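; OutlineSelector is a selector in the RTS selection subsystem that shows an actor's selected state with an outline.
; Select sets the selected flag, turns on the owner's outline component and unbinds cursor-over events on its mouse-hover-responsive components.
; Deselect clears the flag, cancels the outline and rebinds those begin and end hover events.
; A Selected query returns the current flag.
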(event `self.Select`
  (bind _owner (`self.Owner`))
  (set `self.ActorSelected?` true)
  (bind _outlinecomponent (`/Game/RTSMultiplayer/SelectionSubsystem/Blueprints/I_CanBeOutlined.GetOutlineComponent` _owner))
  (`/Game/RTSMultiplayer/SelectionSubsystem/Blueprints/OutlineComponent.Outline` _outlinecomponent)
  (bind _primitivecomponent (`/Game/RTSMultiplayer/SelectionSubsystem/Blueprints/I_CanBeOutlined.GetMouseHoverResponsiveComponents` _owner))
  (for _array_element _primitivecomponent
    (remove `PrimitiveComponent.OnBeginCursorOver` _array_element (`|CreateDelegate` _outlinecomponent :!event `OnBeginCursorOver`))
    (remove `PrimitiveComponent.OnEndCursorOver` _array_element (`|CreateDelegate` _outlinecomponent :!event `OnEndCursorOver`))))

(event `self.Deselect`
  (bind _owner (`self.Owner`))
  (set `self.ActorSelected?` false)
  (bind _outlinecomponent (`/Game/RTSMultiplayer/SelectionSubsystem/Blueprints/I_CanBeOutlined.GetOutlineComponent` _owner))
  (`/Game/RTSMultiplayer/SelectionSubsystem/Blueprints/OutlineComponent.CancelOutline` _outlinecomponent)
  (bind _primitivecomponent (`/Game/RTSMultiplayer/SelectionSubsystem/Blueprints/I_CanBeOutlined.GetMouseHoverResponsiveComponents` _owner))
  (for _array_element _primitivecomponent
    (add `PrimitiveComponent.OnBeginCursorOver` _array_element (`|CreateDelegate` _outlinecomponent :!event `OnBeginCursorOver`))
    (add `PrimitiveComponent.OnEndCursorOver` _array_element (`|CreateDelegate` _outlinecomponent :!event `OnEndCursorOver`))))

(fn `Selected?`
  (returns (`Selected?` :type Boolean))
  (return (`self.ActorSelected?`)))