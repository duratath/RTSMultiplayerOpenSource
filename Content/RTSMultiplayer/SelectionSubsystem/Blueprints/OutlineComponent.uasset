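; Actor component that outlines its owner on mouse hover, tinted by the owner faction's relationship to the local player, for RTS selection feedback.
; It reads meshes, hover components and faction through the owner's I_CanBeOutlined interface, including mesh children of optional scene components.
; Initialization sets custom depth stencil values from the player controller's relationship map and reruns after player faction changes.
; Cursor over events toggle custom depth rendering.
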(event `OnPlayerFactionChanged`
  (params (PlayerCharacter :type "/Game/RTSMultiplayer/RTSCharacters/Blueprints/BasePlayerCharacter Object Reference"))
  ;[1 1 1] Set initial stencil on begin play.
  (`KismetSystemLibrary.Delay` 2.0)
  (`self.Initialize`))

(event `self.ReceiveBeginPlay`
  ;[1 1 1] Set initial stencil on begin play.
  (`self.Initialize`)
  (bind _asbase_player_character (cast `/Game/RTSMultiplayer/RTSCharacters/Blueprints/BasePlayerCharacter` (`GameplayStatics.GetPlayerCharacter` 0)))
  (add `/Game/RTSMultiplayer/RTSCharacters/Blueprints/BasePlayerCharacter.FactionChanged` _asbase_player_character (`|CreateDelegate` :!event `OnPlayerFactionChanged`)))

(event `Initialize`
  ;[1 1 1] Set initial stencil on begin play.
  (`KismetSystemLibrary.Delay` 0.0)
  (bind _asi_can_be_outlined (cast `/Game/RTSMultiplayer/SelectionSubsystem/Blueprints/I_CanBeOutlined` (`self.GetOwner`))
    (:`then`
      (bind _primitivecomponent (`/Game/RTSMultiplayer/SelectionSubsystem/Blueprints/I_CanBeOutlined.GetMouseHoverResponsiveComponents` _asi_can_be_outlined))
      (for _array_element _primitivecomponent
        (add `PrimitiveComponent.OnBeginCursorOver` _array_element (delegate `OnBeginCursorOver`))
        (add `PrimitiveComponent.OnEndCursorOver` _array_element (delegate `OnEndCursorOver`)))
      (bind _faction (`/Game/RTSMultiplayer/SelectionSubsystem/Blueprints/I_CanBeOutlined.GetFactionAsCanBeOutlined` _asi_can_be_outlined))
      (bind (_optionalscenecomponents _meshcomponents) (`/Game/RTSMultiplayer/SelectionSubsystem/Blueprints/I_CanBeOutlined.GetOutlineMeshes` _asi_can_be_outlined))
      (for _array_element_2 _meshcomponents
        (bind _asbase_player_character (cast `/Game/RTSMultiplayer/RTSCharacters/Blueprints/BasePlayerCharacter` (`GameplayStatics.GetPlayerCharacter` 0)))
        (bind _asrtsplayer_controller (cast `/Game/RTSMultiplayer/RTSCharacters/Blueprints/RTSPlayerController` (`GameplayStatics.GetPlayerController` 0)))
        (`PrimitiveComponent.SetCustomDepthStencilValue` _array_element_2 (`BlueprintMapLibrary.Map_Find` (`/Game/RTSMultiplayer/RTSCharacters/Blueprints/RTSPlayerController.StencilValueByRelationships` _asrtsplayer_controller) (`/Game/RTSMultiplayer/RTSCharacters/Blueprints/BasePlayerCharacter.GetRelationships` _asbase_player_character _faction))))
      (for _array_element_3 _optionalscenecomponents
        (bind _asbase_player_character_2 (cast `/Game/RTSMultiplayer/RTSCharacters/Blueprints/BasePlayerCharacter` (`GameplayStatics.GetPlayerCharacter` 0)))
        (bind _asrtsplayer_controller_2 (cast `/Game/RTSMultiplayer/RTSCharacters/Blueprints/RTSPlayerController` (`GameplayStatics.GetPlayerController` 0)))
        (for _array_element_4 (`SceneComponent.GetChildrenComponents` _array_element_3 true)
          (bind _asmesh_component (cast `MeshComponent` _array_element_4))
          (`PrimitiveComponent.SetCustomDepthStencilValue` _asmesh_component (`BlueprintMapLibrary.Map_Find` (`/Game/RTSMultiplayer/RTSCharacters/Blueprints/RTSPlayerController.StencilValueByRelationships` _asrtsplayer_controller_2) (`/Game/RTSMultiplayer/RTSCharacters/Blueprints/BasePlayerCharacter.GetRelationships` _asbase_player_character_2 _faction))))))
    (:`CastFailed`
      (`KismetSystemLibrary.PrintString` "OutlineComponent: owner must implement I_CanBeOutlined interface." true true (struct :`R` 1.0 :`G` 0.038718 :`A` 1.0) 5.0))))

(event `OnBeginCursorOver`
  (params (TouchedComponent :type "PrimitiveComponent Object Reference"))
  ;[1 1 1] Set initial stencil on begin play.
  (`self.Outline`))

(event `OnEndCursorOver`
  (params (TouchedComponent :type "PrimitiveComponent Object Reference"))
  ;[1 1 1] Set initial stencil on begin play.
  (`self.CancelOutline`))

(event `Outline`
  ;[1 1 1] Outline.
  (bind (_optionalscenecomponents _meshcomponents) (`/Game/RTSMultiplayer/SelectionSubsystem/Blueprints/I_CanBeOutlined.GetOutlineMeshes` (cast `/Game/RTSMultiplayer/SelectionSubsystem/Blueprints/I_CanBeOutlined` (`self.GetOwner`) :!pure true)))
  (for _array_element _meshcomponents
    (`PrimitiveComponent.SetRenderCustomDepth` _array_element true))
  (for _array_element_2 _optionalscenecomponents
    (for _array_element_3 (`SceneComponent.GetChildrenComponents` _array_element_2 true)
      (bind _asmesh_component (cast `MeshComponent` _array_element_3))
      (`PrimitiveComponent.SetRenderCustomDepth` _asmesh_component true))))

(event `CancelOutline`
  ;[1 1 1] Cancel outline.
  (bind (_optionalscenecomponents _meshcomponents) (`/Game/RTSMultiplayer/SelectionSubsystem/Blueprints/I_CanBeOutlined.GetOutlineMeshes` (cast `/Game/RTSMultiplayer/SelectionSubsystem/Blueprints/I_CanBeOutlined` (`self.GetOwner`) :!pure true)))
  (for _array_element _meshcomponents
    (`PrimitiveComponent.SetRenderCustomDepth` _array_element false))
  (for _array_element_2 _optionalscenecomponents
    (for _array_element_3 (`SceneComponent.GetChildrenComponents` _array_element_2 true)
      (bind _asmesh_component (cast `MeshComponent` _array_element_3))
      (`PrimitiveComponent.SetRenderCustomDepth` _asmesh_component false))))