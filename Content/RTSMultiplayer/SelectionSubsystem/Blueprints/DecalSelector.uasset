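; DecalSelector is a selection Blueprint in the RTS selection subsystem that shows whether something is selected by means of a decal.
; Select and Deselect call their parent implementations, then show or hide the decal component without propagating to its children.
; The Selected query returns the decal's visibility, so that visibility doubles as the selection state.
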(event `self.Select`
  (`parent.Select`)
  (`SceneComponent.SetVisibility` (`self.DecalComponent`) true false))

(event `self.Deselect`
  (`parent.Deselect`)
  (`SceneComponent.SetVisibility` (`self.DecalComponent`) false false))

(fn `Selected?`
  (returns (`Selected?` :type Boolean))
  (return (`SceneComponent.bVisible` (`self.DecalComponent`))))