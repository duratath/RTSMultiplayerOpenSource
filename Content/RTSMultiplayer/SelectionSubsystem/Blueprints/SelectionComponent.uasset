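; Actor component that makes its owner selectable by the local RTS player when the owner's faction matches the player's.
; On BeginPlay and on faction selection, it registers with the controller's SelectionEnvironment, or binds to that environment's reset event if it is not yet valid.
; Registration also binds to the owner's combat component death event.
; EndPlay and the owner death handler unregister the owner from selection.
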(event `OnPlayerFactionSelected`
  (params (Faction :type "/Game/RTSMultiplayer/RTSCoreBP/E_Faction Enum" :default "NewEnumerator0"))
  ;[1 1 1] Register owner as selectable.
  (bind _asrtsplayer_controller (cast `/Game/RTSMultiplayer/RTSCharacters/Blueprints/RTSPlayerController` (`GameplayStatics.GetPlayerController` 0) :!label _label))
  (bind _selectionenvironment (`/Game/RTSMultiplayer/RTSCharacters/Blueprints/RTSPlayerController.SelectionEnvironment` _asrtsplayer_controller)
    (:`then`
      (`self.RegisterAsSelectable` _selectionenvironment))
    (:`else`
      (add `/Game/RTSMultiplayer/RTSCharacters/Blueprints/RTSPlayerController.OnSelectionEnvironmentReset` _asrtsplayer_controller (delegate `RegisterAsSelectable`)))))

(event `self.ReceiveBeginPlay`
  ;[1 1 1] Register owner as selectable.
  (bind _asrtsplayer_controller (cast `/Game/RTSMultiplayer/RTSCharacters/Blueprints/RTSPlayerController` (`GameplayStatics.GetPlayerController` 0)))
  (add `/Game/RTSMultiplayer/RTSCharacters/Blueprints/RTSPlayerController.PlayerFactionSelected` _asrtsplayer_controller (delegate `OnPlayerFactionSelected`))
  (goto _label))

(event `RegisterAsSelectable`
  (params (SelectionEnvironment :type "/Game/RTSMultiplayer/SelectionSubsystem/Widgets/W_SelectionEnvironment Object Reference"))
  (bind _returnvalue (`self.GetOwner`))
  ;[1 1 1] Register owner as selectable.
  (bind _asrtsgame_instance (cast `/Game/RTSMultiplayer/RTSCoreBP/RTSGameInstance` (`GameplayStatics.GetGameInstance`)))
  (bind _asi_selectable (cast `/Game/RTSMultiplayer/SelectionSubsystem/Blueprints/I_Selectable` (`self.GetOwner`)))
  (bind _faction (`/Game/RTSMultiplayer/SelectionSubsystem/Blueprints/I_Selectable.GetFactionAsSelectable` _asi_selectable))
  (if (`|EnumEquality` _faction (`/Game/RTSMultiplayer/RTSCoreBP/RTSGameInstance.PlayerFaction` _asrtsgame_instance))
    (`/Game/RTSMultiplayer/SelectionSubsystem/Widgets/W_SelectionEnvironment.RegisterAsSelectable` SelectionEnvironment _returnvalue)
    (bind _asi_able_to_fight (cast `/Game/RTSMultiplayer/CombatSubsystem/Blueprints/I_AbleToFight` _returnvalue))
    (bind _combatcomponent (`/Game/RTSMultiplayer/CombatSubsystem/Blueprints/I_AbleToFight.GetCombatComponent` _asi_able_to_fight))
    (add `/Game/RTSMultiplayer/CombatSubsystem/Blueprints/CombatComponent.OwnerDeath` _combatcomponent (`|CreateDelegate` :!event `OnOwnerDeath`))))

(event `self.ReceiveEndPlay`
  (params (EndPlayReason :type "EEndPlayReason Enum" :default "Destroyed"))
  ;[1 1 1] Unregister owner on end play.
  (bind _asrtsplayer_controller (cast `/Game/RTSMultiplayer/RTSCharacters/Blueprints/RTSPlayerController` (`GameplayStatics.GetPlayerController` 0) :!label _label_2))
  (bind _selectionenvironment (`/Game/RTSMultiplayer/RTSCharacters/Blueprints/RTSPlayerController.SelectionEnvironment` _asrtsplayer_controller)
    (:`then`
      (cast `/Game/RTSMultiplayer/RTSCoreBP/RTSGameInstance` (`GameplayStatics.GetGameInstance`))
      (`/Game/RTSMultiplayer/SelectionSubsystem/Widgets/W_SelectionEnvironment.UnregisterActor` _selectionenvironment (`self.GetOwner`)))
    (:`else`)))

(event `OnOwnerDeath`
  (params (Owner :type "Actor Object Reference"))
  ;[1 1 1] Unregister owner on end play.
  (goto _label_2))