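; Fog of war manager actor for an RTS that reveals fog around registered units on the local player's render target.
; A looping timer set on BeginPlay drives updates at a configurable interval.
; Each reveal clears the target to black, converts unit locations and radii to level-normalized UV space, and draws an additive brush material per unit.
; It broadcasts each revealed position and exposes events to register, remove or clear units.
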(event `Reveal`
  (bind (_levelsize_x _levelsize_y) (`KismetMathLibrary.BreakVector2D` (`self.LevelSize`)))
  (bind _levelsize_x_2 (`KismetMathLibrary.BreakVector2D` (`self.LevelSize`)))
  ;[1 1 1] Reveal the fog for every registered unit.
  (bind _asbase_player_character (cast `/Game/RTSMultiplayer/RTSCharacters/Blueprints/BasePlayerCharacter` (`GameplayStatics.GetPlayerPawn` 0)))
  (`KismetRenderingLibrary.ClearRenderTarget2D` (`/Game/RTSMultiplayer/RTSCharacters/Blueprints/BasePlayerCharacter.FogRenderTarget` _asbase_player_character))
  (for _array_element (`self.ObservableUnits`)
    (bind _worldlocation (`/Game/RTSMultiplayer/FogSubsystem/Blueprints/I_CanAffectFog.GetWorldLocation` _array_element))
    (bind _radius (`/Game/RTSMultiplayer/FogSubsystem/Blueprints/I_CanAffectFog.GetFogRevealRadius` _array_element))
    (`/Game/RTSMultiplayer/RTSCharacters/Blueprints/BasePlayerCharacter.SetFogRevealRadius` _asbase_player_character (/ _radius _levelsize_x_2))
    (bind _returnvalue (+ (`KismetMathLibrary.MakeVector2D` (/ (.x _worldlocation) _levelsize_x) (/ (.y _worldlocation) _levelsize_y)) 0.5))
    (`self.RevealAtPosition` _returnvalue)
    (`self.OnPositionRevealed` _array_element _returnvalue)))

(event `self.ReceiveBeginPlay`
  (`KismetSystemLibrary.K2_SetTimerDelegate` (`|CreateDelegate` :!event `Reveal`) (`self.FogUpdateDelta`) true))

(event `RevealAtPosition`
  (params (Position :type "Vector2D Structure"))
  ;[1 1 1] Reveal the fog at specified position.
  (bind _asbase_player_character (cast `/Game/RTSMultiplayer/RTSCharacters/Blueprints/BasePlayerCharacter` (`GameplayStatics.GetPlayerPawn` 0)))
  (bind _additivefogbrush (`/Game/RTSMultiplayer/RTSCharacters/Blueprints/BasePlayerCharacter.AdditiveFogBrush` _asbase_player_character))
  (`MaterialInstanceDynamic.SetVectorParameterValue` _additivefogbrush "DrawLocation" (`KismetMathLibrary.Conv_VectorToLinearColor` (`KismetMathLibrary.Conv_Vector2DToVector` Position)))
  (`KismetRenderingLibrary.DrawMaterialToRenderTarget` (`/Game/RTSMultiplayer/RTSCharacters/Blueprints/BasePlayerCharacter.FogRenderTarget` _asbase_player_character) _additivefogbrush))

(event `RegisterUnit`
  (params (Unit :type "/Game/RTSMultiplayer/FogSubsystem/Blueprints/I_CanAffectFog Interface"))
  ;[1 1 1] Register new unit supposed to reveal the fog.
  (`KismetArrayLibrary.Array_Add` (`self.ObservableUnits`) Unit))

(event `RemoveObservableActor`
  (params (Actor :type "/Game/RTSMultiplayer/FogSubsystem/Blueprints/I_CanAffectFog Interface"))
  ;[1 1 1] Remove single actor from observable units array.
  (`KismetArrayLibrary.Array_RemoveItem` (`self.ObservableUnits`) Actor))

(event `ClearObservable`
  ;[1 1 1] Clear observable units array.
  (`KismetArrayLibrary.Array_Clear` (`self.ObservableUnits`)))

(fn `UserConstructionScript`)