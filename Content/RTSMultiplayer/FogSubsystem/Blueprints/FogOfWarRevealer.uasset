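; Fog of war revealer actor for the RTS multiplayer fog subsystem, providing a faction with a spherical reveal area.
; On BeginPlay it registers its Sphere as the vision collision of its FogOfWarComponent.
; Getter functions expose the faction, component, world location and reveal radius, which comes from the sphere's scaled radius.
; Its visibility query always returns false.
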(event `self.ReceiveBeginPlay`
  (`/Game/RTSMultiplayer/FogSubsystem/Blueprints/FogOfWarComponent.SetSphereVisionCollision` (`self.FogOfWarComponent`) (`self.Sphere`)))

(fn `GetFactionAsFogAffectable`
  (returns (Faction :type "/Game/RTSMultiplayer/RTSCoreBP/E_Faction Enum"))
  (return (`self.Faction`)))

(fn `GetFogOfWarComponent`
  (returns (FogOfWarComponent :type "/Game/RTSMultiplayer/FogSubsystem/Blueprints/FogOfWarComponent Object Reference"))
  (return (`self.FogOfWarComponent`)))

(fn `GetFogRevealRadius`
  (returns (Radius :type "Float (double-precision)"))
  (return (`SphereComponent.GetScaledSphereRadius` (`self.Sphere`))))

(fn `GetWorldLocation`
  (returns (WorldLocation :type "Vector Structure"))
  (return (`self.K2_GetActorLocation`)))

(fn `IsVisible?`
  (returns (Visible :type Boolean))
  (return false))

(fn `UserConstructionScript`)