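; Actor component that ties an RTS unit into fog of war, controlling whether enemies of the player's faction are visible.
; Player-faction owners register with the FogOfWar actor on BeginPlay and unregister on EndPlay; other owners start hidden unless already seen.
; A supplied vision sphere's tagged overlaps, including existing ones, adjust each enemy's VisibleByCount through I_CanAffectFog.
; This reference count keeps enemies shown while any player unit sees them.
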(event `UnregisterActor`
  ;[1 1 1] Remove owner from the fog system.
  (bind _outactors (`GameplayStatics.GetAllActorsOfClass` "/Game/RTSMultiplayer/FogSubsystem/Blueprints/FogOfWar.FogOfWar_C"))
  (bind _asrtsgame_instance (cast `/Game/RTSMultiplayer/RTSCoreBP/RTSGameInstance` (`GameplayStatics.GetGameInstance`)))
  (bind _asi_can_affect_fog (cast `/Game/RTSMultiplayer/FogSubsystem/Blueprints/I_CanAffectFog` (`self.GetOwner`)))
  (bind _faction (`/Game/RTSMultiplayer/FogSubsystem/Blueprints/I_CanAffectFog.GetFactionAsFogAffectable` _asi_can_affect_fog))
  (if (`|EnumEquality` _faction (`/Game/RTSMultiplayer/RTSCoreBP/RTSGameInstance.PlayerFaction` _asrtsgame_instance))
    (`/Game/RTSMultiplayer/FogSubsystem/Blueprints/FogOfWar.RemoveObservableActor` (`|GetArrayItem` _outactors) _asi_can_affect_fog)))

(event `self.ReceiveBeginPlay`
  ;[1 1 1] Begin play.
  (bind _outactors (`GameplayStatics.GetAllActorsOfClass` "/Game/RTSMultiplayer/FogSubsystem/Blueprints/FogOfWar.FogOfWar_C"))
  (bind _asrtsgame_instance (cast `/Game/RTSMultiplayer/RTSCoreBP/RTSGameInstance` (`GameplayStatics.GetGameInstance`)))
  (bind _asi_can_affect_fog (cast `/Game/RTSMultiplayer/FogSubsystem/Blueprints/I_CanAffectFog` (`self.GetOwner`)))
  (bind _faction (`/Game/RTSMultiplayer/FogSubsystem/Blueprints/I_CanAffectFog.GetFactionAsFogAffectable` _asi_can_affect_fog))
  (if (`|EnumEquality` _faction (`/Game/RTSMultiplayer/RTSCoreBP/RTSGameInstance.PlayerFaction` _asrtsgame_instance))
    (`/Game/RTSMultiplayer/FogSubsystem/Blueprints/FogOfWar.RegisterUnit` (`|GetArrayItem` _outactors) _asi_can_affect_fog)
    (`/Game/RTSMultiplayer/FogSubsystem/Blueprints/I_CanAffectFog.SetVisible` _asi_can_affect_fog)
    (else
      (bind _fogofwarcomponent (`/Game/RTSMultiplayer/FogSubsystem/Blueprints/I_CanAffectFog.GetFogOfWarComponent` _asi_can_affect_fog))
      (if (== (`/Game/RTSMultiplayer/FogSubsystem/Blueprints/FogOfWarComponent.VisibleByCount` _fogofwarcomponent) 0)
        (`/Game/RTSMultiplayer/FogSubsystem/Blueprints/I_CanAffectFog.SetInvisible` _asi_can_affect_fog)))))

(event `OnCollisionEndOverlap`
  (params (OverlappedComponent :type "PrimitiveComponent Object Reference") (OtherActor :type "Actor Object Reference") (OtherComp :type "PrimitiveComponent Object Reference") (OtherBodyIndex :type Integer))
  (bind _returnvalue (`self.GetOwner`))
  (bind _playerfaction (`/Game/RTSMultiplayer/RTSCoreBP/RTSGameInstance.PlayerFaction` (cast `/Game/RTSMultiplayer/RTSCoreBP/RTSGameInstance` (`GameplayStatics.GetGameInstance`) :!pure true)))
  ;[1 1 1] End overlap vision sphere.
  (if (`self.ComponentHasTag` OtherComp (`self.VisionCollisionTag`))
    (`/Engine/EditorBlueprintResources/StandardMacros.IsValid` _returnvalue
      (:`Is Valid`
        (bind _asi_can_affect_fog (cast `/Game/RTSMultiplayer/FogSubsystem/Blueprints/I_CanAffectFog` _returnvalue))
        (bind _faction (`/Game/RTSMultiplayer/FogSubsystem/Blueprints/I_CanAffectFog.GetFactionAsFogAffectable` _asi_can_affect_fog))
        (if (`|EnumEquality` _faction _playerfaction)
          (bind _asi_can_affect_fog_2 (cast `/Game/RTSMultiplayer/FogSubsystem/Blueprints/I_CanAffectFog` OtherActor))
          (bind _faction_2 (`/Game/RTSMultiplayer/FogSubsystem/Blueprints/I_CanAffectFog.GetFactionAsFogAffectable` _asi_can_affect_fog_2))
          (if (not (`|EnumEquality` _faction_2 _playerfaction))
            (bind _fogofwarcomponent (`/Game/RTSMultiplayer/FogSubsystem/Blueprints/I_CanAffectFog.GetFogOfWarComponent` _asi_can_affect_fog_2))
            (bind _result (`/Engine/EditorBlueprintResources/StandardMacros.DecrementInt` (`/Game/RTSMultiplayer/FogSubsystem/Blueprints/FogOfWarComponent.VisibleByCount` _fogofwarcomponent))
              (:`  `
                (if (== _result 0)
                  (`/Game/RTSMultiplayer/FogSubsystem/Blueprints/I_CanAffectFog.SetInvisible` _asi_can_affect_fog_2)
                  (elif (< _result 0)
                    (set `/Game/RTSMultiplayer/FogSubsystem/Blueprints/FogOfWarComponent.VisibleByCount` 0 _fogofwarcomponent)))))))))))

(event `OnCollisionBeginOverlap`
  (params (OverlappedComponent :type "PrimitiveComponent Object Reference") (OtherActor :type "Actor Object Reference") (OtherComp :type "PrimitiveComponent Object Reference") (OtherBodyIndex :type Integer) (BoolValue :type Boolean) (SweepResult :type "HitResult Structure (by ref)"))
  (bind _playerfaction (`/Game/RTSMultiplayer/RTSCoreBP/RTSGameInstance.PlayerFaction` (cast `/Game/RTSMultiplayer/RTSCoreBP/RTSGameInstance` (`GameplayStatics.GetGameInstance`) :!pure true)))
  ;[1 1 1] Begin overlap vision sphere.
  (if (`self.ComponentHasTag` OtherComp (`self.VisionCollisionTag`))
    (bind _asi_can_affect_fog (cast `/Game/RTSMultiplayer/FogSubsystem/Blueprints/I_CanAffectFog` (`self.GetOwner`)))
    (bind _faction (`/Game/RTSMultiplayer/FogSubsystem/Blueprints/I_CanAffectFog.GetFactionAsFogAffectable` _asi_can_affect_fog))
    (if (`|EnumEquality` _faction _playerfaction)
      (bind _asi_can_affect_fog_2 (cast `/Game/RTSMultiplayer/FogSubsystem/Blueprints/I_CanAffectFog` OtherActor))
      (bind _faction_2 (`/Game/RTSMultiplayer/FogSubsystem/Blueprints/I_CanAffectFog.GetFactionAsFogAffectable` _asi_can_affect_fog_2))
      (if (not (`|EnumEquality` _faction_2 _playerfaction))
        (bind _fogofwarcomponent (`/Game/RTSMultiplayer/FogSubsystem/Blueprints/I_CanAffectFog.GetFogOfWarComponent` _asi_can_affect_fog_2))
        (bind _result (`/Engine/EditorBlueprintResources/StandardMacros.IncrementInt` (`/Game/RTSMultiplayer/FogSubsystem/Blueprints/FogOfWarComponent.VisibleByCount` _fogofwarcomponent))
          (:`  `
            (if (> _result 0)
              (`/Game/RTSMultiplayer/FogSubsystem/Blueprints/I_CanAffectFog.SetVisible` _asi_can_affect_fog_2))))))))

(event `SetSphereVisionCollision`
  (params (SphereVisionCollision :type "SphereComponent Object Reference"))
  (bind _playerfaction (`/Game/RTSMultiplayer/RTSCoreBP/RTSGameInstance.PlayerFaction` (cast `/Game/RTSMultiplayer/RTSCoreBP/RTSGameInstance` (`GameplayStatics.GetGameInstance`) :!pure true)))
  ;[1 1 1] Set sphere vision collision.
  (bind _output_get (set `self.SphereVisionCollision` SphereVisionCollision))
  (add `PrimitiveComponent.OnComponentBeginOverlap` _output_get (`|CreateDelegate` :!event `OnCollisionBeginOverlap`))
  (add `PrimitiveComponent.OnComponentEndOverlap` _output_get (`|CreateDelegate` :!event `OnCollisionEndOverlap`))
  (for _array_element (`PrimitiveComponent.GetOverlappingComponents` SphereVisionCollision)
    (if (and (`self.ComponentHasTag` _array_element (`self.VisionCollisionTag`)) (!= _array_element SphereVisionCollision))
      (bind _asi_can_affect_fog (cast `/Game/RTSMultiplayer/FogSubsystem/Blueprints/I_CanAffectFog` (`self.GetOwner`)))
      (bind _faction (`/Game/RTSMultiplayer/FogSubsystem/Blueprints/I_CanAffectFog.GetFactionAsFogAffectable` _asi_can_affect_fog))
      (if (`|EnumEquality` _faction _playerfaction)
        (bind _asi_can_affect_fog_2 (cast `/Game/RTSMultiplayer/FogSubsystem/Blueprints/I_CanAffectFog` (`self.GetOwner` _array_element)))
        (bind _faction_2 (`/Game/RTSMultiplayer/FogSubsystem/Blueprints/I_CanAffectFog.GetFactionAsFogAffectable` _asi_can_affect_fog_2))
        (if (not (`|EnumEquality` _faction_2 _playerfaction))
          (bind _fogofwarcomponent (`/Game/RTSMultiplayer/FogSubsystem/Blueprints/I_CanAffectFog.GetFogOfWarComponent` _asi_can_affect_fog_2))
          (`/Engine/EditorBlueprintResources/StandardMacros.IncrementInt` (`/Game/RTSMultiplayer/FogSubsystem/Blueprints/FogOfWarComponent.VisibleByCount` _fogofwarcomponent)
            (:`  `
              (`/Game/RTSMultiplayer/FogSubsystem/Blueprints/I_CanAffectFog.SetVisible` _asi_can_affect_fog_2))))))))

(event `self.ReceiveEndPlay`
  (params (EndPlayReason :type "EEndPlayReason Enum" :default "Destroyed"))
  ;[1 1 1] Unregister owner on end play.
  (`self.UnregisterActor`))