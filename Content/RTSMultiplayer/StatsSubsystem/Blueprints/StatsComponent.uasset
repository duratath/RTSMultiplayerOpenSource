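; Actor component that gives I_HaveStats owners their RTS stats, loaded from a data table by owner ID, plus an overhead nameplate.
; Current and maximum changes go through Multicast events that update the stats map and broadcast StatHasBeenChanged.
; The speed stat drives walk and crouch speeds, while looping timers feed health and mana regeneration back through stat changes.
; The nameplate faces the local camera's spring arm each tick and recolors on player faction change.
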(event `OnPlayerFactionChanged`
  (params (PlayerCharacter :type "/Game/RTSMultiplayer/RTSCharacters/Blueprints/BasePlayerCharacter Object Reference"))
  ;[1 1 1] Changing health bar color on player faction changed.
  (`KismetSystemLibrary.Delay` 2.0)
  (bind _nameplate (`self.Nameplate`)
    (:`then`
      (`/Game/RTSMultiplayer/StatsSubsystem/Widgets/W_Nameplate.SetHealthBarColor` (cast `/Game/RTSMultiplayer/StatsSubsystem/Widgets/W_Nameplate` (`WidgetComponent.GetUserWidgetObject` _nameplate) :!pure true)))
    (:`else`)))

(event `self.ReceiveBeginPlay`
  (bind _asbase_player_character (cast `/Game/RTSMultiplayer/RTSCharacters/Blueprints/BasePlayerCharacter` (`GameplayStatics.GetPlayerCharacter` 0))
    (:`then`
      (add `/Game/RTSMultiplayer/RTSCharacters/Blueprints/BasePlayerCharacter.FactionChanged` _asbase_player_character (`|CreateDelegate` :!event `OnPlayerFactionChanged`)))
    (:`CastFailed`
      _))
  (bind _asi_have_stats (cast `/Game/RTSMultiplayer/StatsSubsystem/Blueprints/I_HaveStats` (`self.GetOwner`))
    (:`then`
      (bind _id (`/Game/RTSMultiplayer/StatsSubsystem/Blueprints/I_HaveStats.GetIdAsHaveStats` _asi_have_stats))
      (bind _returnvalue (`|GetDataTableRow` "/Game/RTSMultiplayer/StatsSubsystem/Data/ActorsStatsDataTable.ActorsStatsDataTable" _id)
        (:`then`
          (set `self.Stats` (break `/Game/RTSMultiplayer/StatsSubsystem/Data/S_StatsMap` _returnvalue))
          ;[1 1 1] Call StatHasBeenChanged.
          (`KismetSystemLibrary.Delay` 0.0)
          (bind _keys (`BlueprintMapLibrary.Map_Keys` (`self.Stats`)))
          (for _array_element _keys
            (`self.StatHasBeenChanged` _array_element (`BlueprintMapLibrary.Map_Find` (`self.Stats`) _array_element)))
          (`self.ChangeOwnerMovementSpeed`)
          (`self.SetupRegeneration`))
        (:`RowNotFound`
          (`KismetSystemLibrary.PrintString` "Row in the ActorsStatsDataTable table not found." true true (struct :`R` 1.0 :`G` 0.038718 :`A` 1.0) 5.0))))
    (:`CastFailed`
      (`KismetSystemLibrary.PrintString` "Actor doesn't implement I_HaveStats interface." true true (struct :`R` 1.0 :`G` 0.038718 :`A` 1.0) 5.0))))

(event `ChangeCurrentStatValue`
  (params (StatToChange :type "/Game/RTSMultiplayer/StatsSubsystem/Blueprints/E_Stat Enum" :default "NewEnumerator0") (ValueDelta :type "Float (double-precision)"))
  ;[1 1 1] Change current stat value.
  (`self.ChangeCurrentStatValueMulticast` StatToChange ValueDelta)
  (if (`|EnumEquality` StatToChange (enumliteral `/Game/RTSMultiplayer/StatsSubsystem/Blueprints/E_Stat` "NewEnumerator5"))
    (`self.ChangeOwnerMovementSpeed`)))

(event `ChangeOwnerMovementSpeed`
  (bind (_value _returnvalue) (`BlueprintMapLibrary.Map_Find` (`self.Stats`) "NewEnumerator5"))
  ;[1 1 1] Changing movement speed stat.
  (if _returnvalue
    (bind _asi_have_stats (cast `/Game/RTSMultiplayer/StatsSubsystem/Blueprints/I_HaveStats` (`self.GetOwner`)))
    (bind _movementcomponent (`/Game/RTSMultiplayer/StatsSubsystem/Blueprints/I_HaveStats.GetCharacterMovementComponent` _asi_have_stats))
    (set `CharacterMovementComponent.MaxWalkSpeed` (break `/Game/RTSMultiplayer/StatsSubsystem/Blueprints/S_Stat` _value) _movementcomponent)
    (set `CharacterMovementComponent.MaxWalkSpeedCrouched` (/ (break `/Game/RTSMultiplayer/StatsSubsystem/Blueprints/S_Stat` _value) 2.0) _movementcomponent)))

(event `ChangeCurrentStatValueMulticast`
  (params (StatToChange :type "/Game/RTSMultiplayer/StatsSubsystem/Blueprints/E_Stat Enum" :default "NewEnumerator0") (ValueDelta :type "Float (double-precision)"))
  (bind _stats (`self.Stats`))
  (bind (_value _returnvalue) (`BlueprintMapLibrary.Map_Find` (`self.Stats`) StatToChange))
  (bind (_current _basemaximum _maximumboost _baseminimum _minimumboost) (break `/Game/RTSMultiplayer/StatsSubsystem/Blueprints/S_Stat` _value))
  ;[1 1 1] Change current stat value.
  (if _returnvalue
    (`BlueprintMapLibrary.Map_Add` _stats StatToChange (make `/Game/RTSMultiplayer/StatsSubsystem/Blueprints/S_Stat` (`KismetMathLibrary.FClamp` (+ _current ValueDelta) (+ _baseminimum _minimumboost) (+ _basemaximum _maximumboost)) _basemaximum _maximumboost))
    (`self.StatHasBeenChanged` StatToChange (`BlueprintMapLibrary.Map_Find` _stats StatToChange))))

(event `SetupRegeneration`
  ;[1 1 1] Setup health and mana regeneration events.
  (if (`.ReturnValue` (`BlueprintMapLibrary.Map_Find` (`self.Stats`) "NewEnumerator9"))
    (bind _returnvalue (`KismetSystemLibrary.K2_SetTimerDelegate` (`|CreateDelegate` :!event `HealthPassiveRegeneration`) 0.2 true))
    (set `self.HealthRegenerationHandle` _returnvalue))
  (if (`.ReturnValue` (`BlueprintMapLibrary.Map_Find` (`self.Stats`) "NewEnumerator10"))
    (bind _returnvalue_2 (`KismetSystemLibrary.K2_SetTimerDelegate` (`|CreateDelegate` :!event `ManaPassiveRegeneration`) 0.2 true))
    (set `self.ManaRegenerationHandle` _returnvalue_2)))

(event `ChangeMaxStatValue`
  (params (StatToChange :type "/Game/RTSMultiplayer/StatsSubsystem/Blueprints/E_Stat Enum" :default "NewEnumerator0") (ValueDelta :type "Float (double-precision)"))
  ;[1 1 1] Change maximum stat value.
  (`self.ChangeMaxStatValueMulticast` StatToChange ValueDelta)
  (if (`|EnumEquality` StatToChange (enumliteral `/Game/RTSMultiplayer/StatsSubsystem/Blueprints/E_Stat` "NewEnumerator5"))
    (`self.ChangeOwnerMovementSpeed`)))

(event `ChangeMaxStatValueMulticast`
  (params (StatToChange :type "/Game/RTSMultiplayer/StatsSubsystem/Blueprints/E_Stat Enum" :default "NewEnumerator0") (ValueDelta :type "Float (double-precision)"))
  (bind _stats (`self.Stats`))
  (bind (_value _returnvalue) (`BlueprintMapLibrary.Map_Find` (`self.Stats`) StatToChange))
  (bind (_current _basemaximum _maximumboost) (break `/Game/RTSMultiplayer/StatsSubsystem/Blueprints/S_Stat` _value))
  ;[1 1 1] Change maximum stat value.
  (if _returnvalue
    (`BlueprintMapLibrary.Map_Add` _stats StatToChange (make `/Game/RTSMultiplayer/StatsSubsystem/Blueprints/S_Stat` (+ _current ValueDelta) _basemaximum (+ _maximumboost ValueDelta)))
    (`self.StatHasBeenChanged` StatToChange (`BlueprintMapLibrary.Map_Find` _stats StatToChange))))

(event `HealthPassiveRegeneration`
  ;[1 1 1] Health and mana regeneration events.
  (`self.ChangeCurrentStatValue` (enumliteral `/Game/RTSMultiplayer/StatsSubsystem/Blueprints/E_Stat` "NewEnumerator0") (/ (break `/Game/RTSMultiplayer/StatsSubsystem/Blueprints/S_Stat` (`BlueprintMapLibrary.Map_Find` (`self.Stats`) "NewEnumerator9")) 5.0)))

(event `ManaPassiveRegeneration`
  ;[1 1 1] Health and mana regeneration events.
  (`self.ChangeCurrentStatValue` (enumliteral `/Game/RTSMultiplayer/StatsSubsystem/Blueprints/E_Stat` "NewEnumerator1") (/ (break `/Game/RTSMultiplayer/StatsSubsystem/Blueprints/S_Stat` (`BlueprintMapLibrary.Map_Find` (`self.Stats`) "NewEnumerator10")) 5.0)))

(event `AddNameplate`
  (params (NameplateWidgetComponent :type "WidgetComponent Object Reference"))
  (bind _returnvalue (enumliteral `/Game/RTSMultiplayer/StatsSubsystem/Blueprints/E_Stat` "NewEnumerator0"))
  (bind (_value _returnvalue_2) (`BlueprintMapLibrary.Map_Find` (`self.Stats`) _returnvalue))
  ;[1 1 1] Add nameplate widget.
  (bind _output_get (set `self.Nameplate` NameplateWidgetComponent))
  (bind _asw_nameplate (cast `/Game/RTSMultiplayer/StatsSubsystem/Widgets/W_Nameplate` (`WidgetComponent.GetUserWidgetObject` _output_get) :!pure true))
  (`/Game/RTSMultiplayer/StatsSubsystem/Widgets/W_Nameplate.SetOwner` _asw_nameplate (cast `/Game/RTSMultiplayer/StatsSubsystem/Blueprints/I_HaveStats` (`self.GetOwner`) :!pure true))
  (`KismetSystemLibrary.Delay` 0.2)
  (if _returnvalue_2
    (`/Game/RTSMultiplayer/StatsSubsystem/Widgets/W_Nameplate.SetHealthBarColor` _asw_nameplate)
    (`/Game/RTSMultiplayer/StatsSubsystem/Widgets/W_Nameplate.ShowHealthBar` _asw_nameplate)
    (`self.StatHasBeenChanged` _returnvalue _value)))

(event `self.ReceiveTick`
  (params (DeltaSeconds :type "Float (single-precision)"))
  ;[1 1 1] Set health bar rotation due to camera position on tick.
  (bind _nameplate (`self.Nameplate`)
    (:`then`
      (bind _asbase_player_character (cast `/Game/RTSMultiplayer/RTSCharacters/Blueprints/BasePlayerCharacter` (`GameplayStatics.GetPlayerCharacter` 0)))
      (`SceneComponent.K2_SetWorldRotation` _nameplate (`KismetMathLibrary.Conv_VectorToRotator` (* (`KismetMathLibrary.Conv_RotatorToVector` (`SceneComponent.K2_GetComponentRotation` (`/Game/RTSMultiplayer/RTSCharacters/Blueprints/BasePlayerCharacter.SpringArm` _asbase_player_character))) -1)) false false))
    (:`else`)))

(event `ShowNameplate`
  ;[1 1 1] Show/hide nameplate.
  (bind _nameplate (`self.Nameplate`)
    (:`then`
      (`SceneComponent.SetVisibility` _nameplate true false))
    (:`else`)))

(event `HideNameplate`
  ;[1 1 1] Show/hide nameplate.
  (bind _nameplate (`self.Nameplate`)
    (:`then`
      (`SceneComponent.SetVisibility` _nameplate false false))
    (:`else`)))

(event `ToggleNameplateVisibility`
  ;[1 1 1] Show/hide nameplate.
  (bind _nameplate (`self.Nameplate`)
    (:`then`
      (`SceneComponent.ToggleVisibility` _nameplate false))
    (:`else`)))

(fn `GetOwnerFaction`
  (returns (Faction :type "/Game/RTSMultiplayer/RTSCoreBP/E_Faction Enum"))
  (bind _faction (`/Game/RTSMultiplayer/StatsSubsystem/Blueprints/I_HaveStats.GetFactionAsHaveStats` (cast `/Game/RTSMultiplayer/StatsSubsystem/Blueprints/I_HaveStats` (`self.GetOwner`) :!pure true)))
  (return _faction))