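; Actor component that shows its owner on the RTS minimap, registering after a short delay and unregistering on end play.
; Sizes the level from two LevelCornerPoint actors to normalize location and fog reveal radius.
; Supplies icons by relationship, plus faction and visibility through I_CanAffectFog.
; Relays owner selection changes from HUD events, and clears the minimap and re-registers when the player's faction changes.
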(event `OnPlayerFactionChanged`
  (params (PlayerCharacter :type "/Game/RTSMultiplayer/RTSCharacters/Blueprints/BasePlayerCharacter Object Reference"))
  ;[1 1 1] Add actor to minimap on begin play.
  (`/Game/RTSMultiplayer/MapSubsystem/Widgets/W_MiniMap.ClearMinimap` (`/Game/RTSMultiplayer/MapSubsystem/Widgets/W_MinimapWindow.W_Minimap` (`/Game/RTSMultiplayer/RTSCoreUI/Widgets/W_PlayerHUD.W_MinimapWindow` (`/Game/RTSMultiplayer/RTSCharacters/Blueprints/RTSPlayerController.PlayerHUD` (cast `/Game/RTSMultiplayer/RTSCharacters/Blueprints/RTSPlayerController` (`GameplayStatics.GetPlayerController` 0) :!pure true)))))
  (`self.Initialize`))

(event `self.ReceiveBeginPlay`
  ;[1 1 1] Add actor to minimap on begin play.
  (`self.Initialize`)
  (bind _asbase_player_character (cast `/Game/RTSMultiplayer/RTSCharacters/Blueprints/BasePlayerCharacter` (`GameplayStatics.GetPlayerCharacter` 0)))
  (add `/Game/RTSMultiplayer/RTSCharacters/Blueprints/BasePlayerCharacter.FactionChanged` _asbase_player_character (`|CreateDelegate` :!event `OnPlayerFactionChanged`)))

(event `Initialize`
  ;[1 1 1] Add actor to minimap on begin play.
  (bind _outactors (`GameplayStatics.GetAllActorsOfClass` "/Game/RTSMultiplayer/FogSubsystem/Blueprints/LevelCornerPoint.LevelCornerPoint_C"))
  (if (== (`KismetArrayLibrary.Array_Length` _outactors) 2)
    (bind (_returnvalue_x _returnvalue_y) (`KismetMathLibrary.BreakVector` (- (`Actor.K2_GetActorLocation` (`|GetArrayItem` _outactors)) (`Actor.K2_GetActorLocation` (`|GetArrayItem` _outactors 1)))))
    (set `self.LevelSize` (`KismetMathLibrary.MakeVector2D` (`KismetMathLibrary.Abs` _returnvalue_x) (`KismetMathLibrary.Abs` _returnvalue_y)))
    (`KismetSystemLibrary.Delay` 2.0)
    (bind _asrtsplayer_controller (cast `/Game/RTSMultiplayer/RTSCharacters/Blueprints/RTSPlayerController` (`GameplayStatics.GetPlayerController` 0)))
    (bind _playerhud (`/Game/RTSMultiplayer/RTSCharacters/Blueprints/RTSPlayerController.PlayerHUD` _asrtsplayer_controller)
      (:`then`
        (add `/Game/RTSMultiplayer/SelectionSubsystem/Widgets/W_SelectionEnvironment.ActorsSelected` (`/Game/RTSMultiplayer/RTSCoreUI/Widgets/W_PlayerHUD.W_SelectionEnvironment` _playerhud) (delegate `OnActorsSelected`))
        (bind _output_get (set `self.MinimapWidget` (`/Game/RTSMultiplayer/MapSubsystem/Widgets/W_MinimapWindow.W_Minimap` (`/Game/RTSMultiplayer/RTSCoreUI/Widgets/W_PlayerHUD.W_MinimapWindow` _playerhud))))
        (`/Game/RTSMultiplayer/MapSubsystem/Widgets/W_MiniMap.AddActor` _output_get self))
      (:`else`))
    (else
      (`KismetSystemLibrary.PrintString` "MapComponent: please, place 2 LevelCornerPoint actors in level." true true (struct :`R` 1.0 :`G` 0.038718 :`A` 1.0) 5.0))))

(event `OnActorsSelected`
  (params (SelectedActors :type "Array of Actor Object Reference (by ref)"))
  ;[1 1 1] Add actor to minimap on begin play.
  (bind _asi_selectable (cast `/Game/RTSMultiplayer/SelectionSubsystem/Blueprints/I_Selectable` (`self.GetOwner`)))
  (bind _selector (`/Game/RTSMultiplayer/SelectionSubsystem/Blueprints/I_Selectable.GetSelector` _asi_selectable))
  (if (`/Game/RTSMultiplayer/SelectionSubsystem/Blueprints/Selector.Selected?` _selector)
    (set `self.WasOwnerSelected?` true)
    (`self.OnOwnerSelected`)
    (elif (`self.WasOwnerSelected?`)
      (`self.OnOwnerDeselected`)
      (set `self.WasOwnerSelected?` false))))

(event `self.ReceiveEndPlay`
  (params (EndPlayReason :type "EEndPlayReason Enum" :default "Destroyed"))
  ;[1 1 1] Remove actor from minimap on end play.
  (bind _minimapwidget (`self.MinimapWidget`)
    (:`then`
      (`/Game/RTSMultiplayer/MapSubsystem/Widgets/W_MiniMap.RemoveFromObservables` _minimapwidget self))
    (:`else`)))

(fn `GetActorFaction`
  (returns (Faction :type "/Game/RTSMultiplayer/RTSCoreBP/E_Faction Enum"))
  (bind _faction (`/Game/RTSMultiplayer/FogSubsystem/Blueprints/I_CanAffectFog.GetFactionAsFogAffectable` (cast `/Game/RTSMultiplayer/FogSubsystem/Blueprints/I_CanAffectFog` (`self.GetOwner`) :!pure true)))
  (return _faction))

(fn `GetIcon`
  (params (Relationships :type "/Game/RTSMultiplayer/CombatSubsystem/Blueprints/E_RelationshipType Enum (by ref)" :default "NewEnumerator0"))
  (returns (Icon :type "Texture2D Object Reference"))
  (return (`BlueprintMapLibrary.Map_Find` (`self.MinimapIcons`) Relationships)))

(fn `GetNormalizedLocation`
  (returns (MapLocation :type "Vector2D Structure"))
  (bind (_levelsize_x _levelsize_y) (`KismetMathLibrary.BreakVector2D` (`self.LevelSize`)))
  (return (+ (`KismetMathLibrary.MakeVector2D` (/ (.x (`Actor.K2_GetActorLocation` (`self.GetOwner`))) _levelsize_x) (/ (.y (`Actor.K2_GetActorLocation` (`self.GetOwner`))) _levelsize_y)) 0.5)))

(fn `GetNormalizedRevealRadius`
  (returns (NormalizedRadius :type "Float (double-precision)"))
  (bind _levelsize_x (`KismetMathLibrary.BreakVector2D` (`self.LevelSize`)))
  (bind _radius (`/Game/RTSMultiplayer/FogSubsystem/Blueprints/I_CanAffectFog.GetFogRevealRadius` (cast `/Game/RTSMultiplayer/FogSubsystem/Blueprints/I_CanAffectFog` (`self.GetOwner`) :!pure true)))
  (return (/ _radius _levelsize_x)))

(fn `IsActorHidden?`
  (returns (Hidden :type Boolean))
  (bind _visible (`/Game/RTSMultiplayer/FogSubsystem/Blueprints/I_CanAffectFog.IsVisible?` (cast `/Game/RTSMultiplayer/FogSubsystem/Blueprints/I_CanAffectFog` (`self.GetOwner`) :!pure true)))
  (return (not _visible)))