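; FrostMage is a demo character Blueprint for the RTS multiplayer game that configures a parent class through getter overrides.
; It supplies Sevarog montages for death and instant casts, and randomly picks one of two medium swing montages for attacks.
; It also reports the free space it needs, while its construction script only calls the parent.
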(fn `GetAttackAnimMontageSettings`
  (returns (AnimMontage :type "AnimMontage Object Reference") (PlayRate :type "Float (double-precision)"))
  (return (select `int` (`KismetMathLibrary.RandomInteger` 2) :`0` "/Game/RTSMultiplayer/DemoCharacters/Sevarog/Sevarog/Animations/Swing1_Medium_Montage.Swing1_Medium_Montage" :`1` "/Game/RTSMultiplayer/DemoCharacters/Sevarog/Sevarog/Animations/Swing2_Medium_Montage.Swing2_Medium_Montage" :!type "AnimMontage Object Reference") 1.0))

(fn `GetDeathAnimMontageSettings`
  (returns (AnimMontage :type "AnimMontage Object Reference") (PlayRate :type "Float (double-precision)"))
  (return "/Game/RTSMultiplayer/DemoCharacters/Sevarog/Sevarog/Animations/Sevarog_Death_Montage.Sevarog_Death_Montage" 1.0))

(fn `GetInstantCastAnimationSettings`
  (returns (AnimMontage :type "AnimMontage Object Reference") (PlayRate :type "Float (double-precision)"))
  (return "/Game/RTSMultiplayer/DemoCharacters/Sevarog/Sevarog/Animations/Sevarog_Instant_Montage.Sevarog_Instant_Montage" 1.0))

(fn `GetNecessaryFreeSpace`
  (returns (FreeSpace :type "Float (double-precision)"))
  (return 2.0))

(fn `UserConstructionScript`
  (`parent.UserConstructionScript`))