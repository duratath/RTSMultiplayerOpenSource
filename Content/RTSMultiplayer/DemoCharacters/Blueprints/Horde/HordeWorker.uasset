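; HordeWorker is the Horde worker unit among the RTS demo characters, supplying Greystone montages for its combat and labor actions.
; Getter functions return a montage and play rate for attack, death, building, tree chopping, mining and instant casting.
; Attacks pick randomly from three primary montages, while mining reuses the chopping montage at a faster play rate.
; The construction script only calls its parent.
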(fn `GetAttackAnimMontageSettings`
  (returns (AnimMontage :type "AnimMontage Object Reference") (PlayRate :type "Float (double-precision)"))
  (return (select `int` (`KismetMathLibrary.RandomInteger` 3) :`0` "/Game/RTSMultiplayer/DemoCharacters/Greystone/Greystone/Animations/Attack_PrimaryA_Montage.Attack_PrimaryA_Montage" :`1` "/Game/RTSMultiplayer/DemoCharacters/Greystone/Greystone/Animations/Attack_PrimaryB_Montage.Attack_PrimaryB_Montage" :`2` "/Game/RTSMultiplayer/DemoCharacters/Greystone/Greystone/Animations/Attack_PrimaryC_Montage.Attack_PrimaryC_Montage" :!type "AnimMontage Object Reference") 1.0))

(fn `GetBuildAnimationSettings`
  (returns (AnimMontage :type "AnimMontage Object Reference") (PlayRate :type "Float (double-precision)"))
  (return "/Game/RTSMultiplayer/DemoCharacters/Greystone/Greystone/Animations/Greystone_Build_Montage.Greystone_Build_Montage" 1.0))

(fn `GetChopTreeAnimationSettings`
  (returns (AnimMontage :type "AnimMontage Object Reference") (PlayRate :type "Float (double-precision)"))
  (return "/Game/RTSMultiplayer/DemoCharacters/Greystone/Greystone/Animations/Greystone_Chopping_Montage.Greystone_Chopping_Montage" 1.0))

(fn `GetDeathAnimMontageSettings`
  (returns (AnimMontage :type "AnimMontage Object Reference") (PlayRate :type "Float (double-precision)"))
  (return "/Game/RTSMultiplayer/DemoCharacters/Greystone/Greystone/Animations/Greystone_Death_Montage.Greystone_Death_Montage" 1.0))

(fn `GetInstantCastAnimationSettings`
  (returns (AnimMontage :type "AnimMontage Object Reference") (PlayRate :type "Float (double-precision)"))
  (return "/Game/RTSMultiplayer/DemoCharacters/Greystone/Greystone/Animations/Greystone_Instant_Montage.Greystone_Instant_Montage" 1.0))

(fn `GetMineAnimationSettings`
  (returns (AnimMontage :type "AnimMontage Object Reference") (PlayRate :type "Float (double-precision)"))
  (return "/Game/RTSMultiplayer/DemoCharacters/Greystone/Greystone/Animations/Greystone_Chopping_Montage.Greystone_Chopping_Montage" 2.1))

(fn `UserConstructionScript`
  (`parent.UserConstructionScript`))