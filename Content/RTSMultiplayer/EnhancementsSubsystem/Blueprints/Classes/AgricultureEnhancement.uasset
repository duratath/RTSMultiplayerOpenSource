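; Agriculture enhancement for an RTS that unlocks the Build Granary ability on the actor it enhances.
; On BeginPlay it looks up and caches the granary build row from the abilities data table, printing a message if the row is missing.
; Apply casts the target actor to I_HaveAbilities and adds the cached ability to its ability component, doing nothing if the cast fails.
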(event `self.ReceiveBeginPlay`
  (`parent.ReceiveBeginPlay`)
  (bind _returnvalue (`|GetDataTableRow` "/Game/RTSMultiplayer/AbilitySubsystem/Data/AbilitiesDataTable.AbilitiesDataTable" "BUILD_GRANARY")
    (:`then`
      (set `self.BuildGranaryAbilityInfo` _returnvalue))
    (:`RowNotFound`
      (`KismetSystemLibrary.PrintString` "AgricultureEnhancement: ability not found." true true (struct :`R` 1.0 :`G` 0.038718 :`A` 1.0) 5.0))))

(event `/Game/RTSMultiplayer/EnhancementsSubsystem/Blueprints/Enhancement.Apply`
  (bind _asi_have_abilities (cast `/Game/RTSMultiplayer/AbilitySubsystem/Blueprints/I_HaveAbilities` (`self.ActorToEnhance`)))
  (bind _abilitycomponent (`/Game/RTSMultiplayer/AbilitySubsystem/Blueprints/I_HaveAbilities.GetAbilityComponent` _asi_have_abilities))
  (`/Game/RTSMultiplayer/AbilitySubsystem/Blueprints/AbilityComponent.AddAbility` _abilitycomponent (`self.BuildGranaryAbilityInfo`)))

(fn `UserConstructionScript`
  (`parent.UserConstructionScript`))