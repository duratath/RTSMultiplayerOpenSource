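; High magic enhancement that grants a target actor the ability to recruit High Mages.
; On BeginPlay it looks up the high mage recruitment row in the abilities data table and caches it, printing a message if the row is missing.
; Apply casts the actor to enhance to the abilities interface and adds the cached ability to that actor's ability component.
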(event `self.ReceiveBeginPlay`
  (`parent.ReceiveBeginPlay`)
  (bind _returnvalue (`|GetDataTableRow` "/Game/RTSMultiplayer/AbilitySubsystem/Data/AbilitiesDataTable.AbilitiesDataTable" "RECRUIT_HIGH_MAGE")
    (:`then`
      (set `self.RecruitHighMageAbilityInfo` _returnvalue))
    (:`RowNotFound`
      (`KismetSystemLibrary.PrintString` "HighMagicEnhancement: ability not found." true true (struct :`R` 1.0 :`G` 0.038718 :`A` 1.0) 5.0))))

(event `/Game/RTSMultiplayer/EnhancementsSubsystem/Blueprints/Enhancement.Apply`
  (bind _asi_have_abilities (cast `/Game/RTSMultiplayer/AbilitySubsystem/Blueprints/I_HaveAbilities` (`self.ActorToEnhance`)))
  (bind _abilitycomponent (`/Game/RTSMultiplayer/AbilitySubsystem/Blueprints/I_HaveAbilities.GetAbilityComponent` _asi_have_abilities))
  (`/Game/RTSMultiplayer/AbilitySubsystem/Blueprints/AbilityComponent.AddAbility` _abilitycomponent (`self.RecruitHighMageAbilityInfo`)))

(fn `UserConstructionScript`
  (`parent.UserConstructionScript`))