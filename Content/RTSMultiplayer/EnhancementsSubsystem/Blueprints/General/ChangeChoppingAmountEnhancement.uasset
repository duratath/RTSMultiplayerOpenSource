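; Enhancement that changes how much wood-chopping yields for the owning player's faction by scaling the collecting amount on tree resources.
; On Apply, it runs the parent logic, then iterates over every TreeResourceSeed actor in the world.
; Each tree's current amount for that faction is multiplied by the first enhancement constant, so only trees present at that moment change and repeated applications compound.
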(event `self.Apply`
  (bind _playerfaction (`/Game/RTSMultiplayer/RTSCharacters/Blueprints/BasePlayerCharacter.PlayerFaction` (cast `/Game/RTSMultiplayer/RTSCharacters/Blueprints/BasePlayerCharacter` (`self.GetOwner`) :!pure true)))
  (`parent.Apply`)
  (bind _outactors (`GameplayStatics.GetAllActorsOfClass` "/Game/RTSMultiplayer/ResourcesSubsystem/Blueprints/TreeResourceSeed.TreeResourceSeed_C"))
  (for _array_element _outactors
    (`/Game/RTSMultiplayer/ResourcesSubsystem/Blueprints/ResourceSeed.ChangeCollectingAmount` _array_element _playerfaction (* (`BlueprintMapLibrary.Map_Find` (`/Game/RTSMultiplayer/ResourcesSubsystem/Blueprints/ResourceSeed.CollectingAmount` _array_element) _playerfaction) (`|GetArrayItem` (`self.EhancementConstants`))))))

(fn `UserConstructionScript`
  (`parent.UserConstructionScript`))