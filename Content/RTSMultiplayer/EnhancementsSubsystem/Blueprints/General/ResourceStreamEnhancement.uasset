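; ResourceStreamEnhancement is an enhancement that periodically grants its owning player a consumable resource.
; On Apply it starts a looping timer, with the interval and amount per tick read from the enhancement constants array.
; IncreaseResources casts the owner to BasePlayerCharacter and adds the configured resource type, printing an error if the owner is of another class.
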(event `self.Apply`
  (`KismetSystemLibrary.K2_SetTimerDelegate` (`|CreateDelegate` :!event `IncreaseResources`) (`|GetArrayItem` (`self.EhancementConstants`)) true))

(event `IncreaseResources`
  (bind _asbase_player_character (cast `/Game/RTSMultiplayer/RTSCharacters/Blueprints/BasePlayerCharacter` (`self.GetOwner`))
    (:`then`
      (`/Game/RTSMultiplayer/RTSCharacters/Blueprints/BasePlayerCharacter.AddConsumableResource` _asbase_player_character (`self.ResourceType`) (`|GetArrayItem` (`self.EhancementConstants`) 1)))
    (:`CastFailed`
      (`KismetSystemLibrary.PrintString` "ResourceStreamEnhancement: owner must be a child of BasePlayerCharacter."))))

(fn `UserConstructionScript`
  (`parent.UserConstructionScript`))