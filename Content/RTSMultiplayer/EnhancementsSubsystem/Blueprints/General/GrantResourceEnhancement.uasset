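; Enhancement Blueprint that grants the owning player character a resource when applied.
; After the parent Apply runs, it switches on ResourceType and passes the first enhancement constant to the BasePlayerCharacter.
; Tree and Gold are added as consumable resources, Space raises the allocatable maximum, and Science changes the streaming resource.
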(event `self.Apply`
  (bind _resourcetype (`self.ResourceType`))
  (bind _asbase_player_character (cast `/Game/RTSMultiplayer/RTSCharacters/Blueprints/BasePlayerCharacter` (`self.GetOwner`) :!pure true))
  (bind _output (`|GetArrayItem` (`self.EhancementConstants`)))
  (`parent.Apply`)
  (switch `/Game/RTSMultiplayer/ResourcesSubsystem/Blueprints/E_ResourceType` _resourcetype
    (:`NewEnumerator0`
      (`/Game/RTSMultiplayer/RTSCharacters/Blueprints/BasePlayerCharacter.AddConsumableResource` _asbase_player_character _resourcetype _output :!label _label))
    (:`NewEnumerator1`
      (goto _label))
    (:`NewEnumerator2`
      (`/Game/RTSMultiplayer/RTSCharacters/Blueprints/BasePlayerCharacter.ChangeAllocatableResourceMaximum` _asbase_player_character _resourcetype _output))
    (:`NewEnumerator3`
      (`/Game/RTSMultiplayer/RTSCharacters/Blueprints/BasePlayerCharacter.ChangeStreamingResource` _asbase_player_character _resourcetype _output))))

(fn `UserConstructionScript`
  (`parent.UserConstructionScript`))