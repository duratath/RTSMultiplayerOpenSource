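; Ability enhancement for the RTS multiplayer enhancements subsystem that scales an ability's consumable costs.
; EnhanceAbility loops over every key in the ability's ConsumableCost map, multiplies its value by the first enhancement constant and rounds it to a whole number.
; It writes the map back into the returned ability info and passes combat constants through unchanged.
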(fn `EnhanceAbility`
  (params (AbilityInfo :type "/Game/RTSMultiplayer/AbilitySubsystem/Data/S_AbilityInfo Structure") (CombatConstants :type "/Game/RTSMultiplayer/AbilitySubsystem/Data/S_AbilityCombatConstants Structure"))
  (returns (NewAbilityInfo :type "/Game/RTSMultiplayer/AbilitySubsystem/Data/S_AbilityInfo Structure") (NewCombatConstants :type "/Game/RTSMultiplayer/AbilitySubsystem/Data/S_AbilityCombatConstants Structure"))
  (bind _consumablecost (`self.ConsumableCost`))
  (set `self.ConsumableCost` (`.ConsumableCost_26_03C7DBCC41457F4251BFB0AF879BEE44` (break `/Game/RTSMultiplayer/AbilitySubsystem/Data/S_AbilityInfo` AbilityInfo)))
  (bind _keys (`BlueprintMapLibrary.Map_Keys` (`self.ConsumableCost`)))
  (for _array_element _keys
    (`BlueprintMapLibrary.Map_Add` _consumablecost _array_element (`KismetMathLibrary.Conv_IntToDouble` (`KismetMathLibrary.Round` (* (`|GetArrayItem` (`self.EhancementConstants`)) (`BlueprintMapLibrary.Map_Find` _consumablecost _array_element))))))
  (bind _structout (setmembers `/Game/RTSMultiplayer/AbilitySubsystem/Data/S_AbilityInfo` :`StructRef` AbilityInfo :`ConsumableCost` (`self.ConsumableCost`)))
  (return _structout CombatConstants))

(fn `UserConstructionScript`
  (`parent.UserConstructionScript`))