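; Ability enhancement in the RTS enhancements subsystem that changes an ability's stat costs.
; EnhanceAbility multiplies every entry in the ability info's StatsCost map by the first enhancement constant and rounds it to a whole number.
; It returns the updated ability info and passes combat constants through unchanged.
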(fn `EnhanceAbility`
  (params (AbilityInfo :type "/Game/RTSMultiplayer/AbilitySubsystem/Data/S_AbilityInfo Structure") (CombatConstants :type "/Game/RTSMultiplayer/AbilitySubsystem/Data/S_AbilityCombatConstants Structure"))
  (returns (NewAbilityInfo :type "/Game/RTSMultiplayer/AbilitySubsystem/Data/S_AbilityInfo Structure") (NewCombatConstants :type "/Game/RTSMultiplayer/AbilitySubsystem/Data/S_AbilityCombatConstants Structure"))
  (bind _statscost (`self.StatsCost`))
  (set `self.StatsCost` (`.StatsCost_32_40B8335549DA9465E8F6F09CDA3E9E24` (break `/Game/RTSMultiplayer/AbilitySubsystem/Data/S_AbilityInfo` AbilityInfo)))
  (bind _keys (`BlueprintMapLibrary.Map_Keys` (`self.StatsCost`)))
  (for _array_element _keys
    (`BlueprintMapLibrary.Map_Add` _statscost _array_element (`KismetMathLibrary.Conv_IntToDouble` (`KismetMathLibrary.Round` (* (`|GetArrayItem` (`self.EhancementConstants`)) (`BlueprintMapLibrary.Map_Find` _statscost _array_element))))))
  (bind _structout (setmembers `/Game/RTSMultiplayer/AbilitySubsystem/Data/S_AbilityInfo` :`StructRef` AbilityInfo :`StatsCost` (`self.StatsCost`)))
  (return _structout CombatConstants))

(fn `UserConstructionScript`
  (`parent.UserConstructionScript`))