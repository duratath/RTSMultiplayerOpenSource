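; Base task Blueprint for the RTS multiplayer task subsystem, with Initialize, Start and End lifecycle events.
; On Start, a non-zero ability range is checked against the executor's distance to the target location, unless its owner has an RTS AI controller.
; Out-of-range tasks post an attention message to the player, set TooFarAway and end.
; Helper events show failure messages and broadcast completion or failure dispatchers, passing the task itself.
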(event `ShowFailedMessage`
  ;[1 1 1] Show failed message.
  (bind _playercontroller (`self.PlayerController`)
    (:`then`
      (`/Game/RTSMultiplayer/RTSCharacters/Blueprints/RTSPlayerController.AddAttentionMessage` _playercontroller (`self.FailedMessageId`)))
    (:`else`)))

(event `Initialize`
  ;[1 1 1] Initialize/Start/End task.
)

(event `Start`
  ;[1 1 1] Initialize/Start/End task.
  ;[1 1 1] Check ability range on start event.
  (if (!= (`self.InstigatorAbilityRange`) 0.0)
    (bind _asactor (cast `Actor` (`self.TaskExecutor`)))
    (cast `/Game/RTSMultiplayer/RTSCharacters/Blueprints/RTSAIController` (`AIBlueprintHelperLibrary.GetAIController` (`Actor.GetOwner` _asactor))
      (:`CastFailed`
        (if (not (<= (`KismetMathLibrary.VSize` (- (`Actor.K2_GetActorLocation` _asactor) (`self.InstigatorAbilityTargetLocation`))) (`self.InstigatorAbilityRange`)))
          (bind _playercontroller (`self.PlayerController`)
            (:`then`
              (`/Game/RTSMultiplayer/RTSCharacters/Blueprints/RTSPlayerController.AddAttentionMessage` _playercontroller "TOO_FAR_AWAY"))
            (:`else`
              _))
          (set `self.TooFarAway?` true)
          (`self.End`))))))

(event `End`
  ;[1 1 1] Initialize/Start/End task.
)

(event `CallTaskCompleted`
  ;[1 1 1] Task completed/failed.
  (`self.TaskCompleted` self))

(event `CallTaskFailed`
  ;[1 1 1] Task completed/failed.
  (`self.TaskFailed` self))