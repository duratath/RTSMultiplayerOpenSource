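; MoveTask is a task in the RTS multiplayer task subsystem that moves its executor to a goal location or actor.
; Start runs AIMoveTo on the executor's AI controller, stores the async proxy and reports completion when the move finishes or failure when the request fails.
; End stops a still-valid move proxy and reports the task as failed.
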(event `self.Start`
  ;[1 1 1] Start move task.
  (`parent.Start`)
  (bind _controller (`/Game/RTSMultiplayer/TaskSubsystem/Blueprints/I_TaskExecutor.GetAIController` (`self.TaskExecutor`)))
  (bind _asynctaskproxy (`AITask_MoveTo.AIMoveTo` _controller (`self.GoalLocation`) (`self.GoalActor`) (`self.AcceptanceRadius`) "Default" (`self.AcceptPartialPath`) true false)
    (:`then`
      (set `self.MoveTaskProxy` _asynctaskproxy))
    (:`OnRequestFailed`
      (`self.CallTaskFailed`))
    (:`OnMoveFinished`
      (`self.CallTaskCompleted`))))

(event `self.End`
  ;[1 1 1] End move task.
  (`parent.End`)
  (bind _movetaskproxy (`self.MoveTaskProxy`)
    (:`then`
      (`GameplayTask.EndTask` _movetaskproxy)
      (`self.CallTaskFailed`))
    (:`else`)))