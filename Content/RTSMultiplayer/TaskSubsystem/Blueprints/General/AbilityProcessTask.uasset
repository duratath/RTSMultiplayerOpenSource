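; AbilityProcessTask is an RTS task Blueprint that runs an ability process as part of the task system.
; On initialization it binds to the process's completed and aborted events, and on start it launches the process unless the TooFarAway flag is set.
; Completion ends the process and reports task success, while an abort destroys the process actor and reports failure.
; Ending the task aborts the process.
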(event `self.Initialize`
  ;[1 1 1] Initialize task.
  (bind _abilityprocess (`self.AbilityProcess`)
    (:`then`
      (add `/Game/RTSMultiplayer/AbilitySubsystem/Blueprints/AbilityProcess.ProcessCompleted` _abilityprocess (`|CreateDelegate` :!event `OnProcessCompleted`))
      (add `/Game/RTSMultiplayer/AbilitySubsystem/Blueprints/AbilityProcess.ProcessAborted` _abilityprocess (`|CreateDelegate` :!event `OnProcessAborted`)))
    (:`else`)))

(event `self.Start`
  ;[1 1 1] Start task.
  (`parent.Start`)
  (if (not (`self.TooFarAway?`))
    (bind _abilityprocess (`self.AbilityProcess`)
      (:`then`
        (`/Game/RTSMultiplayer/AbilitySubsystem/Blueprints/AbilityProcess.StartProcess` _abilityprocess))
      (:`else`))))

(event `OnProcessCompleted`
  ;[1 1 1] Process completed.
  (`/Game/RTSMultiplayer/AbilitySubsystem/Blueprints/AbilityProcess.EndProcess` (`self.AbilityProcess`))
  (`self.CallTaskCompleted`))

(event `OnProcessAborted`
  ;[1 1 1] Process aborted.
  (`Actor.K2_DestroyActor` (`self.AbilityProcess`))
  (`self.CallTaskFailed`))

(event `self.End`
  ;[1 1 1] End task.
  (`parent.End`)
  (bind _abilityprocess (`self.AbilityProcess`)
    (:`then`
      (`/Game/RTSMultiplayer/AbilitySubsystem/Blueprints/AbilityProcess.AbortProcess` _abilityprocess))
    (:`else`)))