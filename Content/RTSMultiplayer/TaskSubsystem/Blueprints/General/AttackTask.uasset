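; RTS task that makes the executing actor chase and repeatedly attack a target actor.
; An AI move brings it within the AttackRange stat, using the nearest slot for buildings, then a looping timer polls TryAttack.
; In range, it faces the target and attacks through its combat component on an AttackSpeed cooldown; out of range, it resumes following.
; Target death or EndPlay stops timer and movement, reporting the task as failed.
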(event `FollowTarget`
  (params (AcceptanceRadius :type "Float (double-precision)"))
  ;[1 1 1] Follow ActorToAttack.
  (bind _asbase_rtsbuilding (cast `/Game/RTSMultiplayer/BuildingSubsystem/Blueprints/BaseRTSBuilding` (`self.ActorToAttack`))
    (:`then`
      (bind _controller (`/Game/RTSMultiplayer/TaskSubsystem/Blueprints/I_TaskExecutor.GetAIController` (`self.TaskExecutor`)))
      (bind _unitslot (`/Game/RTSMultiplayer/BuildingSubsystem/Blueprints/BaseRTSBuilding.GetNearestSlot` _asbase_rtsbuilding (cast `Actor` (`self.TaskExecutor`) :!pure true)))
      (bind _asynctaskproxy (`AITask_MoveTo.AIMoveTo` _controller (0.0 0.0 0.0) _unitslot (- AcceptanceRadius (+ (`KismetMathLibrary.VSize` (- (`/Game/RTSMultiplayer/BuildingSubsystem/Blueprints/UnitSlot.GetLocation` _unitslot) (`Actor.K2_GetActorLocation` _asbase_rtsbuilding))) 30.0)) "Disable" "Enable" true false)
        (:`then`
          (set `self.MoveAITask` _asynctaskproxy))
        (:`OnRequestFailed`
          (`KismetSystemLibrary.PrintString` null "AttackTask: Move task failed." true true (struct :`R` 1.0 :`G` 0.038718 :`A` 1.0) 5.0 :!label _label))
        (:`OnMoveFinished`
          (bind _asactor (cast `Actor` (`self.TaskExecutor`) :!label _label_2))
          (bind (_returnvalue_roll _returnvalue_pitch) (`KismetMathLibrary.BreakRotator` (`Actor.K2_GetActorRotation` _asactor)))
          (bind (_returnvalue_roll_2 _returnvalue_pitch_2 _returnvalue_yaw) (`KismetMathLibrary.BreakRotator` (`KismetMathLibrary.FindLookAtRotation` (`Actor.K2_GetActorLocation` _asactor) (`Actor.K2_GetActorLocation` (`self.ActorToAttack`)))))
          (`SceneComponent.K2_SetWorldRotation` (`Actor.RootComponent` _asactor) (`KismetMathLibrary.MakeRotator` _returnvalue_roll _returnvalue_pitch _returnvalue_yaw) false false)
          (set `self.MoveAITask` null)
          (bind _returnvalue (`KismetSystemLibrary.K2_SetTimerDelegate` (`|CreateDelegate` :!event `TryAttack`) 0.05 true))
          (set `self.TryAttackHandle` _returnvalue))))
    (:`CastFailed`
      (bind _controller_2 (`/Game/RTSMultiplayer/TaskSubsystem/Blueprints/I_TaskExecutor.GetAIController` (`self.TaskExecutor`)))
      (bind _asynctaskproxy_2 (`AITask_MoveTo.AIMoveTo` _controller_2 (0.0 0.0 0.0) (`self.ActorToAttack`) (- AcceptanceRadius 45.0) "Disable" "Enable" true false)
        (:`then`
          (set `self.MoveAITask` _asynctaskproxy_2))
        (:`OnRequestFailed`
          (goto _label))
        (:`OnMoveFinished`
          (goto _label_2))))))

(event `self.Start`
  (bind _actortoattack (`self.ActorToAttack`))
  ;[1 1 1] Event start. Start follow ActorToAttack.
  (`parent.Start`)
  (add `Actor.OnEndPlay` _actortoattack (delegate `OnTargetEndPlay`))
  (bind _asi_able_to_fight (cast `/Game/RTSMultiplayer/CombatSubsystem/Blueprints/I_AbleToFight` _actortoattack)
    (:`then`
      (bind _combatcomponent (`/Game/RTSMultiplayer/CombatSubsystem/Blueprints/I_AbleToFight.GetCombatComponent` _asi_able_to_fight))
      (add `/Game/RTSMultiplayer/CombatSubsystem/Blueprints/CombatComponent.OwnerDeath` _combatcomponent (delegate `OnTargetDeath`))
      (bind _asi_have_stats (cast `/Game/RTSMultiplayer/StatsSubsystem/Blueprints/I_HaveStats` (`self.TaskExecutor`))
        (:`then`
          (bind _statscomponent (`/Game/RTSMultiplayer/StatsSubsystem/Blueprints/I_HaveStats.GetStatsComponent` _asi_have_stats))
          (if (`.ReturnValue` (`BlueprintMapLibrary.Map_Find` (`/Game/RTSMultiplayer/StatsSubsystem/Blueprints/StatsComponent.Stats` _statscomponent) "NewEnumerator4"))
            (bind (_value _returnvalue) (`BlueprintMapLibrary.Map_Find` (`/Game/RTSMultiplayer/StatsSubsystem/Blueprints/StatsComponent.Stats` _statscomponent) "NewEnumerator2"))
            (if _returnvalue
              (`self.FollowTarget` (break `/Game/RTSMultiplayer/StatsSubsystem/Blueprints/S_Stat` _value))
              (else
                (`KismetSystemLibrary.PrintString` null "AttackTask: executor doesn't have AttackRange stat." true true (struct :`R` 1.0 :`G` 0.038718 :`A` 1.0) 5.0)))
            (else
              (`KismetSystemLibrary.PrintString` null "AttackTask: executor doesn't have AttackSpeed stat." true true (struct :`R` 1.0 :`G` 0.038718 :`A` 1.0) 5.0))))
        (:`CastFailed`
          (`KismetSystemLibrary.PrintString` null "AttackTask: executor must implement I_HaveStats interface." true true (struct :`R` 1.0 :`G` 0.038718 :`A` 1.0) 5.0))))
    (:`CastFailed`
      (`KismetSystemLibrary.PrintString` null "AttackTask: executor must implement I_AbleToFight interface." true true (struct :`R` 1.0 :`G` 0.038718 :`A` 1.0) 5.0))))

(event `OnTargetEndPlay`
  (params (Actor :type "Actor Object Reference") (EndPlayReason :type "EEndPlayReason Enum" :default "Destroyed"))
  ;[1 1 1] Event start. Start follow ActorToAttack.
  (`self.End`))

(event `OnTargetDeath`
  (params (Owner :type "Actor Object Reference"))
  ;[1 1 1] Event start. Start follow ActorToAttack.
  (`self.End`))

(event `TryAttack`
  ;[1 1 1] Try attack target.
  (if (`KismetSystemLibrary.K2_IsValidTimerHandle` (`self.TryAttackHandle`))
    (bind _statscomponent (`/Game/RTSMultiplayer/StatsSubsystem/Blueprints/I_HaveStats.GetStatsComponent` (cast `/Game/RTSMultiplayer/StatsSubsystem/Blueprints/I_HaveStats` (`self.TaskExecutor`) :!pure true)))
    (bind _stats (`/Game/RTSMultiplayer/StatsSubsystem/Blueprints/StatsComponent.Stats` _statscomponent))
    (bind _value (`BlueprintMapLibrary.Map_Find` _stats "NewEnumerator2"))
    (if (<= (`KismetMathLibrary.VSize` (- (`Actor.K2_GetActorLocation` (cast `Actor` (`self.TaskExecutor`) :!pure true)) (`Actor.K2_GetActorLocation` (`self.ActorToAttack`)))) (break `/Game/RTSMultiplayer/StatsSubsystem/Blueprints/S_Stat` _value))
      (bind _isoncooldown_ (`/Game/RTSMultiplayer/CombatSubsystem/Blueprints/I_AbleToFight.IsAttackOnCooldown?` (cast `/Game/RTSMultiplayer/CombatSubsystem/Blueprints/I_AbleToFight` (`self.TaskExecutor`) :!pure true)))
      (if (not _isoncooldown_)
        (`self.Attack` (break `/Game/RTSMultiplayer/StatsSubsystem/Blueprints/S_Stat` (`BlueprintMapLibrary.Map_Find` _stats "NewEnumerator4"))))
      (else
        (`KismetSystemLibrary.K2_InvalidateTimerHandle` (`self.TryAttackHandle`))
        (`self.FollowTarget` (break `/Game/RTSMultiplayer/StatsSubsystem/Blueprints/S_Stat` _value))))))

(event `Attack`
  (params (CooldownTime :type "Float (double-precision)"))
  (bind _taskexecutor (`self.TaskExecutor`))
  (bind _asi_able_to_fight (cast `/Game/RTSMultiplayer/CombatSubsystem/Blueprints/I_AbleToFight` _taskexecutor :!pure true))
  (bind _asactor (cast `Actor` _taskexecutor :!pure true))
  ;[1 1 1] Attack.
  (`Actor.K2_SetActorRotation` _asactor (`KismetMathLibrary.FindLookAtRotation` (`Actor.K2_GetActorLocation` _asactor) (`Actor.K2_GetActorLocation` (`self.ActorToAttack`))) false)
  (`/Game/RTSMultiplayer/CombatSubsystem/Blueprints/I_AbleToFight.StartAttackCooldown` _asi_able_to_fight CooldownTime)
  (bind _combatcomponent (`/Game/RTSMultiplayer/CombatSubsystem/Blueprints/I_AbleToFight.GetCombatComponent` _asi_able_to_fight))
  (`/Game/RTSMultiplayer/CombatSubsystem/Blueprints/CombatComponent.Attack` _combatcomponent (`self.ActorToAttack`)))

(event `self.End`
  (bind _moveaitask (`self.MoveAITask`))
  ;[1 1 1] End task.
  (if (not (`self.WasAlreadyEnded?`))
    (set `self.WasAlreadyEnded?` true)
    (if (`KismetSystemLibrary.K2_IsValidTimerHandle` (`self.TryAttackHandle`))
      (`KismetSystemLibrary.K2_InvalidateTimerHandle` (`self.TryAttackHandle`)))
    (`/Engine/EditorBlueprintResources/StandardMacros.IsValid` _moveaitask
      (:`Is Valid`
        (`GameplayTask.EndTask` _moveaitask))
      (:`Is Not Valid`
        _))
    (`self.CallTaskFailed`)))