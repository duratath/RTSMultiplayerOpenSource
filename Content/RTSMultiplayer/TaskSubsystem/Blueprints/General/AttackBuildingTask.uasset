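; AttackBuildingTask is an RTS unit task that attacks a target building from one of its free slots.
; On start it takes the nearest free slot as the move goal, or warns the player and ends if none is available.
; Once the action starts, a fast looping timer attacks through the combat component whenever the stat-driven cooldown allows.
; The task also ends on target EndPlay, and every end reports failure.
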(event `self.Start`
  ;[1 1 1] Start task. Take free building slot.
  (bind _optionaltargetactor (`self.OptionalTargetActor`)
    (:`then`
      (add `Actor.OnEndPlay` _optionaltargetactor (delegate `OnTargetEndPlay`))
      (bind _asbase_rtsbuilding (cast `/Game/RTSMultiplayer/BuildingSubsystem/Blueprints/BaseRTSBuilding` _optionaltargetactor)
        (:`then`
          (bind _freeslot (`/Game/RTSMultiplayer/BuildingSubsystem/Blueprints/BaseRTSBuilding.TakeNearestFreeSlot` _asbase_rtsbuilding (cast `Actor` (`self.TaskExecutor`) :!pure true)))
          (if (`KismetSystemLibrary.IsValid` _freeslot)
            (`/Game/RTSMultiplayer/BuildingSubsystem/Blueprints/UnitSlot.BindResetTarget` _freeslot self)
            (set `self.GoalLocation` (`Actor.K2_GetActorLocation` _freeslot))
            (`parent.Start`)
            (else
              (bind _asrtsplayer_controller (cast `/Game/RTSMultiplayer/RTSCharacters/Blueprints/RTSPlayerController` (`Pawn.GetController` (`self.InstigatorPlayerPawn`))))
              (`/Game/RTSMultiplayer/RTSCharacters/Blueprints/RTSPlayerController.AddAttentionMessage` _asrtsplayer_controller "CANT_WALK_UP_BUILDING")
              (`self.End`))))
        (:`CastFailed`
          (`self.End` :!label _label))))
    (:`else`
      (goto _label))))

(event `OnTargetEndPlay`
  (params (Actor :type "Actor Object Reference") (EndPlayReason :type "EEndPlayReason Enum" :default "Destroyed"))
  ;[1 1 1] Start task. Take free building slot.
  (`self.End`))

(event `self.StartAction`
  (params (Task :type "/Game/RTSMultiplayer/TaskSubsystem/Blueprints/Task Object Reference"))
  ;[1 1 1] Start task.
  (bind _returnvalue (`KismetSystemLibrary.K2_SetTimerDelegate` (`|CreateDelegate` :!event `TryAttack`) 0.05 true))
  (set `self.TryAttackHandle` _returnvalue))

(event `self.End`
  (bind _tryattackhandle (`self.TryAttackHandle`))
  ;[1 1 1] End task.
  (`parent.End`)
  (if (`KismetSystemLibrary.K2_IsValidTimerHandle` _tryattackhandle)
    (`KismetSystemLibrary.K2_InvalidateTimerHandle` _tryattackhandle))
  (`self.CallTaskFailed`))

(event `TryAttack`
  ;[1 1 1] Try attack.
  (if (`KismetSystemLibrary.K2_IsValidTimerHandle` (`self.TryAttackHandle`))
    (bind _isoncooldown_ (`/Game/RTSMultiplayer/CombatSubsystem/Blueprints/I_AbleToFight.IsAttackOnCooldown?` (cast `/Game/RTSMultiplayer/CombatSubsystem/Blueprints/I_AbleToFight` (`self.TaskExecutor`) :!pure true)))
    (if (not _isoncooldown_)
      (bind _statscomponent (`/Game/RTSMultiplayer/StatsSubsystem/Blueprints/I_HaveStats.GetStatsComponent` (cast `/Game/RTSMultiplayer/StatsSubsystem/Blueprints/I_HaveStats` (`self.TaskExecutor`) :!pure true)))
      (`self.Attack` (break `/Game/RTSMultiplayer/StatsSubsystem/Blueprints/S_Stat` (`BlueprintMapLibrary.Map_Find` (`/Game/RTSMultiplayer/StatsSubsystem/Blueprints/StatsComponent.Stats` _statscomponent) "NewEnumerator4"))))))

(event `Attack`
  (params (CooldownTime :type "Float (double-precision)"))
  (bind _asi_able_to_fight (cast `/Game/RTSMultiplayer/CombatSubsystem/Blueprints/I_AbleToFight` (`self.TaskExecutor`) :!pure true))
  ;[1 1 1] Attack.
  (`/Game/RTSMultiplayer/CombatSubsystem/Blueprints/I_AbleToFight.StartAttackCooldown` _asi_able_to_fight CooldownTime)
  (bind _combatcomponent (`/Game/RTSMultiplayer/CombatSubsystem/Blueprints/I_AbleToFight.GetCombatComponent` _asi_able_to_fight))
  (`/Game/RTSMultiplayer/CombatSubsystem/Blueprints/CombatComponent.Attack` _combatcomponent (`self.OptionalTargetActor`)))