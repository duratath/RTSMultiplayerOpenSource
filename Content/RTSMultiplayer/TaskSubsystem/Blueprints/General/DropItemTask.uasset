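; DropItemTask is a task in the RTS multiplayer task subsystem that drops a set of inventory items at a goal location.
; On start it runs the parent action, drops each entry in ItemsToDrop through the inventory component, then immediately reports the task complete.
; SmoothLocation gives each drop a small random horizontal offset within a box around the goal, preserving height so items scatter.
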(event `self.StartAction`
  (params (Task :type "/Game/RTSMultiplayer/TaskSubsystem/Blueprints/Task Object Reference"))
  (`parent.StartAction` Task)
  (for _array_element (`self.ItemsToDrop`)
    (`/Game/RTSMultiplayer/InventorySubsystem/Blueprints/InventoryComponent.Dropitem` (`self.InventoryComponent`) _array_element (`self.ItemSlot`) (`self.SmoothLocation` (`self.GoalLocation`))))
  (`self.CallTaskCompleted`))

(fn `SmoothLocation`
  (params (Location :type "Vector Structure"))
  (returns (NewLocation :type "Vector Structure"))
  (return (`KismetMathLibrary.MakeVector` (.x (`KismetMathLibrary.RandomPointInBoundingBox` Location (35.0 35.0 0.0))) (.y (`KismetMathLibrary.RandomPointInBoundingBox` Location (35.0 35.0 0.0))) (.z Location))))