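; GiveItemTask is an RTS task that hands a set of items from the owner's inventory to a target actor's inventory.
; On start it sets the target as the goal actor and ends if that actor ends play.
; Its action finds a suitable target slot using the first item, then moves all items there, firing unequip and equip calls.
; If no slot fits, it shows an attention message and ends.
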(event `OnTargetEndPlay`
  (params (Actor :type "Actor Object Reference") (EndPlayReason :type "EEndPlayReason Enum" :default "Destroyed"))
  ;[1 1 1] Event start.
  (`self.End`))

(event `self.Start`
  (bind _optionaltargetactor (`self.OptionalTargetActor`))
  ;[1 1 1] Event start.
  (set `self.GoalActor` _optionaltargetactor)
  (add `Actor.OnEndPlay` _optionaltargetactor (delegate `OnTargetEndPlay`))
  (`parent.Start`))

(event `self.StartAction`
  (params (Task :type "/Game/RTSMultiplayer/TaskSubsystem/Blueprints/Task Object Reference"))
  (bind _items (`self.Items`))
  (bind _targetinventorycomponent (`self.TargetInventoryComponent`))
  (bind _ownerinventorycomponent (`self.OwnerInventoryComponent`))
  ;[1 1 1] Start action.
  (`parent.StartAction` Task)
  (bind _output_get (set `self.SuitableSlot` (`/Game/RTSMultiplayer/InventorySubsystem/Blueprints/InventoryComponent.FindSuitableSlotForItem` (`self.TargetInventoryComponent`) (`|GetArrayItem` (`self.Items`)))))
  (if (!= _output_get -1)
    (for _array_element (`self.Items`)
      (`/Game/RTSMultiplayer/InventorySubsystem/Blueprints/InventoryComponent.DetachItemFromSlot` _ownerinventorycomponent (`self.SlotIndex`) _array_element)
      (`/Game/RTSMultiplayer/InventorySubsystem/Blueprints/InventoryComponent.CallItemUnequiped` _ownerinventorycomponent _array_element))
    (`/Game/RTSMultiplayer/InventorySubsystem/Blueprints/InventoryComponent.AttachAllItemsToSlot` _targetinventorycomponent (`self.SuitableSlot`) _items)
    (for _array_element_2 _items
      (`/Game/RTSMultiplayer/InventorySubsystem/Blueprints/InventoryComponent.CallItemEquiped` _targetinventorycomponent _array_element_2))
    (`self.CallTaskCompleted`)
    (else
      (`/Game/RTSMultiplayer/RTSCharacters/Blueprints/RTSPlayerController.AddAttentionMessage` (`self.PlayerController`) "CANNOT_COLLECT_ITEM")
      (`self.End`))))