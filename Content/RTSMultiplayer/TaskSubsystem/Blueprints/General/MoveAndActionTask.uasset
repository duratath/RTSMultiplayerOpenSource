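; Base task for RTS orders that first move to a target and then perform an action.
; Start caches the player controller, then constructs and starts a child MoveTask toward the goal actor, or the goal location if no valid actor exists, passing on the task executor.
; Move completion triggers StartAction, an empty event here; failure logs and ends the task.
; End unbinds both callbacks and ends the move task.
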(event `MoveTaskFailed` :!signature `self.TaskFailed`
  (params (MoveTask :type "/Game/RTSMultiplayer/TaskSubsystem/Blueprints/Task Object Reference"))
  ;[1 1 1] Create move task and bind StartAction event to TaskCompleted.
  (`KismetSystemLibrary.PrintString` null "Move failed")
  (`self.End`))

(event `self.Start`
  (bind _acceptanceradius (`self.AcceptanceRadius`))
  (bind _acceptpartialpath (`self.AcceptPartialPath`))
  (bind _movetask (`self.MoveTask`))
  ;[1 1 1] Create move task and bind StartAction event to TaskCompleted.
  (`parent.Start`)
  (bind _instigatorplayerpawn (`self.InstigatorPlayerPawn`)
    (:`then`
      (bind _asrtsplayer_controller (cast `/Game/RTSMultiplayer/RTSCharacters/Blueprints/RTSPlayerController` (`Pawn.GetController` _instigatorplayerpawn))
        (:`then`
          (set `self.PlayerController` _asrtsplayer_controller))
        (:`CastFailed`
          _)))
    (:`else`
      _))
  (bind _goalactor (`self.GoalActor`)
    (:`then`
      (bind _returnvalue (`|GenericCreateObject` "/Game/RTSMultiplayer/TaskSubsystem/Blueprints/General/MoveTask.MoveTask_C" (`self.InstigatorPlayerPawn`) (0.0 0.0 0.0) _goalactor _acceptanceradius _acceptpartialpath (`self.PlayerController`) null))
      (set `self.MoveTask` _returnvalue))
    (:`else`
      (bind _returnvalue_2 (`|GenericCreateObject` "/Game/RTSMultiplayer/TaskSubsystem/Blueprints/General/MoveTask.MoveTask_C" (`self.InstigatorPlayerPawn`) (`self.GoalLocation`) null _acceptanceradius _acceptpartialpath (`self.PlayerController`) null))
      (set `self.MoveTask` _returnvalue_2)))
  (add `self.TaskFailed` _movetask (`|CreateDelegate` :!event `MoveTaskFailed`))
  (add `self.TaskCompleted` _movetask (delegate `StartAction`))
  (set `/Game/RTSMultiplayer/TaskSubsystem/Blueprints/Task.TaskExecutor` (`self.TaskExecutor`) _movetask)
  (`self.Start` _movetask))

(event `StartAction` :!signature `self.TaskCompleted`
  (params (Task :type "/Game/RTSMultiplayer/TaskSubsystem/Blueprints/Task Object Reference"))
  ;[1 1 1] Create move task and bind StartAction event to TaskCompleted.
)

(event `self.End`
  (bind _movetask (`self.MoveTask`))
  ;[1 1 1] End task.
  (bind _movetask_2 (`self.MoveTask`)
    (:`then`
      (remove `self.TaskFailed` _movetask (`|CreateDelegate` :!event `MoveTaskFailed`))
      (remove `self.TaskCompleted` _movetask (delegate `StartAction`))
      (`self.End` _movetask_2))
    (:`else`)))