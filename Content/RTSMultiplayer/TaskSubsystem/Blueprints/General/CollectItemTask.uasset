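; Task Blueprint for the RTS task subsystem that has its executor collect an inventory item passed as the optional target actor.
; On start, it validates the item and its AbleToCollect flag, then calls CollectItem on the executor's inventory component through I_HaveInventory and reports completion.
; An invalid or uncollectable target routes to End, which reports failure.
; An executor without the interface only prints an error, leaving the task unresolved.
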(event `self.StartAction`
  (params (Task :type "/Game/RTSMultiplayer/TaskSubsystem/Blueprints/Task Object Reference"))
  (`parent.StartAction` Task)
  (bind _optionaltargetactor (`self.OptionalTargetActor`)
    (:`then`
      (bind _asinventory_item (cast `/Game/RTSMultiplayer/InventorySubsystem/Blueprints/InventoryItem` _optionaltargetactor)
        (:`then`
          (if (`/Game/RTSMultiplayer/InventorySubsystem/Blueprints/InventoryItem.AbleToCollect?` _asinventory_item)
            (bind _asi_have_inventory (cast `/Game/RTSMultiplayer/InventorySubsystem/Blueprints/I_HaveInventory` (`self.TaskExecutor`))
              (:`then`
                (bind _inventorycomponent (`/Game/RTSMultiplayer/InventorySubsystem/Blueprints/I_HaveInventory.GetInventoryComponent` _asi_have_inventory))
                (`/Game/RTSMultiplayer/InventorySubsystem/Blueprints/InventoryComponent.CollectItem` _inventorycomponent _asinventory_item (`self.PlayerController`))
                (`self.CallTaskCompleted`))
              (:`CastFailed`
                (`KismetSystemLibrary.PrintString` _asinventory_item "CollectItemTask: Executor must implement I_HaveInventory interface." true true (struct :`R` 1.0 :`G` 0.038718 :`A` 1.0) 5.0)))
            (else
              (`self.End` :!label _label))))
        (:`CastFailed`
          (goto _label))))
    (:`else`
      (goto _label))))

(event `self.End`
  (`parent.End`)
  (`self.CallTaskFailed`))