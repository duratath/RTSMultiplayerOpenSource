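; Worker task that gathers a resource from a ResourceSeed and carries it to storage, looping while the seed lasts.
; The parent task moves to the seed, then a faction-based timer deducts the yield.
; A child MoveTask walks to a free slot at the nearest storage, where a second timer credits the player and restarts.
; End clears timers and the child task; PlayPossibleAnimation is an empty hook.
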(event `StopPossibleAnimation`
  ;[1 1 1] Start/stop possible animation.
  (bind _asbase_rtsunit (cast `/Game/RTSMultiplayer/RTSCharacters/Blueprints/BaseRTSUnit` (`self.TaskExecutor`)))
  (`/Engine/EditorBlueprintResources/StandardMacros.IsValid` _asbase_rtsunit
    (:`Is Valid`
      (`/Game/RTSMultiplayer/RTSCharacters/Blueprints/BaseRTSUnit.StopCurrentAnimationMulticast` _asbase_rtsunit))))

(event `PlayPossibleAnimation`
  ;[1 1 1] Start/stop possible animation.
)

(event `self.Start`
  (bind _instigatorplayerpawn (`self.InstigatorPlayerPawn`))
  ;[1 1 1] Event start. Check for having resource storage.
  (set `self.CanAbort?` false)
  (if (> (`KismetArrayLibrary.Array_Length` (`/Game/RTSMultiplayer/RTSCharacters/Blueprints/BasePlayerCharacter.GetDefaultResourceStorages` (cast `/Game/RTSMultiplayer/RTSCharacters/Blueprints/BasePlayerCharacter` _instigatorplayerpawn :!pure true) (`self.ResourceType`))) 0)
    (bind _optionaltargetactor (`self.OptionalTargetActor`)
      (:`then`
        (set `self.GoalActor` _optionaltargetactor)
        (set `self.AcceptPartialPath` "Enable")
        (set `self.AcceptanceRadius` (`/Game/RTSMultiplayer/ResourcesSubsystem/Blueprints/ResourceSeed.MoveAcceptanceRadius` (cast `/Game/RTSMultiplayer/ResourcesSubsystem/Blueprints/ResourceSeed` _optionaltargetactor :!pure true)))
        (`parent.Start`))
      (:`else`
        (`self.CallTaskCompleted`)))
    (else
      (bind _asrtsplayer_controller (cast `/Game/RTSMultiplayer/RTSCharacters/Blueprints/RTSPlayerController` (`Pawn.GetController` _instigatorplayerpawn))
        (:`then`
          (`/Game/RTSMultiplayer/RTSCharacters/Blueprints/RTSPlayerController.AddAttentionMessage` _asrtsplayer_controller "HAVE_NOT_RESOURCE_STORAGE")
          (`self.CallTaskCompleted`))
        (:`CastFailed`
          (`self.End`))))))

(event `self.StartAction`
  (params (Task :type "/Game/RTSMultiplayer/TaskSubsystem/Blueprints/Task Object Reference"))
  ;[1 1 1] Wait CollectingTime second, then collect.
  (bind _optionaltargetactor (`self.OptionalTargetActor`)
    (:`then`
      (set `self.SeedLocation` (`Actor.K2_GetActorLocation` _optionaltargetactor))
      (bind _asresource_seed (cast `/Game/RTSMultiplayer/ResourcesSubsystem/Blueprints/ResourceSeed` _optionaltargetactor)
        (:`then`
          (if (`/Game/RTSMultiplayer/ResourcesSubsystem/Blueprints/ResourceSeed.HasResources?` _asresource_seed)
            (`self.PlayPossibleAnimation`)
            (bind _returnvalue (`KismetSystemLibrary.K2_SetTimerDelegate` (`|CreateDelegate` :!event `CollectResource`) (`BlueprintMapLibrary.Map_Find` (`/Game/RTSMultiplayer/ResourcesSubsystem/Blueprints/ResourceSeed.CollectingTime` _asresource_seed) (`/Game/RTSMultiplayer/RTSCharacters/Blueprints/BasePlayerCharacter.PlayerFaction` (cast `/Game/RTSMultiplayer/RTSCharacters/Blueprints/BasePlayerCharacter` (`self.InstigatorPlayerPawn`) :!pure true)))))
            (set `self.CollectResourceHandle` _returnvalue)
            (else
              (`self.CallTaskCompleted`))))
        (:`CastFailed`
          (`self.End`))))
    (:`else`
      (`self.CallTaskCompleted`))))

(event `CollectResource`
  (bind _collectresourcehandle (`self.CollectResourceHandle`))
  (bind _building (`/Game/RTSMultiplayer/RTSCharacters/Blueprints/BasePlayerCharacter.GetDefaultResourceStorages` (cast `/Game/RTSMultiplayer/RTSCharacters/Blueprints/BasePlayerCharacter` (`self.InstigatorPlayerPawn`) :!pure true) (`self.ResourceType`)))
  ;[1 1 1] Go to the default resource storage.
  (if (`KismetSystemLibrary.K2_IsValidTimerHandle` _collectresourcehandle)
    (`KismetSystemLibrary.K2_InvalidateTimerHandle` _collectresourcehandle)
    (`self.StopPossibleAnimation`)
    (bind _optionaltargetactor (`self.OptionalTargetActor`)
      (:`then`
        (bind _asresource_seed (cast `/Game/RTSMultiplayer/ResourcesSubsystem/Blueprints/ResourceSeed` _optionaltargetactor)
          (:`then`
            (if (`/Game/RTSMultiplayer/ResourcesSubsystem/Blueprints/ResourceSeed.HasResources?` _asresource_seed)
              (bind _output_get (set `self.CollectedResourceAmount` (`/Game/RTSMultiplayer/ResourcesSubsystem/Blueprints/ResourceSeed.GetPossibleCollectingAmount` _asresource_seed (`/Game/RTSMultiplayer/RTSCharacters/Blueprints/BasePlayerCharacter.PlayerFaction` (cast `/Game/RTSMultiplayer/RTSCharacters/Blueprints/BasePlayerCharacter` (`self.InstigatorPlayerPawn`) :!pure true)))))
              (`/Game/RTSMultiplayer/ResourcesSubsystem/Blueprints/ResourceSeed.ReduceRemainingResources` _asresource_seed _output_get)
              (if (> (`KismetArrayLibrary.Array_Length` _building) 0)
                (bind _storage (`self.GetNearestResourceStorage` _building))
                (bind _freeslot (`/Game/RTSMultiplayer/BuildingSubsystem/Blueprints/BaseRTSBuilding.TakeNearestFreeSlot` _storage (cast `Actor` (`self.TaskExecutor`) :!pure true)))
                (`/Engine/EditorBlueprintResources/StandardMacros.IsValid` _freeslot
                  (:`Is Valid`
                    (bind _returnvalue (`|GenericCreateObject` "/Game/RTSMultiplayer/TaskSubsystem/Blueprints/General/MoveTask.MoveTask_C" (`self.InstigatorPlayerPawn`) (`Actor.K2_GetActorLocation` _freeslot) null 15.0 "Enable" null null))
                    (`/Game/RTSMultiplayer/BuildingSubsystem/Blueprints/UnitSlot.BindResetTarget` _freeslot _returnvalue)
                    (bind _output_get_2 (set `self.MoveToStorageTask` _returnvalue))
                    (add `self.TaskCompleted` _output_get_2 (`|CreateDelegate` :!event `DropResources`))
                    (set `/Game/RTSMultiplayer/TaskSubsystem/Blueprints/Task.TaskExecutor` (`self.TaskExecutor`) _output_get_2)
                    (`self.Start` _output_get_2))
                  (:`Is Not Valid`
                    (`self.End` :!label _label)))
                (else
                  (bind _asrtsplayer_controller (cast `/Game/RTSMultiplayer/RTSCharacters/Blueprints/RTSPlayerController` (`Pawn.GetController` (`self.InstigatorPlayerPawn`))))
                  (`/Game/RTSMultiplayer/RTSCharacters/Blueprints/RTSPlayerController.AddAttentionMessage` _asrtsplayer_controller "CANT_WALK_UP_BUILDING")
                  (goto _label)))
              (else
                (`self.CallTaskCompleted`))))
          (:`CastFailed`
            (`self.End`))))
      (:`else`
        (`self.CallTaskCompleted`)))
    (else
      (`self.End`))))

(event `DropResources` :!signature `self.TaskCompleted`
  (params (MoveToStorageTask :type "/Game/RTSMultiplayer/TaskSubsystem/Blueprints/Task Object Reference"))
  ;[1 1 1] Wait DropResourceTime second, then back to work.
  (set `self.CanAbort?` true)
  (bind _returnvalue (`KismetSystemLibrary.K2_SetTimerDelegate` (`|CreateDelegate` :!event `BackToWork`) (`self.DropResourcesTime`)))
  (set `self.BackToWorkHandle` _returnvalue))

(event `BackToWork`
  (bind _backtoworkhandle (`self.BackToWorkHandle`))
  ;[1 1 1] Wait DropResourceTime second, then back to work.
  (if (`KismetSystemLibrary.K2_IsValidTimerHandle` _backtoworkhandle)
    (`KismetSystemLibrary.K2_InvalidateTimerHandle` _backtoworkhandle)
    (`/Game/RTSMultiplayer/RTSCharacters/Blueprints/BasePlayerCharacter.AddConsumableResource` (cast `/Game/RTSMultiplayer/RTSCharacters/Blueprints/BasePlayerCharacter` (`self.InstigatorPlayerPawn`) :!pure true) (`self.ResourceType`) (`self.CollectedResourceAmount`))
    (`self.OptionalTargetActor`
      (:`then`
        (`self.Start`))
      (:`else`
        (`self.CallTaskCompleted`)))
    (else
      (`self.End`))))

(event `self.End`
  (bind _backtoworkhandle (`self.BackToWorkHandle`))
  (bind _collectresourcehandle (`self.CollectResourceHandle`))
  ;[1 1 1] End event.
  (`parent.End`)
  (`self.StopPossibleAnimation`)
  (if (`KismetSystemLibrary.K2_IsValidTimerHandle` _backtoworkhandle)
    (`KismetSystemLibrary.K2_InvalidateTimerHandle` _backtoworkhandle))
  (if (`KismetSystemLibrary.K2_IsValidTimerHandle` _collectresourcehandle)
    (`KismetSystemLibrary.K2_InvalidateTimerHandle` _collectresourcehandle))
  (bind _movetostoragetask (`self.MoveToStorageTask`)
    (:`then`
      (remove `self.TaskCompleted` (`self.MoveToStorageTask`) (`|CreateDelegate` :!event `DropResources`))
      (`self.End` _movetostoragetask))
    (:`else`
      _))
  (`self.CallTaskFailed`))

(fn `GetNearestResourceStorage`
  (params (ResourceStorages :type "Array of /Game/RTSMultiplayer/BuildingSubsystem/Blueprints/BaseRTSBuilding Object Reference"))
  (returns (Storage :type "/Game/RTSMultiplayer/BuildingSubsystem/Blueprints/BaseRTSBuilding Object Reference"))
  (locals (NearestDistance :type "Float (double-precision)" :default 999999.0) (NearestStorage :type "/Game/RTSMultiplayer/BuildingSubsystem/Blueprints/BaseRTSBuilding Object Reference"))
  (bind _asactor (cast `Actor` (`self.TaskExecutor`)))
  (for _array_element ResourceStorages
    (bind _returnvalue (`Actor.GetDistanceTo` _array_element _asactor))
    (if (< _returnvalue (`local.NearestDistance`))
      (set `local.NearestDistance` _returnvalue)
      (set `local.NearestStorage` _array_element)))
  (return (`local.NearestStorage`)))