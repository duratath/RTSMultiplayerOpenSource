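; Worker task for the RTS task subsystem that sends its executor to repair or build a target building.
; On start it claims the nearest free building slot as the move goal, or posts an attention message and ends if none is free.
; The action adds the executor to the building's builders list and completes when the building-built event fires.
; Ending removes the executor from that list and reports the task as failed.
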(event `self.Start`
  ;[1 1 1] Start task. Take free building slot.
  (bind _optionaltargetactor (`self.OptionalTargetActor`)
    (:`then`
      (bind _asbase_rtsbuilding (cast `/Game/RTSMultiplayer/BuildingSubsystem/Blueprints/BaseRTSBuilding` _optionaltargetactor)
        (:`then`
          (bind _freeslot (`/Game/RTSMultiplayer/BuildingSubsystem/Blueprints/BaseRTSBuilding.TakeNearestFreeSlot` _asbase_rtsbuilding (cast `Actor` (`self.TaskExecutor`) :!pure true)))
          (if (`KismetSystemLibrary.IsValid` _freeslot)
            (`/Game/RTSMultiplayer/BuildingSubsystem/Blueprints/UnitSlot.BindResetTarget` _freeslot self)
            (set `self.GoalLocation` (`Actor.K2_GetActorLocation` _freeslot))
            (`parent.Start`)
            (else
              (bind _asrtsplayer_controller (cast `/Game/RTSMultiplayer/RTSCharacters/Blueprints/RTSPlayerController` (`Pawn.GetController` (`self.InstigatorPlayerPawn`)))
                (:`then`
                  (`/Game/RTSMultiplayer/RTSCharacters/Blueprints/RTSPlayerController.AddAttentionMessage` _asrtsplayer_controller "CANT_WALK_UP_BUILDING"))
                (:`CastFailed`
                  _))
              (`self.End`))))
        (:`CastFailed`
          (`self.End` :!label _label))))
    (:`else`
      (goto _label))))

(event `self.StartAction`
  (params (Task :type "/Game/RTSMultiplayer/TaskSubsystem/Blueprints/Task Object Reference"))
  ;[1 1 1] Start build task.
  (bind _optionaltargetactor (`self.OptionalTargetActor`)
    (:`then`
      (bind _asbase_rtsbuilding (cast `/Game/RTSMultiplayer/BuildingSubsystem/Blueprints/BaseRTSBuilding` _optionaltargetactor))
      (`/Game/RTSMultiplayer/BuildingSubsystem/Blueprints/BaseRTSBuilding.AddActorToBuildersList` _asbase_rtsbuilding (`self.TaskExecutor`))
      (add `/Game/RTSMultiplayer/BuildingSubsystem/Blueprints/BaseRTSBuilding.BuildingBuilt` _asbase_rtsbuilding (delegate `OnBuilt`)))
    (:`else`
      (`self.End`))))

(event `OnBuilt`
  ;[1 1 1] Start build task.
  (`self.CallTaskCompleted`))

(event `self.End`
  ;[1 1 1] End build task.
  (`parent.End`)
  (bind _optionaltargetactor (`self.OptionalTargetActor`)
    (:`then`
      (bind _asbase_rtsbuilding (cast `/Game/RTSMultiplayer/BuildingSubsystem/Blueprints/BaseRTSBuilding` _optionaltargetactor)
        (:`then`
          (`/Game/RTSMultiplayer/BuildingSubsystem/Blueprints/BaseRTSBuilding.RemoveActorFromBuildersList` _asbase_rtsbuilding (`self.TaskExecutor`)))
        (:`CastFailed`
          _)))
    (:`else`
      _))
  (`self.CallTaskFailed`))