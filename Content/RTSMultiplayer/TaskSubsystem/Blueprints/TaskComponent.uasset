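; Task component that gives an RTS task executor, such as a unit, a queue of tasks run one at a time.
; Setting a task ends and replaces the queue, while adding appends, starting immediately if empty.
; Completion or failure events stop unit animation and advance the queue, with failures also showing a message.
; Queue changes and ability process starts are relayed through Call events, and owner death or EndPlay ends all tasks.
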(event `StopPossibleAnimation`
  ;[1 1 1] Stop possible character animation.
  (bind _asbase_rtsunit (cast `/Game/RTSMultiplayer/RTSCharacters/Blueprints/BaseRTSUnit` (`self.GetOwner`)))
  (`/Game/RTSMultiplayer/RTSCharacters/Blueprints/BaseRTSUnit.StopCurrentAnimation` _asbase_rtsunit))

(event `OnCurrentTaskFailed`
  (params (Task :type "/Game/RTSMultiplayer/TaskSubsystem/Blueprints/Task Object Reference"))
  ;[1 1 1] On current task failed.
  ; Show attention message.
  (`self.StopPossibleAnimation`)
  (`self.TaskRemovedFromQueue` Task)
  (`/Game/RTSMultiplayer/TaskSubsystem/Blueprints/Task.ShowFailedMessage` Task)
  (`self.OnTaskEnded` Task))

(event `OnCurrentTaskCompleted`
  (params (Task :type "/Game/RTSMultiplayer/TaskSubsystem/Blueprints/Task Object Reference"))
  ;[1 1 1] On current task completed.
  (`self.StopPossibleAnimation`)
  (`self.CurrentTaskCompleted` Task)
  (`self.OnTaskEnded` Task))

(event `CallProcessTaskStarted`
  (params (DelayProcess :type "/Game/RTSMultiplayer/AbilitySubsystem/Blueprints/AbilityProcess Object Reference"))
  ;[1 1 1] Call current task started. Multicast.
  (`self.CurrentTaskStarted` DelayProcess))

(event `SetCurrentTask`
  (params (NewTask :type "/Game/RTSMultiplayer/TaskSubsystem/Blueprints/Task Object Reference"))
  (bind _taskqueue (`self.TaskQueue`))
  (bind _taskqueue_2 (`self.TaskQueue`))
  (bind _output (`|GetArrayItem` _taskqueue))
  ;[1 1 1] Set new current task.
  (set `self.IsCurrentlySettingNewTask?` true)
  (`self.TaskAddedToQueue` NewTask)
  (bind _asi_task_executor (cast `/Game/RTSMultiplayer/TaskSubsystem/Blueprints/I_TaskExecutor` (`self.GetOwner`))
    (:`then`
      (if (!= (`KismetArrayLibrary.Array_Length` _taskqueue) 0)
        (remove `/Game/RTSMultiplayer/TaskSubsystem/Blueprints/Task.TaskCompleted` _output (`|CreateDelegate` :!event `OnCurrentTaskCompleted`))
        (remove `/Game/RTSMultiplayer/TaskSubsystem/Blueprints/Task.TaskFailed` _output (`|CreateDelegate` :!event `OnCurrentTaskFailed`))
        (for (_array_element _array_index) (`self.TaskQueue`)
          (bind _asability_process_task (cast `/Game/RTSMultiplayer/TaskSubsystem/Blueprints/General/AbilityProcessTask` _array_element)
            (:`then`
              (if (and (== _array_index 0) (`KismetMathLibrary.ClassIsChildOf` (`GameplayStatics.GetObjectClass` (`/Game/RTSMultiplayer/TaskSubsystem/Blueprints/General/AbilityProcessTask.AbilityProcess` _asability_process_task)) "/Game/RTSMultiplayer/AbilitySubsystem/Blueprints/CombatAbilities/SpellChannelingProcess.SpellChannelingProcess_C"))
                (`self.CurrentTaskCompleted` _array_element)
                (else
                  (`self.TaskRemovedFromQueue` _array_element)))
              (`/Game/RTSMultiplayer/TaskSubsystem/Blueprints/Task.End` _asability_process_task))
            (:`CastFailed`
              (`self.TaskRemovedFromQueue` _array_element))))
        (`/Game/RTSMultiplayer/TaskSubsystem/Blueprints/Task.End` _output))
      (`self.StopPossibleAnimation`)
      (`KismetArrayLibrary.Array_Clear` _taskqueue_2)
      (`KismetArrayLibrary.Array_Add` _taskqueue_2 NewTask)
      (set `/Game/RTSMultiplayer/TaskSubsystem/Blueprints/Task.TaskExecutor` _asi_task_executor NewTask)
      (add `/Game/RTSMultiplayer/TaskSubsystem/Blueprints/Task.TaskCompleted` NewTask (`|CreateDelegate` :!event `OnCurrentTaskCompleted`))
      (add `/Game/RTSMultiplayer/TaskSubsystem/Blueprints/Task.TaskFailed` NewTask (`|CreateDelegate` :!event `OnCurrentTaskFailed`))
      (`/Game/RTSMultiplayer/TaskSubsystem/Blueprints/Task.Initialize` NewTask)
      (`/Game/RTSMultiplayer/TaskSubsystem/Blueprints/Task.Start` NewTask)
      (bind _asability_process_task_2 (cast `/Game/RTSMultiplayer/TaskSubsystem/Blueprints/General/AbilityProcessTask` NewTask)
        (:`then`
          (`self.CallProcessTaskStarted` (`/Game/RTSMultiplayer/TaskSubsystem/Blueprints/General/AbilityProcessTask.AbilityProcess` _asability_process_task_2)))
        (:`CastFailed`
          _))
      (set `self.IsCurrentlySettingNewTask?` false))
    (:`CastFailed`
      (set `self.IsCurrentlySettingNewTask?` false))))

(event `OnTaskEnded`
  (params (Task :type "/Game/RTSMultiplayer/TaskSubsystem/Blueprints/Task Object Reference"))
  (bind _output (`|GetArrayItem` (`self.TaskQueue`)))
  ;[1 1 1] Set new current task.
  (`KismetArrayLibrary.Array_Remove` (`self.TaskQueue`))
  (if (`self.IsCurrentlySettingNewTask?`)
    _
    (elif (!= (`KismetArrayLibrary.Array_Length` (`self.TaskQueue`)) 0)
      (remove `/Game/RTSMultiplayer/TaskSubsystem/Blueprints/Task.TaskFailed` _output (`|CreateDelegate` :!event `RemoveTaskFromQueue`))
      (add `/Game/RTSMultiplayer/TaskSubsystem/Blueprints/Task.TaskCompleted` _output (`|CreateDelegate` :!event `OnCurrentTaskCompleted`))
      (add `/Game/RTSMultiplayer/TaskSubsystem/Blueprints/Task.TaskFailed` _output (`|CreateDelegate` :!event `OnCurrentTaskFailed`))
      (`/Game/RTSMultiplayer/TaskSubsystem/Blueprints/Task.Start` _output)
      (bind _asability_process_task (cast `/Game/RTSMultiplayer/TaskSubsystem/Blueprints/General/AbilityProcessTask` _output))
      (`self.CallProcessTaskStarted` (`/Game/RTSMultiplayer/TaskSubsystem/Blueprints/General/AbilityProcessTask.AbilityProcess` _asability_process_task)))))

(event `AddTaskToQueue`
  (params (NewTask :type "/Game/RTSMultiplayer/TaskSubsystem/Blueprints/Task Object Reference"))
  ;[1 1 1] Add task to the queue and remove task from queue.
  (bind _asi_task_executor (cast `/Game/RTSMultiplayer/TaskSubsystem/Blueprints/I_TaskExecutor` (`self.GetOwner`)))
  (if (== (`KismetArrayLibrary.Array_Length` (`self.TaskQueue`)) 0)
    (`self.SetCurrentTask` NewTask)
    (else
      (set `/Game/RTSMultiplayer/TaskSubsystem/Blueprints/Task.TaskExecutor` _asi_task_executor NewTask)
      (add `/Game/RTSMultiplayer/TaskSubsystem/Blueprints/Task.TaskFailed` NewTask (`|CreateDelegate` :!event `RemoveTaskFromQueue`))
      (`/Game/RTSMultiplayer/TaskSubsystem/Blueprints/Task.Initialize` NewTask)
      (`KismetArrayLibrary.Array_Add` (`self.TaskQueue`) NewTask)
      (`self.TaskAddedToQueue` NewTask))))

(event `RemoveTaskFromQueue`
  (params (Task :type "/Game/RTSMultiplayer/TaskSubsystem/Blueprints/Task Object Reference"))
  ;[1 1 1] Add task to the queue and remove task from queue.
  (if (not (`self.IsCurrentlySettingNewTask?`))
    (`self.TaskRemovedFromQueue` Task)
    (remove `/Game/RTSMultiplayer/TaskSubsystem/Blueprints/Task.TaskFailed` Task (`|CreateDelegate` :!event `RemoveTaskFromQueue`))
    (`KismetArrayLibrary.Array_RemoveItem` (`self.TaskQueue`) Task)))

(event `self.ReceiveBeginPlay`
  ;[1 1 1] Bind event to owner death on begin play.
  (bind _asi_able_to_fight (cast `/Game/RTSMultiplayer/CombatSubsystem/Blueprints/I_AbleToFight` (`self.GetOwner`)))
  (bind _combatcomponent (`/Game/RTSMultiplayer/CombatSubsystem/Blueprints/I_AbleToFight.GetCombatComponent` _asi_able_to_fight))
  (add `/Game/RTSMultiplayer/CombatSubsystem/Blueprints/CombatComponent.OwnerDeath` _combatcomponent (`|CreateDelegate` :!event `OnOwnerDeath`)))

(event `self.ReceiveEndPlay`
  (params (EndPlayReason :type "EEndPlayReason Enum" :default "Destroyed"))
  ;[1 1 1] End all tasks on end play.
  (for _array_element (`self.TaskQueue`) :!label _label
    (`/Engine/EditorBlueprintResources/StandardMacros.IsValid` _array_element
      (:`Is Valid`
        (`/Game/RTSMultiplayer/TaskSubsystem/Blueprints/Task.End` _array_element)))))

(event `OnOwnerDeath`
  (params (Owner :type "Actor Object Reference"))
  ;[1 1 1] End all tasks on end play.
  (goto _label))