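; TriangleSquad is an RTS movement squad Blueprint that arranges its actors in a triangle formation.
; RecalculateSquadDisplacements rebuilds SquadTargetDisplacements with one offset per actor, filling rows that each hold one more slot than the row ahead.
; Rows step back along negative X by DistanceBetweenActors and center on Y, with even-sized rows shifted half a spacing to stay symmetric.
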(event `self.RecalculateSquadDisplacements`
  (params (GoalLocation :type "Vector Structure"))
  (bind _currentrow (`self.CurrentRow`))
  (bind _squadtargetdisplacements (`self.SquadTargetDisplacements`))
  (set `self.CurrentRowIndex` 0)
  (set `self.CurrentRow` 0)
  (`KismetArrayLibrary.Array_Clear` _squadtargetdisplacements)
  (for _ (`self.Actors`)
    (`KismetArrayLibrary.Array_Add` _squadtargetdisplacements (`KismetMathLibrary.MakeVector` (* (* (`self.CurrentRow`) -1) (`self.DistanceBetweenActors`)) (- (* (- (`self.CurrentRowIndex`) (/ (`self.CurrentRow`) 2)) (`self.DistanceBetweenActors`)) (select `bool` (== (mod (+ (`self.CurrentRow`) 1) 2) 0) :`true` (/ (`self.DistanceBetweenActors`) 2.0)))))
    (bind _result (`/Engine/EditorBlueprintResources/StandardMacros.IncrementInt` (`self.CurrentRowIndex`))
      (:`  `
        (if (== (+ _currentrow 1) _result)
          (`/Engine/EditorBlueprintResources/StandardMacros.IncrementInt` _currentrow
            (:`  `
              (set `self.CurrentRowIndex` 0))))))))