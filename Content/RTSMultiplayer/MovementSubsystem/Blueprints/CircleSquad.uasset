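; CircleSquad is a squad formation Blueprint for RTS unit movement that spreads units evenly around a circle.
; RecalculateSquadDisplacements rebuilds the target displacement list by stepping an angle by 2π over actor count at the set Radius, taking Z from the goal location.
; A lone actor gets a single displacement without the circle math.
; Unit rotation is unimplemented: RotateUnits is empty and FindUnitRotationAngle always returns zero.
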(event `self.RecalculateSquadDisplacements`
  (params (GoalLocation :type "Vector Structure"))
  (bind _squadtargetdisplacements (`self.SquadTargetDisplacements`))
  (`KismetArrayLibrary.Array_Clear` _squadtargetdisplacements)
  (if (== (`KismetArrayLibrary.Array_Length` (`self.Actors`)) 1)
    (`KismetArrayLibrary.Array_Add` (`self.SquadTargetDisplacements`))
    (else
      (set `self.TDelta` (/ (* (`KismetMathLibrary.GetPI`) 2.0) (`KismetMathLibrary.Conv_IntToDouble` (`KismetArrayLibrary.Array_Length` (`self.Actors`)))))
      (for _ (`self.Actors`)
        (`KismetArrayLibrary.Array_Add` _squadtargetdisplacements (`KismetMathLibrary.MakeVector` (* (`self.Radius`) (`KismetMathLibrary.Cos` (`self.CurrentT`))) (* (`self.Radius`) (`KismetMathLibrary.Sin` (`self.CurrentT`))) (.z GoalLocation)))
        (set `self.CurrentT` (+ (`self.CurrentT`) (`self.TDelta`)))))))

(event `self.RotateUnits`
  (params (Angle :type "Float (single-precision)")))

(fn `FindUnitRotationAngle`
  (params (TargetLocation :type "Vector Structure (by ref)"))
  (returns (Angle :type "Float (double-precision)"))
  (return 0.0))