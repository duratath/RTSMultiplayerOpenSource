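; Component for the RTS camera that turns static mesh actors translucent when they block the view of selected actors.
; A looping timer runs multi line traces from the camera to each actor in the HUD selection.
; Hit meshes have their materials and Visibility response saved, then get a translucent dynamic material and ignore the Visibility channel.
; A per-mesh flag map, reset each pass, identifies meshes no longer hit so their saved state is restored.
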(event `self.ReceiveBeginPlay`
  ;[1 1 1] Multi line tracing, create dynamic transparent material instance.
  (`KismetSystemLibrary.K2_SetTimerDelegate` (delegate `TryToMakeTransparent`) (`self.ObstacleTraceDelta`) true))

(event `TryToMakeTransparent`
  (bind _transparentstaticmeshes (`self.TransparentStaticMeshes`))
  (bind _transparentstaticmeshes_2 (`self.TransparentStaticMeshes`))
  (bind _transparentstaticmeshes_3 (`self.TransparentStaticMeshes`))
  ;[1 1 1] Multi line tracing, create dynamic transparent material instance.
  (bind _camera (`self.Camera`)
    (:`then`
      (bind _asrtsplayer_controller (cast `/Game/RTSMultiplayer/RTSCharacters/Blueprints/RTSPlayerController` (`GameplayStatics.GetPlayerController` 0)))
      (bind _playerhud (`/Game/RTSMultiplayer/RTSCharacters/Blueprints/RTSPlayerController.PlayerHUD` _asrtsplayer_controller)
        (:`then`
          (bind _keys (`BlueprintMapLibrary.Map_Keys` _transparentstaticmeshes))
          (for _array_element _keys
            (`BlueprintMapLibrary.Map_Add` _transparentstaticmeshes _array_element))
          (for _array_element_2 (`/Game/RTSMultiplayer/SelectionSubsystem/Widgets/W_SelectionEnvironment.SelectedActors` (`/Game/RTSMultiplayer/RTSCoreUI/Widgets/W_PlayerHUD.W_SelectionEnvironment` _playerhud))
            (bind _outhits (`KismetSystemLibrary.LineTraceMultiForObjects` :`Start` (`SceneComponent.K2_GetComponentLocation` _camera) :`End` (`Actor.K2_GetActorLocation` _array_element_2) :`ObjectTypes` (`|MakeArray` "ObjectTypeQuery1" "ObjectTypeQuery2" :!type "EObjectTypeQuery Enum") :`bTraceComplex` true :`DrawTime` 1.0))
            (for _array_element_3 _outhits
              (bind _asstatic_mesh_actor (cast `StaticMeshActor` (`.HitActor` (`GameplayStatics.BreakHitResult` _array_element_3))))
              (if (`.ReturnValue` (`BlueprintMapLibrary.Map_Find` _transparentstaticmeshes_2 _asstatic_mesh_actor))
                (`BlueprintMapLibrary.Map_Add` _transparentstaticmeshes_2 _asstatic_mesh_actor true)
                (else
                  (bind _staticmeshcomponent (`StaticMeshActor.StaticMeshComponent` _asstatic_mesh_actor))
                  (`BlueprintMapLibrary.Map_Add` (`self.SavedStaticMeshesMaterials`) _asstatic_mesh_actor (make `/Game/RTSMultiplayer/MovementSubsystem/Blueprints/S_ArrayOfMaterialInstances` (`MeshComponent.GetMaterials` _staticmeshcomponent)))
                  (for _index (range (`PrimitiveComponent.GetNumMaterials` _staticmeshcomponent))
                    (`PrimitiveComponent.CreateDynamicMaterialInstance` _staticmeshcomponent _index "/Game/RTSMultiplayer/MovementSubsystem/Materials/M_SimpleTranslucent.M_SimpleTranslucent" "None")
                    (`BlueprintMapLibrary.Map_Add` (`self.SavedVisibilityResoponses`) _asstatic_mesh_actor (`PrimitiveComponent.GetCollisionResponseToChannel` _staticmeshcomponent "ECC_Visibility"))
                    (`PrimitiveComponent.SetCollisionResponseToChannel` _staticmeshcomponent "ECC_Visibility" "ECR_Ignore")
                    (`BlueprintMapLibrary.Map_Add` (`self.TransparentStaticMeshes`) _asstatic_mesh_actor true))))))
          (bind _keys_2 (`BlueprintMapLibrary.Map_Keys` _transparentstaticmeshes_3))
          (for _array_element_4 _keys_2
            (if (not (`BlueprintMapLibrary.Map_Find` _transparentstaticmeshes_3 _array_element_4))
              (bind (_value _returnvalue) (`BlueprintMapLibrary.Map_Find` (`self.SavedStaticMeshesMaterials`) _array_element_4))
              (if _returnvalue
                (bind _staticmeshcomponent_2 (`StaticMeshActor.StaticMeshComponent` _array_element_4))
                (for _index_2 (range (`PrimitiveComponent.GetNumMaterials` _staticmeshcomponent_2))
                  (`PrimitiveComponent.CreateDynamicMaterialInstance` _staticmeshcomponent_2 _index_2 (`|GetArrayItem` (break `/Game/RTSMultiplayer/MovementSubsystem/Blueprints/S_ArrayOfMaterialInstances` _value) _index_2) "None")
                  (`PrimitiveComponent.SetCollisionResponseToChannel` _staticmeshcomponent_2 "ECC_Visibility" (`BlueprintMapLibrary.Map_Find` (`self.SavedVisibilityResoponses`) _array_element_4)))
                (`BlueprintMapLibrary.Map_Remove` (`self.SavedStaticMeshesMaterials`) _array_element_4)
                (`BlueprintMapLibrary.Map_Remove` (`self.SavedVisibilityResoponses`) _array_element_4)
                (`BlueprintMapLibrary.Map_Remove` (`self.TransparentStaticMeshes`) _array_element_4)
                (else
                  (`KismetSystemLibrary.PrintString` "ObstacleTransparencyComponent: Materials not found."))))))
        (:`else`)))
    (:`else`)))