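; SquareSquad is a squad formation Blueprint that lays out its actors in a roughly square grid for the RTS movement system.
; On recalculation, it derives the column count from the rounded-up square root of the actor count, respecting a minimum, and makes the middle of the front row the leader.
; It then rebuilds per-actor target displacements, stacking rows backward along X and centering columns on Y at fixed spacing, with single actors handled separately.
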(event `self.RecalculateSquadDisplacements`
  (params (GoalLocation :type "Vector Structure"))
  (bind _columnscount (`self.ColumnsCount`))
  (bind _squadtargetdisplacements (`self.SquadTargetDisplacements`))
  (bind _returnvalue (`KismetArrayLibrary.Array_Length` (`self.Actors`)))
  (set `self.ColumnsCount` (`KismetMathLibrary.Max` (`KismetMathLibrary.FCeil` (`KismetMathLibrary.Sqrt` (`KismetMathLibrary.Conv_IntToDouble` _returnvalue))) (`self.MinColumnsCount`)))
  (set `self.LeaderIndex` (/ (`KismetMathLibrary.Min` (`self.ColumnsCount`) _returnvalue) 2))
  (`KismetArrayLibrary.Array_Clear` _squadtargetdisplacements)
  (if (== (`KismetArrayLibrary.Array_Length` (`self.Actors`)) 1)
    (`KismetArrayLibrary.Array_Add` (`self.SquadTargetDisplacements`))
    (else
      (for (_ _array_index) (`self.Actors`)
        (`KismetArrayLibrary.Array_Add` _squadtargetdisplacements (`KismetMathLibrary.MakeVector` (* (* (/ _array_index (`self.ColumnsCount`)) -1) (`self.DistanceBetweenActors`)) (* (- (mod _array_index _columnscount) (/ _columnscount 2)) (`self.DistanceBetweenActors`))))))))