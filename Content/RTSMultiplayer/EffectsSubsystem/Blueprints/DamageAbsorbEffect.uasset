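; DamageAbsorbEffect is an effect Blueprint in the RTS multiplayer effects subsystem that tracks a pool of damage absorption.
; Apply fills AbsorbAmount from the first EffectConstants entry, then calls the parent Apply.
; ReceiveDamage subtracts incoming damage from the pool and, once it is depleted, starts a short one-shot timer whose bound event is not shown.
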(event `ReceiveDamage`
  (params (Amount :type "Float (double-precision)"))
  (bind _output_get (set `self.AbsorbAmount` (- (`self.AbsorbAmount`) Amount)))
  (if (<= _output_get 0.0)
    (`KismetSystemLibrary.K2_SetTimerDelegate` (`|CreateDelegate` :!event `Dispel`) 0.05)))

(event `self.Apply`
  (set `self.AbsorbAmount` (`|GetArrayItem` (`self.EffectConstants`)))
  (`parent.Apply`))

(fn `UserConstructionScript`
  (`parent.UserConstructionScript`))