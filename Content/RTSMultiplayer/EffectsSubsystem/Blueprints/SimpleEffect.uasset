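; Timed effect actor for RTS abilities that deals periodic damage or healing to a target, such as a DoT or HoT.
; On begin play it loads data table rows and derives the tick count from duration and frequency.
; Apply attaches optional particles, registers with the target's effect component and starts a looping tick timer plus a timeline for progress queries.
; Ticks act through combat component interfaces; the last calls Dispel, which unregisters and destroys the actor.
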(event `self.ReceiveBeginPlay`
  (bind (_abilitycombatconstants_basedamage _abilitycombatconstants_basehealing _abilitycombatconstants_effectbaseduration _abilitycombatconstants_tickfrequency) (break `/Game/RTSMultiplayer/AbilitySubsystem/Data/S_AbilityCombatConstants` (`self.AbilityCombatConstants`)))
  (bind (_abilitycombatconstants_basedamage_2 _abilitycombatconstants_basehealing_2 _abilitycombatconstants_effectbaseduration_2 _abilitycombatconstants_tickfrequency_2) (break `/Game/RTSMultiplayer/AbilitySubsystem/Data/S_AbilityCombatConstants` (`self.AbilityCombatConstants`)))
  ;[1 1 1] Begin play.
  (bind _returnvalue (`|GetDataTableRow` "/Game/RTSMultiplayer/EffectsSubsystem/Data/EffectsDataTable.EffectsDataTable" (`self.EffectId`))
    (:`then`
      (set `self.EffectInfo` _returnvalue)
      (bind _returnvalue_2 (`|GetDataTableRow` "/Game/RTSMultiplayer/AbilitySubsystem/Data/CustomConstantsDataTable.CustomConstantsDataTable" (`self.EffectConstantsId`))
        (:`then`
          (set `self.EffectConstants` (break `/Game/RTSMultiplayer/AbilitySubsystem/Data/S_FloatArray` _returnvalue_2)))
        (:`RowNotFound`
          _))
      (set `self.RemainingTickCount` (`KismetMathLibrary.FTrunc` (/ _abilitycombatconstants_effectbaseduration_2 _abilitycombatconstants_tickfrequency_2)))
      (if (or (== _abilitycombatconstants_effectbaseduration 0.0) (== _abilitycombatconstants_tickfrequency 0.0))
        (`KismetSystemLibrary.PrintString` "Effect: Frequency or Duration = 0." true true (struct :`R` 1.0 :`G` 0.038718 :`A` 1.0) 5.0)))
    (:`RowNotFound`
      (`KismetSystemLibrary.PrintString` "Effect: data table row not found." true true (struct :`R` 1.0 :`G` 0.038718 :`A` 1.0) 5.0))))

(event `SpawnPossibleParticleSystem`
  ;[1 1 1] Spawn and destroy possible particle system.
  (bind _onapplyparticlesystem (`self.OnApplyParticleSystem`)
    (:`then`
      (bind _returnvalue (`GameplayStatics.SpawnEmitterAttached` _onapplyparticlesystem (`Actor.RootComponent` (`self.Target`)) "None" (0.0 0.0 0.0) (struct) (`self.ParticleSystemScale`) "KeepRelativeOffset" false))
      (set `self.AttachedParticleSystemComponent` _returnvalue))
    (:`else`)))

(event `DestroyPossibleParticleSystem`
  ;[1 1 1] Spawn and destroy possible particle system.
  (bind _attachedparticlesystemcomponent (`self.AttachedParticleSystemComponent`)
    (:`then`
      (`ActorComponent.K2_DestroyComponent` _attachedparticlesystemcomponent))
    (:`else`)))

(event `Apply`
  (bind (_abilitycombatconstants_basedamage _abilitycombatconstants_basehealing _abilitycombatconstants_effectbaseduration _abilitycombatconstants_tickfrequency) (break `/Game/RTSMultiplayer/AbilitySubsystem/Data/S_AbilityCombatConstants` (`self.AbilityCombatConstants`)))
  ;[1 1 1] Apply event. Start ticking process.
  (`self.SpawnPossibleParticleSystem`)
  (`self.CallEffectHasBeenApplied`)
  (bind _returnvalue (`KismetSystemLibrary.K2_SetTimerDelegate` (`|CreateDelegate` :!event `EffectTick`) _abilitycombatconstants_tickfrequency true))
  (set `self.EffectTickHandle` _returnvalue)
  (`self.StartEffectTimeline`)
  (bind _asi_effect_receiver (cast `/Game/RTSMultiplayer/EffectsSubsystem/Blueprints/I_EffectReceiver` (`self.Target`))
    (:`then`
      (bind _effectcomponent (`/Game/RTSMultiplayer/EffectsSubsystem/Blueprints/I_EffectReceiver.GetEffectComponent` _asi_effect_receiver))
      (`/Game/RTSMultiplayer/EffectsSubsystem/Blueprints/EffectComponent.AddEffect` _effectcomponent self))
    (:`CastFailed`
      (`KismetSystemLibrary.PrintString` "Effect: target must implement I_EffectReceiver interface." true true (struct :`R` 1.0 :`G` 0.038718 :`A` 1.0) 5.0))))

(event `CallEffectHasBeenApplied`
  (`self.EffectHasBeenApplied` self))

(event `Dispel`
  ;[1 1 1] Dispel effect.
  (`self.DestroyPossibleParticleSystem`)
  (`self.StopEffectTimeline`)
  (`self.CallEffectHasBeenDispeled`)
  (bind _target (`self.Target`)
    (:`then`
      (bind _asi_effect_receiver (cast `/Game/RTSMultiplayer/EffectsSubsystem/Blueprints/I_EffectReceiver` _target)
        (:`then`
          (bind _effectcomponent (`/Game/RTSMultiplayer/EffectsSubsystem/Blueprints/I_EffectReceiver.GetEffectComponent` _asi_effect_receiver))
          (`/Game/RTSMultiplayer/EffectsSubsystem/Blueprints/EffectComponent.RemoveEffect` _effectcomponent self)
          (`self.K2_DestroyActor`))
        (:`CastFailed`
          (`KismetSystemLibrary.PrintString` "Effect: target must implement I_EffectReceiver interface." true true (struct :`R` 1.0 :`G` 0.038718 :`A` 1.0) 5.0))))
    (:`else`)))

(event `CallEffectHasBeenDispeled`
  (`self.EffectHasBeenDispeled` self))

(event `EffectTick`
  ;[1 1 1] Effect tick. Dispel event if there are no ticks anymore.
  (`/Engine/EditorBlueprintResources/StandardMacros.DecrementInt` (`self.RemainingTickCount`)
    (:`  `
      (`self.TryDealDamageAndHeal`)
      (if (== (`self.RemainingTickCount`) 0)
        (`self.Dispel`)))))

(event `TryDealDamageAndHeal`
  (bind (_abilitycombatconstants_basedamage _abilitycombatconstants_basehealing _abilitycombatconstants_effectbaseduration _abilitycombatconstants_tickfrequency _abilitycombatconstants_tickdamage _abilitycombatconstants_tickhealing) (break `/Game/RTSMultiplayer/AbilitySubsystem/Data/S_AbilityCombatConstants` (`self.AbilityCombatConstants`)))
  (bind (_abilitycombatconstants_basedamage_2 _abilitycombatconstants_basehealing_2 _abilitycombatconstants_effectbaseduration_2 _abilitycombatconstants_tickfrequency_2 _abilitycombatconstants_tickdamage_2 _abilitycombatconstants_tickhealing_2) (break `/Game/RTSMultiplayer/AbilitySubsystem/Data/S_AbilityCombatConstants` (`self.AbilityCombatConstants`)))
  (bind (_abilitycombatconstants_basedamage_3 _abilitycombatconstants_basehealing_3 _abilitycombatconstants_effectbaseduration_3 _abilitycombatconstants_tickfrequency_3 _abilitycombatconstants_tickdamage_3) (break `/Game/RTSMultiplayer/AbilitySubsystem/Data/S_AbilityCombatConstants` (`self.AbilityCombatConstants`)))
  (bind (_abilitycombatconstants_basedamage_4 _abilitycombatconstants_basehealing_4 _abilitycombatconstants_effectbaseduration_4 _abilitycombatconstants_tickfrequency_4 _abilitycombatconstants_tickdamage_4 _abilitycombatconstants_tickhealing_3 _abilitycombatconstants_damagetype) (break `/Game/RTSMultiplayer/AbilitySubsystem/Data/S_AbilityCombatConstants` (`self.AbilityCombatConstants`)))
  ;[1 1 1] Try deal damage and heal if necessary.
  (if (!= _abilitycombatconstants_tickdamage_3 0.0)
    (bind _caster (`self.Caster`)
      (:`then`
        (bind _asi_able_to_fight (cast `/Game/RTSMultiplayer/CombatSubsystem/Blueprints/I_AbleToFight` _caster)
          (:`then`
            (bind _combatcomponent (`/Game/RTSMultiplayer/CombatSubsystem/Blueprints/I_AbleToFight.GetCombatComponent` _asi_able_to_fight))
            (bind _target (`self.Target`)
              (:`then`
                (bind _asi_able_to_fight_2 (cast `/Game/RTSMultiplayer/CombatSubsystem/Blueprints/I_AbleToFight` _target))
                (bind _combatcomponent_2 (`/Game/RTSMultiplayer/CombatSubsystem/Blueprints/I_AbleToFight.GetCombatComponent` _asi_able_to_fight_2))
                (`/Game/RTSMultiplayer/CombatSubsystem/Blueprints/CombatComponent.ReceiveDamage` _combatcomponent_2 (make `/Game/RTSMultiplayer/CombatSubsystem/Blueprints/S_DamageInfo` _abilitycombatconstants_damagetype (`/Game/RTSMultiplayer/CombatSubsystem/Blueprints/CombatComponent.WeaponType` _combatcomponent) _abilitycombatconstants_tickdamage_4))
                (if (!= _abilitycombatconstants_tickhealing 0.0) :!label _label
                  (bind _target_2 (`self.Target`)
                    (:`then`
                      (bind _asi_able_to_fight_3 (cast `/Game/RTSMultiplayer/CombatSubsystem/Blueprints/I_AbleToFight` _target_2)
                        (:`then`
                          (bind _combatcomponent_3 (`/Game/RTSMultiplayer/CombatSubsystem/Blueprints/I_AbleToFight.GetCombatComponent` _asi_able_to_fight_3))
                          (`/Game/RTSMultiplayer/CombatSubsystem/Blueprints/CombatComponent.ReceiveHealing` _combatcomponent_3 _abilitycombatconstants_tickhealing_2))
                        (:`CastFailed`
                          (`KismetSystemLibrary.PrintString` "Effect: caster and target must implement I_AbleToFight interface." true true (struct :`R` 1.0 :`G` 0.038718 :`A` 1.0) 5.0 :!label _label_2))))
                    (:`else`))))
              (:`else`)))
          (:`CastFailed`
            (goto _label_2))))
      (:`else`))
    (else
      (goto _label))))

(event `StartEffectTimeline`
  (bind (_abilitycombatconstants_basedamage _abilitycombatconstants_basehealing _abilitycombatconstants_effectbaseduration) (break `/Game/RTSMultiplayer/AbilitySubsystem/Data/S_AbilityCombatConstants` (`self.AbilityCombatConstants`)))
  ;[1 1 1] Start and stop effect timeline.
  (`TimelineComponent.SetTimelineLength` (`self.EffectTimeline`) _abilitycombatconstants_effectbaseduration)
  (`Timeline|EffectTimeline` :!via `PlayFromStart`))

(event `StopEffectTimeline`
  ;[1 1 1] Start and stop effect timeline.
  (`TimelineComponent.Stop` (`self.EffectTimeline`)))

(fn `GetEffectProgress`
  (returns (Progress :type "Float (double-precision)"))
  (bind _effecttimeline (`self.EffectTimeline`))
  (return (/ (`TimelineComponent.GetPlaybackPosition` _effecttimeline) (`TimelineComponent.GetTimelineLength` _effecttimeline))))

(fn `GetTimeRemains`
  (returns (Time :type "Float (double-precision)"))
  (bind _effecttimeline (`self.EffectTimeline`))
  (return (- (`TimelineComponent.GetTimelineLength` _effecttimeline) (`TimelineComponent.GetPlaybackPosition` _effecttimeline))))

(fn `UserConstructionScript`)