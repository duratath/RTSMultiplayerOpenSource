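; DamageImmuneEffect is an effect in the RTS effects subsystem that, by its name, makes its target immune to damage while active.
; Apply gets the StatsComponent through the I_HaveStats interface and raises the max values of two stats by a fixed amount.
; Dispel subtracts the same amount from both stats.
; Both events call their parent implementation only when the target is valid.
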(event `self.Apply`
  (bind _target (`self.Target`)
    (:`then`
      (bind _asi_have_stats (cast `/Game/RTSMultiplayer/StatsSubsystem/Blueprints/I_HaveStats` _target)
        (:`then`
          (bind _statscomponent (`/Game/RTSMultiplayer/StatsSubsystem/Blueprints/I_HaveStats.GetStatsComponent` _asi_have_stats))
          (`/Game/RTSMultiplayer/StatsSubsystem/Blueprints/StatsComponent.ChangeMaxStatValue` _statscomponent "NewEnumerator6" 100.0)
          (`/Game/RTSMultiplayer/StatsSubsystem/Blueprints/StatsComponent.ChangeMaxStatValue` _statscomponent "NewEnumerator7" 100.0))
        (:`CastFailed`
          _))
      (`parent.Apply`))
    (:`else`)))

(event `self.Dispel`
  (bind _target (`self.Target`)
    (:`then`
      (bind _asi_have_stats (cast `/Game/RTSMultiplayer/StatsSubsystem/Blueprints/I_HaveStats` _target)
        (:`then`
          (bind _statscomponent (`/Game/RTSMultiplayer/StatsSubsystem/Blueprints/I_HaveStats.GetStatsComponent` _asi_have_stats))
          (`/Game/RTSMultiplayer/StatsSubsystem/Blueprints/StatsComponent.ChangeMaxStatValue` _statscomponent "NewEnumerator6" -100.0)
          (`/Game/RTSMultiplayer/StatsSubsystem/Blueprints/StatsComponent.ChangeMaxStatValue` _statscomponent "NewEnumerator7" -100.0))
        (:`CastFailed`
          _))
      (`parent.Dispel`))
    (:`else`)))

(fn `UserConstructionScript`
  (`parent.UserConstructionScript`))