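; Effect in the RTS effects subsystem that scales the maximum value of a chosen stat on its target while active.
; On Apply, it gets the target's stats component through I_HaveStats and multiplies the stat's base maximum by the first effect constant.
; It stores the resulting difference and applies it as a delta to the maximum.
; Dispel reverses the change by applying the negated stored delta.
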(event `self.Apply`
  (bind _target (`self.Target`)
    (:`then`
      (bind _asi_have_stats (cast `/Game/RTSMultiplayer/StatsSubsystem/Blueprints/I_HaveStats` _target)
        (:`then`
          (bind _statscomponent (`/Game/RTSMultiplayer/StatsSubsystem/Blueprints/I_HaveStats.GetStatsComponent` _asi_have_stats))
          (bind (_value _returnvalue) (`BlueprintMapLibrary.Map_Find` (`/Game/RTSMultiplayer/StatsSubsystem/Blueprints/StatsComponent.Stats` _statscomponent) (`self.StatToChange`)))
          (if _returnvalue
            (bind _output_get (set `self.StatDelta` (- (* (`.BaseMaximum_6_CE344B0C47CFD1A25C77DDA1AD165190` (break `/Game/RTSMultiplayer/StatsSubsystem/Blueprints/S_Stat` _value)) (`|GetArrayItem` (`self.EffectConstants`))) (`.BaseMaximum_6_CE344B0C47CFD1A25C77DDA1AD165190` (break `/Game/RTSMultiplayer/StatsSubsystem/Blueprints/S_Stat` _value)))))
            (`/Game/RTSMultiplayer/StatsSubsystem/Blueprints/StatsComponent.ChangeMaxStatValue` _statscomponent (`self.StatToChange`) _output_get)))
        (:`CastFailed`
          _))
      (`parent.Apply`))
    (:`else`)))

(event `self.Dispel`
  (bind _target (`self.Target`)
    (:`then`
      (bind _asi_have_stats (cast `/Game/RTSMultiplayer/StatsSubsystem/Blueprints/I_HaveStats` _target)
        (:`then`
          (bind _statscomponent (`/Game/RTSMultiplayer/StatsSubsystem/Blueprints/I_HaveStats.GetStatsComponent` _asi_have_stats))
          (`/Game/RTSMultiplayer/StatsSubsystem/Blueprints/StatsComponent.ChangeMaxStatValue` _statscomponent (`self.StatToChange`) (* -1 (`self.StatDelta`))))
        (:`CastFailed`
          _))
      (`parent.Dispel`))
    (:`else`)))

(fn `UserConstructionScript`
  (`parent.UserConstructionScript`))