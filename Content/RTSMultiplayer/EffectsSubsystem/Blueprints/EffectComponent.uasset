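; Effect component from the RTS multiplayer effects subsystem that tracks the effects currently applied and announces changes through added and removed event dispatchers.
; AddEffect stores each effect and also records non-stackable ones by class.
; Adding a non-stackable effect of an already recorded class first dispels and removes the existing instance, so the new one replaces it.
; RemoveEffect clears both records and broadcasts the removal.
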(event `CallEffectRemoved`
  (params (Effect :type "/Game/RTSMultiplayer/EffectsSubsystem/Blueprints/SimpleEffect Object Reference"))
  ;[1 1 1] Call effect added/removed. Multicast.
  (`self.EffectRemoved` Effect))

(event `CallEffectAdded`
  (params (Effect :type "/Game/RTSMultiplayer/EffectsSubsystem/Blueprints/SimpleEffect Object Reference"))
  ;[1 1 1] Call effect added/removed. Multicast.
  (`self.EffectAdded` Effect))

(event `AddEffect`
  (params (Effect :type "/Game/RTSMultiplayer/EffectsSubsystem/Blueprints/SimpleEffect Object Reference"))
  (bind _returnvalue (`GameplayStatics.GetObjectClass` Effect))
  ;[1 1 1] Add new effect. Check for stackable effects.
  (if (`.Stackable?_11_F649E0C745F0D1E1881CD28A878EDE76` (break `/Game/RTSMultiplayer/EffectsSubsystem/Data/S_EffectInfo` (`/Game/RTSMultiplayer/EffectsSubsystem/Blueprints/SimpleEffect.EffectInfo` Effect)))
    _
    (elif (`BlueprintSetLibrary.Set_Contains` (`self.NotStackableEffectClasses`) _returnvalue)
      (`self.RemoveNotStackableEffect` _returnvalue)
      (else
        (`BlueprintSetLibrary.Set_Add` (`self.NotStackableEffectClasses`) _returnvalue))))
  (`KismetArrayLibrary.Array_Add` (`self.CurrentEffects`) Effect)
  (`self.CallEffectAdded` Effect))

(event `RemoveEffect`
  (params (Effect :type "/Game/RTSMultiplayer/EffectsSubsystem/Blueprints/SimpleEffect Object Reference (by ref)"))
  ;[1 1 1] Remove effect from CurrentEffects array.
  (bind _returnvalue (`KismetArrayLibrary.Array_RemoveItem` (`self.CurrentEffects`) Effect))
  (if _returnvalue
    (`BlueprintSetLibrary.Set_Remove` (`self.NotStackableEffectClasses`) (`GameplayStatics.GetObjectClass` Effect))
    (`self.CallEffectRemoved` Effect)))

(event `RemoveNotStackableEffect`
  (params (EffectClass :type "/Game/RTSMultiplayer/EffectsSubsystem/Blueprints/SimpleEffect Class Reference"))
  (bind _currenteffects (`self.CurrentEffects`))
  ;[1 1 1] Remove not stackable effect by class.
  (for _array_element _currenteffects
    (if (== (`GameplayStatics.GetObjectClass` _array_element) EffectClass)
      (bind _output_get (set `self.NotStackableToRemoveEffect` _array_element))
      (`KismetArrayLibrary.Array_RemoveItem` _currenteffects _array_element)
      (`/Game/RTSMultiplayer/EffectsSubsystem/Blueprints/SimpleEffect.Dispel` _output_get)
      (`self.CallEffectRemoved` _output_get)
      (break))))