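; StunEffect is an effect Blueprint in the RTS multiplayer effects subsystem that changes the control state of a targeted unit.
; On Apply, it casts a valid Target to BaseRTSUnit, sets CurrentControlState to one enum value, then calls the parent Apply.
; On Dispel, it sets the other enum value the same way, without saving the prior state, then calls the parent Dispel.
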(event `self.Apply`
  (bind _target (`self.Target`)
    (:`then`
      (bind _asbase_rtsunit (cast `/Game/RTSMultiplayer/RTSCharacters/Blueprints/BaseRTSUnit` _target)
        (:`then`
          (set `/Game/RTSMultiplayer/RTSCharacters/Blueprints/BaseRTSUnit.CurrentControlState` "NewEnumerator1" _asbase_rtsunit))
        (:`CastFailed`
          _))
      (`parent.Apply`))
    (:`else`)))

(event `self.Dispel`
  (bind _target (`self.Target`)
    (:`then`
      (bind _asbase_rtsunit (cast `/Game/RTSMultiplayer/RTSCharacters/Blueprints/BaseRTSUnit` _target)
        (:`then`
          (set `/Game/RTSMultiplayer/RTSCharacters/Blueprints/BaseRTSUnit.CurrentControlState` "NewEnumerator0" _asbase_rtsunit))
        (:`CastFailed`
          _))
      (`parent.Dispel`))
    (:`else`)))

(fn `UserConstructionScript`
  (`parent.UserConstructionScript`))