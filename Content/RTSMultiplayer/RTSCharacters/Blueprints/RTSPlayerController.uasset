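; RTS player controller that sets up the HUD, faction selection and spawn, camera zoom and game-over screen.
; It forwards mouse, camera and ability input to a swappable receiver object for selection or abilities.
; Move and item-pickup orders build formation squads from selected units, while item drop and give orders become queueable tasks on the owner's task component.
; It also handles unit group hotkeys with double-press camera jump and outline and nameplate toggles.
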(event `SetupCharacterSelection`
  (bind _asbase_player_character (cast `/Game/RTSMultiplayer/RTSCharacters/Blueprints/BasePlayerCharacter` (`self.K2_GetPawn`) :!pure true))
  ;[1 1 1] Setup faction selection if PlayWelcomeSequence is true.
  (`self.DisableInput` (cast `/Game/RTSMultiplayer/RTSCharacters/Blueprints/BasePlayerCharacter` (`self.K2_GetPawn`) :!pure true) self)
  (`self.DisableInput` self)
  (bind _outactors (`GameplayStatics.GetAllActorsOfClass` "/Script/Engine.PlayerStart"))
  (for _array_element _outactors
    (if (== (`PlayerStart.PlayerStartTag` _array_element) "FACTION_SELECTION_SPAWN")
      (`/Game/RTSMultiplayer/RTSCharacters/Blueprints/BasePlayerCharacter.TeleportToLocation` _asbase_player_character (`self.K2_GetActorLocation` _array_element))
      (`SceneComponent.K2_SetWorldRotation` (`/Game/RTSMultiplayer/RTSCharacters/Blueprints/BasePlayerCharacter.SpringArm` _asbase_player_character) (struct :`Pitch` -5.0 :`Yaw` -60.0) false false)
      (break)))
  (bind _returnvalue (`|CreateWidget` "/Game/RTSMultiplayer/RTSCoreUI/Widgets/W_CharacterSelection.W_CharacterSelection_C" self))
  (bind _output_get (set `self.FactionSelectionWidget` _returnvalue))
  (`UserWidget.AddToViewport` _output_get 0)
  (add `/Game/RTSMultiplayer/RTSCoreUI/Widgets/W_CharacterSelection.FactionSelected` _output_get (delegate `OnFactionSelected`)))

(event `GameOver`
  (params (`Defeated?` :type Boolean))
  ;[1 1 1] Game over.
  (`self.DisableInput` self)
  (`self.DisableInput` (`self.K2_GetPawn` self) self)
  (bind _playerhud (`self.PlayerHUD`)
    (:`then`
      (`Widget.RemoveFromParent` _playerhud)
      (bind _returnvalue (`|CreateWidget` "/Game/RTSMultiplayer/RTSCoreUI/Widgets/W_GameOverScreen.W_GameOverScreen_C" self `Defeated?`))
      (`UserWidget.AddToViewport` _returnvalue 0))
    (:`else`)))

(event `OnFactionSelected`
  (params (Faction :type "/Game/RTSMultiplayer/RTSCoreBP/E_Faction Enum" :default "NewEnumerator0"))
  ;[1 1 1] Setup faction selection if PlayWelcomeSequence is true.
  (`Widget.RemoveFromParent` (`self.FactionSelectionWidget`))
  (`self.SetPlayerFaction` Faction)
  (`self.PlayerFactionSelected` Faction))

(event `TeleportToFactionSpawn`
  (params (Faction :type "/Game/RTSMultiplayer/RTSCoreBP/E_Faction Enum" :default "NewEnumerator0"))
  ;[1 1 1] Teleport to faction spawn.
  (bind _outactors (`GameplayStatics.GetAllActorsOfClass` "/Script/Engine.PlayerStart"))
  (for _array_element _outactors
    (if (== (`PlayerStart.PlayerStartTag` _array_element) (select `/Game/RTSMultiplayer/RTSCoreBP/E_Faction` Faction :`NewEnumerator0` "HUMANS_SPAWN" :`NewEnumerator1` "HORDE_SPAWN" :!type "Name"))
      (bind _asbase_player_character (cast `/Game/RTSMultiplayer/RTSCharacters/Blueprints/BasePlayerCharacter` (`self.K2_GetPawn`)))
      (`/Game/RTSMultiplayer/RTSCharacters/Blueprints/BasePlayerCharacter.TeleportToLocation` _asbase_player_character (`self.K2_GetActorLocation` _array_element))
      (break))))

(event `self.ReceiveBeginPlay`
  ;[1 1 1] Setup player HUD, initialize input receivers.
  (`self.SetupHUD`)
  (`self.InitializeReceivers`)
  (if (`self.PlayWelcomeSequence?`)
    (`self.SetupCharacterSelection`)
    (else
      (`self.TeleportToFactionSpawn` "NewEnumerator0"))))

(event `SetupHUD`
  ;[1 1 1] Setup player HUD, initialize input receivers.
  (`WidgetLayoutLibrary.RemoveAllWidgets`)
  (bind _returnvalue (`|CreateWidget` "/Game/RTSMultiplayer/RTSCoreUI/Widgets/W_PlayerHUD.W_PlayerHUD_C" self))
  (set `self.PlayerHUD` _returnvalue)
  (set `self.SelectionEnvironment` (`/Game/RTSMultiplayer/RTSCoreUI/Widgets/W_PlayerHUD.W_SelectionEnvironment` _returnvalue))
  (`UserWidget.AddToViewport` _returnvalue 0)
  (`self.OnSelectionEnvironmentReset` (`self.SelectionEnvironment`))
  (add `/Game/RTSMultiplayer/MovementSubsystem/WIdgets/W_SquadeTypeSelection.OnSqaudeTypeChanged` (`/Game/RTSMultiplayer/RTSCoreUI/Widgets/W_PlayerHUD.W_SquadeTypeSelection` _returnvalue) (`|CreateDelegate` :!event `ChangeControlledUnitsSquadeType`))
  (if (`self.PlayWelcomeSequence?`)
    (`Widget.SetVisibility` (`self.PlayerHUD`) "Hidden")))

(event `InputAction|OpenPerkTree`
  (params (Key :type "Key Structure"))
  ;[1 1 1] Receive input.
  (:`Pressed`
    (bind _playerhud (`self.PlayerHUD`)
      (:`then`
        (`/Game/RTSMultiplayer/RTSCoreUI/Widgets/W_PlayerHUD.TogglePerkTree` _playerhud))
      (:`else`))))

(event `InitializeReceivers`
  ;[1 1 1] Setup player HUD, initialize input receivers.
  (bind _returnvalue (`|GenericCreateObject` "/Game/RTSMultiplayer/InputSubsystem/Blueprints/SelectionInputReceiver.SelectionInputReceiver_C" self (`self.SelectionEnvironment`) self))
  (`BlueprintMapLibrary.Map_Add` (`self.InputReceivers`) "NewEnumerator0" _returnvalue)
  (set `self.CurrentInputReceiver` _returnvalue)
  (bind _returnvalue_2 (`|GenericCreateObject` "/Game/RTSMultiplayer/InputSubsystem/Blueprints/AbilityInputReceiver.AbilityInputReceiver_C" self self))
  (`BlueprintMapLibrary.Map_Add` (`self.InputReceivers`) "NewEnumerator1" _returnvalue_2))

(event `InputAxis|RotateRight`
  (params (AxisValue :type "Float (single-precision)"))
  ;[1 1 1] Receive input.
  (bind _currentinputreceiver (`self.CurrentInputReceiver`)
    (:`then`
      (`/Game/RTSMultiplayer/InputSubsystem/Blueprints/InputReceiver.RotateRight` _currentinputreceiver AxisValue))
    (:`else`)))

(event `InputAxisKey|MouseX`
  (params (AxisValue :type "Float (single-precision)"))
  ;[1 1 1] Receive input.
  (bind _currentinputreceiver (`self.CurrentInputReceiver`)
    (:`then`
      (`/Game/RTSMultiplayer/InputSubsystem/Blueprints/InputReceiver.MouseX` _currentinputreceiver AxisValue))
    (:`else`)))

(event `InputAction|RotateCamera`
  (params (Key :type "Key Structure"))
  ;[1 1 1] Receive input.
  (:`Pressed`
    (bind _currentinputreceiver (`self.CurrentInputReceiver`)
      (:`then`
        (`/Game/RTSMultiplayer/InputSubsystem/Blueprints/InputReceiver.RotatePressed` _currentinputreceiver))
      (:`else`)))
  (:`Released`
    (bind _currentinputreceiver_2 (`self.CurrentInputReceiver`)
      (:`then`
        (`/Game/RTSMultiplayer/InputSubsystem/Blueprints/InputReceiver.RotateReleased` _currentinputreceiver_2))
      (:`else`))))

(event `InitializeResourceBar`
  (params (ConsumableResources :type "Map of /Game/RTSMultiplayer/ResourcesSubsystem/Blueprints/E_ResourceType Enum to /Game/RTSMultiplayer/ResourcesSubsystem/Blueprints/S_ConsumableResource Structure") (AllocatableResources :type "Map of /Game/RTSMultiplayer/ResourcesSubsystem/Blueprints/E_ResourceType Enum to /Game/RTSMultiplayer/ResourcesSubsystem/Blueprints/S_AllocatableResource Structure") (StreamingResources :type "Map of /Game/RTSMultiplayer/ResourcesSubsystem/Blueprints/E_ResourceType Enum to /Game/RTSMultiplayer/ResourcesSubsystem/Blueprints/S_StreamingResource Structure"))
  ;[1 1 1] Iniitalize resource bar.
  (`/Game/RTSMultiplayer/ResourcesSubsystem/Widgets/W_ResourcesBar.SetResources` (`/Game/RTSMultiplayer/RTSCoreUI/Widgets/W_PlayerHUD.W_ResourcesBar` (`self.PlayerHUD`)) ConsumableResources AllocatableResources StreamingResources))

(event `InputAction|ToggleBarsVisibility`
  (params (Key :type "Key Structure"))
  ;[1 1 1] Toggle bars visibility.
  (:`Pressed`
    (bind _outactors (`GameplayStatics.GetAllActorsWithInterface` "/Game/RTSMultiplayer/StatsSubsystem/Blueprints/I_HaveStats.I_HaveStats_C"))
    (for _array_element _outactors
      (bind _asi_have_stats (cast `/Game/RTSMultiplayer/StatsSubsystem/Blueprints/I_HaveStats` _array_element))
      (bind _statscomponent (`/Game/RTSMultiplayer/StatsSubsystem/Blueprints/I_HaveStats.GetStatsComponent` _asi_have_stats))
      (`/Game/RTSMultiplayer/StatsSubsystem/Blueprints/StatsComponent.ToggleNameplateVisibility` _statscomponent))))

(event `InputAxisKey|MouseY`
  (params (AxisValue :type "Float (single-precision)"))
  ;[1 1 1] Receive input.
  (bind _currentinputreceiver (`self.CurrentInputReceiver`)
    (:`then`
      (`/Game/RTSMultiplayer/InputSubsystem/Blueprints/InputReceiver.MouseY` _currentinputreceiver AxisValue))
    (:`else`)))

(event `Key|RightMouseButton`
  (params (Key :type "Key Structure"))
  ;[1 1 1] Receive input.
  (:`Pressed`
    (bind _currentinputreceiver (`self.CurrentInputReceiver`)
      (:`then`
        (`/Game/RTSMultiplayer/InputSubsystem/Blueprints/InputReceiver.RightMouseButtonPressed` _currentinputreceiver Key))
      (:`else`)))
  (:`Released`
    (bind _currentinputreceiver_2 (`self.CurrentInputReceiver`)
      (:`then`
        (`/Game/RTSMultiplayer/InputSubsystem/Blueprints/InputReceiver.RightMouseButtonReleased` _currentinputreceiver_2 Key))
      (:`else`))))

(event `ChangeControlledUnitsSquadeType`
  (params (NewType :type "/Game/RTSMultiplayer/MovementSubsystem/Blueprints/E_SquadeType Enum" :default "NewEnumerator0"))
  ;[1 1 1] Movement squade type changed callback.
  (set `self.MovementSquadeType` NewType))

(event `InputAction|ToggleActorsOutline`
  (params (Key :type "Key Structure"))
  ;[1 1 1] Toggle actors outline.
  (:`Pressed`
    (if (`self.bEnableMouseOverEvents`)
      (bind _outactors (`GameplayStatics.GetAllActorsWithInterface` "/Game/RTSMultiplayer/SelectionSubsystem/Blueprints/I_CanBeOutlined.I_CanBeOutlined_C"))
      (for _array_element _outactors
        (if (not (`KismetArrayLibrary.Array_Contains` (`/Game/RTSMultiplayer/SelectionSubsystem/Widgets/W_SelectionEnvironment.SelectedActors` (`self.SelectionEnvironment`)) _array_element))
          (bind _asi_can_be_outlined (cast `/Game/RTSMultiplayer/SelectionSubsystem/Blueprints/I_CanBeOutlined` _array_element))
          (bind _outlinecomponent (`/Game/RTSMultiplayer/SelectionSubsystem/Blueprints/I_CanBeOutlined.GetOutlineComponent` _asi_can_be_outlined))
          (`/Game/RTSMultiplayer/SelectionSubsystem/Blueprints/OutlineComponent.CancelOutline` _outlinecomponent))))
    (set `self.bEnableMouseOverEvents` (not (`self.bEnableMouseOverEvents`)))))

(event `Key|LeftMouseButton`
  (params (Key :type "Key Structure"))
  ;[1 1 1] Receive input.
  (:`Pressed`
    (bind _currentinputreceiver (`self.CurrentInputReceiver`)
      (:`then`
        (`/Game/RTSMultiplayer/InputSubsystem/Blueprints/InputReceiver.LeftMouseButtonPressed` _currentinputreceiver Key))
      (:`else`)))
  (:`Released`
    (bind _currentinputreceiver_2 (`self.CurrentInputReceiver`)
      (:`then`
        (`/Game/RTSMultiplayer/InputSubsystem/Blueprints/InputReceiver.LeftMouseButtonReleased` _currentinputreceiver_2 Key))
      (:`else`))))

(event `MoveUnderMousePosition`
  (bind (_bblockinghit _binitialoverlap _time _distance _location _impactpoint _normal _impactnormal _physmat _hitactor) (`GameplayStatics.BreakHitResult` (`self.GetHitResultUnderCursorByChannel` "TraceTypeQuery1" false)))
  ;[1 1 1] Move units.
  (bind (_abletomoveactors _notabletomove_) (`self.GetAbleToMoveActors` (`/Game/RTSMultiplayer/SelectionSubsystem/Widgets/W_SelectionEnvironment.SelectedActors` (`self.SelectionEnvironment`))))
  (if _notabletomove_
    (`self.AddAttentionMessage` "CANT_DO_THAT"))
  (if (> (`KismetArrayLibrary.Array_Length` _abletomoveactors) 0)
    (`/Engine/EditorBlueprintResources/StandardMacros.IsValid` _hitactor
      (:`Is Valid`
        (bind _asinventory_item (cast `/Game/RTSMultiplayer/InventorySubsystem/Blueprints/InventoryItem` _hitactor)
          (:`then`
            (cast `/Game/RTSMultiplayer/InventorySubsystem/Blueprints/I_HaveInventory` (`|GetArrayItem` _abletomoveactors)
              (:`then`
                (`self.CollectInventoryItem` (`/Game/RTSMultiplayer/SelectionSubsystem/Widgets/W_SelectionEnvironment.SelectedActors` (`self.SelectionEnvironment`)) (`self.IsQueueTaskModifierDown?`) self (select `/Game/RTSMultiplayer/MovementSubsystem/Blueprints/E_SquadeType` (`self.MovementSquadeType`) :`NewEnumerator0` "/Game/RTSMultiplayer/MovementSubsystem/Blueprints/SquareSquad.SquareSquad_C" :`NewEnumerator1` "/Game/RTSMultiplayer/MovementSubsystem/Blueprints/TriangleSquad.TriangleSquad_C" :`NewEnumerator2` "/Game/RTSMultiplayer/MovementSubsystem/Blueprints/CircleSquad.CircleSquad_C" :!type "/Game/RTSMultiplayer/MovementSubsystem/Blueprints/Squad Class Reference") _asinventory_item))
              (:`CastFailed`
                (`self.MoveToLocation` _location :!label _label)
                (`GameplayStatics.SpawnEmitterAtLocation` "/Game/RTSMultiplayer/DemoEffects/AbilitiesParticles/P_MoveTo.P_MoveTo" _location (struct) (0.3 0.3 0.3)))))
          (:`CastFailed`
            (goto _label))))
      (:`Is Not Valid`
        (goto _label)))))

(event `MoveToLocation`
  (params (GoalLocation :type "Vector Structure"))
  ;[1 1 1] Move units.
  (bind _abletomoveactors (`self.GetAbleToMoveActors` (`/Game/RTSMultiplayer/SelectionSubsystem/Widgets/W_SelectionEnvironment.SelectedActors` (`self.SelectionEnvironment`))))
  (`self.MoveSquadTo` _abletomoveactors GoalLocation (`self.MovementSquadeType`) (`self.IsQueueTaskModifierDown?`) self))

(event `Key|Ctrl+LeftMouseButton`
  (params (Key :type "Key Structure"))
  ;[1 1 1] Receive input.
  (:`Pressed`
    (bind _currentinputreceiver (`self.CurrentInputReceiver`)
      (:`then`
        (`/Game/RTSMultiplayer/InputSubsystem/Blueprints/InputReceiver.CtrlLeftMouseButtonPressed` _currentinputreceiver Key))
      (:`else`))))

(event `Key|Shift+LeftMouseButton`
  (params (Key :type "Key Structure"))
  ;[1 1 1] Receive input.
  (:`Pressed`
    (bind _currentinputreceiver (`self.CurrentInputReceiver`)
      (:`then`
        (`/Game/RTSMultiplayer/InputSubsystem/Blueprints/InputReceiver.ShiftLeftMouseButtonPressed` _currentinputreceiver Key))
      (:`else`))))

(event `Key|Alt+One`
  (params (Key :type "Key Structure"))
  ;[1 1 1] Input: change player faction (for debug).
  (:`Pressed`
    (`self.SetPlayerFaction` "NewEnumerator0")))

(event `Key|Ctrl+Shift+LeftMouseButton`
  (params (Key :type "Key Structure"))
  ;[1 1 1] Receive input.
  (:`Pressed`
    (bind _currentinputreceiver (`self.CurrentInputReceiver`)
      (:`then`
        (`/Game/RTSMultiplayer/InputSubsystem/Blueprints/InputReceiver.CtrlShiftLeftMouseButtonPressed` _currentinputreceiver Key))
      (:`else`))))

(event `Key|Alt+Two`
  (params (Key :type "Key Structure"))
  ;[1 1 1] Input: change player faction (for debug).
  (:`Pressed`
    (`self.SetPlayerFaction` "NewEnumerator1")))

(event `AttachAllItemsToSlot`
  (params (InventoryComponent :type "/Game/RTSMultiplayer/InventorySubsystem/Blueprints/InventoryComponent Object Reference") (Slot :type Integer) (Items :type "Array of /Game/RTSMultiplayer/InventorySubsystem/Blueprints/InventoryItem Object Reference"))
  ;[1 1 1] Inventory management.
  (`/Game/RTSMultiplayer/InventorySubsystem/Blueprints/InventoryComponent.AttachAllItemsToSlot` InventoryComponent Slot Items))

(event `CollectInventoryItem`
  (params (SelectedActors :type "Array of Actor Object Reference") (QueueModifier :type Boolean) (PlayerController :type "/Game/RTSMultiplayer/RTSCharacters/Blueprints/RTSPlayerController Object Reference") (SquadClass :type "/Game/RTSMultiplayer/MovementSubsystem/Blueprints/Squad Class Reference") (ItemToCollect :type "/Game/RTSMultiplayer/InventorySubsystem/Blueprints/InventoryItem Object Reference"))
  ;[1 1 1] Inventory management.
  (bind _returnvalue (`|GenericCreateObject` SquadClass self))
  (for _array_element SelectedActors
    (`/Game/RTSMultiplayer/MovementSubsystem/Blueprints/Squad.AddToSquad` _returnvalue _array_element))
  (`/Game/RTSMultiplayer/MovementSubsystem/Blueprints/Squad.SetMoveAndActionTask` _returnvalue (`self.K2_GetPawn` PlayerController) "/Game/RTSMultiplayer/TaskSubsystem/Blueprints/General/CollectItemTask.CollectItemTask_C" (`self.K2_GetActorLocation` ItemToCollect) ItemToCollect QueueModifier PlayerController))

(event `AttachItemToSlot`
  (params (InventoryComponent :type "/Game/RTSMultiplayer/InventorySubsystem/Blueprints/InventoryComponent Object Reference") (Slot :type Integer) (Item :type "/Game/RTSMultiplayer/InventorySubsystem/Blueprints/InventoryItem Object Reference"))
  ;[1 1 1] Inventory management.
  (`/Game/RTSMultiplayer/InventorySubsystem/Blueprints/InventoryComponent.AttachItemToSlot` InventoryComponent Slot Item))

(event `MoveSquadTo`
  (params (Squad :type "Array of Actor Object Reference") (GoalLocation :type "Vector Structure") (MovementSquadeType :type "/Game/RTSMultiplayer/MovementSubsystem/Blueprints/E_SquadeType Enum" :default "NewEnumerator0") (QueueModifier :type Boolean) (PlayerController :type "/Game/RTSMultiplayer/RTSCharacters/Blueprints/RTSPlayerController Object Reference"))
  ;[1 1 1] Create and move squad (on server).
  (switch `/Game/RTSMultiplayer/MovementSubsystem/Blueprints/E_SquadeType` MovementSquadeType
    (:`NewEnumerator0`
      (bind _returnvalue (`|GenericCreateObject` "/Game/RTSMultiplayer/MovementSubsystem/Blueprints/SquareSquad.SquareSquad_C" self))
      (for _array_element Squad
        (`/Game/RTSMultiplayer/MovementSubsystem/Blueprints/Squad.AddToSquad` _returnvalue _array_element))
      (`/Game/RTSMultiplayer/MovementSubsystem/Blueprints/Squad.MoveToLocation` _returnvalue GoalLocation QueueModifier PlayerController))
    (:`NewEnumerator1`
      (bind _returnvalue_2 (`|GenericCreateObject` "/Game/RTSMultiplayer/MovementSubsystem/Blueprints/TriangleSquad.TriangleSquad_C" self))
      (for _array_element_2 Squad
        (`/Game/RTSMultiplayer/MovementSubsystem/Blueprints/Squad.AddToSquad` _returnvalue_2 _array_element_2))
      (`/Game/RTSMultiplayer/MovementSubsystem/Blueprints/Squad.MoveToLocation` _returnvalue_2 GoalLocation QueueModifier PlayerController))
    (:`NewEnumerator2`
      (bind _returnvalue_3 (`|GenericCreateObject` "/Game/RTSMultiplayer/MovementSubsystem/Blueprints/CircleSquad.CircleSquad_C" self (`self.DefaultSquadRadius`)))
      (for _array_element_3 Squad
        (`/Game/RTSMultiplayer/MovementSubsystem/Blueprints/Squad.AddToSquad` _returnvalue_3 _array_element_3))
      (`/Game/RTSMultiplayer/MovementSubsystem/Blueprints/Squad.MoveToLocation` _returnvalue_3 GoalLocation QueueModifier PlayerController))))

(event `DetachAllItemsFromSlot`
  (params (InventoryComponent :type "/Game/RTSMultiplayer/InventorySubsystem/Blueprints/InventoryComponent Object Reference") (Slot :type Integer))
  ;[1 1 1] Inventory management.
  (`/Game/RTSMultiplayer/InventorySubsystem/Blueprints/InventoryComponent.DetachAllItemsFromSlot` InventoryComponent Slot))

(event `SetPlayerFaction`
  (params (PlayerFaction :type "/Game/RTSMultiplayer/RTSCoreBP/E_Faction Enum" :default "NewEnumerator0"))
  (bind _asbase_player_character (cast `/Game/RTSMultiplayer/RTSCharacters/Blueprints/BasePlayerCharacter` (`self.K2_GetPawn`) :!pure true))
  ;[1 1 1] Set player faction.
  (bind _asrtsgame_instance (cast `/Game/RTSMultiplayer/RTSCoreBP/RTSGameInstance` (`GameplayStatics.GetGameInstance`)))
  (bind _output_get (set `/Game/RTSMultiplayer/RTSCoreBP/RTSGameInstance.PlayerFaction` PlayerFaction _asrtsgame_instance))
  (`/Game/RTSMultiplayer/RTSCharacters/Blueprints/BasePlayerCharacter.SetFaction` (cast `/Game/RTSMultiplayer/RTSCharacters/Blueprints/BasePlayerCharacter` (`GameplayStatics.GetPlayerCharacter` 0) :!pure true) PlayerFaction)
  (`/Game/RTSMultiplayer/SelectionSubsystem/Widgets/W_SelectionEnvironment.ResetAll` (`self.SelectionEnvironment`))
  (`self.OnSelectionEnvironmentReset` (`self.SelectionEnvironment`))
  (`/Game/RTSMultiplayer/RTSCharacters/Blueprints/BasePlayerCharacter.SetupFogOfWar` _asbase_player_character)
  (`/Game/RTSMultiplayer/RTSCharacters/Blueprints/BasePlayerCharacter.AddAllControlledUnitsToFogSystem` _asbase_player_character)
  (`KismetSystemLibrary.Delay` 0.2)
  (`/Game/RTSMultiplayer/RTSCharacters/Blueprints/BasePlayerCharacter.SetupRelationships` _asbase_player_character)
  (`self.TeleportToFactionSpawn` _output_get))

(event `DetachItemFromSlot`
  (params (InventoryComponent :type "/Game/RTSMultiplayer/InventorySubsystem/Blueprints/InventoryComponent Object Reference") (Slot :type Integer) (Item :type "/Game/RTSMultiplayer/InventorySubsystem/Blueprints/InventoryItem Object Reference"))
  ;[1 1 1] Inventory management.
  (`/Game/RTSMultiplayer/InventorySubsystem/Blueprints/InventoryComponent.DetachItemFromSlot` InventoryComponent Slot Item))

(event `ConsumeInventoryItem`
  (params (Item :type "/Game/RTSMultiplayer/InventorySubsystem/Blueprints/InventoryItem Object Reference") (SlotIndex :type Integer) (InventoryComponent :type "/Game/RTSMultiplayer/InventorySubsystem/Blueprints/InventoryComponent Object Reference"))
  ;[1 1 1] Inventory management.
  (`/Game/RTSMultiplayer/InventorySubsystem/Blueprints/InventoryComponent.DetachItemFromSlot` InventoryComponent SlotIndex Item)
  (`/Game/RTSMultiplayer/InventorySubsystem/Blueprints/InventoryComponent.CallItemUnequiped` InventoryComponent Item)
  (`self.K2_DestroyActor` Item))

(event `SwapSlotsContent`
  (params (InventoryComponent :type "/Game/RTSMultiplayer/InventorySubsystem/Blueprints/InventoryComponent Object Reference") (Slot1 :type Integer) (Slot2 :type Integer))
  ;[1 1 1] Inventory management.
  (`/Game/RTSMultiplayer/InventorySubsystem/Blueprints/InventoryComponent.SwapSlotsContent` InventoryComponent Slot1 Slot2))

(event `DropInventoryItems`
  (params (ItemOwner :type "Actor Object Reference") (ItemsToDrop :type "Array of /Game/RTSMultiplayer/InventorySubsystem/Blueprints/InventoryItem Object Reference") (SlotIndex :type Integer) (LocationToDrop :type "Vector Structure"))
  ;[1 1 1] Inventory management.
  (`self.DropInventoryItemsServer` ItemOwner ItemsToDrop SlotIndex self LocationToDrop (`self.IsQueueTaskModifierDown?`)))

(event `AddAttentionMessage`
  (params (MessageId :type Name))
  ;[1 1 1] Add attention message to the screen.
  (`/Game/RTSMultiplayer/LogSubsystem/Widgets/W_AttentionMessagesWindow.AddNewMessage` (`/Game/RTSMultiplayer/RTSCoreUI/Widgets/W_PlayerHUD.W_AttentionMessagesWindow` (`self.PlayerHUD`)) MessageId))

(event `DropInventoryItemsServer`
  (params (ItemOwner :type "Actor Object Reference") (ItemsToDrop :type "Array of /Game/RTSMultiplayer/InventorySubsystem/Blueprints/InventoryItem Object Reference") (SlotIndex :type Integer) (PlayerController :type "/Game/RTSMultiplayer/RTSCharacters/Blueprints/RTSPlayerController Object Reference") (LocationToDrop :type "Vector Structure") (`QueueModifier?` :type Boolean))
  ;[1 1 1] Inventory management.
  (bind _asi_have_inventory (cast `/Game/RTSMultiplayer/InventorySubsystem/Blueprints/I_HaveInventory` ItemOwner))
  (bind _inventorycomponent (`/Game/RTSMultiplayer/InventorySubsystem/Blueprints/I_HaveInventory.GetInventoryComponent` _asi_have_inventory))
  (bind _returnvalue (`|GenericCreateObject` "/Game/RTSMultiplayer/TaskSubsystem/Blueprints/General/DropItemTask.DropItemTask_C" self ItemOwner _inventorycomponent ItemsToDrop SlotIndex (`self.K2_GetPawn` PlayerController) LocationToDrop null PlayerController null))
  (bind _asi_task_executor (cast `/Game/RTSMultiplayer/TaskSubsystem/Blueprints/I_TaskExecutor` ItemOwner)
    (:`then`
      (bind _taskcomponent (`/Game/RTSMultiplayer/TaskSubsystem/Blueprints/I_TaskExecutor.GetTaskComponent` _asi_task_executor))
      (if `QueueModifier?`
        (`/Game/RTSMultiplayer/TaskSubsystem/Blueprints/TaskComponent.AddTaskToQueue` _taskcomponent _returnvalue)
        (else
          (`/Game/RTSMultiplayer/TaskSubsystem/Blueprints/TaskComponent.SetCurrentTask` _taskcomponent _returnvalue))))
    (:`CastFailed`
      (`KismetSystemLibrary.PrintString` "RTSPlayerController: Actor should implement I_TaskExecutor interface." true true (struct :`R` 1.0 :`G` 0.038718 :`A` 1.0) 5.0))))

(event `Key|MouseScrollUp`
  (params (Key :type "Key Structure"))
  ;[1 1 1] Camera position.
  (:`Pressed`
    (bind _asbase_player_character (cast `/Game/RTSMultiplayer/RTSCharacters/Blueprints/BasePlayerCharacter` (`self.K2_GetPawn`)))
    (bind _springarm (`/Game/RTSMultiplayer/RTSCharacters/Blueprints/BasePlayerCharacter.SpringArm` _asbase_player_character))
    (set `SpringArmComponent.TargetArmLength` (`KismetMathLibrary.FClamp` (- (`SpringArmComponent.TargetArmLength` _springarm) (`self.ArmLengthScrollDelta`)) (`self.ArmMinLength`) (`self.ArmMaxLength`)) _springarm)))

(event `GiveItemsTo`
  (params (OwnerInventoryComponent :type "/Game/RTSMultiplayer/InventorySubsystem/Blueprints/InventoryComponent Object Reference") (TargetInventoryComponent :type "/Game/RTSMultiplayer/InventorySubsystem/Blueprints/InventoryComponent Object Reference") (Items :type "Array of /Game/RTSMultiplayer/InventorySubsystem/Blueprints/InventoryItem Object Reference") (ItemSlot :type Integer))
  ;[1 1 1] Inventory management.
  (`self.GiveItemsToServer` OwnerInventoryComponent TargetInventoryComponent Items ItemSlot self (`self.IsQueueTaskModifierDown?`)))

(event `Key|MouseScrollDown`
  (params (Key :type "Key Structure"))
  ;[1 1 1] Camera position.
  (:`Pressed`
    (bind _asbase_player_character (cast `/Game/RTSMultiplayer/RTSCharacters/Blueprints/BasePlayerCharacter` (`self.K2_GetPawn`)))
    (bind _springarm (`/Game/RTSMultiplayer/RTSCharacters/Blueprints/BasePlayerCharacter.SpringArm` _asbase_player_character))
    (set `SpringArmComponent.TargetArmLength` (`KismetMathLibrary.FClamp` (+ (`SpringArmComponent.TargetArmLength` _springarm) (`self.ArmLengthScrollDelta`)) (`self.ArmMinLength`) (`self.ArmMaxLength`)) _springarm)))

(event `GiveItemsToServer`
  (params (OwnerInventoryComponent :type "/Game/RTSMultiplayer/InventorySubsystem/Blueprints/InventoryComponent Object Reference") (TargetInventoryComponent :type "/Game/RTSMultiplayer/InventorySubsystem/Blueprints/InventoryComponent Object Reference") (Items :type "Array of /Game/RTSMultiplayer/InventorySubsystem/Blueprints/InventoryItem Object Reference") (ItemSlot :type Integer) (PlayerController :type "/Game/RTSMultiplayer/RTSCharacters/Blueprints/RTSPlayerController Object Reference") (`QueueModifier?` :type Boolean))
  ;[1 1 1] Inventory management.
  (bind _returnvalue (`|GenericCreateObject` "/Game/RTSMultiplayer/TaskSubsystem/Blueprints/General/GiveItemTask.GiveItemTask_C" self OwnerInventoryComponent TargetInventoryComponent ItemSlot Items (`self.K2_GetPawn` PlayerController) (0.0 0.0 0.0) (`ActorComponent.GetOwner` TargetInventoryComponent) PlayerController null))
  (bind _asi_task_executor (cast `/Game/RTSMultiplayer/TaskSubsystem/Blueprints/I_TaskExecutor` (`ActorComponent.GetOwner` OwnerInventoryComponent))
    (:`then`
      (bind _taskcomponent (`/Game/RTSMultiplayer/TaskSubsystem/Blueprints/I_TaskExecutor.GetTaskComponent` _asi_task_executor))
      (if `QueueModifier?`
        (`/Game/RTSMultiplayer/TaskSubsystem/Blueprints/TaskComponent.AddTaskToQueue` _taskcomponent _returnvalue)
        (else
          (`/Game/RTSMultiplayer/TaskSubsystem/Blueprints/TaskComponent.SetCurrentTask` _taskcomponent _returnvalue))))
    (:`CastFailed`
      (`KismetSystemLibrary.PrintString` "RTSPlayerController: Actor should implement I_TaskExecutor interface." true true (struct :`R` 1.0 :`G` 0.038718 :`A` 1.0) 5.0))))

(event `TrySelectBoundUnits`
  (params (Key :type "Key Structure (by ref)") (`ShouldMoveToUnits?` :type Boolean))
  (bind (_value _returnvalue) (`BlueprintMapLibrary.Map_Find` (`self.UnitsBinding`) Key))
  ;[1 1 1] Try to select bound units.
  (if _returnvalue
    (if (!= (`KismetArrayLibrary.Array_Length` (break `/Game/RTSMultiplayer/RTSCharacters/Blueprints/S_ArrayOfActors` _value)) 0)
      (bind _asselection_input_receiver (cast `/Game/RTSMultiplayer/InputSubsystem/Blueprints/SelectionInputReceiver` (`self.CurrentInputReceiver`))
        (:`then`
          (`/Game/RTSMultiplayer/InputSubsystem/Blueprints/SelectionInputReceiver.DeselectPossibleAlienUnit` _asselection_input_receiver))
        (:`CastFailed`
          _))
      (`/Game/RTSMultiplayer/SelectionSubsystem/Widgets/W_SelectionEnvironment.ForceSelectActors` (`self.SelectionEnvironment`) (break `/Game/RTSMultiplayer/RTSCharacters/Blueprints/S_ArrayOfActors` _value))
      (if `ShouldMoveToUnits?`
        (`/Game/RTSMultiplayer/RTSCharacters/Blueprints/BasePlayerCharacter.TeleportToLocation` (cast `/Game/RTSMultiplayer/RTSCharacters/Blueprints/BasePlayerCharacter` (`self.K2_GetPawn`) :!pure true) (`self.K2_GetActorLocation` (`|GetArrayItem` (break `/Game/RTSMultiplayer/RTSCharacters/Blueprints/S_ArrayOfActors` _value))))))))

(event `AddNewUnitsBind`
  (params (Key :type "Key Structure (by ref)"))
  ;[1 1 1] Add new bind.
  (`BlueprintMapLibrary.Map_Add` (`self.UnitsBinding`) Key))

(event `InputAction|Ability`
  (params (Key :type "Key Structure"))
  ;[1 1 1] Ability and serving ability input.
  (:`Pressed`
    (bind _currentinputreceiver (`self.CurrentInputReceiver`)
      (:`then`
        (`/Game/RTSMultiplayer/InputSubsystem/Blueprints/InputReceiver.AbilitySlotKeyPressed` _currentinputreceiver Key))
      (:`else`))))

(event `InputAction|UnitsBinding`
  (params (Key :type "Key Structure"))
  ;[1 1 1] Units binding.
  (:`Pressed`
    (`self.AddNewUnitsBind` Key)))

(event `InputAction|ServingAbility`
  (params (Key :type "Key Structure"))
  ;[1 1 1] Ability and serving ability input.
  (:`Pressed`
    (bind _currentinputreceiver (`self.CurrentInputReceiver`)
      (:`then`
        (`/Game/RTSMultiplayer/InputSubsystem/Blueprints/InputReceiver.ServingAbilitySlotKeyPressed` _currentinputreceiver Key))
      (:`else`))))

(event `InputAction|UnitsQuickSelection`
  (params (Key :type "Key Structure"))
  ;[1 1 1] Units binding.
  (:`Pressed`
    (`self.TrySelectBoundUnits` Key (`self.DoublePress?`))
    (`KismetSystemLibrary.K2_SetTimerDelegate` (delegate `ResetDoubleClick`) (`self.DoublePressTimeDelta`))
    (set `self.DoublePress?` true)))

(event `ResetDoubleClick`
  ;[1 1 1] Units binding.
  (set `self.DoublePress?` false))

(fn `GetAbleToMoveActors`
  (params (Actors :type "Array of Actor Object Reference"))
  (returns (AbleToMoveActors :type "Array of Actor Object Reference") (`NotAbleToMove?` :type Boolean))
  (locals (Result :type "Array of Actor Object Reference") (NotAbleToMove :type Boolean))
  (set `local.NotAbleToMove` (> (`KismetArrayLibrary.Array_Length` Actors) 0))
  (for _array_element Actors
    (bind _asbase_rtsunit (cast `/Game/RTSMultiplayer/RTSCharacters/Blueprints/BaseRTSUnit` _array_element))
    (if (`|EnumEquality` (`/Game/RTSMultiplayer/RTSCharacters/Blueprints/BaseRTSUnit.CurrentControlState` _asbase_rtsunit) "NewEnumerator0")
      (`KismetArrayLibrary.Array_Add` (`local.Result`) _array_element)))
  (return (`local.Result`) (and (`local.NotAbleToMove`) (== (`KismetArrayLibrary.Array_Length` (`local.Result`)) 0))))

(fn `IsQueueTaskModifierDown?`
  (returns (ResultValue :type Boolean))
  (return (`self.IsInputKeyDown` (`self.QueueTaskModifier`))))

(fn `SetInputReceiver`
  (params (ReceiverType :type "/Game/RTSMultiplayer/InputSubsystem/Blueprints/E_InputReceiverType Enum" :default "NewEnumerator0"))
  (bind (_value _returnvalue) (`BlueprintMapLibrary.Map_Find` (`self.InputReceivers`) ReceiverType))
  (if _returnvalue
    (`/Game/RTSMultiplayer/InputSubsystem/Blueprints/InputReceiver.Detached` (`self.CurrentInputReceiver`))
    (bind _output_get (set `self.CurrentInputReceiver` _value))
    (`/Game/RTSMultiplayer/InputSubsystem/Blueprints/InputReceiver.Attached` _output_get)))

(fn `UserConstructionScript`)