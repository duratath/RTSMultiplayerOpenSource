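; Base character for RTS units, implementing the interfaces for selection, combat, abilities, stats, inventory, outlining and fog of war.
; BeginPlay binds combat and task events, creates decal and outline selectors, and loads display info from a data table.
; Spawn adds war and science score to the player; death removes it and frees allocated resources.
; Montages for attacking, working and instant casts come from getters with empty defaults, with multicast events for mining and chopping.
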(event `PlayMineAnimation`
  (bind (_animmontage _playrate) (`self.GetMineAnimationSettings`))
  ;[1 1 1] Animations.
  (`/Engine/EditorBlueprintResources/StandardMacros.IsValid` _animmontage
    (:`Is Valid`
      (bind _output_get (set `self.CurrentAnimationMontage` _animmontage))
      (`self.PlayAnimMontage` _output_get _playrate))))

(event `StopCurrentAnimationMulticast`
  ;[1 1 1] Animations.
  (`self.StopCurrentAnimation`))

(event `PlayMineAnimationMulticast`
  ;[1 1 1] Animations.
  (`self.PlayMineAnimation`))

(event `PlayChopTreeAnimation`
  (bind (_animmontage _playrate) (`self.GetChopTreeAnimationSettings`))
  ;[1 1 1] Animations.
  (`/Engine/EditorBlueprintResources/StandardMacros.IsValid` _animmontage
    (:`Is Valid`
      (bind _output_get (set `self.CurrentAnimationMontage` _animmontage))
      (`self.PlayAnimMontage` _output_get _playrate))))

(event `PlayChopTreeAnimationMulticast`
  ;[1 1 1] Animations.
  (`self.PlayChopTreeAnimation`))

(event `PlayBuildAnimation`
  (bind (_animmontage _playrate) (`self.GetBuildAnimationSettings`))
  ;[1 1 1] Animations.
  (`/Engine/EditorBlueprintResources/StandardMacros.IsValid` _animmontage
    (:`Is Valid`
      (bind _output_get (set `self.CurrentAnimationMontage` _animmontage))
      (`self.PlayAnimMontage` _output_get _playrate))))

(event `StopCurrentAnimation`
  ;[1 1 1] Animations.
  (bind _currentanimationmontage (`self.CurrentAnimationMontage`)
    (:`then`
      (`self.StopAnimMontage` _currentanimationmontage))
    (:`else`)))

(event `OnNewCastStarted`
  (params (DelayProcess :type "/Game/RTSMultiplayer/AbilitySubsystem/Blueprints/AbilityProcess Object Reference"))
  (bind (_animmontage _playrate) (`self.GetInstantCastAnimationSettings`))
  ;[1 1 1] Animations.
  (`/Engine/EditorBlueprintResources/StandardMacros.IsValid` DelayProcess
    (:`Is Valid`
      (if (!= (`TimelineComponent.GetTimelineLength` (`/Game/RTSMultiplayer/AbilitySubsystem/Blueprints/AbilityProcess.ProcessTimeline` DelayProcess)) 0.0)
        (set `self.CurrentCastProcess` DelayProcess)
        (else
          (`self.StopCurrentAnimation`)
          (`/Engine/EditorBlueprintResources/StandardMacros.IsValid` _animmontage
            (:`Is Valid`
              (`self.PlayAnimMontage` _animmontage _playrate))))))))

(event `OnAttacking`
  (params (Actor :type "Actor Object Reference"))
  (bind (_animmontage _playrate) (`self.GetAttackAnimMontageSettings`))
  ;[1 1 1] Animations.
  (`/Engine/EditorBlueprintResources/StandardMacros.IsValid` _animmontage
    (:`Is Valid`
      (bind _output_get (set `self.CurrentAnimationMontage` _animmontage))
      (`self.PlayAnimMontage` _output_get _playrate))))

(event `IncreaseWarScoreClient`
  (bind _asbase_player_character (cast `/Game/RTSMultiplayer/RTSCharacters/Blueprints/BasePlayerCharacter` (`GameplayStatics.GetPlayerCharacter` 0) :!pure true))
  ;[1 1 1] Begin play. Initialize all necessary components.
  (`/Game/RTSMultiplayer/RTSCharacters/Blueprints/BasePlayerCharacter.IncreaseWarScore` _asbase_player_character (`self.WarScorePoints`))
  (`/Game/RTSMultiplayer/RTSCharacters/Blueprints/BasePlayerCharacter.IncreaseScienceScore` _asbase_player_character (`self.ScienceScorePoints`)))

(event `self.ReceiveBeginPlay`
  ;[1 1 1] Begin play. Initialize all necessary components.
  (bind _asbase_player_character (cast `/Game/RTSMultiplayer/RTSCharacters/Blueprints/BasePlayerCharacter` (`self.GetOwner`))
    (:`then`
      (`/Game/RTSMultiplayer/RTSCharacters/Blueprints/BasePlayerCharacter.IncreaseWarScore` _asbase_player_character (`self.WarScorePoints`))
      (`/Game/RTSMultiplayer/RTSCharacters/Blueprints/BasePlayerCharacter.IncreaseScienceScore` _asbase_player_character (`self.ScienceScorePoints`)))
    (:`CastFailed`
      (`self.IncreaseWarScoreClient`)))
  (add `/Game/RTSMultiplayer/CombatSubsystem/Blueprints/CombatComponent.Attacking` (`self.CombatComponent`) (`|CreateDelegate` :!event `OnAttacking`))
  (add `/Game/RTSMultiplayer/TaskSubsystem/Blueprints/TaskComponent.CurrentTaskStarted` (`self.TaskComponent`) (`|CreateDelegate` :!event `OnNewCastStarted`))
  (add `/Game/RTSMultiplayer/CombatSubsystem/Blueprints/CombatComponent.OwnerDeath` (`self.CombatComponent`) (`|CreateDelegate` :!event `OnUnitDeath`))
  (`/Game/RTSMultiplayer/FogSubsystem/Blueprints/FogOfWarComponent.SetSphereVisionCollision` (`self.FogOfWarComponent`) (`self.VisionSphere`))
  (bind _returnvalue (`|GenericCreateObject` "/Game/RTSMultiplayer/SelectionSubsystem/Blueprints/DecalSelector.DecalSelector_C" self (`self.SelectionDecal`)))
  (set `self.Selector` _returnvalue)
  (bind _returnvalue_2 (`|GenericCreateObject` "/Game/RTSMultiplayer/SelectionSubsystem/Blueprints/OutlineSelector.OutlineSelector_C" self (cast `/Game/RTSMultiplayer/SelectionSubsystem/Blueprints/I_CanBeOutlined` self :!pure true)))
  (set `self.AlienSelector` _returnvalue_2)
  (`/Game/RTSMultiplayer/StatsSubsystem/Blueprints/StatsComponent.AddNameplate` (`self.StatsComponent`) (`self.Nameplate`))
  (bind _returnvalue_3 (`|GetDataTableRow` "/Game/RTSMultiplayer/SelectionSubsystem/Data/SelectableActorsInfoDataTable.SelectableActorsInfoDataTable" (`self.UnitId`))
    (:`then`
      (set `self.SelectableActorInfo` _returnvalue_3))))

(event `OnUnitDeath`
  (params (Owner :type "Actor Object Reference"))
  (bind _asbase_player_character (cast `/Game/RTSMultiplayer/RTSCharacters/Blueprints/BasePlayerCharacter` (`GameplayStatics.GetPlayerCharacter` 0) :!pure true))
  ;[1 1 1] Free allocated resources on unit death.
  (bind _asbase_player_character_2 (cast `/Game/RTSMultiplayer/RTSCharacters/Blueprints/BasePlayerCharacter` (`self.GetOwner`))
    (:`then`
      (if (`|EnumEquality` (`/Game/RTSMultiplayer/RTSCharacters/Blueprints/BasePlayerCharacter.PlayerFaction` _asbase_player_character_2) (`self.Faction`))
        (`/Game/RTSMultiplayer/RTSCharacters/Blueprints/BasePlayerCharacter.FreeAllocatedResource` _asbase_player_character_2 "NewEnumerator2" (`self.GetNecessaryFreeSpace`))
        (`/Game/RTSMultiplayer/RTSCharacters/Blueprints/BasePlayerCharacter.DecreaseWarScore` _asbase_player_character_2 (`self.WarScorePoints`))
        (`/Game/RTSMultiplayer/RTSCharacters/Blueprints/BasePlayerCharacter.DecreaseScienceScore` _asbase_player_character_2 (`self.ScienceScorePoints`))))
    (:`CastFailed`
      (if (`|EnumEquality` (`/Game/RTSMultiplayer/RTSCharacters/Blueprints/BasePlayerCharacter.PlayerFaction` _asbase_player_character) (`self.Faction`))
        (`/Game/RTSMultiplayer/RTSCharacters/Blueprints/BasePlayerCharacter.FreeAllocatedResource` _asbase_player_character "NewEnumerator2" (`self.GetNecessaryFreeSpace`))
        (`/Game/RTSMultiplayer/RTSCharacters/Blueprints/BasePlayerCharacter.DecreaseWarScore` _asbase_player_character (`self.WarScorePoints`))
        (`/Game/RTSMultiplayer/RTSCharacters/Blueprints/BasePlayerCharacter.DecreaseScienceScore` _asbase_player_character (`self.ScienceScorePoints`))))))

(event `/Game/RTSMultiplayer/FogSubsystem/Blueprints/I_CanAffectFog.SetVisible`
  ;[1 1 1] I_CanAffectFog: set visible/invisible.
  (`SceneComponent.SetHiddenInGame` (`self.Mesh`) false false)
  (`SceneComponent.SetHiddenInGame` (`self.Nameplate`) false false))

(event `/Game/RTSMultiplayer/CombatSubsystem/Blueprints/I_AbleToFight.StartAttackCooldown`
  (params (CooldownTime :type "Float (single-precision)"))
  ;[1 1 1] I_AbleToFight: start attack cooldown.
  (`TimelineComponent.SetTimelineLength` (`self.AttackCooldownTimeline`) CooldownTime)
  (`Timeline|AttackCooldownTimeline` :!via `PlayFromStart`))

(event `/Game/RTSMultiplayer/FogSubsystem/Blueprints/I_CanAffectFog.SetInvisible`
  ;[1 1 1] I_CanAffectFog: set visible/invisible.
  (`SceneComponent.SetHiddenInGame` (`self.Mesh`) true false)
  (`SceneComponent.SetHiddenInGame` (`self.Nameplate`) true false))

(fn `AttackDealDamageNotify`
  (`/Game/RTSMultiplayer/CombatSubsystem/Blueprints/CombatComponent.AttackCallback` (`self.CombatComponent`)))

(fn `GetAbilities`
  (returns (Abilities :type "Array of /Game/RTSMultiplayer/AbilitySubsystem/Data/S_AbilityInfo Structure"))
  (return (`/Game/RTSMultiplayer/AbilitySubsystem/Blueprints/AbilityComponent.Abilities` (`self.AbilityComponent`))))

(fn `GetAbilityComponent`
  (returns (AbilityComponent :type "/Game/RTSMultiplayer/AbilitySubsystem/Blueprints/AbilityComponent Object Reference"))
  (return (`self.AbilityComponent`)))

(fn `GetAIController`
  (returns (Controller :type "AIController Object Reference"))
  (return (`AIBlueprintHelperLibrary.GetAIController` self)))

(fn `GetAlienSelector`
  (returns (Selector :type "/Game/RTSMultiplayer/SelectionSubsystem/Blueprints/Selector Object Reference"))
  (return (`self.AlienSelector`)))

(fn `GetAttackAnimMontageSettings`
  (returns (AnimMontage :type "AnimMontage Object Reference") (PlayRate :type "Float (double-precision)"))
  (return null 1.0))

(fn `GetBuildAnimationSettings`
  (returns (AnimMontage :type "AnimMontage Object Reference") (PlayRate :type "Float (double-precision)"))
  (return null 1.0))

(fn `GetCharacterMovementComponent`
  (returns (MovementComponent :type "CharacterMovementComponent Object Reference"))
  (return (`self.CharacterMovement`)))

(fn `GetChopTreeAnimationSettings`
  (returns (AnimMontage :type "AnimMontage Object Reference") (PlayRate :type "Float (double-precision)"))
  (return null 0.0))

(fn `GetCombatComponent`
  (returns (CombatComponent :type "/Game/RTSMultiplayer/CombatSubsystem/Blueprints/CombatComponent Object Reference"))
  (return (`self.CombatComponent`)))

(fn `GetCost`
  (returns (ConsumableResources :type "Map of /Game/RTSMultiplayer/ResourcesSubsystem/Blueprints/E_ResourceType Enum to Float (double-precision)") (AllocatableResources :type "Map of /Game/RTSMultiplayer/ResourcesSubsystem/Blueprints/E_ResourceType Enum to Float (double-precision)"))
  (return (`|MakeMap` "NewEnumerator1" 50.0 :!type "/Game/RTSMultiplayer/ResourcesSubsystem/Blueprints/E_ResourceType Enum" :!valuetype "Float (single-precision)") (`|MakeMap` "NewEnumerator2" (`self.GetNecessaryFreeSpace`) :!type "/Game/RTSMultiplayer/ResourcesSubsystem/Blueprints/E_ResourceType Enum")))

(fn `GetDamageReceiveModifierForDamageType`
  (params (DamageType :type "/Game/RTSMultiplayer/CombatSubsystem/Blueprints/E_DamageType Enum" :default "NewEnumerator0"))
  (returns (DamageModifier :type "Float (double-precision)"))
  (return 1.0))

(fn `GetDamageReceiveModifierForWeaponType`
  (params (WeaponType :type "/Game/RTSMultiplayer/CombatSubsystem/Blueprints/E_WeaponType Enum" :default "NewEnumerator0"))
  (returns (DamageModifier :type "Float (double-precision)"))
  (return 1.0))

(fn `GetDeathAnimMontageSettings`
  (returns (AnimMontage :type "AnimMontage Object Reference") (PlayRate :type "Float (double-precision)"))
  (return null 0.0))

(fn `GetEffectComponent`
  (returns (EffectComponent :type "/Game/RTSMultiplayer/EffectsSubsystem/Blueprints/EffectComponent Object Reference"))
  (return (`self.EffectComponent`)))

(fn `GetFactionAsAbleToFight`
  (returns (Faction :type "/Game/RTSMultiplayer/RTSCoreBP/E_Faction Enum"))
  (return (`self.Faction`)))

(fn `GetFactionAsCanBeOutlined`
  (returns (Faction :type "/Game/RTSMultiplayer/RTSCoreBP/E_Faction Enum"))
  (return (`self.Faction`)))

(fn `GetFactionAsEffectReceiver`
  (returns (Faction :type "/Game/RTSMultiplayer/RTSCoreBP/E_Faction Enum"))
  (return (`self.Faction`)))

(fn `GetFactionAsEnhanceable`
  (returns (Faction :type "/Game/RTSMultiplayer/RTSCoreBP/E_Faction Enum"))
  (return (`self.Faction`)))

(fn `GetFactionAsFogAffectable`
  (returns (Faction :type "/Game/RTSMultiplayer/RTSCoreBP/E_Faction Enum"))
  (return (`self.Faction`)))

(fn `GetFactionAsHaveInventory`
  (returns (Faction :type "/Game/RTSMultiplayer/RTSCoreBP/E_Faction Enum"))
  (return (`self.Faction`)))

(fn `GetFactionAsHaveStats`
  (returns (Faction :type "/Game/RTSMultiplayer/RTSCoreBP/E_Faction Enum"))
  (return (`self.Faction`)))

(fn `GetFactionAsSelectable`
  (returns (Faction :type "/Game/RTSMultiplayer/RTSCoreBP/E_Faction Enum"))
  (return (`self.Faction`)))

(fn `GetFogOfWarComponent`
  (returns (FogOfWarComponent :type "/Game/RTSMultiplayer/FogSubsystem/Blueprints/FogOfWarComponent Object Reference"))
  (return (`self.FogOfWarComponent`)))

(fn `GetFogRevealRadius`
  (returns (Radius :type "Float (double-precision)"))
  (return (`SphereComponent.GetScaledSphereRadius` (`self.VisionSphere`))))

(fn `GetHomingTargetComponent`
  (returns (HomingTargetComponent :type "PrimitiveComponent Object Reference"))
  (return (`self.CapsuleComponent`)))

(fn `GetIcon`
  (returns (Icon :type "Texture2D Object Reference"))
  (bind _selectableactorinfo_icon (break `/Game/RTSMultiplayer/SelectionSubsystem/Data/S_SelectableActorInfo` (`self.SelectableActorInfo`)))
  (return _selectableactorinfo_icon))

(fn `GetIdAsHaveAbilities`
  (returns (Id :type Name))
  (return (`self.UnitId`)))

(fn `GetIdAsHaveStats`
  (returns (Id :type Name))
  (return (`self.UnitId`)))

(fn `GetInstantCastAnimationSettings`
  (returns (AnimMontage :type "AnimMontage Object Reference") (PlayRate :type "Float (double-precision)"))
  (return null 0.0))

(fn `GetInventoryComponent`
  (returns (InventoryComponent :type "/Game/RTSMultiplayer/InventorySubsystem/Blueprints/InventoryComponent Object Reference"))
  (return (`self.InventoryComponent`)))

(fn `GetMineAnimationSettings`
  (returns (AnimMontage :type "AnimMontage Object Reference") (PlayRate :type "Float (double-precision)"))
  (return null 0.0))

(fn `GetMouseHoverResponsiveComponents`
  (returns (PrimitiveComponent :type "Array of PrimitiveComponent Object Reference"))
  (return (`|MakeArray` (`self.CapsuleComponent`) :!type "PrimitiveComponent Object Reference")))

(fn `GetName`
  (returns (Name :type Text))
  (bind (_selectableactorinfo_icon _selectableactorinfo_name) (break `/Game/RTSMultiplayer/SelectionSubsystem/Data/S_SelectableActorInfo` (`self.SelectableActorInfo`)))
  (return _selectableactorinfo_name))

(fn `GetNearbyActors`
  (params (SpherePos :type "Vector Structure") (SphereRadius :type "Float (double-precision)") (ActorClassFilter :type "Object Class Reference") (ActorsToIgnore :type "Array of Actor Object Reference (by ref)"))
  (returns (OutActors :type "Array of Actor Object Reference") (`Found?` :type Boolean))
  (bind (_outactors _returnvalue) (`KismetSystemLibrary.SphereOverlapActors` SpherePos SphereRadius (`|MakeArray` "ObjectTypeQuery1" "ObjectTypeQuery2" "ObjectTypeQuery3" :!type "EObjectTypeQuery Enum") ActorClassFilter ActorsToIgnore))
  (return _outactors _returnvalue))

(fn `GetNearbyFriends`
  (returns (Enemies :type "Array of /Game/RTSMultiplayer/RTSCharacters/Blueprints/BaseRTSUnit Object Reference"))
  (locals (UsedUnits :type "Set of /Game/RTSMultiplayer/RTSCharacters/Blueprints/BaseRTSUnit Object Reference") (Result :type "Array of /Game/RTSMultiplayer/RTSCharacters/Blueprints/BaseRTSUnit Object Reference"))
  (bind _outcomponents (`KismetSystemLibrary.SphereOverlapComponents` (`self.K2_GetActorLocation`) (* (`SphereComponent.GetScaledSphereRadius` (`self.VisionSphere`)) 2.0) (`|MakeArray` "ObjectTypeQuery2" :!type "EObjectTypeQuery Enum") "/Script/Engine.CapsuleComponent"))
  (for _array_element _outcomponents
    (bind _asbase_rtsunit (cast `/Game/RTSMultiplayer/RTSCharacters/Blueprints/BaseRTSUnit` (`ActorComponent.GetOwner` _array_element)))
    (if (and (`|EnumEquality` (`/Game/RTSMultiplayer/RTSCharacters/Blueprints/BasePlayerCharacter.GetRelationships` (cast `/Game/RTSMultiplayer/RTSCharacters/Blueprints/BasePlayerCharacter` (`self.GetOwner`) :!pure true) (`/Game/RTSMultiplayer/RTSCharacters/Blueprints/BaseRTSUnit.Faction` _asbase_rtsunit)) "NewEnumerator0") (`ActorComponent.ComponentHasTag` _array_element "VisionCollision"))
      (if (not (`BlueprintSetLibrary.Set_Contains` (`local.UsedUnits`) _asbase_rtsunit))
        (`BlueprintSetLibrary.Set_Add` (`local.UsedUnits`) _asbase_rtsunit)
        (`KismetArrayLibrary.Array_Add` (`local.Result`) _asbase_rtsunit))))
  (return (`local.Result`)))

(fn `GetNecessaryFreeSpace`
  (returns (FreeSpace :type "Float (double-precision)"))
  (return 1.0))

(fn `GetOutlineComponent`
  (returns (OutlineComponent :type "/Game/RTSMultiplayer/SelectionSubsystem/Blueprints/OutlineComponent Object Reference"))
  (return (`self.OutlineComponent`)))

(fn `GetOutlineMeshes`
  (returns (OptionalSceneComponents :type "Array of SceneComponent Object Reference") (MeshComponents :type "Array of MeshComponent Object Reference"))
  (return _ (`|MakeArray` (`self.Mesh`) :!type "MeshComponent Object Reference")))

(fn `GetQuickUseAbilityClass`
  (returns (AbilityClasses :type "Array of /Game/RTSMultiplayer/AbilitySubsystem/Blueprints/Ability Class Reference"))
  (return (`|MakeArray` "/Game/RTSMultiplayer/AbilitySubsystem/Blueprints/General/AttackAbility.AttackAbility_C" :!type "/Game/RTSMultiplayer/AbilitySubsystem/Blueprints/Ability Class Reference")))

(fn `GetSelector`
  (returns (Selector :type "/Game/RTSMultiplayer/SelectionSubsystem/Blueprints/Selector Object Reference"))
  (return (`self.Selector`)))

(fn `GetStatsComponent`
  (returns (StatsComponent :type "/Game/RTSMultiplayer/StatsSubsystem/Blueprints/StatsComponent Object Reference"))
  (return (`self.StatsComponent`)))

(fn `GetTaskComponent`
  (returns (TaskComponent :type "/Game/RTSMultiplayer/TaskSubsystem/Blueprints/TaskComponent Object Reference"))
  (return (`self.TaskComponent`)))

(fn `GetWorldLocation`
  (returns (WorldLocation :type "Vector Structure"))
  (return (`self.K2_GetActorLocation`)))

(fn `IsAttackOnCooldown?`
  (returns (`IsOnCooldown?` :type Boolean))
  (return (`TimelineComponent.IsPlaying` (`self.AttackCooldownTimeline`))))

(fn `IsVisible?`
  (returns (Visible :type Boolean))
  (return (not (`SceneComponent.bHiddenInGame` (`self.Mesh`)))))

(fn `UserConstructionScript`)