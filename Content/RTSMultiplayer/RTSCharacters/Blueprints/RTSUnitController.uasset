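; AI controller for RTS units that runs a combat behavior tree and chooses which ability the unit uses.
; On begin play it builds a map of data-table ability info to optional condition objects and starts a looping timer.
; TryToUseAbility fills an empty blackboard ability slot with the first off-cooldown, affordable ability's class and range.
; The condition objects are stored but not evaluated here.
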(event `self.ReceiveBeginPlay`
  ;[1 1 1] Begin play.
  (`self.InitializeThunks`)
  (`self.RunBehaviorTree` "/Game/RTSMultiplayer/AISubsystem/Combat/CombatAIBehaviorTree.CombatAIBehaviorTree")
  (`KismetSystemLibrary.K2_SetTimerDelegate` (`|CreateDelegate` :!event `TryToUseAbility`) 2.0 true))

(event `TryToUseAbility`
  (bind _returnvalue (`AIBlueprintHelperLibrary.GetBlackboard` null))
  ;[1 1 1] Try to use ability.
  (if (== (`BlackboardComponent.GetValueAsClass` (`AIBlueprintHelperLibrary.GetBlackboard` null) (`self.AbilityToUseKey`)) null)
    (bind _keys (`BlueprintMapLibrary.Map_Keys` (`self.AbilityThunksMap`)))
    (for _array_element _keys
      (bind (_abilityclass _abilityid _abilityinfo) (break `/Game/RTSMultiplayer/AISubsystem/Combat/S_AbilityThunk` _array_element))
      (if (`/Game/RTSMultiplayer/AbilitySubsystem/Blueprints/AbilityComponent.IsAbilityOnCooldown?` (`/Game/RTSMultiplayer/RTSCharacters/Blueprints/BaseRTSUnit.AbilityComponent` (cast `/Game/RTSMultiplayer/RTSCharacters/Blueprints/BaseRTSUnit` (`self.K2_GetPawn`) :!pure true)) _abilityclass)
        _
        (elif (`/Game/RTSMultiplayer/RTSCharacters/Blueprints/RTSAIController.CheckForEnoughResources` (cast `/Game/RTSMultiplayer/RTSCharacters/Blueprints/RTSAIController` (`AIBlueprintHelperLibrary.GetAIController` (`self.GetOwner`)) :!pure true) _abilityinfo)
          (`BlackboardComponent.SetValueAsClass` _returnvalue (`self.AbilityToUseKey`) _abilityclass)
          (`BlackboardComponent.SetValueAsFloat` _returnvalue (`self.AbilityToUseRangeKey`) (`.AbilityRange_40_D6C6FE6A4D87A62EFBED188164408101` (break `/Game/RTSMultiplayer/AbilitySubsystem/Data/S_AbilityInfo` _abilityinfo)))
          (break))))))

(fn `InitializeThunks`
  (for (_array_element _array_index) (`self.AbilityThunks`)
    (bind (_abilityclass _abilityid) (break `/Game/RTSMultiplayer/AISubsystem/Combat/S_AbilityThunk` _array_element))
    (bind _returnvalue (`|GetDataTableRow` "/Game/RTSMultiplayer/AbilitySubsystem/Data/AbilitiesDataTable.AbilitiesDataTable" _abilityid)
      (:`then`
        (bind _output (`|GetArrayItem` (`self.AbilityCondClasses`) _array_index))
        (if (== _output null)
          (bind _s_abilitythunk (make `/Game/RTSMultiplayer/AISubsystem/Combat/S_AbilityThunk` _abilityclass _abilityid _returnvalue))
          (`BlueprintMapLibrary.Map_Add` (`self.AbilityThunksMap`) _s_abilitythunk)
          (else
            (bind _returnvalue_2 (`|GenericCreateObject` _output (`self.GetOwner`)))
            (`BlueprintMapLibrary.Map_Add` (`self.AbilityThunksMap`) _s_abilitythunk _returnvalue_2))))
      (:`RowNotFound`
        (`KismetSystemLibrary.PrintString` "RTSUnitController: ability row not found." true true (struct :`R` 1.0 :`G` 0.064054 :`A` 1.0) 5.0)))))

(fn `UserConstructionScript`)