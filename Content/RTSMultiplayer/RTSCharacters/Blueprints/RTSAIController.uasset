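; AI controller for a computer-controlled RTS player that runs building abilities, learns perks and attacks enemy players.
; Data-table thunks with optional condition objects form ordered to-do maps, worked on looping timers as resources allow; FirstNeed entries block later ones.
; Unit and building vision spheres feed a reference-counted visible-enemy list.
; After a delay, a sufficient war-score lead sends some units at an enemy townhouse through their blackboards.
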(event `self.ReceiveBeginPlay`
  ;[1 1 1] Begin play. Initialize thunks, set events by timers.
  (`self.InitializeBuildingsThunks`)
  (`self.InitializeBuildingAbilitiesThunks`)
  (`self.InitializePerkThunks`)
  (`KismetSystemLibrary.Delay` 2.0)
  (bind _returnvalue (`KismetSystemLibrary.K2_SetTimerDelegate` (`|CreateDelegate` :!event `TryToUseBuildingAbility`) 2.5 true))
  (set `self.TryToUseBuildingAbilityHandle` _returnvalue)
  (`self.InitializeEnemyPlayers`)
  (bind _returnvalue_2 (`KismetSystemLibrary.K2_SetTimerDelegate` (`|CreateDelegate` :!event `TryToLearnPerk`) 3.0 true))
  (set `self.LearnPerkHandle` _returnvalue_2)
  (`KismetSystemLibrary.Delay` (`self.AggressiveModeDelay`))
  (bind _returnvalue_3 (`KismetSystemLibrary.K2_SetTimerDelegate` (`|CreateDelegate` :!event `TryToSwitchToAggressiveMode`) 5.0 true))
  (set `self.AggressiveModeHandle` _returnvalue_3))

(event `OnBuildingEndPlay`
  (params (Actor :type "Actor Object Reference") (EndPlayReason :type "EEndPlayReason Enum" :default "Destroyed"))
  ;[1 1 1] On Building End Play.
  (bind _asbase_rtsbuilding (cast `/Game/RTSMultiplayer/BuildingSubsystem/Blueprints/BaseRTSBuilding` Actor))
  (`self.RemoveBuilding` _asbase_rtsbuilding))

(event `OnEnemyUnrevealed`
  (params (Enemy :type "Actor Object Reference"))
  ;[1 1 1] Revealed/Unrevealed enemy.
  (`KismetArrayLibrary.Array_RemoveItem` (`self.VisibleEnemies`) Enemy))

(event `OnEnemyRevealed`
  (params (Enemy :type "Actor Object Reference"))
  ;[1 1 1] Revealed/Unrevealed enemy.
  (`KismetArrayLibrary.Array_Add` (`self.VisibleEnemies`) Enemy))

(event `OnUnitEndPlay`
  (params (Actor :type "Actor Object Reference") (EndPlayReason :type "EEndPlayReason Enum" :default "Destroyed"))
  ;[1 1 1] Revealed/Unrevealed enemy.
  (bind _asbase_rtsunit (cast `/Game/RTSMultiplayer/RTSCharacters/Blueprints/BaseRTSUnit` Actor))
  (`self.RemoveUnit` _asbase_rtsunit))

(event `self.ReceiveTick`
  (params (DeltaSeconds :type "Float (single-precision)"))
  ;[1 1 1] Tick: print debug info (connect nodes if you want to print it).
)

(event `TryToUseBuildingAbility`
  (bind _buildingabilitiesthunksmap (`self.BuildingAbilitiesThunksMap`))
  ;[1 1 1] Try to use building ability.
  (bind _keys (`BlueprintMapLibrary.Map_Keys` _buildingabilitiesthunksmap))
  (for _array_element _keys
    (bind (_rtsbuildingclass _buildingabilityname _isrepeatable_ _firstneed) (break `/Game/RTSMultiplayer/AISubsystem/Buildings/S_BuildingAbilityThunk` _array_element))
    (bind (_value _returnvalue) (`BlueprintMapLibrary.Map_Find` (`self.AvailableBuildings`) _rtsbuildingclass))
    (if _returnvalue
      (bind _success_ (`self.SpawnAndUseBuildingsAbility` _array_element (`BlueprintMapLibrary.Map_Find` _buildingabilitiesthunksmap _array_element) (break `/Game/RTSMultiplayer/AISubsystem/Buildings/S_ArrayOfBuildings` _value)))
      (if _success_
        (if (not _isrepeatable_)
          (`BlueprintMapLibrary.Map_Remove` (`self.BuildingAbilitiesThunksMap`) _array_element))
        (elif _firstneed
          (break)))
      (elif _firstneed
        (break)))))

(event `OnVisionSphereBeginOverlap`
  (params (OverlappedComponent :type "PrimitiveComponent Object Reference") (OtherActor :type "Actor Object Reference") (OtherComp :type "PrimitiveComponent Object Reference") (OtherBodyIndex :type Integer) (bFromSweep :type Boolean) (SweepResult :type "HitResult Structure (by ref)"))
  ;[1 1 1] Revealed/Unrevealed enemy.
  (if (`ActorComponent.ComponentHasTag` OtherComp (`self.VisionCollisionTag`))
    (bind _asi_can_affect_fog (cast `/Game/RTSMultiplayer/FogSubsystem/Blueprints/I_CanAffectFog` OtherActor))
    (bind _faction (`/Game/RTSMultiplayer/FogSubsystem/Blueprints/I_CanAffectFog.GetFactionAsFogAffectable` _asi_can_affect_fog))
    (if (`|EnumInequality` _faction (`/Game/RTSMultiplayer/RTSCharacters/Blueprints/BasePlayerCharacter.PlayerFaction` (cast `/Game/RTSMultiplayer/RTSCharacters/Blueprints/BasePlayerCharacter` (`self.K2_GetPawn`) :!pure true)))
      (`self.AddActorToVisibleEnemiesMap` OtherActor))))

(event `OnVisionSphereEndOverlap`
  (params (OverlappedComponent :type "PrimitiveComponent Object Reference") (OtherActor :type "Actor Object Reference") (OtherComp :type "PrimitiveComponent Object Reference") (OtherBodyIndex :type Integer))
  ;[1 1 1] Revealed/Unrevealed enemy.
  (if (`ActorComponent.ComponentHasTag` OtherComp (`self.VisionCollisionTag`))
    (bind _asi_can_affect_fog (cast `/Game/RTSMultiplayer/FogSubsystem/Blueprints/I_CanAffectFog` OtherActor))
    (bind _faction (`/Game/RTSMultiplayer/FogSubsystem/Blueprints/I_CanAffectFog.GetFactionAsFogAffectable` _asi_can_affect_fog))
    (if (`|EnumInequality` _faction (`/Game/RTSMultiplayer/RTSCharacters/Blueprints/BasePlayerCharacter.PlayerFaction` (cast `/Game/RTSMultiplayer/RTSCharacters/Blueprints/BasePlayerCharacter` (`self.K2_GetPawn`) :!pure true)))
      (`self.RemoveActorFromVisibleEnemiesMap` OtherActor))))

(event `TryToSwitchToAggressiveMode`
  ;[1 1 1] Aggressive mode.
  (`self.CurrentEnemyPlayer`
    (:`then`)
    (:`else`
      (for _array_element (`self.EnemyPlayers`)
        (if (> (* (- 1.0 (`self.AggressiveModeAdvantagePercentage`)) (`/Game/RTSMultiplayer/RTSCharacters/Blueprints/BasePlayerCharacter.WarScore` (cast `/Game/RTSMultiplayer/RTSCharacters/Blueprints/BasePlayerCharacter` (`self.K2_GetPawn`) :!pure true))) (+ (`/Game/RTSMultiplayer/RTSCharacters/Blueprints/BasePlayerCharacter.WarScore` _array_element) (`/Game/RTSMultiplayer/RTSCharacters/Blueprints/BasePlayerCharacter.ScienceScore` _array_element)))
          (set `self.CurrentEnemyPlayer` _array_element)
          (`self.GoAggressive`)
          (break))))))

(event `TryToLearnPerk`
  (bind _asbase_player_character (cast `/Game/RTSMultiplayer/RTSCharacters/Blueprints/BasePlayerCharacter` (`self.K2_GetPawn`) :!pure true))
  ;[1 1 1] Try to learn perks.
  (if (== (`KismetArrayLibrary.Array_Length` (`/Game/RTSMultiplayer/AbilitySubsystem/Blueprints/AbilityComponent.AbilityProcesses` (`/Game/RTSMultiplayer/RTSCharacters/Blueprints/BasePlayerCharacter.AbilityComponent` _asbase_player_character))) 0)
    (bind _keys (`BlueprintMapLibrary.Map_Keys` (`self.PerkThunksMap`)))
    (for _array_element _keys
      (bind (_perkclass _perkid _firstneed _abilityinfo) (break `/Game/RTSMultiplayer/AISubsystem/General/S_PerkThunk` _array_element))
      (if (`self.CheckForEnoughResources` _abilityinfo)
        (`/Game/RTSMultiplayer/RTSCharacters/Blueprints/BasePlayerCharacter.SpawnAndUseAbility` _asbase_player_character _perkclass (`|MakeArray` _asbase_player_character :!type "Actor Object Reference"))
        (`BlueprintMapLibrary.Map_Remove` (`self.PerkThunksMap`) _array_element)
        (break)
        (elif _firstneed
          (break))))))

(event `GoAggressive`
  ;[1 1 1] Aggressive mode.
  (bind _outactors (`GameplayStatics.GetAllActorsOfClass` (`self.MainBuildingClass`)))
  (for _array_element _outactors
    (bind _astownhouse (cast `/Game/RTSMultiplayer/BuildingSubsystem/Blueprints/Buildings/Global/Townhouse` _array_element :!pure true))
    (if (`|EnumEquality` (`/Game/RTSMultiplayer/BuildingSubsystem/Blueprints/BaseRTSBuilding.Faction` _astownhouse) (`/Game/RTSMultiplayer/RTSCharacters/Blueprints/BasePlayerCharacter.PlayerFaction` (`self.CurrentEnemyPlayer`)))
      (set `self.CurrentEnemyMainBuilding` _astownhouse)
      (`self.SetAggressiveMode`)
      (break)))
  (`self.CurrentEnemyMainBuilding`
    (:`then`)
    (:`else`
      (set `self.CurrentEnemyPlayer` null))))

(fn `AddActorToVisibleEnemiesMap`
  (params (Actor :type "Actor Object Reference"))
  (bind _visibleenemiesmap (`self.VisibleEnemiesMap`))
  (bind (_value _returnvalue) (`BlueprintMapLibrary.Map_Find` _visibleenemiesmap Actor))
  (if _returnvalue
    (`BlueprintMapLibrary.Map_Add` _visibleenemiesmap Actor (+ _value 1))
    (else
      (`BlueprintMapLibrary.Map_Add` (`self.VisibleEnemiesMap`) Actor 1)
      (`self.OnEnemyRevealed` Actor))))

(fn `AddNewBuilding`
  (params (Building :type "/Game/RTSMultiplayer/BuildingSubsystem/Blueprints/BaseRTSBuilding Object Reference"))
  (locals (OldBuildings :type "Array of /Game/RTSMultiplayer/BuildingSubsystem/Blueprints/BaseRTSBuilding Object Reference"))
  (bind _returnvalue (`GameplayStatics.GetObjectClass` Building))
  (bind _availablebuildings (`self.AvailableBuildings`))
  (bind _visionsphere (`/Game/RTSMultiplayer/BuildingSubsystem/Blueprints/BaseRTSBuilding.VisionSphere` Building))
  (bind (_value _returnvalue_2) (`BlueprintMapLibrary.Map_Find` _availablebuildings _returnvalue))
  (add `PrimitiveComponent.OnComponentBeginOverlap` _visionsphere (`|CreateDelegate` :!event `OnVisionSphereBeginOverlap`))
  (add `PrimitiveComponent.OnComponentEndOverlap` _visionsphere (`|CreateDelegate` :!event `OnVisionSphereEndOverlap`))
  (if _returnvalue_2
    (bind _output_get (set `local.OldBuildings` (break `/Game/RTSMultiplayer/AISubsystem/Buildings/S_ArrayOfBuildings` _value)))
    (`KismetArrayLibrary.Array_Add` _output_get Building)
    (`BlueprintMapLibrary.Map_Add` _availablebuildings _returnvalue (make `/Game/RTSMultiplayer/AISubsystem/Buildings/S_ArrayOfBuildings` (`local.OldBuildings`)))
    (else
      (`BlueprintMapLibrary.Map_Add` (`self.AvailableBuildings`) _returnvalue (make `/Game/RTSMultiplayer/AISubsystem/Buildings/S_ArrayOfBuildings` (`|MakeArray` Building)))))
  (add `self.OnEndPlay` Building (`|CreateDelegate` :!event `OnBuildingEndPlay`)))

(fn `AddNewUnit`
  (params (Unit :type "/Game/RTSMultiplayer/RTSCharacters/Blueprints/BaseRTSUnit Object Reference"))
  (locals (OldUnits :type "Array of /Game/RTSMultiplayer/RTSCharacters/Blueprints/BaseRTSUnit Object Reference"))
  (bind _returnvalue (`GameplayStatics.GetObjectClass` Unit))
  (bind _visionsphere (`/Game/RTSMultiplayer/RTSCharacters/Blueprints/BaseRTSUnit.VisionSphere` Unit))
  (bind (_value _returnvalue_2) (`BlueprintMapLibrary.Map_Find` (`self.AvailableUnits`) _returnvalue))
  (add `PrimitiveComponent.OnComponentBeginOverlap` _visionsphere (`|CreateDelegate` :!event `OnVisionSphereBeginOverlap`))
  (add `PrimitiveComponent.OnComponentEndOverlap` _visionsphere (`|CreateDelegate` :!event `OnVisionSphereEndOverlap`))
  (add `self.OnEndPlay` Unit (`|CreateDelegate` :!event `OnUnitEndPlay`))
  (if (`BlueprintSetLibrary.Set_Contains` (`self.WorkerUnitsClasses`) _returnvalue)
    (`KismetArrayLibrary.Array_Add` (`self.AvailableWorkers`) Unit)
    (elif _returnvalue_2
      (bind _output_get (set `local.OldUnits` (break `/Game/RTSMultiplayer/RTSCharacters/Blueprints/S_ArrayOfUnits` _value)))
      (`KismetArrayLibrary.Array_Add` _output_get Unit)
      (`BlueprintMapLibrary.Map_Add` (`self.AvailableUnits`) _returnvalue (make `/Game/RTSMultiplayer/RTSCharacters/Blueprints/S_ArrayOfUnits` (`local.OldUnits`)))
      (else
        (`BlueprintMapLibrary.Map_Add` (`self.AvailableUnits`) _returnvalue (make `/Game/RTSMultiplayer/RTSCharacters/Blueprints/S_ArrayOfUnits` (`|MakeArray` Unit)))))))

(fn `CheckForEnoughResources`
  (params (AbilityInfo :type "/Game/RTSMultiplayer/AbilitySubsystem/Data/S_AbilityInfo Structure (by ref)"))
  (returns (`Enough?` :type Boolean))
  (bind ((`ConsumableCost_26_03C7DBCC41457F4251BFB0AF879BEE44` _consumablecost) (`AllocatableCost_29_ED89984B4F4139EABCE6599E8ECB0AB5` _allocatablecost)) (break `/Game/RTSMultiplayer/AbilitySubsystem/Data/S_AbilityInfo` AbilityInfo))
  (bind _keys (`BlueprintMapLibrary.Map_Keys` _consumablecost))
  (for _array_element _keys
    (if (not (`/Game/RTSMultiplayer/RTSCharacters/Blueprints/BasePlayerCharacter.IsThereEnoughResource?` (cast `/Game/RTSMultiplayer/RTSCharacters/Blueprints/BasePlayerCharacter` (`self.K2_GetPawn`) :!pure true) _array_element (`BlueprintMapLibrary.Map_Find` _consumablecost _array_element)))
      (return false)))
  (bind _keys_2 (`BlueprintMapLibrary.Map_Keys` _allocatablecost))
  (for _array_element_2 _keys_2
    (if (not (`/Game/RTSMultiplayer/RTSCharacters/Blueprints/BasePlayerCharacter.IsThereEnoughResource?` (cast `/Game/RTSMultiplayer/RTSCharacters/Blueprints/BasePlayerCharacter` (`self.K2_GetPawn`) :!pure true) _array_element_2 (`BlueprintMapLibrary.Map_Find` _allocatablecost _array_element_2)))
      (return false)))
  (return true))

(fn `GetBestEnemy`
  (params (ForUnit :type "/Game/RTSMultiplayer/RTSCharacters/Blueprints/BaseRTSUnit Object Reference"))
  (returns (Enemy :type "Actor Object Reference"))
  (locals (BestEnemy :type "Actor Object Reference") (BestEnemyPriority :type "Float (double-precision)") (MaxRangeToAttack :type "Float (double-precision)" :default 15000.0))
  (for _array_element (`self.VisibleEnemies`)
    (bind _returnvalue (* (`BlueprintMapLibrary.Map_Find` (`self.EnemyClassesPriority`) (`GameplayStatics.GetObjectClass` _array_element)) (- 1.0 (`KismetMathLibrary.MapRangeClamped` (`self.GetDistanceTo` ForUnit _array_element) 0.0 (`self.MaxUnitsAttackRange`) 0.0 1.0))))
    (if (> _returnvalue (`local.BestEnemyPriority`))
      (set `local.BestEnemyPriority` _returnvalue)
      (set `local.BestEnemy` _array_element)))
  (return (`local.BestEnemy`)))

(fn `InitializeBuildingAbilitiesThunks`
  (for (_array_element _array_index) (`self.BuildingAbilitiesThunks`)
    (bind (_rtsbuildingclass _buildingabilityname _isrepeatable_ _firstneed) (break `/Game/RTSMultiplayer/AISubsystem/Buildings/S_BuildingAbilityThunk` _array_element))
    (bind _returnvalue (`|GetDataTableRow` "/Game/RTSMultiplayer/AbilitySubsystem/Data/AbilitiesDataTable.AbilitiesDataTable" _buildingabilityname)
      (:`then`
        (bind _output (`|GetArrayItem` (`self.BuildingAbilitiesCondClasses`) _array_index))
        (if (!= _output null)
          (bind _returnvalue_2 (`|GenericCreateObject` _output (`self.K2_GetPawn`)))
          (bind _s_buildingabilitythunk (make `/Game/RTSMultiplayer/AISubsystem/Buildings/S_BuildingAbilityThunk` _rtsbuildingclass _buildingabilityname _isrepeatable_ _firstneed _returnvalue))
          (`BlueprintMapLibrary.Map_Add` (`self.BuildingAbilitiesThunksMap`) _s_buildingabilitythunk _returnvalue_2)
          (else
            (`BlueprintMapLibrary.Map_Add` (`self.BuildingAbilitiesThunksMap`) _s_buildingabilitythunk))))
      (:`RowNotFound`
        (`KismetSystemLibrary.PrintString` "WorkerAIController: ability info data table row not found." true true (struct :`R` 1.0 :`G` 0.064054 :`A` 1.0) 5.0)))))

(fn `InitializeBuildingsThunks`
  (for (_array_element _array_index) (`self.BuildingThunks`)
    (bind _returnvalue (`|GetDataTableRow` "/Game/RTSMultiplayer/AbilitySubsystem/Data/AbilitiesDataTable.AbilitiesDataTable" (`.BuildAbilityName_13_CD5ADC6C4BE64D6BEF7243A24E29C8DE` (break `/Game/RTSMultiplayer/AISubsystem/General/S_BuildingThunk` _array_element)))
      (:`then`
        (bind _output (`|GetArrayItem` (`self.BuildingThunkCondClasses`) _array_index))
        (if (!= _output null)
          (bind _returnvalue_2 (`|GenericCreateObject` _output (`self.K2_GetPawn`)))
          (bind (_buildingclass _buildabilityname _isrepeatable_) (break `/Game/RTSMultiplayer/AISubsystem/General/S_BuildingThunk` _array_element))
          (bind _s_buildingthunk (make `/Game/RTSMultiplayer/AISubsystem/General/S_BuildingThunk` _buildingclass _buildabilityname _isrepeatable_ false _returnvalue))
          (`BlueprintMapLibrary.Map_Add` (`self.BuildingThunksMap`) _s_buildingthunk _returnvalue_2)
          (else
            (`BlueprintMapLibrary.Map_Add` (`self.BuildingThunksMap`) _s_buildingthunk))))
      (:`RowNotFound`
        (`KismetSystemLibrary.PrintString` "WorkerAIController: ability info data table row not found." true true (struct :`R` 1.0 :`G` 0.064054 :`A` 1.0) 5.0)))))

(fn `InitializeEnemyPlayers`
  (bind _outactors (`GameplayStatics.GetAllActorsOfClass` "/Game/RTSMultiplayer/RTSCharacters/Blueprints/BasePlayerCharacter.BasePlayerCharacter_C"))
  (for _array_element _outactors
    (if (`|EnumEquality` (`/Game/RTSMultiplayer/RTSCharacters/Blueprints/BasePlayerCharacter.GetRelationships` (cast `/Game/RTSMultiplayer/RTSCharacters/Blueprints/BasePlayerCharacter` (`self.K2_GetPawn`) :!pure true) (`/Game/RTSMultiplayer/RTSCharacters/Blueprints/BasePlayerCharacter.PlayerFaction` _array_element)) "NewEnumerator1")
      (`KismetArrayLibrary.Array_Add` (`self.EnemyPlayers`) _array_element))))

(fn `InitializePerkThunks`
  (for (_array_element _array_index) (`self.PerkThunks`)
    (bind (_perkclass _perkid _firstneed) (break `/Game/RTSMultiplayer/AISubsystem/General/S_PerkThunk` _array_element))
    (bind _returnvalue (`|GetDataTableRow` "/Game/RTSMultiplayer/AbilitySubsystem/Data/AbilitiesDataTable.AbilitiesDataTable" _perkid)
      (:`then`
        (bind _output (`|GetArrayItem` (`self.PerkCondClasses`) _array_index))
        (if (!= _output null)
          (bind _returnvalue_2 (`|GenericCreateObject` _output (`self.K2_GetPawn`)))
          (bind _s_perkthunk (make `/Game/RTSMultiplayer/AISubsystem/General/S_PerkThunk` _perkclass _perkid _firstneed _returnvalue))
          (`BlueprintMapLibrary.Map_Add` (`self.PerkThunksMap`) _s_perkthunk _returnvalue_2)
          (else
            (`BlueprintMapLibrary.Map_Add` (`self.PerkThunksMap`) _s_perkthunk))))
      (:`RowNotFound`
        (`KismetSystemLibrary.PrintString` "RTSAIController: perk row not found." true true (struct :`R` 1.0 :`G` 0.064054 :`A` 1.0) 5.0)))))

(fn `RemoveActorFromVisibleEnemiesMap`
  (params (Actor :type "Actor Object Reference (by ref)"))
  (bind _visibleenemiesmap (`self.VisibleEnemiesMap`))
  (bind _value (`BlueprintMapLibrary.Map_Find` _visibleenemiesmap Actor))
  (if (== _value 1)
    (`BlueprintMapLibrary.Map_Remove` _visibleenemiesmap Actor)
    (`self.OnEnemyUnrevealed` Actor)
    (else
      (`BlueprintMapLibrary.Map_Add` (`self.VisibleEnemiesMap`) Actor (- _value 1)))))

(fn `RemoveBuilding`
  (params (Building :type "/Game/RTSMultiplayer/BuildingSubsystem/Blueprints/BaseRTSBuilding Object Reference"))
  (locals (OldBuildings :type "Array of /Game/RTSMultiplayer/BuildingSubsystem/Blueprints/BaseRTSBuilding Object Reference"))
  (bind _returnvalue (`GameplayStatics.GetObjectClass` Building))
  (bind _oldbuildings (`local.OldBuildings`))
  (bind _visionsphere (`/Game/RTSMultiplayer/BuildingSubsystem/Blueprints/BaseRTSBuilding.VisionSphere` Building))
  (bind (_value _returnvalue_2) (`BlueprintMapLibrary.Map_Find` (`self.AvailableBuildings`) _returnvalue))
  (remove `PrimitiveComponent.OnComponentBeginOverlap` _visionsphere (`|CreateDelegate` :!event `OnVisionSphereBeginOverlap`))
  (remove `PrimitiveComponent.OnComponentEndOverlap` _visionsphere (`|CreateDelegate` :!event `OnVisionSphereEndOverlap`))
  (if _returnvalue_2
    (bind _output_get (set `local.OldBuildings` (break `/Game/RTSMultiplayer/AISubsystem/Buildings/S_ArrayOfBuildings` _value)))
    (bind _returnvalue_3 (`KismetArrayLibrary.Array_RemoveItem` _output_get Building))
    (if (and _returnvalue_3 (!= (`KismetArrayLibrary.Array_Length` _oldbuildings) 0))
      (`BlueprintMapLibrary.Map_Add` (`self.AvailableBuildings`) _returnvalue (make `/Game/RTSMultiplayer/AISubsystem/Buildings/S_ArrayOfBuildings` _oldbuildings)))))

(fn `RemoveBuildingThunk`
  (params (BuildingThunk :type "/Game/RTSMultiplayer/AISubsystem/General/S_BuildingThunk Structure"))
  (`BlueprintMapLibrary.Map_Remove` (`self.BuildingThunksMap`) BuildingThunk))

(fn `RemoveUnit`
  (params (Unit :type "/Game/RTSMultiplayer/RTSCharacters/Blueprints/BaseRTSUnit Object Reference"))
  (locals (OldUnits :type "Array of /Game/RTSMultiplayer/RTSCharacters/Blueprints/BaseRTSUnit Object Reference"))
  (bind _returnvalue (`GameplayStatics.GetObjectClass` Unit))
  (bind _visionsphere (`/Game/RTSMultiplayer/RTSCharacters/Blueprints/BaseRTSUnit.VisionSphere` Unit))
  (bind (_value _returnvalue_2) (`BlueprintMapLibrary.Map_Find` (`self.AvailableUnits`) _returnvalue))
  (remove `PrimitiveComponent.OnComponentBeginOverlap` _visionsphere (`|CreateDelegate` :!event `OnVisionSphereBeginOverlap`))
  (remove `PrimitiveComponent.OnComponentEndOverlap` _visionsphere (`|CreateDelegate` :!event `OnVisionSphereEndOverlap`))
  (if _returnvalue_2
    (bind _output_get (set `local.OldUnits` (break `/Game/RTSMultiplayer/RTSCharacters/Blueprints/S_ArrayOfUnits` _value)))
    (bind _returnvalue_3 (`KismetArrayLibrary.Array_RemoveItem` _output_get Unit))
    (if (and _returnvalue_3 (!= (`KismetArrayLibrary.Array_Length` (`local.OldUnits`)) 0))
      (`BlueprintMapLibrary.Map_Add` (`self.AvailableUnits`) _returnvalue (make `/Game/RTSMultiplayer/RTSCharacters/Blueprints/S_ArrayOfUnits` (`local.OldUnits`))))))

(fn `SetAggressiveMode`
  (bind _availableunits (`self.AvailableUnits`))
  (bind _keys (`BlueprintMapLibrary.Map_Keys` _availableunits))
  (for _array_element _keys
    (bind _value (`BlueprintMapLibrary.Map_Find` _availableunits _array_element))
    (bind _returnvalue (`KismetArrayLibrary.Array_Length` (break `/Game/RTSMultiplayer/RTSCharacters/Blueprints/S_ArrayOfUnits` _value)))
    (bind _returnvalue_2 (`KismetMathLibrary.FTrunc` (* _returnvalue (`self.AggressiveModeUnitsAmountPercentage`))))
    (for _index (range (+ (select `bool` (<= _returnvalue_2 2) :`false` (- _returnvalue_2 1) :`true` (- _returnvalue 1)) 1))
      (bind _returnvalue_3 (`AIBlueprintHelperLibrary.GetBlackboard` (`AIBlueprintHelperLibrary.GetAIController` (`|GetArrayItem` (break `/Game/RTSMultiplayer/RTSCharacters/Blueprints/S_ArrayOfUnits` _value) _index))))
      (`BlackboardComponent.SetValueAsObject` _returnvalue_3 (`self.EnemyMainBuildingKey`) (`self.CurrentEnemyMainBuilding`))
      (`BlackboardComponent.SetValueAsBool` _returnvalue_3 (`self.AggressiveModeKey`) true))))

(fn `SpawnAndUseBuildingsAbility`
  (params (AbilityThunk :type "/Game/RTSMultiplayer/AISubsystem/Buildings/S_BuildingAbilityThunk Structure") (ThunkCondition :type "/Game/RTSMultiplayer/AISubsystem/ThunkConditions/ThunkCondition Object Reference") (Buildings :type "Array of /Game/RTSMultiplayer/BuildingSubsystem/Blueprints/BaseRTSBuilding Object Reference"))
  (returns (`Success?` :type Boolean))
  (locals (Result :type Boolean))
  (bind (_rtsbuildingclass _buildingabilityname _isrepeatable_ _firstneed _abilityinfo) (break `/Game/RTSMultiplayer/AISubsystem/Buildings/S_BuildingAbilityThunk` AbilityThunk))
  (bind _asbase_player_character (cast `/Game/RTSMultiplayer/RTSCharacters/Blueprints/BasePlayerCharacter` (`self.K2_GetPawn`) :!pure true))
  (for _array_element Buildings
    (if (`/Game/RTSMultiplayer/BuildingSubsystem/Blueprints/BaseRTSBuilding.WasBuilt?` _array_element)
      (`/Engine/EditorBlueprintResources/StandardMacros.IsValid` ThunkCondition
        (:`Is Valid`
          (bind _result (`/Game/RTSMultiplayer/AISubsystem/ThunkConditions/ThunkCondition.CheckCondition` ThunkCondition null _array_element))
          (if _result
            (if (== (`KismetArrayLibrary.Array_Length` (`/Game/RTSMultiplayer/TaskSubsystem/Blueprints/TaskComponent.TaskQueue` (`/Game/RTSMultiplayer/BuildingSubsystem/Blueprints/BaseRTSBuilding.TaskComponent` _array_element))) 0) :!label _label
              (if (`self.CheckForEnoughResources` _abilityinfo)
                (set `local.Result` true)
                (bind _returnvalue (`|SpawnActorFromClass` (`.Class_5_AD5F1DB1454BA05768809DBC81B23849` (break `/Game/RTSMultiplayer/AbilitySubsystem/Data/S_AbilityInfo` _abilityinfo)) (`KismetMathLibrary.MakeTransform` (0.0 0.0 0.0)) "AlwaysSpawn" "OverrideRootScale" _asbase_player_character _asbase_player_character))
                (`/Game/RTSMultiplayer/AbilitySubsystem/Blueprints/Ability.Use` _returnvalue (`|MakeArray` _array_element :!type "Actor Object Reference"))
                (`/Game/RTSMultiplayer/RTSCharacters/Blueprints/BasePlayerCharacter.AbilityUsed` _asbase_player_character _returnvalue)
                (if _isrepeatable_
                  (return true))))))
        (:`Is Not Valid`
          (goto _label)))))
  (return (`local.Result`)))

(fn `UserConstructionScript`)