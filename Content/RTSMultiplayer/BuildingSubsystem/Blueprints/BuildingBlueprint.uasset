(event `self.ReceiveBeginPlay`
  (bind _buldingmeshactor (`self.BuldingMeshActor`))
  (bind _childactor (`ChildActorComponent.ChildActor` _buldingmeshactor))
  ;[1 1 1] Setting up material instance on begin play.
  (`ChildActorComponent.SetChildActorClass` _buldingmeshactor (`self.BuildingMeshClass`))
  (bind _asbuilding_mesh (cast `/Game/RTSMultiplayer/BuildingSubsystem/Blueprints/BuildingMesh` _childactor))
  (bind _returnvalue (`KismetMaterialLibrary.CreateDynamicMaterialInstance` "/Game/RTSMultiplayer/BuildingSubsystem/Materials/M_Wireframe.M_Wireframe"))
  (`MaterialInstanceDynamic.SetVectorParameterValue` _returnvalue "GridColor" (`self.GoodSlopeMaterialColor`))
  (bind _output_get (set `self.WireframeMaterial` _returnvalue))
  (`/Game/RTSMultiplayer/BuildingSubsystem/Blueprints/BuildingMesh.SetMeshesMaterial` _asbuilding_mesh _output_get)
  (`self.SetActorEnableCollision` _childactor false))

(event `Build`
  (params (Class :type "/Game/RTSMultiplayer/BuildingSubsystem/Blueprints/BaseRTSBuilding Class Reference") (Instigator :type "Pawn Object Reference") (Squad :type "/Game/RTSMultiplayer/MovementSubsystem/Blueprints/Squad Object Reference") (`AddToQueue?` :type Boolean) (Faction :type "/Game/RTSMultiplayer/RTSCoreBP/E_Faction Enum" :default "NewEnumerator0"))
  ;[1 1 1] Build at the current location.
  (bind _returnvalue (`|SpawnActorFromClass` Class (`self.GetTransform`) "AlwaysSpawn" "OverrideRootScale" Instigator Faction false Instigator))
  (`/Game/RTSMultiplayer/MovementSubsystem/Blueprints/Squad.SetMoveAndActionTask` Squad Instigator "/Game/RTSMultiplayer/TaskSubsystem/Blueprints/Worker/RepairTask.RepairTask_C" (0.0 0.0 0.0) _returnvalue `AddToQueue?` null)
  (`self.K2_DestroyActor`))

(event `UpdatePositionAvailability`
  ;[1 1 1] Update position availability. Change material color.
  (if (`self.IsGoodPlace?`)
    (`self.SetGoodMaterial`)
    (else
      (`self.SetBadMaterial`))))

(event `SetBadMaterial`
  ;[1 1 1] Update position availability. Change material color.
  (`MaterialInstanceDynamic.SetVectorParameterValue` (`self.WireframeMaterial`) "GridColor" (`self.BadSlopeMaterialColor`)))

(event `SetGoodMaterial`
  ;[1 1 1] Update position availability. Change material color.
  (`MaterialInstanceDynamic.SetVectorParameterValue` (`self.WireframeMaterial`) "GridColor" (`self.GoodSlopeMaterialColor`)))

(fn `IsGoodPlace?`
  (returns (`IsGood?` :type Boolean))
  (locals (TracePoints :type "Array of Vector Structure"))
  ;[1 1 1] Check for actors collision.
  (bind _asbuilding_mesh (cast `/Game/RTSMultiplayer/BuildingSubsystem/Blueprints/BuildingMesh` (`ChildActorComponent.ChildActor` (`self.BuldingMeshActor`))))
  (bind _buildingblueprintcollision (`/Game/RTSMultiplayer/BuildingSubsystem/Blueprints/BuildingMesh.BuildingBlueprintCollision` _asbuilding_mesh))
  (bind _outcomponents (`KismetSystemLibrary.BoxOverlapComponents` (`SceneComponent.K2_GetComponentLocation` _buildingblueprintcollision) (`BoxComponent.GetScaledBoxExtent` _buildingblueprintcollision) (`|MakeArray` "ObjectTypeQuery1" "ObjectTypeQuery2" "ObjectTypeQuery3" :!type "EObjectTypeQuery Enum") null (`|MakeArray` _asbuilding_mesh :!type "Actor Object Reference")))
  (for _array_element _outcomponents
    (if (`ActorComponent.ComponentHasTag` _array_element "BuildingCollision")
      (return false)))
  ;[1 1 1] Check landscape slope.
  (bind _output_get (set `local.TracePoints` (`/Game/RTSMultiplayer/BuildingSubsystem/Blueprints/BuildingMesh.GetTracePointsForLandscapeCheck` _asbuilding_mesh)))
  (if (== (`KismetArrayLibrary.Array_Length` _output_get) 0)
    (return false)
    (else
      (for _array_element_2 (`local.TracePoints`)
        (bind (_outhit _returnvalue) (`KismetSystemLibrary.LineTraceSingle` :`Start` (`KismetMathLibrary.MakeVector` (.x _array_element_2) (.y _array_element_2) (+ (.z _array_element_2) 100.0)) :`End` (`KismetMathLibrary.MakeVector` (.x _array_element_2) (.y _array_element_2) (- (.z _array_element_2) 100.0)) :`TraceChannel` "TraceTypeQuery1" :`DrawTime` 0.5))
        (if _returnvalue
          (if (and (> (`KismetMathLibrary.Abs` (.x (`.Normal` (`GameplayStatics.BreakHitResult` _outhit)))) (`self.MaxBuildSlope`)) (> (`KismetMathLibrary.Abs` (.y (`.Normal` (`GameplayStatics.BreakHitResult` _outhit)))) (`self.MaxBuildSlope`)))
            (return false))
          (else
            (return false))))
      (return true))))

(fn `UserConstructionScript`)