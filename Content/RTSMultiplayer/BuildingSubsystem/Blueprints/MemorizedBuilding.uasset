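; MemorizedBuilding is a fog-of-war stand-in for a remembered building in the RTS, tied to an owning faction.
; Its construction script spawns the given building mesh class as a child actor with collision disabled.
; When a fog-affecting actor of the owning faction overlaps its RevealingBox, identified through the I_CanAffectFog interface, the stand-in destroys itself.
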(event `self.RevealingBox.OnComponentBeginOverlap`
  (params (OverlappedComponent :type "PrimitiveComponent Object Reference") (OtherActor :type "Actor Object Reference") (OtherComp :type "PrimitiveComponent Object Reference") (OtherBodyIndex :type Integer) (bFromSweep :type Boolean) (SweepResult :type "HitResult Structure (by ref)"))
  (bind _asi_can_affect_fog (cast `/Game/RTSMultiplayer/FogSubsystem/Blueprints/I_CanAffectFog` OtherActor))
  (bind _faction (`/Game/RTSMultiplayer/FogSubsystem/Blueprints/I_CanAffectFog.GetFactionAsFogAffectable` _asi_can_affect_fog))
  (if (`|EnumEquality` _faction (`self.OwnerFaction`))
    (`self.K2_DestroyActor`)))

(fn `UserConstructionScript`
  (bind _buildingmesh (`self.BuildingMesh`))
  (`ChildActorComponent.SetChildActorClass` _buildingmesh (`self.BuildingMeshClass`))
  (`self.SetActorEnableCollision` (`ChildActorComponent.ChildActor` _buildingmesh) false))