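; Building groundwork for an RTS that shows construction progress by progressively revealing tagged static meshes.
; On BeginPlay it fills a map of evenly spaced progress thresholds, all unreached, and reveals stage zero.
; Each progress update marks the first unreached threshold within the completion percentage and unhides meshes tagged with that BuildingStage number.
; Only one stage advances per update, and revealed meshes are never hidden again.
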(event `self.ReceiveBeginPlay`
  (`self.InitializeBuildingStages`)
  (`self.IncBuildingStage` 0))

(event `UpdateBuildingProcess`
  (params (CompletePercentage :type "Float (double-precision)"))
  (bind _buildingstages (`self.BuildingStages`))
  ;[1 1 1] Update building stages.
  (bind _keys (`BlueprintMapLibrary.Map_Keys` _buildingstages))
  (for (_array_element _array_index) _keys
    (if (and (not (`BlueprintMapLibrary.Map_Find` _buildingstages _array_element)) (<= _array_element CompletePercentage))
      (`BlueprintMapLibrary.Map_Add` (`self.BuildingStages`) _array_element true)
      (`self.IncBuildingStage` (+ _array_index 1))
      (break))))

(fn `IncBuildingStage`
  (params (NewStage :type Integer))
  (for _array_element (`self.GetComponentsByTag` "/Script/Engine.StaticMeshComponent" (`KismetStringLibrary.Conv_StringToName` (`KismetTextLibrary.Conv_TextToString` (`|FormatText` "BuildingStage{StageNumber}" NewStage))))
    (`SceneComponent.SetHiddenInGame` _array_element false false)))

(fn `InitializeBuildingStages`
  (locals (ProgressDelta :type "Float (double-precision)" :default 0.037))
  (for _index (range 1 26)
    (`BlueprintMapLibrary.Map_Add` (`self.BuildingStages`) (* _index (`local.ProgressDelta`)))))

(fn `UserConstructionScript`)