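; UnitSlot is a reservable position in the RTS building subsystem that a unit can target, exposing its world location.
; Its collision counts overlaps with BuildingCollision-tagged components, ignoring RTS unit actors, to detect a blocked position.
; TakeSlot marks it as targeted, and delegates bound to a task's completion or failure handle resetting that claim.
; IsFree reports true only when nothing blocks the slot and nobody targets it.
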(event `self.SlotCollision.OnComponentBeginOverlap`
  (params (OverlappedComponent :type "PrimitiveComponent Object Reference") (OtherActor :type "Actor Object Reference") (OtherComp :type "PrimitiveComponent Object Reference") (OtherBodyIndex :type Integer) (bFromSweep :type Boolean) (SweepResult :type "HitResult Structure (by ref)"))
  ;[1 1 1] Begin/end overlapping with any actor.
  (if (and (not (`KismetMathLibrary.ClassIsChildOf` (`GameplayStatics.GetObjectClass` OtherActor) "/Game/RTSMultiplayer/RTSCharacters/Blueprints/BaseRTSUnit.BaseRTSUnit_C")) (`ActorComponent.ComponentHasTag` OtherComp "BuildingCollision"))
    (`/Engine/EditorBlueprintResources/StandardMacros.IncrementInt` (`self.OverlappedActorsCount`))))

(event `self.SlotCollision.OnComponentEndOverlap`
  (params (OverlappedComponent :type "PrimitiveComponent Object Reference") (OtherActor :type "Actor Object Reference") (OtherComp :type "PrimitiveComponent Object Reference") (OtherBodyIndex :type Integer))
  ;[1 1 1] Begin/end overlapping with any actor.
  (if (and (not (`KismetMathLibrary.ClassIsChildOf` (`GameplayStatics.GetObjectClass` OtherActor) "/Game/RTSMultiplayer/RTSCharacters/Blueprints/BaseRTSUnit.BaseRTSUnit_C")) (`ActorComponent.ComponentHasTag` OtherComp "BuildingCollision"))
    (bind _result (`/Engine/EditorBlueprintResources/StandardMacros.DecrementInt` (`self.OverlappedActorsCount`))
      (:`  `
        (if (< _result 0)
          (set `self.OverlappedActorsCount` 0))))))

(event `ResetSomeoneTarget`
  (params (Task :type "/Game/RTSMultiplayer/TaskSubsystem/Blueprints/Task Object Reference"))
  ;[1 1 1] Taske/reset slot.
  (set `self.SomeoneTarget?` false)
  (`/Engine/EditorBlueprintResources/StandardMacros.IsValid` Task
    (:`Is Valid`
      (remove `/Game/RTSMultiplayer/TaskSubsystem/Blueprints/Task.TaskCompleted` Task (`|CreateDelegate` :!event `ResetSomeoneTarget`))
      (remove `/Game/RTSMultiplayer/TaskSubsystem/Blueprints/Task.TaskFailed` Task (`|CreateDelegate` :!event `ResetSomeoneTarget`)))))

(event `BindResetTarget`
  (params (CurrentTask :type "/Game/RTSMultiplayer/TaskSubsystem/Blueprints/Task Object Reference"))
  ;[1 1 1] Taske/reset slot.
  (add `/Game/RTSMultiplayer/TaskSubsystem/Blueprints/Task.TaskCompleted` CurrentTask (`|CreateDelegate` :!event `ResetSomeoneTarget`))
  (add `/Game/RTSMultiplayer/TaskSubsystem/Blueprints/Task.TaskFailed` CurrentTask (`|CreateDelegate` :!event `ResetSomeoneTarget`)))

(event `TakeSlot`
  ;[1 1 1] Taske/reset slot.
  (set `self.SomeoneTarget?` true))

(fn `GetLocation`
  (returns (Location :type "Vector Structure"))
  (return (`SceneComponent.K2_GetComponentLocation` (`self.SlotCollision`))))

(fn `IsFree?`
  (returns (IsFree :type Boolean))
  (return (and (== (`self.OverlappedActorsCount`) 0) (not (`self.SomeoneTarget?`)))))

(fn `UserConstructionScript`)