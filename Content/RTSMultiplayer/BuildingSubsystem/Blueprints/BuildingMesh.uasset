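; Base Blueprint for a building's visual mesh in the RTS building subsystem.
; SetMeshesMaterial applies one material to every slot of all static mesh components under the Meshes component, stopping at the first child that is not a static mesh.
; GetTracePointsForLandscapeCheck returns the world locations of the LandscapeTraces child components as points for a landscape check.
; The upgrade progress and completion events are empty stubs here.
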(event `SetMeshesMaterial`
  (params (NewMaterial :type "MaterialInstanceDynamic Object Reference"))
  (for _array_element (`SceneComponent.GetChildrenComponents` (`self.Meshes`) true)
    (bind _asstatic_mesh_component (cast `StaticMeshComponent` _array_element))
    (for _index (range (`PrimitiveComponent.GetNumMaterials` _asstatic_mesh_component))
      (`PrimitiveComponent.SetMaterial` _asstatic_mesh_component _index NewMaterial))))

(event `UpdateUpgradeProcess`
  (params (Percentage :type "Float (double-precision)")))

(event `EndUpgradeProcess`
  (params (UpgradeLevel :type Integer)))

(fn `GetTracePointsForLandscapeCheck`
  (returns (TracePoints :type "Array of Vector Structure"))
  (locals (Result :type "Array of Vector Structure"))
  (for _array_element (`SceneComponent.GetChildrenComponents` (`self.LandscapeTraces`) true)
    (`KismetArrayLibrary.Array_Add` (`local.Result`) (`SceneComponent.K2_GetComponentLocation` _array_element)))
  (return (`local.Result`)))

(fn `UserConstructionScript`)