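; Perk process for the RTS multiplayer perks system that completes once the owning player has streamed in its required resources.
; On start, it copies the per-type requirements, totals them and binds to the BasePlayerCharacter's streaming resource tick.
; Each tick deducts the gained amount; when every type is paid, it unbinds and multicasts completion.
; Progress derives from remaining versus required totals, and GetRemainingTime returns the remaining resource amount rather than a time.
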(event `CallProcessCompletedFromServer`
  ;[1 1 1] End process.
  (`self.CallProcessCompletedMulticast`))

(event `OnStreamingResourceTick`
  (params (ResourceType :type "/Game/RTSMultiplayer/ResourcesSubsystem/Blueprints/E_ResourceType Enum" :default "NewEnumerator0") (ResourceValue :type "Float (double-precision)"))
  (bind _accumulatedstreamingresources (`self.AccumulatedStreamingResources`))
  (bind (_value _returnvalue) (`BlueprintMapLibrary.Map_Find` (`self.AccumulatedStreamingResources`) ResourceType))
  (bind _returnvalue_2 (- _value ResourceValue))
  ;[1 1 1] Streaming resource gained.
  (if _returnvalue
    (set `self.RemainingStreamingResourcesAmount` (- (`self.RemainingStreamingResourcesAmount`) ResourceValue))
    (if (<= _returnvalue_2 0.0)
      (`BlueprintMapLibrary.Map_Remove` _accumulatedstreamingresources ResourceType)
      (if (== (`BlueprintMapLibrary.Map_Length` _accumulatedstreamingresources) 0)
        (bind _asbase_player_character (cast `/Game/RTSMultiplayer/RTSCharacters/Blueprints/BasePlayerCharacter` (`self.GetOwner`)))
        (remove `/Game/RTSMultiplayer/RTSCharacters/Blueprints/BasePlayerCharacter.StreamingResourceTick` _asbase_player_character (`|CreateDelegate` :!event `OnStreamingResourceTick`))
        (`self.CallProcessCompletedFromServer`))
      (else
        (`BlueprintMapLibrary.Map_Add` _accumulatedstreamingresources ResourceType _returnvalue_2)))))

(event `self.StartProcessMulticast`
  ;[1 1 1] Start process.
  (bind _asbase_player_character (cast `/Game/RTSMultiplayer/RTSCharacters/Blueprints/BasePlayerCharacter` (`self.GetOwner`)))
  (bind _output_get (set `self.AccumulatedStreamingResources` (`self.StreamingResources`)))
  (bind _keys (`BlueprintMapLibrary.Map_Keys` _output_get))
  (for _array_element _keys
    (set `self.NecessaryStreamingResourcesAmount` (+ (`self.NecessaryStreamingResourcesAmount`) (`BlueprintMapLibrary.Map_Find` (`self.AccumulatedStreamingResources`) _array_element))))
  (set `self.RemainingStreamingResourcesAmount` (`self.NecessaryStreamingResourcesAmount`))
  (add `/Game/RTSMultiplayer/RTSCharacters/Blueprints/BasePlayerCharacter.StreamingResourceTick` _asbase_player_character (`|CreateDelegate` :!event `OnStreamingResourceTick`)))

(fn `GetProcessPercentage`
  (returns (Percentage :type "Float (double-precision)"))
  (bind _necessarystreamingresourcesamount (`self.NecessaryStreamingResourcesAmount`))
  (return (/ (- _necessarystreamingresourcesamount (`self.RemainingStreamingResourcesAmount`)) _necessarystreamingresourcesamount)))

(fn `GetRemainingTime`
  (returns (RemainingTime :type "Float (double-precision)"))
  (return (`self.RemainingStreamingResourcesAmount`)))

(fn `InitializeAccumulatedResources`
  (bind _streamingresources (`self.StreamingResources`))
  (bind _keys (`BlueprintMapLibrary.Map_Keys` _streamingresources))
  (for _array_element _keys
    (`BlueprintMapLibrary.Map_Add` (`self.AccumulatedStreamingResources`) _array_element (`BlueprintMapLibrary.Map_Find` _streamingresources _array_element))))

(fn `UserConstructionScript`
  (`parent.UserConstructionScript`))