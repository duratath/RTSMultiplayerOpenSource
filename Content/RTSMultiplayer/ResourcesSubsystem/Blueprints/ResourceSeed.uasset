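; ResourceSeed is a harvestable RTS resource node that is destroyed when its resources run out.
; A StatsComponent holds remaining amount and capacity, while per-faction maps of collecting time and amount update through multicast events, with possible yield capped at what remains.
; Selection, outline and stats interfaces expose data-table name and icon, a fixed faction and an OutlineSelector built at BeginPlay.
; The construction script sizes or disables an optional building-collision box.
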(event `self.ReceiveBeginPlay`
  ;[1 1 1] Begin play.
  (add `self.ResourcesEnded` (`|CreateDelegate` :!event `OnResourcesEnded`))
  (bind _returnvalue (`|GetDataTableRow` "/Game/RTSMultiplayer/SelectionSubsystem/Data/SelectableActorsInfoDataTable.SelectableActorsInfoDataTable" (`self.ResourceId`))
    (:`then`
      (set `self.SelectableInfo` _returnvalue)
      (bind _returnvalue_2 (`|GenericCreateObject` "/Game/RTSMultiplayer/SelectionSubsystem/Blueprints/OutlineSelector.OutlineSelector_C" self (cast `/Game/RTSMultiplayer/SelectionSubsystem/Blueprints/I_CanBeOutlined` self :!pure true)))
      (set `self.AlienSelector` _returnvalue_2))
    (:`RowNotFound`
      (`KismetSystemLibrary.PrintString` "ResourceSeed: data table row not found." true true (struct :`R` 1.0 :`G` 0.038718 :`A` 1.0) 5.0))))

(event `ReduceRemainingResources`
  (params (ResourcesDelta :type "Float (double-precision)"))
  (bind _returnvalue (enumliteral `/Game/RTSMultiplayer/StatsSubsystem/Blueprints/E_Stat` "NewEnumerator0"))
  (bind _statscomponent (`self.StatsComponent`))
  ;[1 1 1] Reduce remaining resources. Change health.
  (`/Game/RTSMultiplayer/StatsSubsystem/Blueprints/StatsComponent.ChangeCurrentStatValue` _statscomponent _returnvalue (* -1 ResourcesDelta))
  (if (<= (break `/Game/RTSMultiplayer/StatsSubsystem/Blueprints/S_Stat` (`BlueprintMapLibrary.Map_Find` (`/Game/RTSMultiplayer/StatsSubsystem/Blueprints/StatsComponent.Stats` _statscomponent) _returnvalue)) 0.0)
    (`self.ResourcesEnded`)))

(event `ChangeCapacity`
  (params (CapacityDelta :type "Float (double-precision)"))
  ;[1 1 1] Change resource seed capacity.
  (`/Game/RTSMultiplayer/StatsSubsystem/Blueprints/StatsComponent.ChangeMaxStatValue` (`self.StatsComponent`) (enumliteral `/Game/RTSMultiplayer/StatsSubsystem/Blueprints/E_Stat` "NewEnumerator0") CapacityDelta))

(event `ChangeCollectingTime`
  (params (ForFaction :type "/Game/RTSMultiplayer/RTSCoreBP/E_Faction Enum" :default "NewEnumerator0") (NewValue :type "Float (double-precision)"))
  ;[1 1 1] Change collecting time/amount.
  (`self.ChangeCollectingTimeMulticast` ForFaction NewValue))

(event `ChangeCollectingTimeMulticast`
  (params (ForFaction :type "/Game/RTSMultiplayer/RTSCoreBP/E_Faction Enum (by ref)" :default "NewEnumerator0") (NewValue :type "Float (double-precision)"))
  ;[1 1 1] Change collecting time/amount.
  (`BlueprintMapLibrary.Map_Add` (`self.CollectingTime`) ForFaction NewValue))

(event `OnResourcesEnded`
  ;[1 1 1] On resources ended.
  (`self.K2_DestroyActor`))

(event `ChangeCollectingAmount`
  (params (ForFaction :type "/Game/RTSMultiplayer/RTSCoreBP/E_Faction Enum" :default "NewEnumerator0") (NewValue :type "Float (double-precision)"))
  ;[1 1 1] Change collecting time/amount.
  (`self.ChangeCollectingAmountMulticast` ForFaction NewValue))

(event `ChangeCollectingAmountMulticast`
  (params (ForFaction :type "/Game/RTSMultiplayer/RTSCoreBP/E_Faction Enum (by ref)" :default "NewEnumerator0") (NewValue :type "Float (double-precision)"))
  ;[1 1 1] Change collecting time/amount.
  (`BlueprintMapLibrary.Map_Add` (`self.CollectingAmount`) ForFaction NewValue))

(fn `GetAbilities`
  (returns (Abilities :type "Array of /Game/RTSMultiplayer/AbilitySubsystem/Data/S_AbilityInfo Structure"))
  (return))

(fn `GetAlienSelector`
  (returns (Selector :type "/Game/RTSMultiplayer/SelectionSubsystem/Blueprints/Selector Object Reference"))
  (return (`self.AlienSelector`)))

(fn `GetCharacterMovementComponent`
  (returns (MovementComponent :type "CharacterMovementComponent Object Reference"))
  (return null))

(fn `GetFactionAsCanBeOutlined`
  (returns (Faction :type "/Game/RTSMultiplayer/RTSCoreBP/E_Faction Enum"))
  (return (enumliteral `/Game/RTSMultiplayer/RTSCoreBP/E_Faction` "NewEnumerator2")))

(fn `GetFactionAsHaveStats`
  (returns (Faction :type "/Game/RTSMultiplayer/RTSCoreBP/E_Faction Enum"))
  (return "NewEnumerator2"))

(fn `GetFactionAsSelectable`
  (returns (Faction :type "/Game/RTSMultiplayer/RTSCoreBP/E_Faction Enum"))
  (return "NewEnumerator2"))

(fn `GetIcon`
  (returns (Icon :type "Texture2D Object Reference"))
  (bind _selectableinfo_icon (break `/Game/RTSMultiplayer/SelectionSubsystem/Data/S_SelectableActorInfo` (`self.SelectableInfo`)))
  (return _selectableinfo_icon))

(fn `GetIdAsHaveStats`
  (returns (Id :type Name))
  (return (`self.ResourceId`)))

(fn `GetMouseHoverResponsiveComponents`
  (returns (PrimitiveComponent :type "Array of PrimitiveComponent Object Reference"))
  (return (`|MakeArray` (`self.StaticMesh`) :!type "PrimitiveComponent Object Reference")))

(fn `GetName`
  (returns (Name :type Text))
  (bind (_selectableinfo_icon _selectableinfo_name) (break `/Game/RTSMultiplayer/SelectionSubsystem/Data/S_SelectableActorInfo` (`self.SelectableInfo`)))
  (return _selectableinfo_name))

(fn `GetOutlineComponent`
  (returns (OutlineComponent :type "/Game/RTSMultiplayer/SelectionSubsystem/Blueprints/OutlineComponent Object Reference"))
  (return (`self.OutlineComponent`)))

(fn `GetOutlineMeshes`
  (returns (OptionalSceneComponents :type "Array of SceneComponent Object Reference") (MeshComponents :type "Array of MeshComponent Object Reference"))
  (return _ (`|MakeArray` (`self.StaticMesh`) :!type "MeshComponent Object Reference")))

(fn `GetPossibleCollectingAmount`
  (params (ForFaction :type "/Game/RTSMultiplayer/RTSCoreBP/E_Faction Enum" :default "NewEnumerator0"))
  (returns (CollectingAmount :type "Float (double-precision)"))
  (bind _value (`BlueprintMapLibrary.Map_Find` (`self.CollectingAmount`) ForFaction))
  (bind _value_2 (`BlueprintMapLibrary.Map_Find` (`/Game/RTSMultiplayer/StatsSubsystem/Blueprints/StatsComponent.Stats` (`self.StatsComponent`)) (enumliteral `/Game/RTSMultiplayer/StatsSubsystem/Blueprints/E_Stat` "NewEnumerator0")))
  (return (select `bool` (> _value (break `/Game/RTSMultiplayer/StatsSubsystem/Blueprints/S_Stat` _value_2)) :`false` _value :`true` (break `/Game/RTSMultiplayer/StatsSubsystem/Blueprints/S_Stat` _value_2))))

(fn `GetQuickUseAbilityClass`
  (returns (AbilityClasses :type "Array of /Game/RTSMultiplayer/AbilitySubsystem/Blueprints/Ability Class Reference"))
  (return))

(fn `GetSelector`
  (returns (Selector :type "/Game/RTSMultiplayer/SelectionSubsystem/Blueprints/Selector Object Reference"))
  (return null))

(fn `GetStatsComponent`
  (returns (StatsComponent :type "/Game/RTSMultiplayer/StatsSubsystem/Blueprints/StatsComponent Object Reference"))
  (return (`self.StatsComponent`)))

(fn `HasResources?`
  (returns (`HasResources?` :type Boolean))
  (return (> (break `/Game/RTSMultiplayer/StatsSubsystem/Blueprints/S_Stat` (`BlueprintMapLibrary.Map_Find` (`/Game/RTSMultiplayer/StatsSubsystem/Blueprints/StatsComponent.Stats` (`self.StatsComponent`)) (enumliteral `/Game/RTSMultiplayer/StatsSubsystem/Blueprints/E_Stat` "NewEnumerator0"))) 0.0)))

(fn `UserConstructionScript`
  (bind _collisionbox (`self.CollisionBox`))
  (bind _collisionbox_2 (`self.CollisionBox`))
  (if (`self.EnableBuildingCollision?`)
    (`SceneComponent.SetWorldScale3D` _collisionbox (`self.CollisionScale`))
    (`SceneComponent.K2_SetRelativeLocation` _collisionbox (`self.CollisionLocation`) false false)
    (else
      (`PrimitiveComponent.SetCollisionEnabled` _collisionbox_2 "NoCollision")
      (`SceneComponent.SetVisibility` _collisionbox_2 false false))))