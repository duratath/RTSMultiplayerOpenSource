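; Actor component for an RTS unit inventory that collects, stacks, moves, swaps and drops item actors.
; Slots are a map of item arrays sized from the HUD inventory bar grid, with same-class stackable items sharing a slot.
; Requests forward to Multicast events that edit slots, hide or show items and broadcast changes.
; Collecting equips and dropping unequips, adding or reverting each item's max-stat deltas on the owner's stats component.
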(event `CallItemEquiped`
  (params (Item :type "/Game/RTSMultiplayer/InventorySubsystem/Blueprints/InventoryItem Object Reference"))
  ;[1 1 1] Call item equiped/unequiped.
  (`self.ItemEquiped` Item self))

(event `CollectItemMulticast`
  (params (Item :type "/Game/RTSMultiplayer/InventorySubsystem/Blueprints/InventoryItem Object Reference") (Slot :type Integer))
  ;[1 1 1] Collect new item.
  (`/Engine/EditorBlueprintResources/StandardMacros.IsValid` Item
    (:`Is Valid`
      (bind _success_ (`self.AddItemTo` Slot Item))
      (`Actor.SetActorEnableCollision` Item false)
      (`Actor.SetActorHiddenInGame` Item true)
      (`PrimitiveComponent.SetCollisionResponseToChannel` (`/Game/RTSMultiplayer/InventorySubsystem/Blueprints/InventoryItem.ItemCollisionBox` Item) "ECC_Visibility" "ECR_Block")
      (if _success_
        (`self.ItemEquiped` Item self)
        (`self.InventoryHasBeenChanged`)))))

(event `CallItemUnequiped`
  (params (Item :type "/Game/RTSMultiplayer/InventorySubsystem/Blueprints/InventoryItem Object Reference"))
  ;[1 1 1] Call item equiped/unequiped.
  (`self.ItemUnequiped` Item self))

(event `OnHUDAvailable`
  (params (SelectionEnvironment :type "/Game/RTSMultiplayer/SelectionSubsystem/Widgets/W_SelectionEnvironment Object Reference"))
  ;[1 1 1] Begin play, initialize inventory.
  (bind _asrtsplayer_controller (cast `/Game/RTSMultiplayer/RTSCharacters/Blueprints/RTSPlayerController` (`GameplayStatics.GetPlayerController` 0)))
  (bind _playerhud (`/Game/RTSMultiplayer/RTSCharacters/Blueprints/RTSPlayerController.PlayerHUD` _asrtsplayer_controller)
    (:`then`
      (bind _w_inventorybar (`/Game/RTSMultiplayer/RTSCoreUI/Widgets/W_PlayerHUD.W_InventoryBar` _playerhud)
        (:`then`
          (if (== (`BlueprintMapLibrary.Map_Length` (`self.Inventory`)) 0)
            (remove `/Game/RTSMultiplayer/RTSCharacters/Blueprints/RTSPlayerController.OnSelectionEnvironmentReset` _asrtsplayer_controller (`|CreateDelegate` :!event `OnHUDAvailable`))
            (for _index (range (* (`/Game/RTSMultiplayer/InventorySubsystem/Widgets/W_InventoryBar.ColumnsCount` _w_inventorybar) (`/Game/RTSMultiplayer/InventorySubsystem/Widgets/W_InventoryBar.RowsCount` _w_inventorybar)))
              (`BlueprintMapLibrary.Map_Add` (`self.Inventory`) _index (make `/Game/RTSMultiplayer/InventorySubsystem/Blueprints/S_ArrayOfInventoryItems` (`|MakeArray`))))))
        (:`else`)))
    (:`else`)))

(event `CollectItem`
  (params (ItemToCollect :type "/Game/RTSMultiplayer/InventorySubsystem/Blueprints/InventoryItem Object Reference") (PlayerController :type "/Game/RTSMultiplayer/RTSCharacters/Blueprints/RTSPlayerController Object Reference"))
  (bind _slotindex (`self.FindSuitableSlotForItem` ItemToCollect))
  ;[1 1 1] Collect new item.
  (if (!= _slotindex -1)
    (set `/Game/RTSMultiplayer/InventorySubsystem/Blueprints/InventoryItem.AbleToCollect?` false ItemToCollect)
    (`self.CollectItemMulticast` ItemToCollect _slotindex)
    (else
      (`/Game/RTSMultiplayer/RTSCharacters/Blueprints/RTSPlayerController.AddAttentionMessage` PlayerController "CANNOT_COLLECT_ITEM"))))

(event `self.ReceiveBeginPlay`
  ;[1 1 1] Begin play, initialize inventory.
  (bind _asrtsplayer_controller (cast `/Game/RTSMultiplayer/RTSCharacters/Blueprints/RTSPlayerController` (`GameplayStatics.GetPlayerController` 0)))
  (add `/Game/RTSMultiplayer/RTSCharacters/Blueprints/RTSPlayerController.OnSelectionEnvironmentReset` _asrtsplayer_controller (`|CreateDelegate` :!event `OnHUDAvailable`))
  (`self.OnHUDAvailable` null)
  (`self.BindChangeStatsEvent`))

(event `BindChangeStatsEvent`
  ;[1 1 1] Begin play, initialize inventory.
  (add `self.ItemEquiped` (`|CreateDelegate` :!event `ChangeStatsOnEquip`))
  (add `self.ItemUnequiped` (`|CreateDelegate` :!event `ChangeStatsOnUnequip`)))

(event `DropItemMulticast`
  (params (Item :type "/Game/RTSMultiplayer/InventorySubsystem/Blueprints/InventoryItem Object Reference"))
  ;[1 1 1] Drop item.
  (`Actor.SetActorEnableCollision` Item true)
  (`Actor.SetActorHiddenInGame` Item false)
  (`self.CallItemUnequiped` Item))

(event `DropItem`
  (params (InventoryItem :type "/Game/RTSMultiplayer/InventorySubsystem/Blueprints/InventoryItem Object Reference") (SlotIndex :type Integer) (DropLocation :type "Vector Structure"))
  (bind (_returnvalue_roll _returnvalue_pitch) (`KismetMathLibrary.BreakRotator` (`Actor.K2_GetActorRotation` InventoryItem)))
  ;[1 1 1] Drop item.
  (`self.DetachItemFromSlot` SlotIndex InventoryItem)
  (`Actor.K2_SetActorLocation` InventoryItem DropLocation false true)
  (`Actor.K2_SetActorRotation` InventoryItem (`KismetMathLibrary.MakeRotator` _returnvalue_roll _returnvalue_pitch (`KismetMathLibrary.RandomFloatInRange` 0.0 359.0)) true)
  (set `/Game/RTSMultiplayer/InventorySubsystem/Blueprints/InventoryItem.AbleToCollect?` true InventoryItem)
  (`self.DropItemMulticast` InventoryItem))

(event `DetachItemFromSlotMulticast`
  (params (SlotIndex :type Integer) (InventoryItem :type "/Game/RTSMultiplayer/InventorySubsystem/Blueprints/InventoryItem Object Reference"))
  ;[1 1 1] Inventory items management.
  (`self.RemoveItemFrom` SlotIndex InventoryItem)
  (`self.InventoryHasBeenChanged`))

(event `DetachItemFromSlot`
  (params (SlotIndex :type Integer) (InventoryItem :type "/Game/RTSMultiplayer/InventorySubsystem/Blueprints/InventoryItem Object Reference"))
  ;[1 1 1] Inventory items management.
  (`self.DetachItemFromSlotMulticast` SlotIndex InventoryItem))

(event `AttachItemToSlotMulticast`
  (params (SlotIndex :type Integer) (InventoryItem :type "/Game/RTSMultiplayer/InventorySubsystem/Blueprints/InventoryItem Object Reference"))
  ;[1 1 1] Inventory items management.
  (`self.AddItemTo` SlotIndex InventoryItem)
  (`self.InventoryHasBeenChanged`))

(event `AttachItemToSlot`
  (params (SlotIndex :type Integer) (InventoryItem :type "/Game/RTSMultiplayer/InventorySubsystem/Blueprints/InventoryItem Object Reference"))
  ;[1 1 1] Inventory items management.
  (`self.AttachItemToSlotMulticast` SlotIndex InventoryItem))

(event `ChangeStatsOnEquip` :!signature `self.ItemEquiped`
  (params (Item :type "/Game/RTSMultiplayer/InventorySubsystem/Blueprints/InventoryItem Object Reference") (InventoryComponent :type "/Game/RTSMultiplayer/InventorySubsystem/Blueprints/InventoryComponent Object Reference"))
  (bind ((`ItemClass_34_8F5AA4EE471466E843574DB3B3EB0514` _itemclass) (`OnEquipStatsDelta_31_6ADFA76E4326A1D0A751888DF69E3E9C` _onequipstatsdelta)) (break `/Game/RTSMultiplayer/InventorySubsystem/Data/S_InventoryItemInfo` (`/Game/RTSMultiplayer/InventorySubsystem/Blueprints/InventoryItem.ItemInfo` Item)))
  ;[1 1 1] Change stats on equip/unequip.
  (bind _asi_have_stats (cast `/Game/RTSMultiplayer/StatsSubsystem/Blueprints/I_HaveStats` (`self.GetOwner`)))
  (bind _statscomponent (`/Game/RTSMultiplayer/StatsSubsystem/Blueprints/I_HaveStats.GetStatsComponent` _asi_have_stats))
  (bind _keys (`BlueprintMapLibrary.Map_Keys` _onequipstatsdelta))
  (for _array_element _keys
    (`/Game/RTSMultiplayer/StatsSubsystem/Blueprints/StatsComponent.ChangeMaxStatValue` _statscomponent _array_element (`BlueprintMapLibrary.Map_Find` _onequipstatsdelta _array_element))))

(event `DetachAllItemsFromSlot`
  (params (SlotIndex :type Integer))
  ;[1 1 1] Inventory items management.
  (`self.DetachAllItemsFromSlotMulticast` SlotIndex))

(event `DetachAllItemsFromSlotMulticast`
  (params (SlotIndex :type Integer))
  (bind _inventory (`self.Inventory`))
  ;[1 1 1] Inventory items management.
  (`BlueprintMapLibrary.Map_Remove` _inventory SlotIndex)
  (`BlueprintMapLibrary.Map_Add` _inventory SlotIndex (make `/Game/RTSMultiplayer/InventorySubsystem/Blueprints/S_ArrayOfInventoryItems` (`|MakeArray`)))
  (`self.InventoryHasBeenChanged`))

(event `AttachAllItemsToSlot`
  (params (SlotIndex :type Integer) (Items :type "Array of /Game/RTSMultiplayer/InventorySubsystem/Blueprints/InventoryItem Object Reference"))
  ;[1 1 1] Inventory items management.
  (`self.AttachAllItemsToSlotMulticast` SlotIndex Items))

(event `AttachAllItemsToSlotMulticast`
  (params (SlotIndex :type Integer) (Items :type "Array of /Game/RTSMultiplayer/InventorySubsystem/Blueprints/InventoryItem Object Reference"))
  ;[1 1 1] Inventory items management.
  (`self.AddAllItemsTo` SlotIndex Items)
  (`self.InventoryHasBeenChanged`))

(event `ChangeStatsOnUnequip` :!signature `self.ItemUnequiped`
  (params (Item :type "/Game/RTSMultiplayer/InventorySubsystem/Blueprints/InventoryItem Object Reference") (InventoryComponent :type "/Game/RTSMultiplayer/InventorySubsystem/Blueprints/InventoryComponent Object Reference"))
  (bind ((`ItemClass_34_8F5AA4EE471466E843574DB3B3EB0514` _itemclass) (`OnEquipStatsDelta_31_6ADFA76E4326A1D0A751888DF69E3E9C` _onequipstatsdelta)) (break `/Game/RTSMultiplayer/InventorySubsystem/Data/S_InventoryItemInfo` (`/Game/RTSMultiplayer/InventorySubsystem/Blueprints/InventoryItem.ItemInfo` Item)))
  ;[1 1 1] Change stats on equip/unequip.
  (bind _asi_have_stats (cast `/Game/RTSMultiplayer/StatsSubsystem/Blueprints/I_HaveStats` (`self.GetOwner`)))
  (bind _statscomponent (`/Game/RTSMultiplayer/StatsSubsystem/Blueprints/I_HaveStats.GetStatsComponent` _asi_have_stats))
  (bind _keys (`BlueprintMapLibrary.Map_Keys` _onequipstatsdelta))
  (for _array_element _keys
    (`/Game/RTSMultiplayer/StatsSubsystem/Blueprints/StatsComponent.ChangeMaxStatValue` _statscomponent _array_element (* (`BlueprintMapLibrary.Map_Find` _onequipstatsdelta _array_element) -1.0))))

(event `SwapSlotsContent`
  (params (Slot1 :type Integer) (Slot2 :type Integer))
  ;[1 1 1] Inventory items management.
  (`self.SwapSlotsContentMulticast` Slot1 Slot2))

(event `SwapSlotsContentMulticast`
  (params (Slot1 :type Integer) (Slot2 :type Integer))
  ;[1 1 1] Inventory items management.
  (`self.SwapSlots` Slot1 Slot2)
  (`self.InventoryHasBeenChanged`))

(fn `AbleToDropAtLocation?`
  (params (Item :type "/Game/RTSMultiplayer/InventorySubsystem/Blueprints/InventoryItem Object Reference") (Location :type "Vector Structure"))
  (returns (`AbleToDrop?` :type Boolean))
  (bind _outcomponents (`KismetSystemLibrary.BoxOverlapComponents` Location (`BoxComponent.GetScaledBoxExtent` (`/Game/RTSMultiplayer/InventorySubsystem/Blueprints/InventoryItem.ItemCollisionBox` Item)) (`|MakeArray` "ObjectTypeQuery1" "ObjectTypeQuery2" "ObjectTypeQuery3" :!type "EObjectTypeQuery Enum") null (`|MakeArray` Item :!type "Actor Object Reference")))
  (for _array_element _outcomponents
    (if (`self.ComponentHasTag` _array_element "ItemCollision")
      (return false)))
  (return true))

(fn `AddAllItemsTo`
  (params (SlotIndex :type Integer) (Items :type "Array of /Game/RTSMultiplayer/InventorySubsystem/Blueprints/InventoryItem Object Reference"))
  (returns (`Success?` :type Boolean))
  (locals (SavedItems :type "Array of /Game/RTSMultiplayer/InventorySubsystem/Blueprints/InventoryItem Object Reference"))
  (bind _output (`|GetArrayItem` Items))
  (bind (_value _returnvalue) (`BlueprintMapLibrary.Map_Find` (`self.Inventory`) SlotIndex))
  (if _returnvalue
    (bind _output_get (set `local.SavedItems` (break `/Game/RTSMultiplayer/InventorySubsystem/Blueprints/S_ArrayOfInventoryItems` _value)))
    (if (> (`KismetArrayLibrary.Array_Length` _output_get) 0)
      (if (and (== (`GameplayStatics.GetObjectClass` (`|GetArrayItem` (`local.SavedItems`))) (`GameplayStatics.GetObjectClass` _output)) (`.IsStackable?_15_52AEF5B44590CC70FEA13BA716ADF761` (break `/Game/RTSMultiplayer/InventorySubsystem/Data/S_InventoryItemInfo` (`/Game/RTSMultiplayer/InventorySubsystem/Blueprints/InventoryItem.ItemInfo` _output))))
        (for _array_element Items
          (`KismetArrayLibrary.Array_Add` (`local.SavedItems`) _array_element))
        (`BlueprintMapLibrary.Map_Add` (`self.Inventory`) SlotIndex (make `/Game/RTSMultiplayer/InventorySubsystem/Blueprints/S_ArrayOfInventoryItems` (`local.SavedItems`)))
        (return true)
        (else
          (return false)))
      (else
        (`BlueprintMapLibrary.Map_Add` (`self.Inventory`) SlotIndex (make `/Game/RTSMultiplayer/InventorySubsystem/Blueprints/S_ArrayOfInventoryItems` Items))
        (return true)))
    (else
      (return false))))

(fn `AddItemTo`
  (params (SlotIndex :type Integer) (ItemToAdd :type "/Game/RTSMultiplayer/InventorySubsystem/Blueprints/InventoryItem Object Reference"))
  (returns (`Success?` :type Boolean))
  (locals (SavedItems :type "Array of /Game/RTSMultiplayer/InventorySubsystem/Blueprints/InventoryItem Object Reference"))
  (bind (_value _returnvalue) (`BlueprintMapLibrary.Map_Find` (`self.Inventory`) SlotIndex))
  (bind _items (break `/Game/RTSMultiplayer/InventorySubsystem/Blueprints/S_ArrayOfInventoryItems` _value))
  (if _returnvalue
    (if (> (`KismetArrayLibrary.Array_Length` _items) 0)
      (if (and (== (`GameplayStatics.GetObjectClass` ItemToAdd) (`GameplayStatics.GetObjectClass` (`|GetArrayItem` _items))) (`.IsStackable?_15_52AEF5B44590CC70FEA13BA716ADF761` (break `/Game/RTSMultiplayer/InventorySubsystem/Data/S_InventoryItemInfo` (`/Game/RTSMultiplayer/InventorySubsystem/Blueprints/InventoryItem.ItemInfo` ItemToAdd))))
        (bind _output_get (set `local.SavedItems` _items))
        (`KismetArrayLibrary.Array_Add` _output_get ItemToAdd)
        (`BlueprintMapLibrary.Map_Add` (`self.Inventory`) SlotIndex (make `/Game/RTSMultiplayer/InventorySubsystem/Blueprints/S_ArrayOfInventoryItems` (`local.SavedItems`)))
        (return true)
        (else
          (return false)))
      (else
        (`BlueprintMapLibrary.Map_Add` (`self.Inventory`) SlotIndex (make `/Game/RTSMultiplayer/InventorySubsystem/Blueprints/S_ArrayOfInventoryItems` (`|MakeArray` ItemToAdd)))
        (return true)))
    (else
      (return false))))

(fn `FindSuitableSlot`
  (params (S_InventoryItemInfo :type "/Game/RTSMultiplayer/InventorySubsystem/Data/S_InventoryItemInfo Structure (by ref)"))
  (returns (SlotIndex :type Integer))
  (locals (FreeSlot :type Integer :default -1))
  (bind ((`ItemClass_34_8F5AA4EE471466E843574DB3B3EB0514` _itemclass) (`ConsumableCost_26_B4B62B7546567E6FFDB323B3F3599370` _consumablecost) (`IsStackable?_15_52AEF5B44590CC70FEA13BA716ADF761` _isstackable_)) (break `/Game/RTSMultiplayer/InventorySubsystem/Data/S_InventoryItemInfo` S_InventoryItemInfo))
  (bind _keys (`BlueprintMapLibrary.Map_Keys` (`self.Inventory`)))
  (for _array_element _keys
    (bind _value (`BlueprintMapLibrary.Map_Find` (`self.Inventory`) _array_element))
    (if (> (`KismetArrayLibrary.Array_Length` (break `/Game/RTSMultiplayer/InventorySubsystem/Blueprints/S_ArrayOfInventoryItems` _value)) 0)
      (if (and _isstackable_ (== _itemclass (`GameplayStatics.GetObjectClass` (`|GetArrayItem` (break `/Game/RTSMultiplayer/InventorySubsystem/Blueprints/S_ArrayOfInventoryItems` _value)))))
        (return _array_element))
      (elif (== (`local.FreeSlot`) -1)
        (set `local.FreeSlot` _array_element))))
  (return (`local.FreeSlot`)))

(fn `FindSuitableSlotForItem`
  (params (NewItem :type "/Game/RTSMultiplayer/InventorySubsystem/Blueprints/InventoryItem Object Reference"))
  (returns (SlotIndex :type Integer))
  (locals (FreeSlot :type Integer :default -1))
  (bind _keys (`BlueprintMapLibrary.Map_Keys` (`self.Inventory`)))
  (for _array_element _keys
    (bind _value (`BlueprintMapLibrary.Map_Find` (`self.Inventory`) _array_element))
    (if (> (`KismetArrayLibrary.Array_Length` (break `/Game/RTSMultiplayer/InventorySubsystem/Blueprints/S_ArrayOfInventoryItems` _value)) 0)
      (if (and (`.IsStackable?_15_52AEF5B44590CC70FEA13BA716ADF761` (break `/Game/RTSMultiplayer/InventorySubsystem/Data/S_InventoryItemInfo` (`/Game/RTSMultiplayer/InventorySubsystem/Blueprints/InventoryItem.ItemInfo` NewItem))) (== (`GameplayStatics.GetObjectClass` NewItem) (`GameplayStatics.GetObjectClass` (`|GetArrayItem` (break `/Game/RTSMultiplayer/InventorySubsystem/Blueprints/S_ArrayOfInventoryItems` _value)))))
        (return _array_element))
      (elif (== (`local.FreeSlot`) -1)
        (set `local.FreeSlot` _array_element))))
  (return (`local.FreeSlot`)))

(fn `RemoveItemFrom`
  (params (Index :type Integer) (Item :type "/Game/RTSMultiplayer/InventorySubsystem/Blueprints/InventoryItem Object Reference"))
  (locals (SavedItems :type "Array of /Game/RTSMultiplayer/InventorySubsystem/Blueprints/InventoryItem Object Reference"))
  (bind (_value _returnvalue) (`BlueprintMapLibrary.Map_Find` (`self.Inventory`) Index))
  (if _returnvalue
    (bind _output_get (set `local.SavedItems` (break `/Game/RTSMultiplayer/InventorySubsystem/Blueprints/S_ArrayOfInventoryItems` _value)))
    (bind _returnvalue_2 (`KismetArrayLibrary.Array_RemoveItem` _output_get Item))
    (if _returnvalue_2
      (`BlueprintMapLibrary.Map_Add` (`self.Inventory`) Index (make `/Game/RTSMultiplayer/InventorySubsystem/Blueprints/S_ArrayOfInventoryItems` (`local.SavedItems`))))))

(fn `SwapSlots`
  (params (Slot1 :type Integer) (Slot2 :type Integer))
  (locals (Slot1Content :type "Array of /Game/RTSMultiplayer/InventorySubsystem/Blueprints/InventoryItem Object Reference") (Slot2Content :type "Array of /Game/RTSMultiplayer/InventorySubsystem/Blueprints/InventoryItem Object Reference"))
  (bind (_value _returnvalue) (`BlueprintMapLibrary.Map_Find` (`self.Inventory`) Slot2))
  (bind (_value_2 _returnvalue_2) (`BlueprintMapLibrary.Map_Find` (`self.Inventory`) Slot1))
  (if _returnvalue_2
    (set `local.Slot1Content` (break `/Game/RTSMultiplayer/InventorySubsystem/Blueprints/S_ArrayOfInventoryItems` _value_2))
    (if _returnvalue
      (set `local.Slot2Content` (break `/Game/RTSMultiplayer/InventorySubsystem/Blueprints/S_ArrayOfInventoryItems` _value))
      (`BlueprintMapLibrary.Map_Add` (`self.Inventory`) Slot2 (make `/Game/RTSMultiplayer/InventorySubsystem/Blueprints/S_ArrayOfInventoryItems` (`local.Slot1Content`)))
      (`BlueprintMapLibrary.Map_Add` (`self.Inventory`) Slot1 (make `/Game/RTSMultiplayer/InventorySubsystem/Blueprints/S_ArrayOfInventoryItems` (`local.Slot2Content`))))))