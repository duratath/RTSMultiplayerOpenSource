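; InventoryItem is a world item actor for the RTS inventory system, with an optional attached ability.
; BeginPlay loads item and ability info from data tables by ID.
; Cursor hover over the collision box starts a delayed timer that spawns a tooltip on the player HUD at the mouse, removed on exit.
; It implements fog-of-war and outline interfaces; fog hides the actor and ignores Visibility traces only while it is collectable.
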(event `self.ReceiveBeginPlay`
  ;[1 1 1] Begin play, read data table info.
  (bind _returnvalue (`|GetDataTableRow` "/Game/RTSMultiplayer/InventorySubsystem/Data/InventoryItemsDataTable.InventoryItemsDataTable" (`self.ItemId`))
    (:`then`
      (bind _output_get (set `self.ItemInfo` _returnvalue))
      (bind _returnvalue_2 (`|GetDataTableRow` "/Game/RTSMultiplayer/AbilitySubsystem/Data/AbilitiesDataTable.AbilitiesDataTable" (`.AttachedAbilityId_19_C8CD61CE47256311D7B85A903166611C` (break `/Game/RTSMultiplayer/InventorySubsystem/Data/S_InventoryItemInfo` _output_get)))
        (:`then`
          (set `self.HasAttachedAbility?` true)
          (set `self.AbilityInfo` _returnvalue_2))))
    (:`RowNotFound`
      (`KismetSystemLibrary.PrintString` "InventoryItem: data table row not found." true true (struct :`R` 1.0 :`G` 0.038718 :`A` 1.0) 5.0))))

(event `ShowTooltip`
  (bind _returnvalue (`GameplayStatics.GetPlayerController` 0))
  ;[1 1 1] Show/hide tooltip.
  (`KismetSystemLibrary.K2_ClearAndInvalidateTimerHandle` (`self.TooltipHandle`))
  (`self.ItemTooltip`
    (:`then`)
    (:`else`
      (bind _asrtsplayer_controller (cast `/Game/RTSMultiplayer/RTSCharacters/Blueprints/RTSPlayerController` _returnvalue))
      (bind _returnvalue_2 (`|CreateWidget` "/Game/RTSMultiplayer/InventorySubsystem/Widgets/W_ItemTooltip.W_ItemTooltip_C" _returnvalue (`self.ItemInfo`) (`self.AbilityInfo`) (`self.HasAttachedAbility?`)))
      (bind _output_get (set `self.ItemTooltip` _returnvalue_2))
      (bind _returnvalue_3 (`CanvasPanel.AddChildToCanvas` (`/Game/RTSMultiplayer/RTSCoreUI/Widgets/W_PlayerHUD.HUDCanvasPanel` (`/Game/RTSMultiplayer/RTSCharacters/Blueprints/RTSPlayerController.PlayerHUD` _asrtsplayer_controller)) _output_get))
      (`CanvasPanelSlot.SetAutoSize` _returnvalue_3 true)
      (`CanvasPanelSlot.SetZOrder` _returnvalue_3 5)
      (bind _returnvalue_4 (`WidgetLayoutLibrary.GetMousePositionOnViewport`))
      (`CanvasPanelSlot.SetPosition` _returnvalue_3 (+ _returnvalue_4 (10.0 10.0))))))

(event `self.ItemCollisionBox.OnBeginCursorOver`
  (params (TouchedComponent :type "PrimitiveComponent Object Reference"))
  ;[1 1 1] Show/hide tooltip.
  (bind _returnvalue (`KismetSystemLibrary.K2_SetTimerDelegate` (delegate `ShowTooltip`) (`self.TooltipDisplayLatency`)))
  (set `self.TooltipHandle` _returnvalue))

(event `self.ItemCollisionBox.OnEndCursorOver`
  (params (TouchedComponent :type "PrimitiveComponent Object Reference"))
  ;[1 1 1] Show/hide tooltip.
  (`KismetSystemLibrary.K2_ClearAndInvalidateTimerHandle` (`self.TooltipHandle`))
  (bind _itemtooltip (`self.ItemTooltip`)
    (:`then`
      (`Widget.RemoveFromParent` _itemtooltip)
      (set `self.ItemTooltip` null))
    (:`else`)))

(event `/Game/RTSMultiplayer/FogSubsystem/Blueprints/I_CanAffectFog.SetVisible`
  ;[1 1 1] I_CanAffectFog: set visible/invisible.
  (if (`self.AbleToCollect?`)
    (`self.SetActorHiddenInGame` false)
    (`PrimitiveComponent.SetCollisionResponseToChannel` (`self.ItemCollisionBox`) "ECC_Visibility" "ECR_Block"))
  (set `self.IsInFog?` false))

(event `/Game/RTSMultiplayer/FogSubsystem/Blueprints/I_CanAffectFog.SetInvisible`
  ;[1 1 1] I_CanAffectFog: set visible/invisible.
  (if (`self.AbleToCollect?`)
    (`self.SetActorHiddenInGame` true)
    (`PrimitiveComponent.SetCollisionResponseToChannel` (`self.ItemCollisionBox`) "ECC_Visibility" "ECR_Ignore"))
  (set `self.IsInFog?` true))

(fn `GetFactionAsCanBeOutlined`
  (returns (Faction :type "/Game/RTSMultiplayer/RTSCoreBP/E_Faction Enum"))
  (return "NewEnumerator2"))

(fn `GetFactionAsFogAffectable`
  (returns (Faction :type "/Game/RTSMultiplayer/RTSCoreBP/E_Faction Enum"))
  (return "NewEnumerator2"))

(fn `GetFogOfWarComponent`
  (returns (FogOfWarComponent :type "/Game/RTSMultiplayer/FogSubsystem/Blueprints/FogOfWarComponent Object Reference"))
  (return (`self.FogOfWarComponent`)))

(fn `GetFogRevealRadius`
  (returns (Radius :type "Float (double-precision)"))
  (return 0.0))

(fn `GetMouseHoverResponsiveComponents`
  (returns (PrimitiveComponent :type "Array of PrimitiveComponent Object Reference"))
  (return (`|MakeArray` (`self.ItemCollisionBox`) :!type "PrimitiveComponent Object Reference")))

(fn `GetOutlineComponent`
  (returns (OutlineComponent :type "/Game/RTSMultiplayer/SelectionSubsystem/Blueprints/OutlineComponent Object Reference"))
  (return (`self.OutlineComponent`)))

(fn `GetOutlineMeshes`
  (returns (OptionalSceneComponents :type "Array of SceneComponent Object Reference") (MeshComponents :type "Array of MeshComponent Object Reference"))
  (return (`|MakeArray` (`self.Meshes`))))

(fn `GetQuickUseAbilityClass`
  (returns (AbilityClasses :type "Array of /Game/RTSMultiplayer/AbilitySubsystem/Blueprints/Ability Class Reference") (AbilityClasses :type "Array of /Game/RTSMultiplayer/AbilitySubsystem/Blueprints/Ability Class Reference"))
  (return))

(fn `GetWorldLocation`
  (returns (WorldLocation :type "Vector Structure"))
  (return (`self.K2_GetActorLocation`)))

(fn `IsVisible?`
  (returns (Visible :type Boolean))
  (return (not (`self.IsInFog?`))))

(fn `UserConstructionScript`)