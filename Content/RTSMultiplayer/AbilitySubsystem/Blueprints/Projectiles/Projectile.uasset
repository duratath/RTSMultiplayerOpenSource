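; Homing ability projectile that chases a Target actor and delivers damage, healing and effects on impact.
; Tick turns it toward the target and rebuilds its velocity along that heading, scaled by VelocityMultiplier.
; Only overlap with the target's I_AbleToFight homing component counts as a hit, routing damage and healing through combat components.
; It spawns an end emitter when destroyed on hit, missing target, or target or caster EndPlay.
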(event `self.ReceiveTick`
  (params (DeltaSeconds :type "Float (single-precision)"))
  (bind (_returnvalue_roll _returnvalue_pitch _returnvalue_yaw) (`KismetMathLibrary.BreakRotator` (`self.K2_GetActorRotation`)))
  ;[1 1 1] Move and rotate projectile to the target.
  (`self.K2_SetActorRotation` (`KismetMathLibrary.FindLookAtRotation` (`self.K2_GetActorLocation`) (`self.K2_GetActorLocation` (`self.Target`))))
  (set `MovementComponent.Velocity` (* (`KismetMathLibrary.CreateVectorFromYawPitch` _returnvalue_yaw _returnvalue_pitch (`KismetMathLibrary.VSize` (`self.GetVelocity`))) (`self.VelocityMultiplier`)) (`self.ProjectileMovement`)))

(event `BindOnEndPlay`
  ;[1 1 1] Begin play. Set homing target component, bind on end play event.
  (add `self.OnEndPlay` (`self.Target`) (delegate `OnTargetEndPlay`))
  (add `self.OnEndPlay` (`self.Caster`) (delegate `OnTargetEndPlay`)))

(event `self.ReceiveBeginPlay`
  ;[1 1 1] Begin play. Set homing target component, bind on end play event.
  (bind _target (`self.Target`)
    (:`then`
      (bind _asi_able_to_fight (cast `/Game/RTSMultiplayer/CombatSubsystem/Blueprints/I_AbleToFight` _target)
        (:`then`
          (`/Game/RTSMultiplayer/CombatSubsystem/Blueprints/I_AbleToFight.GetHomingTargetComponent` _asi_able_to_fight)
          (`self.BindOnEndPlay`))
        (:`CastFailed`
          (`KismetSystemLibrary.PrintString` "Projectile: target must implement I_AbleToFight interface." true true (struct :`R` 1.0 :`G` 0.038718 :`A` 1.0) 5.0))))
    (:`else`
      (`self.DestroyProjectile`))))

(event `OnTargetEndPlay` :!signature `self.OnEndPlay`
  (params (Actor :type "Actor Object Reference") (EndPlayReason :type "EEndPlayReason Enum" :default "Destroyed"))
  ;[1 1 1] Begin play. Set homing target component, bind on end play event.
  (`self.DestroyProjectile`))

(event `DestroyProjectile`
  ;[1 1 1] Destroy projectile.
  (`self.SpawnPossibleOnEndEmitter`)
  (`self.K2_DestroyActor`))

(event `self.ProjectileCollision.OnComponentBeginOverlap`
  (params (OverlappedComponent :type "PrimitiveComponent Object Reference") (OtherActor :type "Actor Object Reference") (OtherComp :type "PrimitiveComponent Object Reference") (OtherBodyIndex :type Integer) (bFromSweep :type Boolean) (SweepResult :type "HitResult Structure (by ref)"))
  ;[1 1 1] On projectile overlap something.
  (bind _asi_able_to_fight (cast `/Game/RTSMultiplayer/CombatSubsystem/Blueprints/I_AbleToFight` (`self.Target`)))
  (bind _homingtargetcomponent (`/Game/RTSMultiplayer/CombatSubsystem/Blueprints/I_AbleToFight.GetHomingTargetComponent` _asi_able_to_fight))
  (if (== _homingtargetcomponent OtherComp)
    (`self.OnProjectileHitTarget`)
    (`self.DestroyProjectile`)))

(event `SpawnPossibleOnEndEmitter`
  ;[1 1 1] Spawn possible on end play emitter.
  (`GameplayStatics.SpawnEmitterAtLocation` (`self.OnEndPlayEmitter`) (`self.K2_GetActorLocation`)))

(event `ApplyPossibleEffects`
  ;[1 1 1] Apply possible effects.
  (for _array_element (`self.Effects`)
    (`/Game/RTSMultiplayer/EffectsSubsystem/Blueprints/SimpleEffect.Apply` _array_element)))

(event `OnProjectileHitTarget`
  ;[1 1 1] On projectile hit target.
  (`self.TryDealDamageAndHeal`)
  (`self.ApplyPossibleEffects`))

(event `TryDealDamageAndHeal`
  (bind _abilitycombatconstants_basedamage (break `/Game/RTSMultiplayer/AbilitySubsystem/Data/S_AbilityCombatConstants` (`self.AbilityCombatConstants`)))
  (bind (_abilitycombatconstants_basedamage_2 _abilitycombatconstants_basehealing _abilitycombatconstants_effectbaseduration _abilitycombatconstants_tickfrequency _abilitycombatconstants_tickdamage _abilitycombatconstants_tickhealing _abilitycombatconstants_damagetype) (break `/Game/RTSMultiplayer/AbilitySubsystem/Data/S_AbilityCombatConstants` (`self.AbilityCombatConstants`)))
  (bind (_abilitycombatconstants_basedamage_3 _abilitycombatconstants_basehealing_2) (break `/Game/RTSMultiplayer/AbilitySubsystem/Data/S_AbilityCombatConstants` (`self.AbilityCombatConstants`)))
  (bind (_abilitycombatconstants_basedamage_4 _abilitycombatconstants_basehealing_3) (break `/Game/RTSMultiplayer/AbilitySubsystem/Data/S_AbilityCombatConstants` (`self.AbilityCombatConstants`)))
  ;[1 1 1] Try deal damage and heal target if possible.
  (if (!= _abilitycombatconstants_basedamage 0.0)
    (bind _asi_able_to_fight (cast `/Game/RTSMultiplayer/CombatSubsystem/Blueprints/I_AbleToFight` (`self.Caster`))
      (:`then`
        (bind _combatcomponent (`/Game/RTSMultiplayer/CombatSubsystem/Blueprints/I_AbleToFight.GetCombatComponent` _asi_able_to_fight))
        (bind _asi_able_to_fight_2 (cast `/Game/RTSMultiplayer/CombatSubsystem/Blueprints/I_AbleToFight` (`self.Target`)))
        (bind _combatcomponent_2 (`/Game/RTSMultiplayer/CombatSubsystem/Blueprints/I_AbleToFight.GetCombatComponent` _asi_able_to_fight_2))
        (`/Game/RTSMultiplayer/CombatSubsystem/Blueprints/CombatComponent.ReceiveDamage` _combatcomponent_2 (make `/Game/RTSMultiplayer/CombatSubsystem/Blueprints/S_DamageInfo` _abilitycombatconstants_damagetype (`/Game/RTSMultiplayer/CombatSubsystem/Blueprints/CombatComponent.WeaponType` _combatcomponent) _abilitycombatconstants_basedamage_2))
        (if (!= _abilitycombatconstants_basehealing_3 0.0) :!label _label
          (bind _asi_able_to_fight_3 (cast `/Game/RTSMultiplayer/CombatSubsystem/Blueprints/I_AbleToFight` (`self.Target`))
            (:`then`
              (bind _combatcomponent_3 (`/Game/RTSMultiplayer/CombatSubsystem/Blueprints/I_AbleToFight.GetCombatComponent` _asi_able_to_fight_3))
              (`/Game/RTSMultiplayer/CombatSubsystem/Blueprints/CombatComponent.ReceiveHealing` _combatcomponent_3 _abilitycombatconstants_basehealing_2))
            (:`CastFailed`
              (`KismetSystemLibrary.PrintString` "Projectile: caster and caster must implement I_AbleToFight interface." true true (struct :`R` 1.0 :`G` 0.038718 :`A` 1.0) 5.0 :!label _label_2)))))
      (:`CastFailed`
        (goto _label_2)))
    (else
      (goto _label))))

(fn `UserConstructionScript`)