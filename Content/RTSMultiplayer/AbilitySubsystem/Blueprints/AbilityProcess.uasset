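; AbilityProcess is a timed, multicast ability process that tracks its spent resources and reports progress and remaining time.
; Initializing records resource costs and registers it with the instigator's ability component.
; Starting plays a timeline sized to ProcessTime, which signals completion when finished.
; Ending unregisters it, while aborting also refunds consumable, allocatable and stat resources (not streaming) and resets one-time-use abilities.
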(event `AbortProcessMulticast`
  ;[1 1 1] Abort process. Add spent resources.
  (`TimelineComponent.Stop` (`self.ProcessTimeline`))
  (bind _asi_have_abilities (cast `/Game/RTSMultiplayer/AbilitySubsystem/Blueprints/I_HaveAbilities` (`self.ProcessInstigator`)))
  (bind _abilitycomponent (`/Game/RTSMultiplayer/AbilitySubsystem/Blueprints/I_HaveAbilities.GetAbilityComponent` _asi_have_abilities))
  (`/Game/RTSMultiplayer/AbilitySubsystem/Blueprints/AbilityComponent.RemoveProcess` _abilitycomponent self)
  (`/Game/RTSMultiplayer/AbilitySubsystem/Blueprints/AbilityComponent.CallProcessRemoved` _abilitycomponent)
  (`self.ProcessAborted`))

(event `AbortProcess`
  ;[1 1 1] Abort process. Add spent resources.
  (`self.MakeAmendsClient`)
  (`self.AmendStatResources`)
  (`self.AbortProcessMulticast`))

(event `AmendStatResources`
  ;[1 1 1] Abort process. Add spent resources.
  (bind _keys (`BlueprintMapLibrary.Map_Keys` (`self.StatResources`)))
  (for _array_element _keys
    (bind _asi_have_stats (cast `/Game/RTSMultiplayer/StatsSubsystem/Blueprints/I_HaveStats` (`self.ProcessInstigator`))
      (:`then`
        (bind _statscomponent (`/Game/RTSMultiplayer/StatsSubsystem/Blueprints/I_HaveStats.GetStatsComponent` _asi_have_stats))
        (`/Game/RTSMultiplayer/StatsSubsystem/Blueprints/StatsComponent.ChangeCurrentStatValue` _statscomponent _array_element (`BlueprintMapLibrary.Map_Find` (`self.StatResources`) _array_element)))
      (:`CastFailed`
        (`KismetSystemLibrary.PrintString` "AbilityDelayProcess: instigator must implement I_HaveStats interface." true true (struct :`R` 1.0 :`G` 0.038718 :`A` 1.0) 5.0)))))

(event `MakeAmendsClient`
  (bind (_abilityinfo_class _abilityinfo_icon _abilityinfo_isserving_ _abilityinfo_isonetimeuse_) (break `/Game/RTSMultiplayer/AbilitySubsystem/Data/S_AbilityInfo` (`self.AbilityInfo`)))
  ;[1 1 1] Abort process. Add spent resources.
  (bind _asbase_player_character (cast `/Game/RTSMultiplayer/RTSCharacters/Blueprints/BasePlayerCharacter` (`GameplayStatics.GetPlayerCharacter` 0)))
  (bind _keys (`BlueprintMapLibrary.Map_Keys` (`self.ConsumableResources`)))
  (for _array_element _keys
    (`/Game/RTSMultiplayer/RTSCharacters/Blueprints/BasePlayerCharacter.AddConsumableResource` _asbase_player_character _array_element (`BlueprintMapLibrary.Map_Find` (`self.ConsumableResources`) _array_element)))
  (bind _keys_2 (`BlueprintMapLibrary.Map_Keys` (`self.AllocatableResources`)))
  (for _array_element_2 _keys_2
    (`/Game/RTSMultiplayer/RTSCharacters/Blueprints/BasePlayerCharacter.FreeAllocatedResource` _asbase_player_character _array_element_2 (`BlueprintMapLibrary.Map_Find` (`self.AllocatableResources`) _array_element_2)))
  (if _abilityinfo_isonetimeuse_
    (`/Game/RTSMultiplayer/RTSCharacters/Blueprints/BasePlayerCharacter.ResetUsedAbility` _asbase_player_character (`self.AbilityInfo`) (`GameplayStatics.GetObjectClass` (`self.ProcessInstigator`)))))

(event `Initialize`
  (params (ConsumableResources :type "Map of /Game/RTSMultiplayer/ResourcesSubsystem/Blueprints/E_ResourceType Enum to Float (double-precision)") (AllocatableResources :type "Map of /Game/RTSMultiplayer/ResourcesSubsystem/Blueprints/E_ResourceType Enum to Float (double-precision)") (StatResources :type "Map of /Game/RTSMultiplayer/StatsSubsystem/Blueprints/E_Stat Enum to Float (double-precision)") (StreamingResources :type "Map of /Game/RTSMultiplayer/ResourcesSubsystem/Blueprints/E_ResourceType Enum to Float (double-precision)"))
  ;[1 1 1] Initialize process.
  (bind _keys (`BlueprintMapLibrary.Map_Keys` ConsumableResources))
  (for _array_element _keys
    (`self.AddConsumableResource` _array_element (`BlueprintMapLibrary.Map_Find` ConsumableResources _array_element)))
  (bind _keys_2 (`BlueprintMapLibrary.Map_Keys` AllocatableResources))
  (for _array_element_2 _keys_2
    (`self.AddAllocatableResource` _array_element_2 (`BlueprintMapLibrary.Map_Find` AllocatableResources _array_element_2)))
  (bind _keys_3 (`BlueprintMapLibrary.Map_Keys` StatResources))
  (for _array_element_3 _keys_3
    (`self.AddStatResource` _array_element_3 (`BlueprintMapLibrary.Map_Find` StatResources _array_element_3)))
  (bind _keys_4 (`BlueprintMapLibrary.Map_Keys` StreamingResources))
  (for _array_element_4 _keys_4
    (`self.AddStreamingResource` _array_element_4 (`BlueprintMapLibrary.Map_Find` StreamingResources _array_element_4)))
  (`self.InitializeMulticast`))

(event `AddConsumableResource`
  (params (Key :type "/Game/RTSMultiplayer/ResourcesSubsystem/Blueprints/E_ResourceType Enum (by ref)") (Value :type "Float (double-precision) (by ref)"))
  ;[1 1 1] Add resources.
  (`BlueprintMapLibrary.Map_Add` (`self.ConsumableResources`) Key Value))

(event `AddAllocatableResource`
  (params (Key :type "/Game/RTSMultiplayer/ResourcesSubsystem/Blueprints/E_ResourceType Enum (by ref)") (Value :type "Float (double-precision) (by ref)"))
  ;[1 1 1] Add resources.
  (`BlueprintMapLibrary.Map_Add` (`self.AllocatableResources`) Key Value))

(event `AddStatResource`
  (params (Key :type "/Game/RTSMultiplayer/StatsSubsystem/Blueprints/E_Stat Enum (by ref)") (Value :type "Float (double-precision) (by ref)"))
  ;[1 1 1] Add resources.
  (`BlueprintMapLibrary.Map_Add` (`self.StatResources`) Key Value))

(event `AddStreamingResource`
  (params (Key :type "/Game/RTSMultiplayer/ResourcesSubsystem/Blueprints/E_ResourceType Enum (by ref)") (Value :type "Float (double-precision) (by ref)"))
  ;[1 1 1] Add resources.
  (`BlueprintMapLibrary.Map_Add` (`self.StreamingResources`) Key Value))

(event `InitializeMulticast`
  ;[1 1 1] Initialize process.
  (bind _asi_have_abilities (cast `/Game/RTSMultiplayer/AbilitySubsystem/Blueprints/I_HaveAbilities` (`self.ProcessInstigator`))
    (:`then`
      (bind _abilitycomponent (`/Game/RTSMultiplayer/AbilitySubsystem/Blueprints/I_HaveAbilities.GetAbilityComponent` _asi_have_abilities))
      (`/Game/RTSMultiplayer/AbilitySubsystem/Blueprints/AbilityComponent.AddProcess` _abilitycomponent self)
      (`/Game/RTSMultiplayer/AbilitySubsystem/Blueprints/AbilityComponent.CallProcessAdded` _abilitycomponent))
    (:`CastFailed`
      (`KismetSystemLibrary.PrintString` "AbilityDelayProcess: process instigator must implement I_HaveAbilities interface." true true (struct :`R` 1.0 :`G` 0.038718 :`A` 1.0) 5.0))))

(event `StartProcessMulticast`
  ;[1 1 1] Start process.
  (`TimelineComponent.SetTimelineLength` (`self.ProcessTimeline`) (`self.ProcessTime`))
  (`Timeline|ProcessTimeline` :!via `PlayFromStart`
    (:`Finished`
      (`self.CallProcessCompletedMulticast`))))

(event `CallProcessCompletedMulticast`
  ;[1 1 1] Start process.
  (`self.ProcessCompleted`))

(event `StartProcess`
  ;[1 1 1] Start process.
  (`self.StartProcessMulticast`))

(event `EndProcess`
  ;[1 1 1] End process.
  (`self.EndProcessMulticast`))

(event `EndProcessMulticast`
  ;[1 1 1] End process.
  (bind _asi_have_abilities (cast `/Game/RTSMultiplayer/AbilitySubsystem/Blueprints/I_HaveAbilities` (`self.ProcessInstigator`)))
  (bind _abilitycomponent (`/Game/RTSMultiplayer/AbilitySubsystem/Blueprints/I_HaveAbilities.GetAbilityComponent` _asi_have_abilities))
  (`/Game/RTSMultiplayer/AbilitySubsystem/Blueprints/AbilityComponent.RemoveProcess` _abilitycomponent self)
  (`/Game/RTSMultiplayer/AbilitySubsystem/Blueprints/AbilityComponent.CallProcessRemoved` _abilitycomponent))

(fn `GetProcessPercentage`
  (returns (Percentage :type "Float (double-precision)"))
  (return (/ (`TimelineComponent.GetPlaybackPosition` (`self.ProcessTimeline`)) (`self.ProcessTime`))))

(fn `GetRemainingTime`
  (returns (RemainingTime :type "Float (double-precision)"))
  (return (- (`self.ProcessTime`) (`TimelineComponent.GetPlaybackPosition` (`self.ProcessTimeline`)))))

(fn `UserConstructionScript`)