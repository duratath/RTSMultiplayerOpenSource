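; SellAbility is an RTS ability that sells the units it is used on and returns their resources to the player.
; For each unit implementing I_CanBeSold, it reads GetCost, adds back consumable resources and frees allocated ones on player character 0, then destroys the actor.
; Units without the interface only print an error, and the ability destroys itself once all units are processed.
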(event `self.Use`
  (params (Units :type "Array of Actor Object Reference (by ref)"))
  ;[1 1 1] Change player's resources amount. Destroy sold actors.
  (`parent.Use` Units)
  (for _array_element Units
    (bind _asi_can_be_sold (cast `/Game/RTSMultiplayer/AbilitySubsystem/Blueprints/I_CanBeSold` _array_element)
      (:`then`
        (bind (_consumableresources _allocatableresources) (`/Game/RTSMultiplayer/AbilitySubsystem/Blueprints/I_CanBeSold.GetCost` _asi_can_be_sold))
        (bind _keys (`BlueprintMapLibrary.Map_Keys` _consumableresources))
        (for _array_element_2 _keys
          (`/Game/RTSMultiplayer/RTSCharacters/Blueprints/BasePlayerCharacter.AddConsumableResource` (cast `/Game/RTSMultiplayer/RTSCharacters/Blueprints/BasePlayerCharacter` (`GameplayStatics.GetPlayerCharacter` 0) :!pure true) _array_element_2 (`BlueprintMapLibrary.Map_Find` _consumableresources _array_element_2)))
        (bind _keys_2 (`BlueprintMapLibrary.Map_Keys` _allocatableresources))
        (for _array_element_3 _keys_2
          (`/Game/RTSMultiplayer/RTSCharacters/Blueprints/BasePlayerCharacter.FreeAllocatedResource` (cast `/Game/RTSMultiplayer/RTSCharacters/Blueprints/BasePlayerCharacter` (`GameplayStatics.GetPlayerCharacter` 0) :!pure true) _array_element_3 (`BlueprintMapLibrary.Map_Find` _allocatableresources _array_element_3)))
        (`self.DestroySoldActor` _array_element))
      (:`CastFailed`
        (`KismetSystemLibrary.PrintString` "SellAbility: executor must implement I_CanBeSold interface." true true (struct :`R` 1.0 :`G` 0.038718 :`A` 1.0) 5.0))))
  (`self.DestroyAbility`))

(event `DestroySoldActor`
  (params (Actor :type "Actor Object Reference"))
  ;[1 1 1] Change player's resources amount. Destroy sold actors.
  (`self.K2_DestroyActor` Actor))

(fn `UserConstructionScript`
  (`parent.UserConstructionScript`))