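; RTS targeted ability that orders the selected units to attack the chosen actor.
; It accepts targets with combat and stats interfaces and the required faction relationship to the local player, otherwise showing an attention message.
; Each unit's task component receives an AttackBuildingTask for buildings when its weapon type matches, or a standard AttackTask otherwise.
; Tasks replace the current one or queue via modifier, then the ability destroys itself.
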(event `self.OnTargetChosen`
  (params (HitResult :type "HitResult Structure"))
  (bind (_bblockinghit _binitialoverlap _time _distance _location _impactpoint _normal _impactnormal _physmat _hitactor) (`GameplayStatics.BreakHitResult` HitResult))
  (bind _asrtsplayer_controller (cast `/Game/RTSMultiplayer/RTSCharacters/Blueprints/RTSPlayerController` (`GameplayStatics.GetPlayerController` 0) :!pure true))
  ;[1 1 1] On target chosen. Target must implement I_AbleToFight and I_HaveStats interfaces.
  (bind _asi_able_to_fight (cast `/Game/RTSMultiplayer/CombatSubsystem/Blueprints/I_AbleToFight` _hitactor)
    (:`then`
      (cast `/Game/RTSMultiplayer/StatsSubsystem/Blueprints/I_HaveStats` _hitactor
        (:`then`
          (bind _faction (`/Game/RTSMultiplayer/CombatSubsystem/Blueprints/I_AbleToFight.GetFactionAsAbleToFight` _asi_able_to_fight))
          (if (`|EnumEquality` (`/Game/RTSMultiplayer/RTSCharacters/Blueprints/BasePlayerCharacter.GetRelationships` (cast `/Game/RTSMultiplayer/RTSCharacters/Blueprints/BasePlayerCharacter` (`GameplayStatics.GetPlayerCharacter` 0) :!pure true) _faction) "NewEnumerator1")
            (`parent.OnTargetChosen` HitResult)
            (`self.SpawnAttackTask` _hitactor _asrtsplayer_controller)
            (`self.DestroyAbility`)
            (else
              (`/Game/RTSMultiplayer/RTSCharacters/Blueprints/RTSPlayerController.AddAttentionMessage` _asrtsplayer_controller "CANT_ATTACK_TARGET" :!label _label))))
        (:`CastFailed`
          (goto _label))))
    (:`CastFailed`
      (goto _label))))

(event `SpawnAttackTask`
  (params (ActorToAttack :type "Actor Object Reference") (PlayerController :type "/Game/RTSMultiplayer/RTSCharacters/Blueprints/RTSPlayerController Object Reference"))
  (bind (_chosentargethitresult_bblockinghit _chosentargethitresult_binitialoverlap _chosentargethitresult_time _chosentargethitresult_distance _chosentargethitresult_location) (`GameplayStatics.BreakHitResult` (`self.ChosenTargetHitResult`)))
  (bind (_chosentargethitresult_bblockinghit_2 _chosentargethitresult_binitialoverlap_2 _chosentargethitresult_time_2 _chosentargethitresult_distance_2 _chosentargethitresult_location_2 _chosentargethitresult_impactpoint _chosentargethitresult_normal _chosentargethitresult_impactnormal _chosentargethitresult_physmat _chosentargethitresult_hitactor) (`GameplayStatics.BreakHitResult` (`self.ChosenTargetHitResult`)))
  (bind ((`Class_5_AD5F1DB1454BA05768809DBC81B23849` _class) (`StreamingCost_56_46CD57F148A7D646CB494DA55173A248` _streamingcost) (`Cooldown_45_24031EA94123C5EE818405B9344E59F6` _cooldown)) (break `/Game/RTSMultiplayer/AbilitySubsystem/Data/S_AbilityInfo` (`self.AbilityInfo`)))
  (bind ((`Class_5_AD5F1DB1454BA05768809DBC81B23849` _class_2) (`StreamingCost_56_46CD57F148A7D646CB494DA55173A248` _streamingcost_2) (`Cooldown_45_24031EA94123C5EE818405B9344E59F6` _cooldown_2)) (break `/Game/RTSMultiplayer/AbilitySubsystem/Data/S_AbilityInfo` (`self.AbilityInfo`)))
  ;[1 1 1] Spawn attack task depends on target.
  (for _array_element (`self.SelectedUnits`)
    (bind _asi_task_executor (cast `/Game/RTSMultiplayer/TaskSubsystem/Blueprints/I_TaskExecutor` _array_element)
      (:`then`
        (bind _taskcomponent (`/Game/RTSMultiplayer/TaskSubsystem/Blueprints/I_TaskExecutor.GetTaskComponent` _asi_task_executor))
        (bind _asbase_rtsbuilding (cast `/Game/RTSMultiplayer/BuildingSubsystem/Blueprints/BaseRTSBuilding` ActorToAttack)
          (:`then`
            (bind _combatcomponent (`/Game/RTSMultiplayer/CombatSubsystem/Blueprints/I_AbleToFight.GetCombatComponent` (cast `/Game/RTSMultiplayer/CombatSubsystem/Blueprints/I_AbleToFight` _array_element :!pure true)))
            (if (`|EnumEquality` (`/Game/RTSMultiplayer/CombatSubsystem/Blueprints/CombatComponent.WeaponType` _combatcomponent) "NewEnumerator0")
              (bind _returnvalue (`|GenericCreateObject` "/Game/RTSMultiplayer/TaskSubsystem/Blueprints/General/AttackBuildingTask.AttackBuildingTask_C" (`self.GetOwner`) (`Controller.K2_GetPawn` PlayerController) (0.0 0.0 0.0) _asbase_rtsbuilding PlayerController _class _cooldown 0.0 _chosentargethitresult_location))
              (if (`self.QueueTaskModifierDown`)
                (`/Game/RTSMultiplayer/TaskSubsystem/Blueprints/TaskComponent.AddTaskToQueue` _taskcomponent _returnvalue)
                (else
                  (`/Game/RTSMultiplayer/TaskSubsystem/Blueprints/TaskComponent.SetCurrentTask` _taskcomponent _returnvalue)))
              (else
                (bind _returnvalue_2 (`|GenericCreateObject` "/Game/RTSMultiplayer/TaskSubsystem/Blueprints/General/AttackTask.AttackTask_C" (`self.GetOwner`) ActorToAttack PlayerController _class_2 _cooldown_2 0.0 (`self.K2_GetActorLocation` _chosentargethitresult_hitactor) :!label _label_2))
                (if (`self.QueueTaskModifierDown`)
                  (`/Game/RTSMultiplayer/TaskSubsystem/Blueprints/TaskComponent.AddTaskToQueue` _taskcomponent _returnvalue_2)
                  (else
                    (`/Game/RTSMultiplayer/TaskSubsystem/Blueprints/TaskComponent.SetCurrentTask` _taskcomponent _returnvalue_2))))))
          (:`CastFailed`
            (goto _label_2))))
      (:`CastFailed`
        (`KismetSystemLibrary.PrintString` "AttackAbility: actors should implement I_TaskExecutor interface." true true (struct :`R` 1.0 :`G` 0.092183 :`A` 1.0) 3.0)))))

(fn `UserConstructionScript`
  (`parent.UserConstructionScript`))