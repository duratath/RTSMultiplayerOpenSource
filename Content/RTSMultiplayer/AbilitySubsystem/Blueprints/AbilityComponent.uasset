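; Actor component that manages an RTS actor's abilities, ability processes and cooldowns.
; BeginPlay fills abilities from data tables by owner ID, skipping those player 0's character already used.
; Owner task-queue events drive cooldowns: queueing spawns an AbilityCooldown actor mapped by class, completion starts it, and removal clears it.
; Ability and cooldown changes route through Multicast-named events, most firing notifications, with queries for cooldown state and remaining time.
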(event `SpawnCooldownActorMulticast`
  (params (AbilityClass :type "/Game/RTSMultiplayer/AbilitySubsystem/Blueprints/Ability Class Reference (by ref)") (CooldownLength :type "Float (double-precision)"))
  ;[1 1 1] Start/finish ability cooldown.
  (bind _returnvalue (`|SpawnActorFromClass` "/Game/RTSMultiplayer/AbilitySubsystem/Blueprints/AbilityCooldown.AbilityCooldown_C" (`KismetMathLibrary.MakeTransform` (0.0 0.0 0.0)) "AlwaysSpawn" "OverrideRootScale" (`self.GetOwner`) CooldownLength AbilityClass (`GameplayStatics.GetPlayerPawn` 0)))
  (`BlueprintMapLibrary.Map_Add` (`self.AbilitiesCooldowns`) AbilityClass _returnvalue)
  (add `/Game/RTSMultiplayer/AbilitySubsystem/Blueprints/AbilityCooldown.CooldownFinished` _returnvalue (`|CreateDelegate` :!event `OnCooldownFinished`))
  (`self.CooldownStarted` AbilityClass))

(event `SpawnCooldownActor`
  (params (AbilityClass :type "/Game/RTSMultiplayer/AbilitySubsystem/Blueprints/Ability Class Reference") (CooldownLength :type "Float (double-precision)"))
  ;[1 1 1] Start/finish ability cooldown.
  (`self.SpawnCooldownActorMulticast` AbilityClass CooldownLength))

(event `OnCooldownFinishedMulticast`
  (params (AbilityClass :type "/Game/RTSMultiplayer/AbilitySubsystem/Blueprints/Ability Class Reference (by ref)"))
  ;[1 1 1] Start/finish ability cooldown.
  (`BlueprintMapLibrary.Map_Remove` (`self.AbilitiesCooldowns`) AbilityClass)
  (`self.CooldownFinished` AbilityClass))

(event `OnCurrentTaskCompleted`
  (params (Task :type "/Game/RTSMultiplayer/TaskSubsystem/Blueprints/Task Object Reference"))
  ;[1 1 1] On current task completed/task added to queue/task removed from queue.
  (`/Engine/EditorBlueprintResources/StandardMacros.IsValid` Task
    (:`Is Valid`
      (if (!= (`/Game/RTSMultiplayer/TaskSubsystem/Blueprints/Task.InstigatorAbilityCooldown` Task) 0.0)
        (`self.StartCooldown` (`/Game/RTSMultiplayer/TaskSubsystem/Blueprints/Task.InstigatorAbilityClass` Task))))))

(event `StartCooldown`
  (params (AbilityClass :type "/Game/RTSMultiplayer/AbilitySubsystem/Blueprints/Ability Class Reference"))
  ;[1 1 1] Start/finish ability cooldown.
  (`self.StartCooldownMulticast` AbilityClass))

(event `OnCooldownFinished`
  (params (AbilityCooldown :type "/Game/RTSMultiplayer/AbilitySubsystem/Blueprints/AbilityCooldown Object Reference"))
  (bind _abilityclass (`/Game/RTSMultiplayer/AbilitySubsystem/Blueprints/AbilityCooldown.AbilityClass` AbilityCooldown))
  ;[1 1 1] Start/finish ability cooldown.
  (`BlueprintMapLibrary.Map_Remove` (`self.AbilitiesCooldowns`) _abilityclass)
  (`self.CooldownFinished` _abilityclass))

(event `OnTaskAddedToQueue`
  (params (Task :type "/Game/RTSMultiplayer/TaskSubsystem/Blueprints/Task Object Reference"))
  (bind _instigatorabilitycooldown (`/Game/RTSMultiplayer/TaskSubsystem/Blueprints/Task.InstigatorAbilityCooldown` Task))
  ;[1 1 1] On current task completed/task added to queue/task removed from queue.
  (`/Engine/EditorBlueprintResources/StandardMacros.IsValid` Task
    (:`Is Valid`
      (if (!= _instigatorabilitycooldown 0.0)
        (`self.SpawnCooldownActor` (`/Game/RTSMultiplayer/TaskSubsystem/Blueprints/Task.InstigatorAbilityClass` Task) _instigatorabilitycooldown)))))

(event `StartCooldownMulticast`
  (params (AbilityClass :type "/Game/RTSMultiplayer/AbilitySubsystem/Blueprints/Ability Class Reference (by ref)"))
  (bind (_value _returnvalue) (`BlueprintMapLibrary.Map_Find` (`self.AbilitiesCooldowns`) AbilityClass))
  ;[1 1 1] Start/finish ability cooldown.
  (if _returnvalue
    (`/Game/RTSMultiplayer/AbilitySubsystem/Blueprints/AbilityCooldown.StartCooldown` _value)))

(event `ResetAbilityCooldown`
  (params (AbilityClass :type "/Game/RTSMultiplayer/AbilitySubsystem/Blueprints/Ability Class Reference"))
  ;[1 1 1] Start/finish ability cooldown.
  (`self.OnCooldownFinishedMulticast` AbilityClass))

(event `OnTaskRemovedFromQueue`
  (params (Task :type "/Game/RTSMultiplayer/TaskSubsystem/Blueprints/Task Object Reference"))
  ;[1 1 1] On current task completed/task added to queue/task removed from queue.
  (`/Engine/EditorBlueprintResources/StandardMacros.IsValid` Task
    (:`Is Valid`
      (if (!= (`/Game/RTSMultiplayer/TaskSubsystem/Blueprints/Task.InstigatorAbilityCooldown` Task) 0.0)
        (`self.ResetAbilityCooldown` (`/Game/RTSMultiplayer/TaskSubsystem/Blueprints/Task.InstigatorAbilityClass` Task))))))

(event `self.ReceiveBeginPlay`
  (bind _returnvalue (`self.GetOwner`))
  ;[1 1 1] Begin play. Load data from abilities data table.
  (bind _asi_task_executor (cast `/Game/RTSMultiplayer/TaskSubsystem/Blueprints/I_TaskExecutor` _returnvalue)
    (:`then`
      (bind _taskcomponent (`/Game/RTSMultiplayer/TaskSubsystem/Blueprints/I_TaskExecutor.GetTaskComponent` _asi_task_executor))
      (add `/Game/RTSMultiplayer/TaskSubsystem/Blueprints/TaskComponent.CurrentTaskCompleted` _taskcomponent (`|CreateDelegate` :!event `OnCurrentTaskCompleted`))
      (add `/Game/RTSMultiplayer/TaskSubsystem/Blueprints/TaskComponent.TaskAddedToQueue` _taskcomponent (`|CreateDelegate` :!event `OnTaskAddedToQueue`))
      (add `/Game/RTSMultiplayer/TaskSubsystem/Blueprints/TaskComponent.TaskRemovedFromQueue` _taskcomponent (`|CreateDelegate` :!event `OnTaskRemovedFromQueue`)))
    (:`CastFailed`
      (`KismetSystemLibrary.PrintString` "AbilityComponent: owner don't implement I_HaveAbilities interface. Ability cooldowns will not work properly." true true (struct :`R` 1.0 :`G` 0.038718 :`A` 1.0) 5.0)))
  (bind _asi_have_abilities (cast `/Game/RTSMultiplayer/AbilitySubsystem/Blueprints/I_HaveAbilities` _returnvalue)
    (:`then`
      (bind _id (`/Game/RTSMultiplayer/AbilitySubsystem/Blueprints/I_HaveAbilities.GetIdAsHaveAbilities` _asi_have_abilities))
      (bind _returnvalue_2 (`|GetDataTableRow` "/Game/RTSMultiplayer/AbilitySubsystem/Data/ActorsAbilitiesDataTable.ActorsAbilitiesDataTable" _id)
        (:`then`
          (for _array_element (break `/Game/RTSMultiplayer/AbilitySubsystem/Data/S_ArrayOfNames` _returnvalue_2)
            (bind _returnvalue_3 (`|GetDataTableRow` "/Game/RTSMultiplayer/AbilitySubsystem/Data/AbilitiesDataTable.AbilitiesDataTable" _array_element)
              (:`then`
                (if (not (`/Game/RTSMultiplayer/RTSCharacters/Blueprints/BasePlayerCharacter.WasAbilityUsed?` (cast `/Game/RTSMultiplayer/RTSCharacters/Blueprints/BasePlayerCharacter` (`GameplayStatics.GetPlayerCharacter` 0) :!pure true) (`.Class_5_AD5F1DB1454BA05768809DBC81B23849` (break `/Game/RTSMultiplayer/AbilitySubsystem/Data/S_AbilityInfo` _returnvalue_3))))
                  (`KismetArrayLibrary.Array_Add` (`self.Abilities`) _returnvalue_3)))
              (:`RowNotFound`
                (`KismetSystemLibrary.PrintString` "AbilityComponent: abilities data table row not found." true true (struct :`R` 1.0 :`G` 0.038718 :`A` 1.0) 5.0)))))
        (:`RowNotFound`
          (`KismetSystemLibrary.PrintString` "AbilityComponent: actors abilities data table row not found." true true (struct :`R` 1.0 :`G` 0.038718 :`A` 1.0) 5.0))))
    (:`CastFailed`
      (`KismetSystemLibrary.PrintString` "AbilityComponent: owner must implement I_HaveAbilities interface." true true (struct :`R` 1.0 :`G` 0.038718 :`A` 1.0) 5.0))))

(event `AddProcess`
  (params (NewRecruitingProcess :type "/Game/RTSMultiplayer/AbilitySubsystem/Blueprints/AbilityProcess Object Reference"))
  ;[1 1 1] Add/remove ability process.
  (`KismetArrayLibrary.Array_Add` (`self.AbilityProcesses`) NewRecruitingProcess))

(event `RemoveAbility`
  (params (AbilityClass :type "/Game/RTSMultiplayer/AbilitySubsystem/Blueprints/Ability Class Reference"))
  ;[1 1 1] Remove and ability.
  (for (_array_element _array_index) (`self.Abilities`)
    (if (== (break `/Game/RTSMultiplayer/AbilitySubsystem/Data/S_AbilityInfo` _array_element) AbilityClass)
      (`self.RemoveAbilityMulticast` _array_index)
      (break))))

(event `RemoveProcess`
  (params (ToRemove :type "/Game/RTSMultiplayer/AbilitySubsystem/Blueprints/AbilityProcess Object Reference"))
  ;[1 1 1] Add/remove ability process.
  (`KismetArrayLibrary.Array_RemoveItem` (`self.AbilityProcesses`) ToRemove))

(event `RemoveAbilityMulticast`
  (params (IndexToRemove :type Integer))
  ;[1 1 1] Remove and ability.
  (`KismetArrayLibrary.Array_Remove` (`self.Abilities`) IndexToRemove)
  (`self.AbilityRemoved`))

(event `CallProcessAdded`
  ;[1 1 1] Add/remove ability process.
  (`self.ProcessAdded`))

(event `CallProcessRemoved`
  ;[1 1 1] Add/remove ability process.
  (`self.ProcessRemoved`))

(event `AddAbility`
  (params (AbilityInfo :type "/Game/RTSMultiplayer/AbilitySubsystem/Data/S_AbilityInfo Structure"))
  ;[1 1 1] Remove and ability.
  (`self.AddAbilityMulticast` AbilityInfo))

(event `AddAbilityMulticast`
  (params (AbilityInfo :type "/Game/RTSMultiplayer/AbilitySubsystem/Data/S_AbilityInfo Structure (by ref)"))
  ;[1 1 1] Remove and ability.
  (`KismetArrayLibrary.Array_Add` (`self.Abilities`) AbilityInfo)
  (`self.AbilityAdded`))

(fn `GetCooldownRemaining`
  (params (AbilityClass :type "/Game/RTSMultiplayer/AbilitySubsystem/Blueprints/Ability Class Reference"))
  (returns (RemainingTime :type "Float (double-precision)"))
  (bind (_value _returnvalue) (`BlueprintMapLibrary.Map_Find` (`self.AbilitiesCooldowns`) AbilityClass))
  (bind _cooldowntimeline (`/Game/RTSMultiplayer/AbilitySubsystem/Blueprints/AbilityCooldown.CooldownTimeline` _value))
  (if _returnvalue
    (return (- (`TimelineComponent.GetTimelineLength` _cooldowntimeline) (`TimelineComponent.GetPlaybackPosition` _cooldowntimeline)))
    (else
      (return 0.0))))

(fn `IsAbilityOnCooldown?`
  (params (AbilityClass :type "/Game/RTSMultiplayer/AbilitySubsystem/Blueprints/Ability Class Reference"))
  (returns (OnCooldown :type Boolean))
  (return (`.ReturnValue` (`BlueprintMapLibrary.Map_Find` (`self.AbilitiesCooldowns`) AbilityClass))))