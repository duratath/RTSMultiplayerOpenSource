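; A targeted RTS ability that sends the selected units to collect from a resource seed of the ability's resource type.
; On a valid target it forms the units into a circle squad, assigns a move-and-action collect task at the seed with optional queuing, then destroys itself.
; A wrong actor or mismatched resource type instead shows an attention message through the player controller.
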(event `self.OnTargetChosen`
  (params (HitResult :type "HitResult Structure"))
  ;[1 1 1] Target chosen.
  (bind _asresource_seed (cast `/Game/RTSMultiplayer/ResourcesSubsystem/Blueprints/ResourceSeed` (`.HitActor` (`GameplayStatics.BreakHitResult` HitResult)))
    (:`then`
      (if (`|EnumEquality` (`/Game/RTSMultiplayer/ResourcesSubsystem/Blueprints/ResourceSeed.ResourceType` _asresource_seed) (`self.ResourceType`))
        (`parent.OnTargetChosen` HitResult)
        (`self.CreateCollectResourceTask` _asresource_seed (`GameplayStatics.GetPlayerCharacter` 0))
        (`self.DestroyAbility`)
        (else
          (`/Game/RTSMultiplayer/RTSCharacters/Blueprints/RTSPlayerController.AddAttentionMessage` (cast `/Game/RTSMultiplayer/RTSCharacters/Blueprints/RTSPlayerController` (`GameplayStatics.GetPlayerController` 0) :!pure true) "CHOOSE_CORRECT_TARGET" :!label _label))))
    (:`CastFailed`
      (goto _label))))

(event `CreateCollectResourceTask`
  (params (ResourceSeed :type "Actor Object Reference") (Instigator :type "Pawn Object Reference"))
  ;[1 1 1] Spawn Squad and set CollectResourceTask.
  (bind _returnvalue (`|GenericCreateObject` "/Game/RTSMultiplayer/MovementSubsystem/Blueprints/CircleSquad.CircleSquad_C" (`self.GetOwner`) (`self.CircleSquadRadius`)))
  (for _array_element (`self.SelectedUnits`)
    (`/Game/RTSMultiplayer/MovementSubsystem/Blueprints/Squad.AddToSquad` _returnvalue _array_element))
  (`/Game/RTSMultiplayer/MovementSubsystem/Blueprints/Squad.SetMoveAndActionTask` _returnvalue Instigator (`self.CollectResourceTaskClass`) (`self.K2_GetActorLocation` ResourceSeed) ResourceSeed (`self.QueueTaskModifierDown`) null))

(fn `UserConstructionScript`
  (`parent.UserConstructionScript`))