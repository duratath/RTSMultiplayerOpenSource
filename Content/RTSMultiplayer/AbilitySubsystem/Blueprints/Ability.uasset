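; Base ability actor for the RTS, owned by the player character and used on a set of selected units.
; On BeginPlay it loads info and combat constants from data tables by Id, then passes them through the owner's enhancements for that ability class.
; On EndPlay, non-aborted one-time abilities are recorded as used per unique unit class.
; Helper functions check the player faction's buildings against required levels.
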(event `self.ReceiveBeginPlay`
  ;[1 1 1] Begin play. Read ability info, check abilities enhancements.
  (bind _returnvalue (`|GetDataTableRow` "/Game/RTSMultiplayer/AbilitySubsystem/Data/AbilitiesCombatConstantsDataTable.AbilitiesCombatConstantsDataTable" (`self.Id`))
    (:`then`
      (set `self.CombatConstants` _returnvalue))
    (:`RowNotFound`
      _))
  (bind _returnvalue_2 (`|GetDataTableRow` "/Game/RTSMultiplayer/AbilitySubsystem/Data/AbilitiesDataTable.AbilitiesDataTable" (`self.Id`))
    (:`then`
      (bind _output_get (set `self.AbilityInfo` _returnvalue_2))
      (bind (_enhancements _found_) (`/Game/RTSMultiplayer/RTSCharacters/Blueprints/BasePlayerCharacter.GetAbilityEnhancements` (cast `/Game/RTSMultiplayer/RTSCharacters/Blueprints/BasePlayerCharacter` (`self.GetOwner`) :!pure true) (`.Class_5_AD5F1DB1454BA05768809DBC81B23849` (break `/Game/RTSMultiplayer/AbilitySubsystem/Data/S_AbilityInfo` _output_get))))
      (if _found_
        (for _array_element (`.Enhancements_3_79066C2542DF933384CFADAA507894E9` (break `/Game/RTSMultiplayer/EnhancementsSubsystem/Blueprints/S_EnhancementsArray` _enhancements))
          (bind _asability_enhancement (cast `/Game/RTSMultiplayer/EnhancementsSubsystem/Blueprints/AbilityEnhancement` _array_element))
          (bind (_newabilityinfo _newcombatconstants) (`/Game/RTSMultiplayer/EnhancementsSubsystem/Blueprints/AbilityEnhancement.EnhanceAbility` _asability_enhancement (`self.AbilityInfo`) (`self.CombatConstants`)))
          (set `self.AbilityInfo` _newabilityinfo)
          (set `self.CombatConstants` _newcombatconstants))))
    (:`RowNotFound`
      (`KismetSystemLibrary.PrintString` "Ability: data table row not found." true true (struct :`R` 1.0 :`G` 0.038718 :`A` 1.0) 5.0))))

(event `CheckForOneTimeAbilities`
  (bind (_abilityinfo_class _abilityinfo_icon _abilityinfo_isserving_ _abilityinfo_isonetimeuse_) (break `/Game/RTSMultiplayer/AbilitySubsystem/Data/S_AbilityInfo` (`self.AbilityInfo`)))
  ;[1 1 1] If ability can be used only once.
  (if (and (not (`self.WasAborted?`)) _abilityinfo_isonetimeuse_)
    (bind _asbase_player_character (cast `/Game/RTSMultiplayer/RTSCharacters/Blueprints/BasePlayerCharacter` (`self.GetOwner`)))
    (for _array_element (`self.GetUniqueSelectedUnitsClasses`)
      (`/Game/RTSMultiplayer/RTSCharacters/Blueprints/BasePlayerCharacter.AddUsedAbility` _asbase_player_character _abilityinfo_class _array_element))))

(event `DestroyAbility`
  (`self.K2_DestroyActor`))

(event `self.ReceiveEndPlay`
  (params (EndPlayReason :type "EEndPlayReason Enum" :default "Destroyed"))
  (`self.CheckForOneTimeAbilities`))

(event `Use`
  (params (Units :type "Array of Actor Object Reference"))
  ;[1 1 1] Use event.
  (`self.SetSelectedUnits` Units))

(event `SetSelectedUnits`
  (params (SelectedUnits :type "Array of Actor Object Reference"))
  (set `self.SelectedUnits` SelectedUnits))

(event `Abort`
  ;[1 1 1] Abort ability.
  (`self.SetWasAborted`)
  (`self.DestroyAbility`))

(event `SetWasAborted`
  ;[1 1 1] Abort ability.
  (set `self.WasAborted?` true))

(fn `CheckForBuildingsRequirements`
  (params (BuildingClasses :type "Array of /Game/RTSMultiplayer/BuildingSubsystem/Blueprints/BaseRTSBuilding Class Reference") (BuildingLevels :type "Array of Integer"))
  (returns (ResultValue :type Boolean))
  (locals (`Satisfied?` :type Boolean))
  (for (_array_element _array_index) BuildingClasses
    (set `local.Satisfied?` false)
    (bind _outactors (`GameplayStatics.GetAllActorsOfClass` _array_element))
    (for _array_element_2 _outactors
      (if (and (== (`/Game/RTSMultiplayer/RTSCharacters/Blueprints/BasePlayerCharacter.PlayerFaction` (cast `/Game/RTSMultiplayer/RTSCharacters/Blueprints/BasePlayerCharacter` (`self.GetOwner`) :!pure true)) (`/Game/RTSMultiplayer/BuildingSubsystem/Blueprints/BaseRTSBuilding.Faction` _array_element_2)) (>= (`/Game/RTSMultiplayer/BuildingSubsystem/Blueprints/BaseRTSBuilding.CurrentBuildingLevel` _array_element_2) (`|GetArrayItem` BuildingLevels _array_index)))
        (set `local.Satisfied?` true)
        (break)))
    (if (not (`local.Satisfied?`))
      (return false)))
  (return true))

(fn `CheckForNecessaryBuildings`
  (params (BuildngClasses :type "Array of /Game/RTSMultiplayer/BuildingSubsystem/Blueprints/BaseRTSBuilding Class Reference") (BuildngLevels :type "Array of Integer"))
  (returns (`Success?` :type Boolean))
  (for (_array_element _array_index) BuildngClasses
    (bind _returnvalue (`self.HaveBuilding?` _array_element (`|GetArrayItem` BuildngLevels _array_index)))
    (if (not _returnvalue)
      (return false)))
  (return true))

(fn `GetUniqueSelectedUnitsClasses`
  (returns (UniqueClasses :type "Array of Actor Class Reference"))
  (locals (Classes :type "Array of Actor Class Reference"))
  (for _array_element (`self.SelectedUnits`)
    (`KismetArrayLibrary.Array_AddUnique` (`local.Classes`) (`GameplayStatics.GetObjectClass` _array_element)))
  (return (`local.Classes`)))

(fn `HaveBuilding?`
  (params (BuildingClass :type "/Game/RTSMultiplayer/BuildingSubsystem/Blueprints/BaseRTSBuilding Class Reference") (BuildingLevel :type Integer))
  (returns (ReturnValue :type Boolean))
  (bind _outactors (`GameplayStatics.GetAllActorsOfClass` BuildingClass))
  (for _array_element _outactors
    (if (and (>= (`/Game/RTSMultiplayer/BuildingSubsystem/Blueprints/BaseRTSBuilding.CurrentBuildingLevel` _array_element) BuildingLevel) (`|EnumEquality` (`/Game/RTSMultiplayer/BuildingSubsystem/Blueprints/BaseRTSBuilding.Faction` _array_element) (`/Game/RTSMultiplayer/RTSCharacters/Blueprints/BasePlayerCharacter.PlayerFaction` (cast `/Game/RTSMultiplayer/RTSCharacters/Blueprints/BasePlayerCharacter` (`self.GetOwner`) :!pure true))) (`/Game/RTSMultiplayer/BuildingSubsystem/Blueprints/BaseRTSBuilding.WasBuilt?` _array_element))
      (return true)))
  (return false))

(fn `UserConstructionScript`)