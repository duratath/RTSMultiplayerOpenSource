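; RTS ability that lets the player place a faction-specific building for selected units to construct.
; Use checks singleton, prerequisite and cost rules, then spawns a server-side placement preview that a looping timer moves to the cursor and input rotates.
; A second timer waits for the preview variable to sync before revealing its mesh.
; Choosing a target validates range, placement and resources, then pays and hands construction to a CircleSquad.
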(event `RotateBuildingBlueprint`
  (params (AxisValue :type "Float (double-precision)"))
  ;[1 1 1] Rotate building blueprint events.
  (`self.RotateBuildingBlueprintServer` AxisValue))

(event `UnbindRotateEvent`
  ;[1 1 1] Bind/unbind rotate event.
  (bind _asability_input_receiver (cast `/Game/RTSMultiplayer/InputSubsystem/Blueprints/AbilityInputReceiver` (`/Game/RTSMultiplayer/RTSCharacters/Blueprints/RTSPlayerController.CurrentInputReceiver` (cast `/Game/RTSMultiplayer/RTSCharacters/Blueprints/RTSPlayerController` (`GameplayStatics.GetPlayerController` 0) :!pure true))))
  (remove `/Game/RTSMultiplayer/InputSubsystem/Blueprints/AbilityInputReceiver.OnRotateRight` _asability_input_receiver (`|CreateDelegate` :!event `RotateBuildingBlueprint`)))

(event `SpawnBuildingBlueprint`
  (params (`Spawn Transform Location` :type "Vector Structure") (Instigator :type "Pawn Object Reference"))
  (bind _returnvalue (`self.GetOwner`))
  (bind _playerfaction (`/Game/RTSMultiplayer/RTSCharacters/Blueprints/BasePlayerCharacter.PlayerFaction` (cast `/Game/RTSMultiplayer/RTSCharacters/Blueprints/BasePlayerCharacter` _returnvalue :!pure true)))
  ;[1 1 1] Spawning building blueprint on server.
  (bind _returnvalue_2 (`|SpawnActorFromClass` "/Game/RTSMultiplayer/BuildingSubsystem/Blueprints/BuildingBlueprint.BuildingBlueprint_C" (`KismetMathLibrary.MakeTransform` `Spawn Transform Location`) "AlwaysSpawn" "OverrideRootScale" _returnvalue (`BlueprintMapLibrary.Map_Find` (`self.BuildingClasses`) _playerfaction) (`BlueprintMapLibrary.Map_Find` (`self.BuildingMeshClasses`) _playerfaction) Instigator))
  (set `self.BuildingBlueprint` _returnvalue_2))

(event `RotateBuildingBlueprintServer`
  (params (AxisValue :type "Float (double-precision)"))
  ;[1 1 1] Rotate building blueprint events.
  (bind _buildingblueprint (`self.BuildingBlueprint`)
    (:`then`
      (bind (_returnvalue_roll _returnvalue_pitch _returnvalue_yaw) (`KismetMathLibrary.BreakRotator` (`self.K2_GetActorRotation` _buildingblueprint)))
      (`self.K2_SetActorRotation` _buildingblueprint (`KismetMathLibrary.MakeRotator` _returnvalue_roll _returnvalue_pitch (+ _returnvalue_yaw (* (`self.RotationSensitivity`) AxisValue))) false))
    (:`else`)))

(event `BindRotateEvent`
  ;[1 1 1] Bind/unbind rotate event.
  (bind _asability_input_receiver (cast `/Game/RTSMultiplayer/InputSubsystem/Blueprints/AbilityInputReceiver` (`/Game/RTSMultiplayer/RTSCharacters/Blueprints/RTSPlayerController.CurrentInputReceiver` (cast `/Game/RTSMultiplayer/RTSCharacters/Blueprints/RTSPlayerController` (`GameplayStatics.GetPlayerController` 0) :!pure true))))
  (add `/Game/RTSMultiplayer/InputSubsystem/Blueprints/AbilityInputReceiver.OnRotateRight` _asability_input_receiver (`|CreateDelegate` :!event `RotateBuildingBlueprint`)))

(event `self.Use`
  (params (Units :type "Array of Actor Object Reference (by ref)"))
  (bind _asrtsplayer_controller (cast `/Game/RTSMultiplayer/RTSCharacters/Blueprints/RTSPlayerController` (`GameplayStatics.GetPlayerController` 0) :!pure true))
  (bind (_hitresult _returnvalue) (`PlayerController.GetHitResultUnderCursorByChannel` _asrtsplayer_controller "TraceTypeQuery1" true))
  ;[1 1 1] Use. Setup building blueprint.
  (if (`self.Singleton?`)
    (bind _returnvalue_2 (`self.HaveBuilding?` (`BlueprintMapLibrary.Map_Find` (`self.BuildingClasses`) (`/Game/RTSMultiplayer/RTSCharacters/Blueprints/BasePlayerCharacter.PlayerFaction` (cast `/Game/RTSMultiplayer/RTSCharacters/Blueprints/BasePlayerCharacter` (`self.GetOwner`) :!pure true)))))
    (if _returnvalue_2
      (`/Game/RTSMultiplayer/RTSCharacters/Blueprints/RTSPlayerController.AddAttentionMessage` (cast `/Game/RTSMultiplayer/RTSCharacters/Blueprints/RTSPlayerController` (`GameplayStatics.GetPlayerController` 0) :!pure true) "CANT_DO_THAT" :!label _label)
      (`self.DestroyAbility`)
      (else
        (bind _success_ (`self.CheckForNecessaryBuildings` (`self.NecessaryBuildngClasses`) (`self.NecessaryBuildingLevels`) :!label _label_2))
        (if _success_
          (if (`self.CheckForEnoughResources`)
            (`parent.Use` Units)
            (`self.BindRotateEvent`)
            (if _returnvalue
              (`self.SpawnBuildingBlueprint` (`.Location` (`GameplayStatics.BreakHitResult` _hitresult)) (`Controller.K2_GetPawn` _asrtsplayer_controller))
              (bind _returnvalue_3 (`KismetSystemLibrary.K2_SetTimerDelegate` (`|CreateDelegate` :!event `SetBuildingBlueprintPosition`) 0.05 true))
              (set `self.SetPositionHandle` _returnvalue_3)
              ;[1 1 1] Waiting BuildingBlueprint variable sync.
              (bind _returnvalue_4 (`KismetSystemLibrary.K2_SetTimerDelegate` (delegate `SetBuildingMeshVisibility`) 0.05 true))
              (set `self.BuildingMeshVisibilityHandle` _returnvalue_4))
            (else
              (`/Game/RTSMultiplayer/RTSCharacters/Blueprints/RTSPlayerController.AddAttentionMessage` (cast `/Game/RTSMultiplayer/RTSCharacters/Blueprints/RTSPlayerController` (`GameplayStatics.GetPlayerController` 0) :!pure true) "NOT_ENOUGH_RESOURCES")
              (`self.DestroyAbility`)))
          (else
            (goto _label)))))
    (else
      (goto _label_2))))

(event `SetBuildingMeshVisibility`
  ;[1 1 1] Waiting BuildingBlueprint variable sync.
  (bind _buildingblueprint (`self.BuildingBlueprint`)
    (:`then`
      (`SceneComponent.SetVisibility` (`/Game/RTSMultiplayer/BuildingSubsystem/Blueprints/BuildingBlueprint.BuldingMeshActor` _buildingblueprint) true false)
      (`KismetSystemLibrary.K2_ClearAndInvalidateTimerHandle` (`self.BuildingMeshVisibilityHandle`)))
    (:`else`)))

(event `UpdateBuildingBlueprintLocation`
  (params (NewLocation :type "Vector Structure"))
  ;[1 1 1] Set building blueprint position to mouse cursor position.
  (`self.K2_SetActorLocation` (`self.BuildingBlueprint`) NewLocation false false))

(event `SetBuildingBlueprintPosition`
  ;[1 1 1] Set building blueprint position to mouse cursor position.
  (bind _asrtsplayer_controller (cast `/Game/RTSMultiplayer/RTSCharacters/Blueprints/RTSPlayerController` (`GameplayStatics.GetPlayerController` 0)))
  (bind (_hitresult _returnvalue) (`PlayerController.GetHitResultUnderCursorForObjects` _asrtsplayer_controller (`|MakeArray` "ObjectTypeQuery1" :!type "EObjectTypeQuery Enum") true))
  (if _returnvalue
    (`self.UpdateBuildingBlueprintLocation` (`.Location` (`GameplayStatics.BreakHitResult` _hitresult)))
    (bind _buildingblueprint (`self.BuildingBlueprint`)
      (:`then`
        (`/Game/RTSMultiplayer/BuildingSubsystem/Blueprints/BuildingBlueprint.UpdatePositionAvailability` _buildingblueprint)
        (if (not (`self.IsInRange?`))
          (`/Game/RTSMultiplayer/BuildingSubsystem/Blueprints/BuildingBlueprint.SetBadMaterial` _buildingblueprint)))
      (:`else`))))

(event `self.OnTargetChosen`
  (params (HitResult :type "HitResult Structure"))
  (bind _asrtsplayer_controller (cast `/Game/RTSMultiplayer/RTSCharacters/Blueprints/RTSPlayerController` (`GameplayStatics.GetPlayerController` 0) :!pure true))
  ;[1 1 1] Place for building has been chosen. Spawn building actor if place is good.
  (if (`self.IsInRange?`)
    (if (`/Game/RTSMultiplayer/BuildingSubsystem/Blueprints/BuildingBlueprint.IsGoodPlace?` (`self.BuildingBlueprint`))
      (`self.UnbindRotateEvent`)
      (`parent.OnTargetChosen` HitResult)
      (if (== (`KismetArrayLibrary.Array_Length` (`self.SelectedUnits`)) 0)
        (`self.Abort`)
        (else
          (`KismetSystemLibrary.K2_ClearAndInvalidateTimerHandle` (`self.SetPositionHandle`))
          (if (`self.CheckForEnoughResources`)
            (`self.PayForBuilding`)
            (`self.Build` (`GameplayStatics.GetPlayerCharacter` 0))
            (`self.DestroyAbility`)
            (else
              (`/Game/RTSMultiplayer/RTSCharacters/Blueprints/RTSPlayerController.AddAttentionMessage` (cast `/Game/RTSMultiplayer/RTSCharacters/Blueprints/RTSPlayerController` (`GameplayStatics.GetPlayerController` 0) :!pure true) "NOT_ENOUGH_RESOURCES")
              (`self.Abort`)))))
      (else
        (`/Game/RTSMultiplayer/RTSCharacters/Blueprints/RTSPlayerController.AddAttentionMessage` _asrtsplayer_controller "CHOOSE_CORRECT_TARGET")))
    (else
      (`/Game/RTSMultiplayer/RTSCharacters/Blueprints/RTSPlayerController.AddAttentionMessage` _asrtsplayer_controller "TOO_FAR_AWAY"))))

(event `Build`
  (params (Instigator :type "Pawn Object Reference"))
  (bind _playerfaction (`/Game/RTSMultiplayer/RTSCharacters/Blueprints/BasePlayerCharacter.PlayerFaction` (cast `/Game/RTSMultiplayer/RTSCharacters/Blueprints/BasePlayerCharacter` Instigator :!pure true)))
  ;[1 1 1] Build by a squad.
  (bind _returnvalue (`|GenericCreateObject` "/Game/RTSMultiplayer/MovementSubsystem/Blueprints/CircleSquad.CircleSquad_C" (`self.GetOwner`) 250.0))
  (for _array_element (`self.SelectedUnits`)
    (`/Game/RTSMultiplayer/MovementSubsystem/Blueprints/Squad.AddToSquad` _returnvalue _array_element))
  (`/Game/RTSMultiplayer/BuildingSubsystem/Blueprints/BuildingBlueprint.Build` (`self.BuildingBlueprint`) (`BlueprintMapLibrary.Map_Find` (`self.BuildingClasses`) _playerfaction) Instigator _returnvalue (`self.QueueTaskModifierDown`) _playerfaction))

(event `self.Abort`
  ;[1 1 1] Abort ability.
  (`KismetSystemLibrary.K2_ClearAndInvalidateTimerHandle` (`self.SetPositionHandle`))
  (`self.UnbindRotateEvent`)
  (`self.DestroyBuildingBlueprint`)
  (`parent.Abort`))

(event `DestroyBuildingBlueprint`
  ;[1 1 1] Abort ability.
  (bind _buildingblueprint (`self.BuildingBlueprint`)
    (:`then`
      (`self.K2_DestroyActor` _buildingblueprint))
    (:`else`)))

(fn `CheckForEnoughResources`
  (returns (`Enough?` :type Boolean))
  (bind ((`ConsumableCost_26_03C7DBCC41457F4251BFB0AF879BEE44` _consumablecost) (`AllocatableCost_29_ED89984B4F4139EABCE6599E8ECB0AB5` _allocatablecost)) (break `/Game/RTSMultiplayer/AbilitySubsystem/Data/S_AbilityInfo` (`self.AbilityInfo`)))
  (bind _keys (`BlueprintMapLibrary.Map_Keys` _consumablecost))
  (for _array_element _keys
    (if (not (`/Game/RTSMultiplayer/RTSCharacters/Blueprints/BasePlayerCharacter.IsThereEnoughResource?` (cast `/Game/RTSMultiplayer/RTSCharacters/Blueprints/BasePlayerCharacter` (`self.GetOwner`) :!pure true) _array_element (`BlueprintMapLibrary.Map_Find` _consumablecost _array_element)))
      (return false)))
  (bind _keys_2 (`BlueprintMapLibrary.Map_Keys` _allocatablecost))
  (for _array_element_2 _keys_2
    (if (not (`/Game/RTSMultiplayer/RTSCharacters/Blueprints/BasePlayerCharacter.IsThereEnoughResource?` (cast `/Game/RTSMultiplayer/RTSCharacters/Blueprints/BasePlayerCharacter` (`self.GetOwner`) :!pure true) _array_element_2 (`BlueprintMapLibrary.Map_Find` _allocatablecost _array_element_2)))
      (return false)))
  (return true))

(fn `IsInRange?`
  (returns (InRange :type Boolean))
  (locals (MinDistance :type "Float (double-precision)" :default 999999.0))
  (bind (_abilityinfo_class _abilityinfo_icon _abilityinfo_isserving_ _abilityinfo_isonetimeuse_ _abilityinfo_displayedname _abilityinfo_displayeddescription _abilityinfo_consumablecost _abilityinfo_allocatablecost _abilityinfo_statscost _abilityinfo_streamingcost _abilityinfo_abilityrange) (break `/Game/RTSMultiplayer/AbilitySubsystem/Data/S_AbilityInfo` (`self.AbilityInfo`)))
  (for _array_element (`self.SelectedUnits`)
    (set `local.MinDistance` (`KismetMathLibrary.FMin` (`local.MinDistance`) (`KismetMathLibrary.VSize` (- (`self.K2_GetActorLocation` _array_element) (`self.K2_GetActorLocation` (`self.BuildingBlueprint`)))))))
  (return (<= (`local.MinDistance`) _abilityinfo_abilityrange)))

(fn `PayForBuilding`
  (bind ((`ConsumableCost_26_03C7DBCC41457F4251BFB0AF879BEE44` _consumablecost) (`AllocatableCost_29_ED89984B4F4139EABCE6599E8ECB0AB5` _allocatablecost)) (break `/Game/RTSMultiplayer/AbilitySubsystem/Data/S_AbilityInfo` (`self.AbilityInfo`)))
  (bind _keys (`BlueprintMapLibrary.Map_Keys` _consumablecost))
  (for _array_element _keys
    (`/Game/RTSMultiplayer/RTSCharacters/Blueprints/BasePlayerCharacter.ConsumeResource` (cast `/Game/RTSMultiplayer/RTSCharacters/Blueprints/BasePlayerCharacter` (`self.GetOwner`) :!pure true) _array_element (`BlueprintMapLibrary.Map_Find` _consumablecost _array_element)))
  (bind _keys_2 (`BlueprintMapLibrary.Map_Keys` _allocatablecost))
  (for _array_element_2 _keys_2
    (`/Game/RTSMultiplayer/RTSCharacters/Blueprints/BasePlayerCharacter.AllocateResource` (cast `/Game/RTSMultiplayer/RTSCharacters/Blueprints/BasePlayerCharacter` (`self.GetOwner`) :!pure true) _array_element_2 (`BlueprintMapLibrary.Map_Find` _allocatablecost _array_element_2))))

(fn `UserConstructionScript`
  (`parent.UserConstructionScript`))