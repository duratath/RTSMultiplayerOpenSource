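; Targeted RTS ability that orders selected units to repair a building of the player's faction.
; A valid target triggers CreateRepairTask, which groups the units into a new CircleSquad and issues a move-and-RepairTask order, queued if the modifier is held.
; The ability then destroys itself, while invalid targets only show an attention message.
; Player character and controller are both fetched at index 0.
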(event `self.OnTargetChosen`
  (params (HitResult :type "HitResult Structure"))
  ;[1 1 1] On target chosen.
  (bind _asbase_rtsbuilding (cast `/Game/RTSMultiplayer/BuildingSubsystem/Blueprints/BaseRTSBuilding` (`.HitActor` (`GameplayStatics.BreakHitResult` HitResult)))
    (:`then`
      (if (`|EnumEquality` (`/Game/RTSMultiplayer/RTSCharacters/Blueprints/BasePlayerCharacter.PlayerFaction` (cast `/Game/RTSMultiplayer/RTSCharacters/Blueprints/BasePlayerCharacter` (`GameplayStatics.GetPlayerCharacter` 0) :!pure true)) (`/Game/RTSMultiplayer/BuildingSubsystem/Blueprints/BaseRTSBuilding.Faction` _asbase_rtsbuilding))
        (`parent.OnTargetChosen` HitResult)
        (`self.CreateRepairTask` _asbase_rtsbuilding (`GameplayStatics.GetPlayerCharacter` 0))
        (`self.DestroyAbility`)
        (else
          (`/Game/RTSMultiplayer/RTSCharacters/Blueprints/RTSPlayerController.AddAttentionMessage` (cast `/Game/RTSMultiplayer/RTSCharacters/Blueprints/RTSPlayerController` (`GameplayStatics.GetPlayerController` 0) :!pure true) "CHOOSE_CORRECT_TARGET"))))
    (:`CastFailed`
      (`/Game/RTSMultiplayer/RTSCharacters/Blueprints/RTSPlayerController.AddAttentionMessage` (cast `/Game/RTSMultiplayer/RTSCharacters/Blueprints/RTSPlayerController` (`GameplayStatics.GetPlayerController` 0) :!pure true) "CHOOSE_CORRECT_TARGET"))))

(event `CreateRepairTask`
  (params (BuildingToRepair :type "/Game/RTSMultiplayer/BuildingSubsystem/Blueprints/BaseRTSBuilding Object Reference") (Instigator :type "Pawn Object Reference"))
  ;[1 1 1] Spawn Squad and set RepairTask.
  (bind _returnvalue (`|GenericCreateObject` "/Game/RTSMultiplayer/MovementSubsystem/Blueprints/CircleSquad.CircleSquad_C" (`self.GetOwner`) 250.0))
  (for _array_element (`self.SelectedUnits`)
    (`/Game/RTSMultiplayer/MovementSubsystem/Blueprints/Squad.AddToSquad` _returnvalue _array_element))
  (`/Game/RTSMultiplayer/MovementSubsystem/Blueprints/Squad.SetMoveAndActionTask` _returnvalue Instigator "/Game/RTSMultiplayer/TaskSubsystem/Blueprints/Worker/RepairTask.RepairTask_C" (0.0 0.0 0.0) BuildingToRepair (`self.QueueTaskModifierDown`) null))

(fn `UserConstructionScript`
  (`parent.UserConstructionScript`))