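; Targeted ability base for the RTS that has the player pick a target point or object for the selected units.
; Use switches the player controller to an ability input receiver and, for AOE abilities, spawns a timer-driven cursor decal showing range validity.
; Choosing a target stores the hit, filters executors by nearest-unit or per-unit range, then restores input, as does Abort.
; AI-controlled units bypass the input and range steps.
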(event `SetAOEDecalLocation`
  (bind _hitresult (`PlayerController.GetHitResultUnderCursorForObjects` (cast `/Game/RTSMultiplayer/RTSCharacters/Blueprints/RTSPlayerController` (`GameplayStatics.GetPlayerController` 0) :!pure true) (`|MakeArray` "ObjectTypeQuery1" :!type "EObjectTypeQuery Enum") true))
  ;[1 1 1] Spawn and move AOEDecalActor.
  (`self.K2_SetActorLocation` (`self.AOEDecalActor`) (`.Location` (`GameplayStatics.BreakHitResult` _hitresult)) false false)
  (if (> (`self.GetNearestExecutorDistance` _hitresult) (`.AbilityRange_40_D6C6FE6A4D87A62EFBED188164408101` (break `/Game/RTSMultiplayer/AbilitySubsystem/Data/S_AbilityInfo` (`self.AbilityInfo`))))
    (`/Game/RTSMultiplayer/AbilitySubsystem/Blueprints/AOEDecalActor.SetBadMaterial` (`self.AOEDecalActor`))
    (else
      (`/Game/RTSMultiplayer/AbilitySubsystem/Blueprints/AOEDecalActor.SetGoodMaterial` (`self.AOEDecalActor`)))))

(event `SetupAOESelection`
  ;[1 1 1] Spawn and move AOEDecalActor.
  (bind _returnvalue (`|SpawnActorFromClass` "/Game/RTSMultiplayer/AbilitySubsystem/Blueprints/AOEDecalActor.AOEDecalActor_C" (`KismetMathLibrary.MakeTransform` (`.Location` (`GameplayStatics.BreakHitResult` (`PlayerController.GetHitResultUnderCursorForObjects` (cast `/Game/RTSMultiplayer/RTSCharacters/Blueprints/RTSPlayerController` (`GameplayStatics.GetPlayerController` 0) :!pure true) (`|MakeArray` "ObjectTypeQuery1" :!type "EObjectTypeQuery Enum") true)))) "AlwaysSpawn" "OverrideRootScale" (`self.GetOwner`) (`self.Instigator`)))
  (bind _output_get (set `self.AOEDecalActor` _returnvalue))
  (bind _returnvalue_2 (`KismetSystemLibrary.K2_SetTimerDelegate` (`|CreateDelegate` :!event `SetAOEDecalLocation`) 0.05 true))
  (set `self.SetAOEDecalLocationHandle` _returnvalue_2)
  (`/Game/RTSMultiplayer/AbilitySubsystem/Blueprints/AOEDecalActor.SetRadius` _output_get (`.AOERadius_51_317D0B6A49E5F0E8833AA8B676668C71` (break `/Game/RTSMultiplayer/AbilitySubsystem/Data/S_AbilityInfo` (`self.AbilityInfo`)))))

(event `self.Use`
  (params (Units :type "Array of Actor Object Reference (by ref)"))
  ;[1 1 1] Use event. Set ability input receiver as current receiver, possibly setup AOEDecalActor.
  (`parent.Use` Units)
  (cast `/Game/RTSMultiplayer/RTSCharacters/Blueprints/RTSAIController` (`AIBlueprintHelperLibrary.GetAIController` (`self.GetOwner` (`|GetArrayItem` Units)))
    (:`CastFailed`
      (bind _asrtsplayer_controller (cast `/Game/RTSMultiplayer/RTSCharacters/Blueprints/RTSPlayerController` (`GameplayStatics.GetPlayerController` 0)))
      (`/Game/RTSMultiplayer/RTSCharacters/Blueprints/RTSPlayerController.SetInputReceiver` _asrtsplayer_controller "NewEnumerator1")
      (bind _asability_input_receiver (cast `/Game/RTSMultiplayer/InputSubsystem/Blueprints/AbilityInputReceiver` (`/Game/RTSMultiplayer/RTSCharacters/Blueprints/RTSPlayerController.CurrentInputReceiver` _asrtsplayer_controller)))
      (add `/Game/RTSMultiplayer/InputSubsystem/Blueprints/AbilityInputReceiver.TargetChosen` _asability_input_receiver (`|CreateDelegate` :!event `OnTargetChosen`))
      (if (`.AOEAbility?_47_9DF26F2A47AC2284D8A6719B65410CF9` (break `/Game/RTSMultiplayer/AbilitySubsystem/Data/S_AbilityInfo` (`self.AbilityInfo`)))
        (`self.SetupAOESelection`)))))

(event `OnTargetChosen`
  (params (HitResult :type "HitResult Structure"))
  (bind _actorsinrange (`self.GetExecutorsInRange` HitResult))
  (bind (_abilityinfo_class _abilityinfo_icon _abilityinfo_isserving_ _abilityinfo_isonetimeuse_ _abilityinfo_displayedname _abilityinfo_displayeddescription _abilityinfo_consumablecost _abilityinfo_allocatablecost _abilityinfo_statscost _abilityinfo_streamingcost _abilityinfo_abilityrange _abilityinfo_casttime _abilityinfo_cooldown _abilityinfo_aoeability_ _abilityinfo_aoeradius _abilityinfo_checknearestexecutorrange_) (break `/Game/RTSMultiplayer/AbilitySubsystem/Data/S_AbilityInfo` (`self.AbilityInfo`)))
  ;[1 1 1] Target was chosen. Call AbleToCast? and check range.
  (`KismetSystemLibrary.K2_ClearAndInvalidateTimerHandle` (`self.SetAOEDecalLocationHandle`))
  (bind _aoedecalactor (`self.AOEDecalActor`)
    (:`then`
      (`self.K2_DestroyActor` _aoedecalactor))
    (:`else`
      _))
  (`self.SetChosenTargetHitResult` HitResult)
  (cast `/Game/RTSMultiplayer/RTSCharacters/Blueprints/RTSAIController` (`AIBlueprintHelperLibrary.GetAIController` (`self.GetOwner`))
    (:`CastFailed`
      (if (== _abilityinfo_abilityrange 0.0)
        _
        (elif _abilityinfo_checknearestexecutorrange_
          (if (not (<= (`self.GetNearestExecutorDistance` HitResult) _abilityinfo_abilityrange))
            (`self.SetSelectedUnits` (`|MakeArray`)))
          (elif (!= (`KismetArrayLibrary.Array_Length` _actorsinrange) (`KismetArrayLibrary.Array_Length` (`self.SelectedUnits`)))
            (cast `/Game/RTSMultiplayer/RTSCharacters/Blueprints/RTSAIController` (`AIBlueprintHelperLibrary.GetAIController` (`self.GetOwner`))
              (:`then`
                _)
              (:`CastFailed`
                (`/Game/RTSMultiplayer/RTSCharacters/Blueprints/RTSPlayerController.AddAttentionMessage` (cast `/Game/RTSMultiplayer/RTSCharacters/Blueprints/RTSPlayerController` (`GameplayStatics.GetPlayerController` 0) :!pure true) "TOO_FAR_AWAY")))
            (`self.SetSelectedUnits` _actorsinrange))))
      (cast `/Game/RTSMultiplayer/RTSCharacters/Blueprints/RTSAIController` (`AIBlueprintHelperLibrary.GetAIController` (`self.GetOwner`))
        (:`CastFailed`
          (bind _asrtsplayer_controller (cast `/Game/RTSMultiplayer/RTSCharacters/Blueprints/RTSPlayerController` (`GameplayStatics.GetPlayerController` 0)))
          (`self.SetQueueTaskModifierDown` (`/Game/RTSMultiplayer/RTSCharacters/Blueprints/RTSPlayerController.IsQueueTaskModifierDown?` _asrtsplayer_controller))
          (bind _asability_input_receiver (cast `/Game/RTSMultiplayer/InputSubsystem/Blueprints/AbilityInputReceiver` (`/Game/RTSMultiplayer/RTSCharacters/Blueprints/RTSPlayerController.CurrentInputReceiver` _asrtsplayer_controller)))
          (remove `/Game/RTSMultiplayer/InputSubsystem/Blueprints/AbilityInputReceiver.TargetChosen` _asability_input_receiver (`|CreateDelegate` :!event `OnTargetChosen`))
          (`/Game/RTSMultiplayer/RTSCharacters/Blueprints/RTSPlayerController.SetInputReceiver` _asrtsplayer_controller "NewEnumerator0"))))))

(event `SetChosenTargetHitResult`
  (params (ChosenTargetHitResult :type "HitResult Structure"))
  ;[1 1 1] Target was chosen. Call AbleToCast? and check range.
  (set `self.ChosenTargetHitResult` ChosenTargetHitResult))

(event `SetQueueTaskModifierDown`
  (params (QueueTaskModifierDown :type Boolean))
  ;[1 1 1] Target was chosen. Call AbleToCast? and check range.
  (set `self.QueueTaskModifierDown` QueueTaskModifierDown))

(event `self.Abort`
  ;[1 1 1] Abort ability.
  (cast `/Game/RTSMultiplayer/RTSCharacters/Blueprints/RTSAIController` (`AIBlueprintHelperLibrary.GetAIController` (`self.GetOwner`))
    (:`then`
      _)
    (:`CastFailed`
      (bind _asrtsplayer_controller (cast `/Game/RTSMultiplayer/RTSCharacters/Blueprints/RTSPlayerController` (`GameplayStatics.GetPlayerController` 0)))
      (bind _asability_input_receiver (cast `/Game/RTSMultiplayer/InputSubsystem/Blueprints/AbilityInputReceiver` (`/Game/RTSMultiplayer/RTSCharacters/Blueprints/RTSPlayerController.CurrentInputReceiver` _asrtsplayer_controller))
        (:`then`
          (remove `/Game/RTSMultiplayer/InputSubsystem/Blueprints/AbilityInputReceiver.TargetChosen` _asability_input_receiver (`|CreateDelegate` :!event `OnTargetChosen`))
          (`/Game/RTSMultiplayer/RTSCharacters/Blueprints/RTSPlayerController.SetInputReceiver` _asrtsplayer_controller "NewEnumerator0"))
        (:`CastFailed`
          _))
      (`KismetSystemLibrary.K2_ClearAndInvalidateTimerHandle` (`self.SetAOEDecalLocationHandle`))
      (bind _aoedecalactor (`self.AOEDecalActor`)
        (:`then`
          (`self.K2_DestroyActor` _aoedecalactor))
        (:`else`
          _))))
  (`parent.Abort`))

(fn `GetExecutorsInRange`
  (params (HitResult :type "HitResult Structure (by ref)"))
  (returns (ActorsInRange :type "Array of Actor Object Reference"))
  (locals (ResultActors :type "Array of Actor Object Reference"))
  (bind _selectedunits (`self.SelectedUnits`))
  (bind (_abilityinfo_class _abilityinfo_icon _abilityinfo_isserving_ _abilityinfo_isonetimeuse_ _abilityinfo_displayedname _abilityinfo_displayeddescription _abilityinfo_consumablecost _abilityinfo_allocatablecost _abilityinfo_statscost _abilityinfo_streamingcost _abilityinfo_abilityrange) (break `/Game/RTSMultiplayer/AbilitySubsystem/Data/S_AbilityInfo` (`self.AbilityInfo`)))
  (cast `/Game/RTSMultiplayer/RTSCharacters/Blueprints/RTSAIController` (`AIBlueprintHelperLibrary.GetAIController` (`self.GetOwner`))
    (:`then`
      (return _selectedunits))
    (:`CastFailed`
      (for _array_element _selectedunits
        (if (<= (`KismetMathLibrary.VSize` (- (`self.K2_GetActorLocation` _array_element) (`.Location` (`GameplayStatics.BreakHitResult` HitResult)))) _abilityinfo_abilityrange)
          (`KismetArrayLibrary.Array_Add` (`local.ResultActors`) _array_element)))
      (return (`local.ResultActors`)))))

(fn `GetNearestExecutorDistance`
  (params (HitResult :type "HitResult Structure"))
  (returns (Distance :type "Float (double-precision)"))
  (locals (MinDistance :type "Float (double-precision)" :default 999999.0))
  (for _array_element (`self.SelectedUnits`)
    (set `local.MinDistance` (`KismetMathLibrary.FMin` (`local.MinDistance`) (`KismetMathLibrary.VSize` (- (`self.K2_GetActorLocation` _array_element) (`.Location` (`GameplayStatics.BreakHitResult` HitResult)))))))
  (return (`local.MinDistance`)))

(fn `UserConstructionScript`
  (`parent.UserConstructionScript`))