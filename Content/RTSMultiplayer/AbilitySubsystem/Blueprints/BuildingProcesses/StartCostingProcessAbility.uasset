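; Base RTS building ability that starts a resource-costing process, with an empty SpawnTask hook.
; Use checks required buildings, then counts how many selected units the owning player can afford from consumable and allocatable resources, capped at one for one-time abilities.
; It pays per affordable unit, passes those to the parent Use, calls SpawnTask once and destroys itself.
; Shortfalls show a warning but still process affordable units; a hardcoded false disables the one-time exception.
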(event `self.Use`
  (params (Units :type "Array of Actor Object Reference (by ref)"))
  (bind (_abilityinfo_class _abilityinfo_icon _abilityinfo_isserving_ _abilityinfo_isonetimeuse_) (break `/Game/RTSMultiplayer/AbilitySubsystem/Data/S_AbilityInfo` (`self.AbilityInfo`)))
  ;[1 1 1] Is there enough resources?
  (bind _success_ (`self.CheckForNecessaryBuildings` (`self.NecessaryBuildingClasses`) (`self.NecessaryBuildingLevels`)))
  (if _success_
    (set `self.SolventUnits` (`self.GetSolventActorsCount` Units))
    (if (and (> (`self.SolventUnits`) 0) _abilityinfo_isonetimeuse_)
      (set `self.SolventUnits` 1))
    (if (< (`self.SolventUnits`) (`KismetArrayLibrary.Array_Length` Units))
      (if (and _abilityinfo_isonetimeuse_ (!= (`self.SolventUnits`) 0) false)
        (for _index (range (`self.SolventUnits`)) :!label _label
          (`KismetArrayLibrary.Array_Add` (`self.WhoPaid`) (`|GetArrayItem` Units _index))
          (`self.PayForProcess`))
        (`parent.Use` (`self.WhoPaid`))
        (`self.SpawnTask`)
        (`self.DestroyAbility`)
        (else
          (`/Game/RTSMultiplayer/RTSCharacters/Blueprints/RTSPlayerController.AddAttentionMessage` (cast `/Game/RTSMultiplayer/RTSCharacters/Blueprints/RTSPlayerController` (`GameplayStatics.GetPlayerController` 0) :!pure true) "NOT_ENOUGH_RESOURCES")
          (if (== (`self.SolventUnits`) 0)
            (`self.DestroyAbility`)
            (else
              (goto _label)))))
      (else
        (goto _label)))
    (else
      (`/Game/RTSMultiplayer/RTSCharacters/Blueprints/RTSPlayerController.AddAttentionMessage` (cast `/Game/RTSMultiplayer/RTSCharacters/Blueprints/RTSPlayerController` (`GameplayStatics.GetPlayerController` 0) :!pure true) "CANT_DO_THAT")
      (`self.DestroyAbility`))))

(event `SpawnTask`
  ;[1 1 1] Is there enough resources?
)

(fn `GetSolventActorsCount`
  (params (Actors :type "Array of Actor Object Reference"))
  (returns (SolventUnits :type Integer))
  (locals (MinimumSolventUnits :type Integer))
  (bind (_abilityinfo_class _abilityinfo_icon _abilityinfo_isserving_ _abilityinfo_isonetimeuse_ _abilityinfo_displayedname _abilityinfo_displayeddescription _abilityinfo_consumablecost _abilityinfo_allocatablecost) (break `/Game/RTSMultiplayer/AbilitySubsystem/Data/S_AbilityInfo` (`self.AbilityInfo`)))
  (bind (_abilityinfo_class_2 _abilityinfo_icon_2 _abilityinfo_isserving__2 _abilityinfo_isonetimeuse__2 _abilityinfo_displayedname_2 _abilityinfo_displayeddescription_2 _abilityinfo_consumablecost_2) (break `/Game/RTSMultiplayer/AbilitySubsystem/Data/S_AbilityInfo` (`self.AbilityInfo`)))
  (set `local.MinimumSolventUnits` (`KismetArrayLibrary.Array_Length` Actors))
  (bind _asbase_player_character (cast `/Game/RTSMultiplayer/RTSCharacters/Blueprints/BasePlayerCharacter` (`self.GetOwner`))
    (:`then`
      (bind _keys (`BlueprintMapLibrary.Map_Keys` _abilityinfo_consumablecost_2))
      (for _array_element _keys
        (bind _value (`BlueprintMapLibrary.Map_Find` _abilityinfo_consumablecost_2 _array_element))
        (if (not (== _value 0.0))
          (bind (_found_ _resource) (`/Game/RTSMultiplayer/RTSCharacters/Blueprints/BasePlayerCharacter.GetConsumableResource` _asbase_player_character _array_element))
          (if _found_
            (set `local.MinimumSolventUnits` (`KismetMathLibrary.Min` (`local.MinimumSolventUnits`) (`KismetMathLibrary.FTrunc` (/ (break `/Game/RTSMultiplayer/ResourcesSubsystem/Blueprints/S_ConsumableResource` _resource) _value))))
            (else
              (return 0)))))
      (bind _keys_2 (`BlueprintMapLibrary.Map_Keys` _abilityinfo_allocatablecost))
      (for _array_element_2 _keys_2
        (bind _value_2 (`BlueprintMapLibrary.Map_Find` _abilityinfo_allocatablecost _array_element_2))
        (if (not (== _value_2 0.0))
          (bind (_found__2 _resource_2) (`/Game/RTSMultiplayer/RTSCharacters/Blueprints/BasePlayerCharacter.GetAllocatableResource` _asbase_player_character _array_element_2))
          (if _found__2
            (set `local.MinimumSolventUnits` (`KismetMathLibrary.Min` (`local.MinimumSolventUnits`) (`KismetMathLibrary.FTrunc` (/ (- (`.MaximumAvailable_4_A59F6CB84091EDDEEFB2EDBECEC97409` (break `/Game/RTSMultiplayer/ResourcesSubsystem/Blueprints/S_AllocatableResource` _resource_2)) (break `/Game/RTSMultiplayer/ResourcesSubsystem/Blueprints/S_AllocatableResource` _resource_2)) _value_2))))
            (else
              (return 0)))))
      (return (`local.MinimumSolventUnits`)))
    (:`CastFailed`
      (return 0))))

(fn `PayForProcess`
  (bind (_abilityinfo_class _abilityinfo_icon _abilityinfo_isserving_ _abilityinfo_isonetimeuse_ _abilityinfo_displayedname _abilityinfo_displayeddescription _abilityinfo_consumablecost) (break `/Game/RTSMultiplayer/AbilitySubsystem/Data/S_AbilityInfo` (`self.AbilityInfo`)))
  (bind (_abilityinfo_class_2 _abilityinfo_icon_2 _abilityinfo_isserving__2 _abilityinfo_isonetimeuse__2 _abilityinfo_displayedname_2 _abilityinfo_displayeddescription_2 _abilityinfo_consumablecost_2 _abilityinfo_allocatablecost) (break `/Game/RTSMultiplayer/AbilitySubsystem/Data/S_AbilityInfo` (`self.AbilityInfo`)))
  (bind _asbase_player_character (cast `/Game/RTSMultiplayer/RTSCharacters/Blueprints/BasePlayerCharacter` (`self.GetOwner`)))
  (bind _keys (`BlueprintMapLibrary.Map_Keys` _abilityinfo_consumablecost))
  (for _array_element _keys
    (`/Game/RTSMultiplayer/RTSCharacters/Blueprints/BasePlayerCharacter.ConsumeResource` _asbase_player_character _array_element (`BlueprintMapLibrary.Map_Find` _abilityinfo_consumablecost _array_element)))
  (bind _keys_2 (`BlueprintMapLibrary.Map_Keys` _abilityinfo_allocatablecost))
  (for _array_element_2 _keys_2
    (`/Game/RTSMultiplayer/RTSCharacters/Blueprints/BasePlayerCharacter.AllocateResource` _asbase_player_character _array_element_2 (`BlueprintMapLibrary.Map_Find` _abilityinfo_allocatablecost _array_element_2))))

(fn `UserConstructionScript`
  (`parent.UserConstructionScript`))