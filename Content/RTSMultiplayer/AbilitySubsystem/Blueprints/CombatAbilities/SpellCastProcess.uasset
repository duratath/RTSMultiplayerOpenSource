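; Spell cast process actor for RTS combat abilities that turns the caster toward the target, resolves the spell when the process ends, then destroys itself.
; On end it spawns effect actors and hands them to a projectile if one is set; otherwise it deals damage and healing, plays the end particle and applies the effects.
; AOE targets come from sphere overlaps on tagged components, filtered by faction relationship and optional class.
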(event `self.StartProcess`
  (bind _processinstigator (`self.ProcessInstigator`))
  (bind (_hitresult_bblockinghit _hitresult_binitialoverlap _hitresult_time _hitresult_distance _hitresult_location) (`GameplayStatics.BreakHitResult` (`self.HitResult`)))
  (bind (_returnvalue_roll _returnvalue_pitch) (`KismetMathLibrary.BreakRotator` (`self.K2_GetActorRotation` _processinstigator)))
  (bind (_returnvalue_roll_2 _returnvalue_pitch_2 _returnvalue_yaw) (`KismetMathLibrary.BreakRotator` (`KismetMathLibrary.FindLookAtRotation` (`self.K2_GetActorLocation` _processinstigator) _hitresult_location)))
  ;[1 1 1] Rotate executor to target on start.
  (`parent.StartProcess`)
  (`SceneComponent.K2_SetWorldRotation` (`Actor.RootComponent` _processinstigator) (`KismetMathLibrary.MakeRotator` _returnvalue_roll _returnvalue_pitch _returnvalue_yaw) false false))

(event `SpawnPossibleAOEEmitter`
  (bind (_hitresult_bblockinghit _hitresult_binitialoverlap _hitresult_time _hitresult_distance _hitresult_location _hitresult_impactpoint _hitresult_normal _hitresult_impactnormal _hitresult_physmat _hitresult_hitactor) (`GameplayStatics.BreakHitResult` (`self.HitResult`)))
  ;[1 1 1] Spawn possible emitter.
  (bind _endcastparticlesystem (`self.EndCastParticleSystem`)
    (:`then`
      (`GameplayStatics.SpawnEmitterAtLocation` _endcastparticlesystem _hitresult_location))
    (:`else`)))

(event `SpawnPossibleTargetEmitter`
  (bind (_hitresult_bblockinghit _hitresult_binitialoverlap _hitresult_time _hitresult_distance _hitresult_location _hitresult_impactpoint _hitresult_normal _hitresult_impactnormal _hitresult_physmat _hitresult_hitactor) (`GameplayStatics.BreakHitResult` (`self.HitResult`)))
  ;[1 1 1] Spawn possible emitter.
  (bind _endcastparticlesystem (`self.EndCastParticleSystem`)
    (:`then`
      (`GameplayStatics.SpawnEmitterAttached` _endcastparticlesystem (`Actor.RootComponent` _hitresult_hitactor)))
    (:`else`)))

(event `self.EndProcess`
  (bind _processinstigator (`self.ProcessInstigator`))
  (bind (_hitresult_bblockinghit _hitresult_binitialoverlap _hitresult_time _hitresult_distance _hitresult_location _hitresult_impactpoint _hitresult_normal _hitresult_impactnormal _hitresult_physmat _hitresult_hitactor) (`GameplayStatics.BreakHitResult` (`self.HitResult`)))
  ;[1 1 1] Spawn projectile if valid on end process, apply effects immediately if there is no projectile.
  (`parent.EndProcess`)
  (bind _projectileclass (`self.ProjectileClass`)
    (:`then`
      (bind _resulteffects (`self.SpawnEffects`))
      (`|SpawnActorFromClass` _projectileclass (`self.GetTransform` _processinstigator) "AlwaysSpawn" "OverrideRootScale" (`self.GetOwner`) _hitresult_hitactor _processinstigator (`self.AbilityConstants`) _resulteffects (`self.Instigator`)))
    (:`else`
      (if (`.AOEAbility?_47_9DF26F2A47AC2284D8A6719B65410CF9` (break `/Game/RTSMultiplayer/AbilitySubsystem/Data/S_AbilityInfo` (`self.AbilityInfo`)))
        (`self.TryDealDamageAndHealAOE`)
        (`self.SpawnPossibleAOEEmitter`)
        (else
          (`self.TryDealDamageAndHealTarget`)
          (`self.SpawnPossibleTargetEmitter`)))
      (bind _resulteffects_2 (`self.SpawnEffects`))
      (for _array_element _resulteffects_2
        (`/Game/RTSMultiplayer/EffectsSubsystem/Blueprints/SimpleEffect.Apply` _array_element))))
  (`self.K2_DestroyActor`))

(event `TryDealDamageAndHealTarget`
  (bind (_hitresult_bblockinghit _hitresult_binitialoverlap _hitresult_time _hitresult_distance _hitresult_location _hitresult_impactpoint _hitresult_normal _hitresult_impactnormal _hitresult_physmat _hitresult_hitactor) (`GameplayStatics.BreakHitResult` (`self.HitResult`)))
  (bind (_abilityconstants_basedamage _abilityconstants_basehealing) (break `/Game/RTSMultiplayer/AbilitySubsystem/Data/S_AbilityCombatConstants` (`self.AbilityConstants`)))
  (bind _abilityconstants_basedamage_2 (break `/Game/RTSMultiplayer/AbilitySubsystem/Data/S_AbilityCombatConstants` (`self.AbilityConstants`)))
  (bind (_abilityconstants_basedamage_3 _abilityconstants_basehealing_2 _abilityconstants_effectbaseduration _abilityconstants_tickfrequency _abilityconstants_tickdamage _abilityconstants_tickhealing _abilityconstants_damagetype) (break `/Game/RTSMultiplayer/AbilitySubsystem/Data/S_AbilityCombatConstants` (`self.AbilityConstants`)))
  (bind (_abilityconstants_basedamage_4 _abilityconstants_basehealing_3) (break `/Game/RTSMultiplayer/AbilitySubsystem/Data/S_AbilityCombatConstants` (`self.AbilityConstants`)))
  ;[1 1 1] Try deal damage and heal specified target if necessary.
  (if (!= _abilityconstants_basedamage_2 0.0)
    (bind _asi_able_to_fight (cast `/Game/RTSMultiplayer/CombatSubsystem/Blueprints/I_AbleToFight` (`self.ProcessInstigator`))
      (:`then`
        (bind _combatcomponent (`/Game/RTSMultiplayer/CombatSubsystem/Blueprints/I_AbleToFight.GetCombatComponent` _asi_able_to_fight))
        (bind _asi_able_to_fight_2 (cast `/Game/RTSMultiplayer/CombatSubsystem/Blueprints/I_AbleToFight` _hitresult_hitactor))
        (bind _combatcomponent_2 (`/Game/RTSMultiplayer/CombatSubsystem/Blueprints/I_AbleToFight.GetCombatComponent` _asi_able_to_fight_2))
        (`/Game/RTSMultiplayer/CombatSubsystem/Blueprints/CombatComponent.ReceiveDamage` _combatcomponent_2 (make `/Game/RTSMultiplayer/CombatSubsystem/Blueprints/S_DamageInfo` _abilityconstants_damagetype (`/Game/RTSMultiplayer/CombatSubsystem/Blueprints/CombatComponent.WeaponType` _combatcomponent) _abilityconstants_basedamage_3))
        (if (!= _abilityconstants_basehealing_3 0.0) :!label _label
          (bind _asi_able_to_fight_3 (cast `/Game/RTSMultiplayer/CombatSubsystem/Blueprints/I_AbleToFight` _hitresult_hitactor)
            (:`then`
              (bind _combatcomponent_3 (`/Game/RTSMultiplayer/CombatSubsystem/Blueprints/I_AbleToFight.GetCombatComponent` _asi_able_to_fight_3))
              (`/Game/RTSMultiplayer/CombatSubsystem/Blueprints/CombatComponent.ReceiveHealing` _combatcomponent_3 _abilityconstants_basehealing))
            (:`CastFailed`
              (`KismetSystemLibrary.PrintString` "SpellCastProcess: instigator and target must implement I_AbleToFight interface." true true (struct :`R` 1.0 :`G` 0.038718 :`A` 1.0) 5.0 :!label _label_2)))))
      (:`CastFailed`
        (goto _label_2)))
    (else
      (goto _label))))

(event `TryDealDamageAndHealAOE`
  (bind ((`BaseDamage_5_67243A2647AD5CEE5DABE38F9040B1C7` _basedamage) (`BaseHealing_6_C34337194E1EB197A8E5DDABD5950921` _basehealing) (`EffectBaseDuration_21_F507FA954AE69DE36891B6B09B366D74` _effectbaseduration) (`DamageType_11_13F3D90246A8A8D2C591B190B076806C` _damagetype)) (break `/Game/RTSMultiplayer/AbilitySubsystem/Data/S_AbilityCombatConstants` (`self.AbilityConstants`)))
  (bind ((`BaseDamage_5_67243A2647AD5CEE5DABE38F9040B1C7` _basedamage_2) (`BaseHealing_6_C34337194E1EB197A8E5DDABD5950921` _basehealing_2)) (break `/Game/RTSMultiplayer/AbilitySubsystem/Data/S_AbilityCombatConstants` (`self.AbilityConstants`)))
  ;[1 1 1] Try deal damage and heal AOE if necessary.
  (if (or (!= _basedamage_2 0.0) (!= _basehealing_2 0.0))
    (bind _actors (`self.GetOverlappedAbleToFightActors`))
    (for _array_element _actors
      (bind _asi_able_to_fight (cast `/Game/RTSMultiplayer/CombatSubsystem/Blueprints/I_AbleToFight` _array_element))
      (bind _faction (`/Game/RTSMultiplayer/CombatSubsystem/Blueprints/I_AbleToFight.GetFactionAsAbleToFight` _asi_able_to_fight))
      (if (`|EnumEquality` (`/Game/RTSMultiplayer/RTSCharacters/Blueprints/BasePlayerCharacter.GetRelationships` (cast `/Game/RTSMultiplayer/RTSCharacters/Blueprints/BasePlayerCharacter` (`self.GetOwner`) :!pure true) _faction) (`self.CorrectTarget`))
        (if (== (`self.CorrectTargetClass`) null)
          (bind _combatcomponent (`/Game/RTSMultiplayer/CombatSubsystem/Blueprints/I_AbleToFight.GetCombatComponent` _asi_able_to_fight :!label _label_3))
          (if (!= _basedamage 0.0)
            (bind _asi_able_to_fight_2 (cast `/Game/RTSMultiplayer/CombatSubsystem/Blueprints/I_AbleToFight` (`self.ProcessInstigator`))
              (:`then`
                (bind _combatcomponent_2 (`/Game/RTSMultiplayer/CombatSubsystem/Blueprints/I_AbleToFight.GetCombatComponent` _asi_able_to_fight_2))
                (`/Game/RTSMultiplayer/CombatSubsystem/Blueprints/CombatComponent.ReceiveDamage` _combatcomponent (make `/Game/RTSMultiplayer/CombatSubsystem/Blueprints/S_DamageInfo` _damagetype (`/Game/RTSMultiplayer/CombatSubsystem/Blueprints/CombatComponent.WeaponType` _combatcomponent_2) _basedamage))
                (if (!= _basehealing 0.0) :!label _label_4
                  (`/Game/RTSMultiplayer/CombatSubsystem/Blueprints/CombatComponent.ReceiveHealing` _combatcomponent _basehealing)))
              (:`CastFailed`
                (`KismetSystemLibrary.PrintString` "SpellCastProcess: process instigator must implement I_AbleToFight interface." true true (struct :`R` 1.0 :`G` 0.038718 :`A` 1.0) 5.0)))
            (else
              (goto _label_4)))
          (elif (`KismetMathLibrary.ClassIsChildOf` (`GameplayStatics.GetObjectClass` _array_element) (`self.CorrectTargetClass`))
            (goto _label_3)))))))

(fn `GetOverlappedAbleToFightActors`
  (returns (Actors :type "Array of Actor Object Reference"))
  (locals (Result :type "Array of Actor Object Reference"))
  (bind (_hitresult_bblockinghit _hitresult_binitialoverlap _hitresult_time _hitresult_distance _hitresult_location) (`GameplayStatics.BreakHitResult` (`self.HitResult`)))
  (bind _outcomponents (`KismetSystemLibrary.SphereOverlapComponents` _hitresult_location (`.AOERadius_51_317D0B6A49E5F0E8833AA8B676668C71` (break `/Game/RTSMultiplayer/AbilitySubsystem/Data/S_AbilityInfo` (`self.AbilityInfo`))) (`|MakeArray` "ObjectTypeQuery1" "ObjectTypeQuery2" "ObjectTypeQuery3" :!type "EObjectTypeQuery Enum") "/Script/Engine.PrimitiveComponent"))
  (for _array_element _outcomponents
    (if (`ActorComponent.ComponentHasTag` _array_element "AOEAbilityCollision")
      (bind _returnvalue (`ActorComponent.GetOwner` _array_element))
      (cast `/Game/RTSMultiplayer/CombatSubsystem/Blueprints/I_AbleToFight` _returnvalue)
      (`KismetArrayLibrary.Array_Add` (`local.Result`) _returnvalue)))
  (return (`local.Result`)))

(fn `GetOverlappedEffectReceiversActors`
  (returns (Actors :type "Array of Actor Object Reference"))
  (locals (Result :type "Array of Actor Object Reference"))
  (bind (_hitresult_bblockinghit _hitresult_binitialoverlap _hitresult_time _hitresult_distance _hitresult_location) (`GameplayStatics.BreakHitResult` (`self.HitResult`)))
  (bind _outcomponents (`KismetSystemLibrary.SphereOverlapComponents` _hitresult_location (`.AOERadius_51_317D0B6A49E5F0E8833AA8B676668C71` (break `/Game/RTSMultiplayer/AbilitySubsystem/Data/S_AbilityInfo` (`self.AbilityInfo`))) (`|MakeArray` "ObjectTypeQuery1" "ObjectTypeQuery2" "ObjectTypeQuery3" :!type "EObjectTypeQuery Enum") "/Script/Engine.PrimitiveComponent"))
  (for _array_element _outcomponents
    (if (`ActorComponent.ComponentHasTag` _array_element "AOEAbilityCollision")
      (bind _returnvalue (`ActorComponent.GetOwner` _array_element))
      (cast `/Game/RTSMultiplayer/EffectsSubsystem/Blueprints/I_EffectReceiver` _returnvalue)
      (`KismetArrayLibrary.Array_Add` (`local.Result`) _returnvalue)))
  (return (`local.Result`)))

(fn `SpawnEffects`
  (returns (ResultEffects :type "Array of /Game/RTSMultiplayer/EffectsSubsystem/Blueprints/SimpleEffect Object Reference"))
  (locals (Effects :type "Array of /Game/RTSMultiplayer/EffectsSubsystem/Blueprints/SimpleEffect Object Reference"))
  (bind (_hitresult_bblockinghit _hitresult_binitialoverlap _hitresult_time _hitresult_distance _hitresult_location _hitresult_impactpoint _hitresult_normal _hitresult_impactnormal _hitresult_physmat _hitresult_hitactor) (`GameplayStatics.BreakHitResult` (`self.HitResult`)))
  (if (`.AOEAbility?_47_9DF26F2A47AC2284D8A6719B65410CF9` (break `/Game/RTSMultiplayer/AbilitySubsystem/Data/S_AbilityInfo` (`self.AbilityInfo`)))
    (bind _actors (`self.GetOverlappedEffectReceiversActors`))
    (for _array_element _actors
      (if (== (`self.CorrectTargetClass`) null)
        (bind _asi_effect_receiver (cast `/Game/RTSMultiplayer/EffectsSubsystem/Blueprints/I_EffectReceiver` _array_element :!label _label)
          (:`then`
            (bind _faction (`/Game/RTSMultiplayer/EffectsSubsystem/Blueprints/I_EffectReceiver.GetFactionAsEffectReceiver` _asi_effect_receiver))
            (if (`|EnumEquality` (`/Game/RTSMultiplayer/RTSCharacters/Blueprints/BasePlayerCharacter.GetRelationships` (cast `/Game/RTSMultiplayer/RTSCharacters/Blueprints/BasePlayerCharacter` (`self.GetOwner`) :!pure true) _faction) (`self.CorrectTarget`))
              (for (_array_element_2 _array_index) (`self.EffectsToApply`)
                (bind _returnvalue (`|SpawnActorFromClass` _array_element_2 (`KismetMathLibrary.MakeTransform` (0.0 0.0 0.0)) "AlwaysSpawn" "OverrideRootScale" (`self.GetOwner`) _array_element (`self.AbilityConstants`) (`|GetArrayItem` (`self.EffectsConstantsId`) _array_index) (`self.ProcessInstigator`) (`self.GetInstigator`)))
                (`KismetArrayLibrary.Array_Add` (`local.Effects`) _returnvalue))))
          (:`CastFailed`
            (`KismetSystemLibrary.PrintString` "SpellCastProcess: target must implement I_EffectReceiver interface." true true (struct :`R` 1.0 :`G` 0.038718 :`A` 1.0) 5.0)))
        (elif (`KismetMathLibrary.ClassIsChildOf` (`GameplayStatics.GetObjectClass` _array_element) (`self.CorrectTargetClass`))
          (goto _label))))
    (return (`local.Effects`))
    (else
      (for (_array_element_3 _array_index_2) (`self.EffectsToApply`)
        (bind _returnvalue_2 (`|SpawnActorFromClass` _array_element_3 (`KismetMathLibrary.MakeTransform` (0.0 0.0 0.0)) "AlwaysSpawn" "OverrideRootScale" (`self.GetOwner`) _hitresult_hitactor (`self.AbilityConstants`) (`|GetArrayItem` (`self.EffectsConstantsId`) _array_index_2) (`self.ProcessInstigator`) (`self.GetInstigator`)))
        (`KismetArrayLibrary.Array_Add` (`local.Effects`) _returnvalue_2))
      (return (`local.Effects`)))))

(fn `UserConstructionScript`
  (`parent.UserConstructionScript`))