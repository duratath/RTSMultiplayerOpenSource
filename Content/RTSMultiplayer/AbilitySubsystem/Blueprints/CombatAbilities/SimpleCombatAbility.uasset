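; Targeted combat ability for RTS units that validates the target, charges casters and queues a spell cast.
; BeginPlay applies the owning player's effect enhancements.
; Use and target selection keep only casters who can afford stat costs (target selection also checks range, faction relationship and class, except for AOE), warning human players on failure.
; Each paying caster gets a SpellCastProcess task, queued or immediate; AI targeting picks the lowest health ratio.
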(event `self.ReceiveBeginPlay`
  (bind (_enhancements _found_) (`/Game/RTSMultiplayer/RTSCharacters/Blueprints/BasePlayerCharacter.GetAbilityEnhancements` (cast `/Game/RTSMultiplayer/RTSCharacters/Blueprints/BasePlayerCharacter` (`self.GetOwner`) :!pure true) (`.Class_5_AD5F1DB1454BA05768809DBC81B23849` (break `/Game/RTSMultiplayer/AbilitySubsystem/Data/S_AbilityInfo` (`self.AbilityInfo`)))))
  ;[1 1 1] Begin play. Apply possible effect enhancements.
  (`parent.ReceiveBeginPlay`)
  (if _found_
    (for _array_element (`.Enhancements_3_79066C2542DF933384CFADAA507894E9` (break `/Game/RTSMultiplayer/EnhancementsSubsystem/Blueprints/S_EnhancementsArray` _enhancements))
      (bind _aseffects_enhancement (cast `/Game/RTSMultiplayer/EnhancementsSubsystem/Blueprints/EffectsEnhancement` _array_element))
      (`/Game/RTSMultiplayer/EnhancementsSubsystem/Blueprints/EffectsEnhancement.EnhanceEffects` _aseffects_enhancement (`self.EffectsToApply`) (`self.EffectsConstantsId`)))))

(event `PayForAbility`
  (params (AbleToPayActors :type "Array of Actor Object Reference"))
  (bind ((`StatsCost_32_40B8335549DA9465E8F6F09CDA3E9E24` _statscost)) (break `/Game/RTSMultiplayer/AbilitySubsystem/Data/S_AbilityInfo` (`self.AbilityInfo`)))
  ;[1 1 1] Pay for ability.
  (for _array_element AbleToPayActors
    (bind _asi_have_stats (cast `/Game/RTSMultiplayer/StatsSubsystem/Blueprints/I_HaveStats` _array_element)
      (:`then`
        (bind _statscomponent (`/Game/RTSMultiplayer/StatsSubsystem/Blueprints/I_HaveStats.GetStatsComponent` _asi_have_stats))
        (bind _keys (`BlueprintMapLibrary.Map_Keys` _statscost))
        (for _array_element_2 _keys
          (`/Game/RTSMultiplayer/StatsSubsystem/Blueprints/StatsComponent.ChangeCurrentStatValue` _statscomponent _array_element_2 (* -1 (`BlueprintMapLibrary.Map_Find` _statscost _array_element_2)))))
      (:`CastFailed`
        (`KismetSystemLibrary.PrintString` "SimpleCombatAbility: caster must implement I_HaveStats interface." true true (struct :`R` 1.0 :`G` 0.038718 :`A` 1.0) 5.0)))))

(event `self.Use`
  (params (Units :type "Array of Actor Object Reference (by ref)"))
  ;[1 1 1] Check for enough resources.
  (bind _abletopayactors (`self.CheckResourcesAvailability` Units))
  (bind _returnvalue (`KismetArrayLibrary.Array_Length` _abletopayactors))
  (set `self.DisplayAttentionMessage` (< _returnvalue (`KismetArrayLibrary.Array_Length` Units)))
  (if (== _returnvalue 0)
    (cast `/Game/RTSMultiplayer/RTSCharacters/Blueprints/RTSAIController` (`AIBlueprintHelperLibrary.GetAIController` (`self.GetOwner`))
      (:`then`
        _)
      (:`CastFailed`
        (`/Game/RTSMultiplayer/RTSCharacters/Blueprints/RTSPlayerController.AddAttentionMessage` (cast `/Game/RTSMultiplayer/RTSCharacters/Blueprints/RTSPlayerController` (`GameplayStatics.GetPlayerController` 0) :!pure true) "NOT_ENOUGH_RESOURCES")))
    (`self.DestroyAbility`)
    (else
      (`parent.Use` _abletopayactors))))

(event `self.OnTargetChosen`
  (params (HitResult :type "HitResult Structure"))
  (bind _actorsinrange (`self.GetExecutorsInRange` HitResult))
  (bind _correcttargetclass (`self.CorrectTargetClass`))
  ;[1 1 1] On target chosen.
  (if (and (`self.IsTargetCorrect?` HitResult) (or (`KismetMathLibrary.ClassIsChildOf` (`GameplayStatics.GetObjectClass` (`.HitActor` (`GameplayStatics.BreakHitResult` HitResult))) _correcttargetclass) (== _correcttargetclass null) (`.AOEAbility?_47_9DF26F2A47AC2284D8A6719B65410CF9` (break `/Game/RTSMultiplayer/AbilitySubsystem/Data/S_AbilityInfo` (`self.AbilityInfo`)))))
    (`parent.OnTargetChosen` HitResult)
    (if (== (`KismetArrayLibrary.Array_Length` _actorsinrange) 0)
      (`self.Abort`)
      (else
        (bind _abletopayactors (`self.CheckResourcesAvailability` _actorsinrange))
        (bind _returnvalue (`KismetArrayLibrary.Array_Length` _abletopayactors))
        (if (or (< _returnvalue (`KismetArrayLibrary.Array_Length` _actorsinrange)) (`self.DisplayAttentionMessage`))
          (cast `/Game/RTSMultiplayer/RTSCharacters/Blueprints/RTSAIController` (`AIBlueprintHelperLibrary.GetAIController` (`self.GetOwner`))
            (:`then`
              _)
            (:`CastFailed`
              (`/Game/RTSMultiplayer/RTSCharacters/Blueprints/RTSPlayerController.AddAttentionMessage` (cast `/Game/RTSMultiplayer/RTSCharacters/Blueprints/RTSPlayerController` (`GameplayStatics.GetPlayerController` 0) :!pure true) "NOT_ENOUGH_RESOURCES")))
          (if (== _returnvalue 0)
            (`self.Abort`)
            (else
              (`self.PayForAbility` _abletopayactors :!label _label)
              (`self.SetSelectedUnits` _abletopayactors)
              (`self.SpawnPossibleProcessTask` (cast `/Game/RTSMultiplayer/RTSCharacters/Blueprints/RTSPlayerController` (`GameplayStatics.GetPlayerController` 0) :!pure true))
              (`self.DestroyAbility`)))
          (else
            (goto _label)))))
    (else
      (cast `/Game/RTSMultiplayer/RTSCharacters/Blueprints/RTSAIController` (`AIBlueprintHelperLibrary.GetAIController` (`self.GetOwner`))
        (:`CastFailed`
          (`/Game/RTSMultiplayer/RTSCharacters/Blueprints/RTSPlayerController.AddAttentionMessage` (cast `/Game/RTSMultiplayer/RTSCharacters/Blueprints/RTSPlayerController` (`GameplayStatics.GetPlayerController` 0) :!pure true) "CHOOSE_CORRECT_TARGET"))))))

(event `SpawnPossibleProcessTask`
  (params (PlayerController :type "/Game/RTSMultiplayer/RTSCharacters/Blueprints/RTSPlayerController Object Reference"))
  (bind _returnvalue (`self.GetOwner`))
  (bind (_abilityinfo_class _abilityinfo_icon _abilityinfo_isserving_ _abilityinfo_isonetimeuse_ _abilityinfo_displayedname _abilityinfo_displayeddescription _abilityinfo_consumablecost _abilityinfo_allocatablecost _abilityinfo_statscost _abilityinfo_streamingcost _abilityinfo_abilityrange _abilityinfo_casttime) (break `/Game/RTSMultiplayer/AbilitySubsystem/Data/S_AbilityInfo` (`self.AbilityInfo`)))
  (bind (_abilityinfo_class_2 _abilityinfo_icon_2 _abilityinfo_isserving__2 _abilityinfo_isonetimeuse__2 _abilityinfo_displayedname_2 _abilityinfo_displayeddescription_2 _abilityinfo_consumablecost_2 _abilityinfo_allocatablecost_2 _abilityinfo_statscost_2 _abilityinfo_streamingcost_2 _abilityinfo_abilityrange_2 _abilityinfo_casttime_2 _abilityinfo_cooldown) (break `/Game/RTSMultiplayer/AbilitySubsystem/Data/S_AbilityInfo` (`self.AbilityInfo`)))
  ;[1 1 1] Spawn spell cast process task.
  (for _array_element (`self.SelectedUnits`)
    (bind _returnvalue_2 (`|SpawnActorFromClass` (`self.SpellCastProcessClass`) (`KismetMathLibrary.MakeTransform` (0.0 0.0 0.0)) "AlwaysSpawn" "OverrideRootScale" _returnvalue (`self.ProjectileClass`) (`self.ChosenTargetHitResult`) (`self.CombatConstants`) (`self.EffectsToApply`) (`self.EffectsConstantsId`) (`self.CorrectTarget`) (`self.CorrectTargetClass`) (`self.EndCastParticleSystem`) _abilityinfo_casttime _abilityinfo_icon _array_element (`self.AbilityInfo`) (`self.Id`) (cast `Pawn` _returnvalue :!pure true)))
    (`/Game/RTSMultiplayer/AbilitySubsystem/Blueprints/AbilityProcess.Initialize` _returnvalue_2 _abilityinfo_consumablecost_2 _abilityinfo_allocatablecost_2 _abilityinfo_statscost_2 _abilityinfo_streamingcost_2)
    (bind _returnvalue_3 (`|GenericCreateObject` "/Game/RTSMultiplayer/TaskSubsystem/Blueprints/General/AbilityProcessTask.AbilityProcessTask_C" (`self.GetOwner`) _returnvalue_2 PlayerController _abilityinfo_class_2 _abilityinfo_cooldown _abilityinfo_abilityrange_2 (`.Location` (`GameplayStatics.BreakHitResult` (`self.ChosenTargetHitResult`)))))
    (bind _asi_task_executor (cast `/Game/RTSMultiplayer/TaskSubsystem/Blueprints/I_TaskExecutor` _array_element)
      (:`then`
        (bind _taskcomponent (`/Game/RTSMultiplayer/TaskSubsystem/Blueprints/I_TaskExecutor.GetTaskComponent` _asi_task_executor))
        (if (`self.QueueTaskModifierDown`)
          (`/Game/RTSMultiplayer/TaskSubsystem/Blueprints/TaskComponent.AddTaskToQueue` _taskcomponent _returnvalue_3)
          (else
            (`/Game/RTSMultiplayer/TaskSubsystem/Blueprints/TaskComponent.SetCurrentTask` _taskcomponent _returnvalue_3))))
      (:`CastFailed`
        (`KismetSystemLibrary.PrintString` "SimpleCombatAbility: instigator must implements I_TaskExecutor interface." true true (struct :`R` 1.0 :`G` 0.038718 :`A` 1.0) 5.0)))))

(fn `AIFindBestTarget`
  (params (PossibleTargets :type "Array of /Game/RTSMultiplayer/RTSCharacters/Blueprints/BaseRTSUnit Object Reference") (Caster :type "/Game/RTSMultiplayer/RTSCharacters/Blueprints/BaseRTSUnit Object Reference"))
  (returns (BestTarget :type "/Game/RTSMultiplayer/RTSCharacters/Blueprints/BaseRTSUnit Object Reference"))
  (locals (MinHealth :type "Float (double-precision)" :default 999999.0) (L_BestTarget :type "/Game/RTSMultiplayer/RTSCharacters/Blueprints/BaseRTSUnit Object Reference"))
  (for _array_element PossibleTargets
    (bind _value (`BlueprintMapLibrary.Map_Find` (`/Game/RTSMultiplayer/StatsSubsystem/Blueprints/StatsComponent.Stats` (`/Game/RTSMultiplayer/RTSCharacters/Blueprints/BaseRTSUnit.StatsComponent` _array_element)) (enumliteral `/Game/RTSMultiplayer/StatsSubsystem/Blueprints/E_Stat` "NewEnumerator0")))
    (bind _returnvalue (/ (break `/Game/RTSMultiplayer/StatsSubsystem/Blueprints/S_Stat` _value) (+ (`.BaseMaximum_6_CE344B0C47CFD1A25C77DDA1AD165190` (break `/Game/RTSMultiplayer/StatsSubsystem/Blueprints/S_Stat` _value)) (`.MaximumBoost_7_EAA8C9EC457DC663ED67AC9ADA29B6FE` (break `/Game/RTSMultiplayer/StatsSubsystem/Blueprints/S_Stat` _value)))))
    (if (< _returnvalue (`local.MinHealth`))
      (set `local.MinHealth` _returnvalue)
      (set `local.L_BestTarget` _array_element)))
  (return (`local.L_BestTarget`)))

(fn `CheckResourcesAvailability`
  (params (Actors :type "Array of Actor Object Reference"))
  (returns (AbleToPayActors :type "Array of Actor Object Reference"))
  (locals (`DoesActorPay?` :type Boolean) (ResultActors :type "Array of Actor Object Reference"))
  (bind ((`StatsCost_32_40B8335549DA9465E8F6F09CDA3E9E24` _statscost)) (break `/Game/RTSMultiplayer/AbilitySubsystem/Data/S_AbilityInfo` (`self.AbilityInfo`)))
  (for _array_element Actors
    (set `local.DoesActorPay?` true)
    (bind _asi_have_stats (cast `/Game/RTSMultiplayer/StatsSubsystem/Blueprints/I_HaveStats` _array_element))
    (bind _statscomponent (`/Game/RTSMultiplayer/StatsSubsystem/Blueprints/I_HaveStats.GetStatsComponent` _asi_have_stats))
    (bind _keys (`BlueprintMapLibrary.Map_Keys` _statscost))
    (for _array_element_2 _keys
      (bind (_value _returnvalue) (`BlueprintMapLibrary.Map_Find` (`/Game/RTSMultiplayer/StatsSubsystem/Blueprints/StatsComponent.Stats` _statscomponent) _array_element_2))
      (if _returnvalue
        (if (not (<= (`BlueprintMapLibrary.Map_Find` _statscost _array_element_2) (break `/Game/RTSMultiplayer/StatsSubsystem/Blueprints/S_Stat` _value)))
          (set `local.DoesActorPay?` false :!label _label)
          (break))
        (else
          (goto _label))))
    (if (`local.DoesActorPay?`)
      (`KismetArrayLibrary.Array_Add` (`local.ResultActors`) _array_element)))
  (return (`local.ResultActors`)))

(fn `IsTargetCorrect?`
  (params (HitResult :type "HitResult Structure (by ref)"))
  (returns (AbleToCast :type Boolean))
  (if (`.AOEAbility?_47_9DF26F2A47AC2284D8A6719B65410CF9` (break `/Game/RTSMultiplayer/AbilitySubsystem/Data/S_AbilityInfo` (`self.AbilityInfo`)))
    (return true)
    (else
      (bind _asi_able_to_fight (cast `/Game/RTSMultiplayer/CombatSubsystem/Blueprints/I_AbleToFight` (`.HitActor` (`GameplayStatics.BreakHitResult` HitResult)))
        (:`then`
          (bind _faction (`/Game/RTSMultiplayer/CombatSubsystem/Blueprints/I_AbleToFight.GetFactionAsAbleToFight` _asi_able_to_fight))
          (return (`|EnumEquality` (`/Game/RTSMultiplayer/RTSCharacters/Blueprints/BasePlayerCharacter.GetRelationships` (cast `/Game/RTSMultiplayer/RTSCharacters/Blueprints/BasePlayerCharacter` (`self.GetOwner`) :!pure true) _faction) (`self.CorrectTarget`))))
        (:`CastFailed`
          (return false))))))

(fn `UserConstructionScript`
  (`parent.UserConstructionScript`))