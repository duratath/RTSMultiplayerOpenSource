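; Channelled combat ability for the RTS that gives each selected unit its own channeling process and a task to perform it.
; Its SpawnPossibleProcessTask override spawns a ChannelingProcess actor per unit, initialized with the chosen target, cast time, combat constants and resource costs, including streaming.
; An AbilityProcessTask wraps each process and goes to the unit's task component through I_TaskExecutor, either queued with the modifier held or replacing the current task.
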(event `self.SpawnPossibleProcessTask`
  (params (PlayerController :type "/Game/RTSMultiplayer/RTSCharacters/Blueprints/RTSPlayerController Object Reference"))
  (bind _returnvalue (`self.GetOwner`))
  (bind (_abilityinfo_class _abilityinfo_icon _abilityinfo_isserving_ _abilityinfo_isonetimeuse_ _abilityinfo_displayedname _abilityinfo_displayeddescription _abilityinfo_consumablecost _abilityinfo_allocatablecost _abilityinfo_statscost _abilityinfo_streamingcost _abilityinfo_abilityrange _abilityinfo_casttime _abilityinfo_cooldown) (break `/Game/RTSMultiplayer/AbilitySubsystem/Data/S_AbilityInfo` (`self.AbilityInfo`)))
  (bind _combatconstants (`self.CombatConstants`))
  (bind (_chosentargethitresult_bblockinghit _chosentargethitresult_binitialoverlap _chosentargethitresult_time _chosentargethitresult_distance _chosentargethitresult_location) (`GameplayStatics.BreakHitResult` (`self.ChosenTargetHitResult`)))
  (bind ((`Icon_6_02A18FEC48E53E41B3DAED9F1C4FC50F` _icon) (`StreamingCost_56_46CD57F148A7D646CB494DA55173A248` _streamingcost) (`CastTime_39_30BE88CD4E8BE0C00F87CA8DDD9798B0` _casttime)) (break `/Game/RTSMultiplayer/AbilitySubsystem/Data/S_AbilityInfo` (`self.AbilityInfo`)))
  ;[1 1 1] Override SpawnPossibleProcessTask and spawn specified ChannelingProcess.
  (for _array_element (`self.SelectedUnits`)
    (bind _returnvalue_2 (`|SpawnActorFromClass` (`self.ChannelingProcessClass`) (`KismetMathLibrary.MakeTransform` (0.0 0.0 0.0)) "AlwaysSpawn" "OverrideRootScale" _returnvalue (`.TickFrequency_14_9CA2529D4A94AC9D976B6FB984571F17` (break `/Game/RTSMultiplayer/AbilitySubsystem/Data/S_AbilityCombatConstants` _combatconstants)) (`self.ChosenTargetHitResult`) _combatconstants (`self.CorrectTarget`) (`self.CorrectTargetClass`) _casttime _icon _array_element (`self.AbilityInfo`) (`self.Id`) (cast `Pawn` _returnvalue :!pure true)))
    (`/Game/RTSMultiplayer/AbilitySubsystem/Blueprints/AbilityProcess.Initialize` _returnvalue_2 _abilityinfo_consumablecost _abilityinfo_allocatablecost _abilityinfo_statscost _abilityinfo_streamingcost)
    (bind _returnvalue_3 (`|GenericCreateObject` "/Game/RTSMultiplayer/TaskSubsystem/Blueprints/General/AbilityProcessTask.AbilityProcessTask_C" (`self.GetOwner`) _returnvalue_2 PlayerController _abilityinfo_class _abilityinfo_cooldown _abilityinfo_abilityrange _chosentargethitresult_location))
    (bind _asi_task_executor (cast `/Game/RTSMultiplayer/TaskSubsystem/Blueprints/I_TaskExecutor` _array_element)
      (:`then`
        (bind _taskcomponent (`/Game/RTSMultiplayer/TaskSubsystem/Blueprints/I_TaskExecutor.GetTaskComponent` _asi_task_executor))
        (if (`self.QueueTaskModifierDown`)
          (`/Game/RTSMultiplayer/TaskSubsystem/Blueprints/TaskComponent.AddTaskToQueue` _taskcomponent _returnvalue_3)
          (else
            (`/Game/RTSMultiplayer/TaskSubsystem/Blueprints/TaskComponent.SetCurrentTask` _taskcomponent _returnvalue_3))))
      (:`CastFailed`
        (`KismetSystemLibrary.PrintString` "ChanneledCombatAbility: instigator must implements I_TaskExecutor interface." true true (struct :`R` 1.0 :`G` 0.038718 :`A` 1.0) 5.0)))))

(fn `UserConstructionScript`
  (`parent.UserConstructionScript`))