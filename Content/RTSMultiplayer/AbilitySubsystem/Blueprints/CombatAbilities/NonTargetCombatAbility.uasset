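; Combat ability that needs no target and applies its effects directly to the selected casting units in the RTS.
; On use it pays the cost, spawns and applies each configured effect with the caster as target, then destroys itself.
; It also gives each caster a spell-cast process task via I_TaskExecutor, intended only to start the cooldown.
; That process uses the first selected unit as hit actor and location.
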(event `ApplyEffects`
  ;[1 1 1] Apply effects on casters.
  (for _array_element (`self.SelectedUnits`)
    (for (_array_element_2 _array_index) (`self.EffectsToApply`)
      (bind _returnvalue (`|SpawnActorFromClass` _array_element_2 (`KismetMathLibrary.MakeTransform` (0.0 0.0 0.0)) "AlwaysSpawn" "OverrideRootScale" (`self.GetOwner`) _array_element (`self.CombatConstants`) (`|GetArrayItem` (`self.EffectsConstantsId`) _array_index) _array_element (`self.GetInstigator`)))
      (`/Game/RTSMultiplayer/EffectsSubsystem/Blueprints/SimpleEffect.Apply` _returnvalue))))

(event `self.Use`
  (params (Units :type "Array of Actor Object Reference (by ref)"))
  ;[1 1 1] Use event.
  (`self.SetSelectedUnits` Units)
  (`self.PayForAbility` Units)
  (`self.ApplyEffects`)
  (`self.SpawnPossibleProcessTask` (cast `/Game/RTSMultiplayer/RTSCharacters/Blueprints/RTSPlayerController` (`GameplayStatics.GetPlayerController` 0) :!pure true))
  (`self.DestroyAbility`))

(event `self.SpawnPossibleProcessTask`
  (params (PlayerController :type "/Game/RTSMultiplayer/RTSCharacters/Blueprints/RTSPlayerController Object Reference"))
  (bind _returnvalue (`self.GetOwner`))
  (bind (_abilityinfo_class _abilityinfo_icon _abilityinfo_isserving_ _abilityinfo_isonetimeuse_ _abilityinfo_displayedname _abilityinfo_displayeddescription _abilityinfo_consumablecost _abilityinfo_allocatablecost _abilityinfo_statscost _abilityinfo_streamingcost _abilityinfo_abilityrange _abilityinfo_casttime) (break `/Game/RTSMultiplayer/AbilitySubsystem/Data/S_AbilityInfo` (`self.AbilityInfo`)))
  (bind (_abilityinfo_class_2 _abilityinfo_icon_2 _abilityinfo_isserving__2 _abilityinfo_isonetimeuse__2 _abilityinfo_displayedname_2 _abilityinfo_displayeddescription_2 _abilityinfo_consumablecost_2 _abilityinfo_allocatablecost_2 _abilityinfo_statscost_2 _abilityinfo_streamingcost_2 _abilityinfo_abilityrange_2 _abilityinfo_casttime_2 _abilityinfo_cooldown) (break `/Game/RTSMultiplayer/AbilitySubsystem/Data/S_AbilityInfo` (`self.AbilityInfo`)))
  (bind _output (`|GetArrayItem` (`self.SelectedUnits`)))
  ;[1 1 1] Spawn spell cast process task to start a cooldown only.
  (for _array_element (`self.SelectedUnits`)
    (bind _returnvalue_2 (`|SpawnActorFromClass` :`Class` (`self.SpellCastProcessClass`) :`SpawnTransform` (`KismetMathLibrary.MakeTransform` (0.0 0.0 0.0)) :`CollisionHandlingOverride` "AlwaysSpawn" :`TransformScaleMethod` "OverrideRootScale" :`Owner` _returnvalue :`ProjectileClass` (`self.ProjectileClass`) :`HitResult` (`GameplayStatics.MakeHitResult` false false 0.0 0.0 (`self.K2_GetActorLocation` _output) (0.0 0.0 0.0) (0.0 0.0 1.0) (0.0 0.0 1.0) null _output) :`AbilityConstants` (`self.CombatConstants`) :`CorrectTarget` (`self.CorrectTarget`) :`CorrectTargetClass` (`self.CorrectTargetClass`) :`EndCastParticleSystem` null :`ProcessTime` _abilityinfo_casttime :`ProcessIcon` _abilityinfo_icon :`ProcessInstigator` _array_element :`AbilityInfo` (`self.AbilityInfo`) :`AbilityId` (`self.Id`) :`Instigator` (cast `Pawn` _returnvalue :!pure true)))
    (`/Game/RTSMultiplayer/AbilitySubsystem/Blueprints/AbilityProcess.Initialize` _returnvalue_2 _abilityinfo_consumablecost_2 _abilityinfo_allocatablecost_2 _abilityinfo_statscost_2 _abilityinfo_streamingcost_2)
    (bind _returnvalue_3 (`|GenericCreateObject` "/Game/RTSMultiplayer/TaskSubsystem/Blueprints/General/AbilityProcessTask.AbilityProcessTask_C" (`self.GetOwner`) _returnvalue_2 PlayerController _abilityinfo_class_2 _abilityinfo_cooldown _abilityinfo_abilityrange_2 (`self.K2_GetActorLocation` (`|GetArrayItem` (`self.SelectedUnits`)))))
    (bind _asi_task_executor (cast `/Game/RTSMultiplayer/TaskSubsystem/Blueprints/I_TaskExecutor` _array_element)
      (:`then`
        (bind _taskcomponent (`/Game/RTSMultiplayer/TaskSubsystem/Blueprints/I_TaskExecutor.GetTaskComponent` _asi_task_executor))
        (`/Game/RTSMultiplayer/TaskSubsystem/Blueprints/TaskComponent.SetCurrentTask` _taskcomponent _returnvalue_3))
      (:`CastFailed`
        (`KismetSystemLibrary.PrintString` "RageAbility: instigator must implements I_TaskExecutor interface." true true (struct :`R` 1.0 :`G` 0.038718 :`A` 1.0) 5.0)))))

(fn `UserConstructionScript`
  (`parent.UserConstructionScript`))