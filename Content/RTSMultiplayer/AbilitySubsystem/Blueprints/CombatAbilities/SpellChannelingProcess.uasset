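; Ability process actor for a channeled spell that periodically deals damage and healing to one target or an area.
; On start it turns the caster toward the hit location, spawns an effect and runs a looping timer.
; Area hits use a tagged-component sphere overlap filtered by faction and class, while a gated Tick keeps single-target beams aimed and sized toward the caster.
; End and abort clean up, with abort also multicasting process removal.
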(event `SpawnPossibleTargetParticleSystem`
  (bind _attachedparticlesystemcomponent (`self.AttachedParticleSystemComponent`))
  (bind (_hitresult_bblockinghit _hitresult_binitialoverlap _hitresult_time _hitresult_distance _hitresult_location _hitresult_impactpoint _hitresult_normal _hitresult_impactnormal _hitresult_physmat _hitresult_hitactor) (`GameplayStatics.BreakHitResult` (`self.HitResult`)))
  (bind _returnvalue (`self.K2_GetActorLocation` (`self.ProcessInstigator`)))
  (bind _returnvalue_2 (`self.K2_GetActorLocation` _hitresult_hitactor))
  (bind _returnvalue_3 (`self.K2_GetActorLocation` (`self.ProcessInstigator`)))
  (bind _returnvalue_4 (`self.K2_GetActorLocation` _hitresult_hitactor))
  (bind _rootcomponent (`Actor.RootComponent` _hitresult_hitactor))
  (bind _rootcomponent_2 (`Actor.RootComponent` _hitresult_hitactor))
  (bind (_returnvalue_roll _returnvalue_pitch _returnvalue_yaw) (`KismetMathLibrary.BreakRotator` (`SceneComponent.K2_GetComponentRotation` _rootcomponent_2)))
  (bind (_returnvalue_roll_2 _returnvalue_pitch_2 _returnvalue_yaw_2) (`KismetMathLibrary.BreakRotator` (`KismetMathLibrary.FindLookAtRotation` _returnvalue_2 _returnvalue)))
  (bind (_returnvalue_roll_3 _returnvalue_pitch_3 _returnvalue_yaw_3) (`KismetMathLibrary.BreakRotator` (`KismetMathLibrary.FindLookAtRotation` _returnvalue_4 _returnvalue_3)))
  (bind (_returnvalue_roll_4 _returnvalue_pitch_4 _returnvalue_yaw_4) (`KismetMathLibrary.BreakRotator` (`SceneComponent.K2_GetComponentRotation` _rootcomponent)))
  ;[1 1 1] Spawn and destroy possible particle system. Rotate beem on tick.
  (`/Engine/EditorBlueprintResources/StandardMacros.IsValid` _hitresult_hitactor
    (:`Is Valid`
      (bind _onapplyparticlesystem (`self.OnApplyParticleSystem`)
        (:`then`
          (bind _returnvalue_5 (`GameplayStatics.SpawnEmitterAttached` _onapplyparticlesystem _rootcomponent "None" (0.0 0.0 0.0) (`KismetMathLibrary.MakeRotator` (- _returnvalue_roll_3 _returnvalue_roll_4) (- _returnvalue_pitch_3 _returnvalue_pitch_4) (- _returnvalue_yaw_3 _returnvalue_yaw_4)) (1.0 1.0 1.0) "KeepRelativeOffset" false))
          (`ParticleSystemComponent.SetFloatParameter` _returnvalue_5 "BeamLength" (`KismetMathLibrary.VSize` (- _returnvalue_3 _returnvalue_4)))
          (set `self.AttachedParticleSystemComponent` _returnvalue_5)
          (goto _label :!via `Open`))
        (:`else`)))))

(event `self.StartProcess`
  (bind _processinstigator (`self.ProcessInstigator`))
  (bind (_hitresult_bblockinghit _hitresult_binitialoverlap _hitresult_time _hitresult_distance _hitresult_location) (`GameplayStatics.BreakHitResult` (`self.HitResult`)))
  (bind (_returnvalue_roll _returnvalue_pitch) (`KismetMathLibrary.BreakRotator` (`self.K2_GetActorRotation` _processinstigator)))
  (bind (_returnvalue_roll_2 _returnvalue_pitch_2 _returnvalue_yaw) (`KismetMathLibrary.BreakRotator` (`KismetMathLibrary.FindLookAtRotation` (`self.K2_GetActorLocation` _processinstigator) _hitresult_location)))
  ;[1 1 1] Set tick timer and rotate executor on start process.
  (`parent.StartProcess`)
  (`SceneComponent.K2_SetWorldRotation` (`Actor.RootComponent` _processinstigator) (`KismetMathLibrary.MakeRotator` _returnvalue_roll _returnvalue_pitch _returnvalue_yaw) false false)
  (bind _returnvalue (`KismetSystemLibrary.K2_SetTimerDelegate` (`|CreateDelegate` :!event `OnChanneledSpellTick`) (`self.TickFrequency`) true))
  (set `self.TickHandle` _returnvalue)
  (if (`.AOEAbility?_47_9DF26F2A47AC2284D8A6719B65410CF9` (break `/Game/RTSMultiplayer/AbilitySubsystem/Data/S_AbilityInfo` (`self.AbilityInfo`)))
    (`self.SpawnPossubleAOEParticleSystem`)
    (else
      (`self.SpawnPossibleTargetParticleSystem`))))

(event `self.ReceiveTick`
  (params (DeltaSeconds :type "Float (single-precision)"))
  (bind _attachedparticlesystemcomponent (`self.AttachedParticleSystemComponent`))
  (bind (_hitresult_bblockinghit _hitresult_binitialoverlap _hitresult_time _hitresult_distance _hitresult_location _hitresult_impactpoint _hitresult_normal _hitresult_impactnormal _hitresult_physmat _hitresult_hitactor) (`GameplayStatics.BreakHitResult` (`self.HitResult`)))
  (bind _returnvalue (`self.K2_GetActorLocation` (`self.ProcessInstigator`)))
  (bind _returnvalue_2 (`self.K2_GetActorLocation` _hitresult_hitactor))
  (bind _rootcomponent (`Actor.RootComponent` _hitresult_hitactor))
  (bind (_returnvalue_roll _returnvalue_pitch _returnvalue_yaw) (`KismetMathLibrary.BreakRotator` (`SceneComponent.K2_GetComponentRotation` _rootcomponent)))
  (bind (_returnvalue_roll_2 _returnvalue_pitch_2 _returnvalue_yaw_2) (`KismetMathLibrary.BreakRotator` (`KismetMathLibrary.FindLookAtRotation` _returnvalue_2 _returnvalue)))
  ;[1 1 1] Spawn and destroy possible particle system. Rotate beem on tick.
  (`/Engine/EditorBlueprintResources/StandardMacros.Gate` true :!label _label
    (:`Exit`
      (`/Engine/EditorBlueprintResources/StandardMacros.IsValid` _hitresult_hitactor
        (:`Is Valid`
          (`/Engine/EditorBlueprintResources/StandardMacros.IsValid` _rootcomponent
            (:`Is Valid`
              (`SceneComponent.K2_SetRelativeRotation` _attachedparticlesystemcomponent (`KismetMathLibrary.MakeRotator` (- _returnvalue_roll_2 _returnvalue_roll) (- _returnvalue_pitch_2 _returnvalue_pitch) (- _returnvalue_yaw_2 _returnvalue_yaw)) false false)
              (`ParticleSystemComponent.SetFloatParameter` _attachedparticlesystemcomponent "BeamLength" (`KismetMathLibrary.VSize` (- _returnvalue _returnvalue_2))))))))))

(event `DestroyPossibleParticleSystem`
  ;[1 1 1] Spawn and destroy possible particle system. Rotate beem on tick.
  (bind _attachedparticlesystemcomponent (`self.AttachedParticleSystemComponent`)
    (:`then`
      (`ActorComponent.K2_DestroyComponent` _attachedparticlesystemcomponent)
      (goto _label :!via `Close`))
    (:`else`)))

(event `SpawnPossubleAOEParticleSystem`
  (bind (_hitresult_bblockinghit _hitresult_binitialoverlap _hitresult_time _hitresult_distance _hitresult_location _hitresult_impactpoint _hitresult_normal _hitresult_impactnormal _hitresult_physmat _hitresult_hitactor) (`GameplayStatics.BreakHitResult` (`self.HitResult`)))
  ;[1 1 1] Spawn and destroy possible particle system. Rotate beem on tick.
  (bind _onapplyparticlesystem (`self.OnApplyParticleSystem`)
    (:`then`
      (bind _returnvalue (`GameplayStatics.SpawnEmitterAtLocation` _onapplyparticlesystem _hitresult_location (struct) (1.0 1.0 1.0) false))
      (set `self.AttachedParticleSystemComponent` _returnvalue))
    (:`else`)))

(event `OnChanneledSpellTick`
  ;[1 1 1] On channeled spell tick.
  (if (`.AOEAbility?_47_9DF26F2A47AC2284D8A6719B65410CF9` (break `/Game/RTSMultiplayer/AbilitySubsystem/Data/S_AbilityInfo` (`self.AbilityInfo`)))
    (`self.TryDealDamageAndHealAOE`)
    (else
      (`self.TryDealDamageAndHealTarget`))))

(event `self.AbortProcess`
  ;[1 1 1] Abort/end process.
  (`KismetSystemLibrary.K2_ClearAndInvalidateTimerHandle` (`self.TickHandle`))
  (`self.MakeAmendsClient`)
  (`self.AbortProcessMulticast`)
  (`self.DestroyPossibleParticleSystem`)
  (`self.K2_DestroyActor`))

(event `self.AbortProcessMulticast`
  ;[1 1 1] Abort/end process.
  (`TimelineComponent.Stop` (`self.ProcessTimeline`))
  (bind _asi_have_abilities (cast `/Game/RTSMultiplayer/AbilitySubsystem/Blueprints/I_HaveAbilities` (`self.ProcessInstigator`)))
  (bind _abilitycomponent (`/Game/RTSMultiplayer/AbilitySubsystem/Blueprints/I_HaveAbilities.GetAbilityComponent` _asi_have_abilities))
  (`/Game/RTSMultiplayer/AbilitySubsystem/Blueprints/AbilityComponent.RemoveProcess` _abilitycomponent self)
  (`/Game/RTSMultiplayer/AbilitySubsystem/Blueprints/AbilityComponent.CallProcessRemoved` _abilitycomponent)
  (bind _asi_task_executor (cast `/Game/RTSMultiplayer/TaskSubsystem/Blueprints/I_TaskExecutor` (`self.ProcessInstigator`))
    (:`then`
      (bind _taskcomponent (`/Game/RTSMultiplayer/TaskSubsystem/Blueprints/I_TaskExecutor.GetTaskComponent` _asi_task_executor))
      (bind _asability_process_task (cast `/Game/RTSMultiplayer/TaskSubsystem/Blueprints/General/AbilityProcessTask` (`|GetArrayItem` (`/Game/RTSMultiplayer/TaskSubsystem/Blueprints/TaskComponent.TaskQueue` _taskcomponent)))
        (:`then`
          (bind _abilityprocess (`/Game/RTSMultiplayer/TaskSubsystem/Blueprints/General/AbilityProcessTask.AbilityProcess` _asability_process_task)
            (:`then`
              (if (== _abilityprocess self)
                (`self.ProcessCompleted`)
                (else
                  (`self.ProcessAborted` :!label _label_2))))
            (:`else`
              (goto _label_2))))
        (:`CastFailed`
          (goto _label_2))))
    (:`CastFailed`
      (`self.ProcessCompleted`))))

(event `self.EndProcess`
  ;[1 1 1] Abort/end process.
  (`KismetSystemLibrary.K2_ClearAndInvalidateTimerHandle` (`self.TickHandle`))
  (`parent.EndProcess`)
  (`self.DestroyPossibleParticleSystem`)
  (`self.K2_DestroyActor`))

(event `TryDealDamageAndHealTarget`
  (bind (_hitresult_bblockinghit _hitresult_binitialoverlap _hitresult_time _hitresult_distance _hitresult_location _hitresult_impactpoint _hitresult_normal _hitresult_impactnormal _hitresult_physmat _hitresult_hitactor) (`GameplayStatics.BreakHitResult` (`self.HitResult`)))
  (bind (_abilityconstants_basedamage _abilityconstants_basehealing _abilityconstants_effectbaseduration _abilityconstants_tickfrequency _abilityconstants_tickdamage _abilityconstants_tickhealing _abilityconstants_damagetype) (break `/Game/RTSMultiplayer/AbilitySubsystem/Data/S_AbilityCombatConstants` (`self.AbilityConstants`)))
  (bind (_abilityconstants_basedamage_2 _abilityconstants_basehealing_2 _abilityconstants_effectbaseduration_2 _abilityconstants_tickfrequency_2 _abilityconstants_tickdamage_2 _abilityconstants_tickhealing_2) (break `/Game/RTSMultiplayer/AbilitySubsystem/Data/S_AbilityCombatConstants` (`self.AbilityConstants`)))
  (bind (_abilityconstants_basedamage_3 _abilityconstants_basehealing_3 _abilityconstants_effectbaseduration_3 _abilityconstants_tickfrequency_3 _abilityconstants_tickdamage_3 _abilityconstants_tickhealing_3) (break `/Game/RTSMultiplayer/AbilitySubsystem/Data/S_AbilityCombatConstants` (`self.AbilityConstants`)))
  (bind (_abilityconstants_basedamage_4 _abilityconstants_basehealing_4 _abilityconstants_effectbaseduration_4 _abilityconstants_tickfrequency_4 _abilityconstants_tickdamage_4) (break `/Game/RTSMultiplayer/AbilitySubsystem/Data/S_AbilityCombatConstants` (`self.AbilityConstants`)))
  ;[1 1 1] Try deal damage and heal specified target if necessary.
  (if (!= _abilityconstants_tickdamage_4 0.0)
    (bind _asi_able_to_fight (cast `/Game/RTSMultiplayer/CombatSubsystem/Blueprints/I_AbleToFight` (`self.ProcessInstigator`))
      (:`then`
        (bind _combatcomponent (`/Game/RTSMultiplayer/CombatSubsystem/Blueprints/I_AbleToFight.GetCombatComponent` _asi_able_to_fight))
        (`/Engine/EditorBlueprintResources/StandardMacros.IsValid` _hitresult_hitactor
          (:`Is Valid`
            (bind _asi_able_to_fight_2 (cast `/Game/RTSMultiplayer/CombatSubsystem/Blueprints/I_AbleToFight` _hitresult_hitactor))
            (bind _combatcomponent_2 (`/Game/RTSMultiplayer/CombatSubsystem/Blueprints/I_AbleToFight.GetCombatComponent` _asi_able_to_fight_2))
            (`/Game/RTSMultiplayer/CombatSubsystem/Blueprints/CombatComponent.ReceiveDamage` _combatcomponent_2 (make `/Game/RTSMultiplayer/CombatSubsystem/Blueprints/S_DamageInfo` _abilityconstants_damagetype (`/Game/RTSMultiplayer/CombatSubsystem/Blueprints/CombatComponent.WeaponType` _combatcomponent) _abilityconstants_tickdamage))
            (if (!= _abilityconstants_tickhealing_2 0.0) :!label _label_3
              (`/Engine/EditorBlueprintResources/StandardMacros.IsValid` _hitresult_hitactor
                (:`Is Valid`
                  (bind _asi_able_to_fight_3 (cast `/Game/RTSMultiplayer/CombatSubsystem/Blueprints/I_AbleToFight` _hitresult_hitactor)
                    (:`then`
                      (bind _combatcomponent_3 (`/Game/RTSMultiplayer/CombatSubsystem/Blueprints/I_AbleToFight.GetCombatComponent` _asi_able_to_fight_3))
                      (`/Game/RTSMultiplayer/CombatSubsystem/Blueprints/CombatComponent.ReceiveHealing` _combatcomponent_3 _abilityconstants_tickhealing_3))
                    (:`CastFailed`
                      (`KismetSystemLibrary.PrintString` "SpellCastProcess: instigator and target must implement I_AbleToFight interface." true true (struct :`R` 1.0 :`G` 0.038718 :`A` 1.0) 5.0 :!label _label_4)))))))))
      (:`CastFailed`
        (goto _label_4)))
    (else
      (goto _label_3))))

(event `TryDealDamageAndHealAOE`
  (bind ((`EffectBaseDuration_21_F507FA954AE69DE36891B6B09B366D74` _effectbaseduration) (`TickDamage_19_29E7014941C65001BC63D5A87C5CEECC` _tickdamage) (`TickHealing_20_B12222B44650394F01B97B9A35563B6F` _tickhealing) (`DamageType_11_13F3D90246A8A8D2C591B190B076806C` _damagetype)) (break `/Game/RTSMultiplayer/AbilitySubsystem/Data/S_AbilityCombatConstants` (`self.AbilityConstants`)))
  (bind ((`EffectBaseDuration_21_F507FA954AE69DE36891B6B09B366D74` _effectbaseduration_2) (`TickDamage_19_29E7014941C65001BC63D5A87C5CEECC` _tickdamage_2) (`TickHealing_20_B12222B44650394F01B97B9A35563B6F` _tickhealing_2)) (break `/Game/RTSMultiplayer/AbilitySubsystem/Data/S_AbilityCombatConstants` (`self.AbilityConstants`)))
  ;[1 1 1] Try deal damage and heal AOE if necessary.
  (if (or (!= _tickdamage_2 0.0) (!= _tickhealing_2 0.0))
    (bind _actors (`self.GetOverlappedAbleToFightActors`))
    (for _array_element _actors
      (bind _asi_able_to_fight (cast `/Game/RTSMultiplayer/CombatSubsystem/Blueprints/I_AbleToFight` _array_element))
      (bind _faction (`/Game/RTSMultiplayer/CombatSubsystem/Blueprints/I_AbleToFight.GetFactionAsAbleToFight` _asi_able_to_fight))
      (if (`|EnumEquality` (`/Game/RTSMultiplayer/RTSCharacters/Blueprints/BasePlayerCharacter.GetRelationships` (cast `/Game/RTSMultiplayer/RTSCharacters/Blueprints/BasePlayerCharacter` (`self.GetOwner`) :!pure true) _faction) (`self.CorrectTarget`))
        (if (== (`self.CorrectTargetClass`) null)
          (bind _combatcomponent (`/Game/RTSMultiplayer/CombatSubsystem/Blueprints/I_AbleToFight.GetCombatComponent` _asi_able_to_fight :!label _label_5))
          (if (!= _tickdamage 0.0)
            (bind _asi_able_to_fight_2 (cast `/Game/RTSMultiplayer/CombatSubsystem/Blueprints/I_AbleToFight` (`self.ProcessInstigator`))
              (:`then`
                (bind _combatcomponent_2 (`/Game/RTSMultiplayer/CombatSubsystem/Blueprints/I_AbleToFight.GetCombatComponent` _asi_able_to_fight_2))
                (`/Game/RTSMultiplayer/CombatSubsystem/Blueprints/CombatComponent.ReceiveDamage` _combatcomponent (make `/Game/RTSMultiplayer/CombatSubsystem/Blueprints/S_DamageInfo` _damagetype (`/Game/RTSMultiplayer/CombatSubsystem/Blueprints/CombatComponent.WeaponType` _combatcomponent_2) _tickdamage))
                (if (!= _tickhealing 0.0) :!label _label_6
                  (`/Game/RTSMultiplayer/CombatSubsystem/Blueprints/CombatComponent.ReceiveHealing` _combatcomponent _tickhealing)))
              (:`CastFailed`
                (`KismetSystemLibrary.PrintString` "SpellCastProcess: process instigator must implement I_AbleToFight interface." true true (struct :`R` 1.0 :`G` 0.038718 :`A` 1.0) 5.0)))
            (else
              (goto _label_6)))
          (elif (`KismetMathLibrary.ClassIsChildOf` (`GameplayStatics.GetObjectClass` _array_element) (`self.CorrectTargetClass`))
            (goto _label_5)))))))

(fn `GetOverlappedAbleToFightActors`
  (returns (Actors :type "Array of Actor Object Reference"))
  (locals (Result :type "Array of Actor Object Reference"))
  (bind (_hitresult_bblockinghit _hitresult_binitialoverlap _hitresult_time _hitresult_distance _hitresult_location) (`GameplayStatics.BreakHitResult` (`self.HitResult`)))
  (bind _outcomponents (`KismetSystemLibrary.SphereOverlapComponents` _hitresult_location (`.AOERadius_51_317D0B6A49E5F0E8833AA8B676668C71` (break `/Game/RTSMultiplayer/AbilitySubsystem/Data/S_AbilityInfo` (`self.AbilityInfo`))) (`|MakeArray` "ObjectTypeQuery1" "ObjectTypeQuery2" "ObjectTypeQuery3" :!type "EObjectTypeQuery Enum") "/Script/Engine.PrimitiveComponent"))
  (for _array_element _outcomponents
    (if (`ActorComponent.ComponentHasTag` _array_element "AOEAbilityCollision")
      (bind _returnvalue (`ActorComponent.GetOwner` _array_element))
      (cast `/Game/RTSMultiplayer/CombatSubsystem/Blueprints/I_AbleToFight` _returnvalue)
      (`KismetArrayLibrary.Array_Add` (`local.Result`) _returnvalue)))
  (return (`local.Result`)))

(fn `UserConstructionScript`
  (`parent.UserConstructionScript`))