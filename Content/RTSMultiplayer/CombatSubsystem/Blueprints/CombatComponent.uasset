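; Actor component that handles attacking, taking damage, healing and death for RTS units and other actors, with damage and weapon types read from a data table.
; Attack saves the target and damage info, and AttackCallback later applies them to the target's CombatComponent.
; Incoming damage passes through type modifiers, armor or magic resistance, and absorb effects before reducing the owner's stat.
; On death, units play a montage before destruction, while other actors are destroyed immediately.
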(event `self.ReceiveBeginPlay`
  ;[1 1 1] Begin play. Set damage and weapon type from data table.
  (bind _asi_have_stats (cast `/Game/RTSMultiplayer/StatsSubsystem/Blueprints/I_HaveStats` (`self.GetOwner`))
    (:`then`
      (bind _id (`/Game/RTSMultiplayer/StatsSubsystem/Blueprints/I_HaveStats.GetIdAsHaveStats` _asi_have_stats))
      (bind _returnvalue (`|GetDataTableRow` "/Game/RTSMultiplayer/CombatSubsystem/Data/ActorsCombatInfoDataTable.ActorsCombatInfoDataTable" _id)
        (:`then`
          (set `self.DamageType` (break `/Game/RTSMultiplayer/CombatSubsystem/Data/S_ActorCombatInfo` _returnvalue))
          (set `self.WeaponType` (`.WeaponType_5_2F015F63484A60FB517CD19F61642851` (break `/Game/RTSMultiplayer/CombatSubsystem/Data/S_ActorCombatInfo` _returnvalue))))
        (:`RowNotFound`
          (`KismetSystemLibrary.PrintString` "CombatComponent: ActorsCombatInfoDataTable row not found." true true (struct :`R` 1.0 :`G` 0.038718 :`A` 1.0) 5.0))))
    (:`CastFailed`
      (`KismetSystemLibrary.PrintString` "CombatComponent: owner must implement I_HaveStats interface." true true (struct :`R` 1.0 :`G` 0.038718 :`A` 1.0) 5.0))))

(event `ReceiveDamage`
  (params (DamageInfo :type "/Game/RTSMultiplayer/CombatSubsystem/Blueprints/S_DamageInfo Structure"))
  (bind (_damagetype _weapontype _basedamage) (break `/Game/RTSMultiplayer/CombatSubsystem/Blueprints/S_DamageInfo` DamageInfo))
  (bind _returnvalue (`self.GetOwner`))
  ;[1 1 1] Receive damage.
  (if (not (`self.Dead?`))
    (set `self.CurrentReceivingDamage` _basedamage)
    (`self.GetOwnerStats`)
    (`self.ChangeBaseCurrentReceivingDamage` DamageInfo)
    (switch `/Game/RTSMultiplayer/CombatSubsystem/Blueprints/E_DamageType` _damagetype
      (:`NewEnumerator0`
        (`self.ChangeCurrentReceivingDamageByArmor`))
      (:`NewEnumerator1`
        (`self.ChangeCurrentReceivingDamageByMagicResistance`))
      (:`NewEnumerator2`
        _))
    (`self.TryToAbsorbDamage`)
    (if (!= (`self.CurrentReceivingDamage`) 0.0)
      (bind _statscomponent (`self.GetOwnerStatsComponent`))
      (`/Game/RTSMultiplayer/StatsSubsystem/Blueprints/StatsComponent.ChangeCurrentStatValue` _statscomponent "NewEnumerator0" (* -1 (`self.CurrentReceivingDamage`)))
      (bind _stats (`self.GetOwnerStats`))
      (if (<= (break `/Game/RTSMultiplayer/StatsSubsystem/Blueprints/S_Stat` (`BlueprintMapLibrary.Map_Find` _stats (enumliteral `/Game/RTSMultiplayer/StatsSubsystem/Blueprints/E_Stat` "NewEnumerator0"))) 0.0)
        (`self.CallOwnerDeath`)
        (bind _asbase_rtsunit (cast `/Game/RTSMultiplayer/RTSCharacters/Blueprints/BaseRTSUnit` _returnvalue)
          (:`then`
            (set `self.Dead?` true)
            (`CharacterMovementComponent.DisableMovement` (`Character.CharacterMovement` _asbase_rtsunit))
            (`self.PlayDeathAnimation` _asbase_rtsunit))
          (:`CastFailed`
            (`Actor.K2_DestroyActor` _returnvalue)))))))

(event `ReceiveHealing`
  (params (Healing :type "Float (double-precision)"))
  ;[1 1 1] Receive healing.
  (if (not (`self.Dead?`))
    (bind _statscomponent (`self.GetOwnerStatsComponent`))
    (`/Game/RTSMultiplayer/StatsSubsystem/Blueprints/StatsComponent.ChangeCurrentStatValue` _statscomponent "NewEnumerator0" Healing)))

(event `PlayDeathAnimation`
  (params (Unit :type "/Game/RTSMultiplayer/RTSCharacters/Blueprints/BaseRTSUnit Object Reference"))
  (bind (_animmontage _playrate) (`/Game/RTSMultiplayer/RTSCharacters/Blueprints/BaseRTSUnit.GetDeathAnimMontageSettings` Unit))
  ;[1 1 1] Owner death. Play death animation.
  (`/Engine/EditorBlueprintResources/StandardMacros.IsValid` _animmontage
    (:`Is Valid`
      (`Character.PlayAnimMontage` Unit _animmontage _playrate "None")
      (bind _returnvalue (`AnimSequenceBase.GetPlayLength` _animmontage))
      (`KismetSystemLibrary.Delay` (/ _returnvalue _playrate))
      (`Actor.K2_DestroyActor` (`self.GetOwner`)))))

(event `Attack`
  (params (ActorToAttack :type "Actor Object Reference"))
  ;[1 1 1] Attack other actor.
  (`self.CallAttacking`)
  (bind _asi_able_to_fight (cast `/Game/RTSMultiplayer/CombatSubsystem/Blueprints/I_AbleToFight` ActorToAttack)
    (:`then`
      (bind _combatcomponent (`/Game/RTSMultiplayer/CombatSubsystem/Blueprints/I_AbleToFight.GetCombatComponent` _asi_able_to_fight))
      (bind _stats (`self.GetOwnerStats`))
      (bind (_value _returnvalue) (`BlueprintMapLibrary.Map_Find` _stats "NewEnumerator8"))
      (if _returnvalue
        (set `self.SavedTargetCombatComponent` _combatcomponent)
        (set `self.SavedDamageInfo` (make `/Game/RTSMultiplayer/CombatSubsystem/Blueprints/S_DamageInfo` (`self.DamageType`) (`self.WeaponType`) (break `/Game/RTSMultiplayer/StatsSubsystem/Blueprints/S_Stat` _value)))
        (else
          (`KismetSystemLibrary.PrintString` "CombatComponent: Owner doesn't have Damage stat." true true (struct :`R` 1.0 :`G` 0.038718 :`A` 1.0) 5.0))))
    (:`CastFailed`
      (`KismetSystemLibrary.PrintString` "CombatComponent: Actor to Attack must implement I_AbleToFight interface." true true (struct :`R` 1.0 :`G` 0.038718 :`A` 1.0) 5.0))))

(event `CallOwnerDeath`
  ;[1 1 1] Owner death. Play death animation.
  (`self.OwnerDeath` (`self.GetOwner`)))

(event `CallAttacking`
  ;[1 1 1] Attack other actor.
  (`self.Attacking` (`self.GetOwner`)))

(event `AttackCallback`
  ;[1 1 1] Attack other actor.
  (bind _savedtargetcombatcomponent (`self.SavedTargetCombatComponent`)
    (:`then`
      (`self.ReceiveDamage` _savedtargetcombatcomponent (`self.SavedDamageInfo`))
      (set `self.SavedTargetCombatComponent` null))
    (:`else`)))

(fn `ChangeBaseCurrentReceivingDamage`
  (params (DamageInfo :type "/Game/RTSMultiplayer/CombatSubsystem/Blueprints/S_DamageInfo Structure"))
  (bind (_damagetype _weapontype) (break `/Game/RTSMultiplayer/CombatSubsystem/Blueprints/S_DamageInfo` DamageInfo))
  (bind _asi_able_to_fight (cast `/Game/RTSMultiplayer/CombatSubsystem/Blueprints/I_AbleToFight` (`self.GetOwner`))
    (:`then`
      (bind _damagemodifier (`/Game/RTSMultiplayer/CombatSubsystem/Blueprints/I_AbleToFight.GetDamageReceiveModifierForWeaponType` _asi_able_to_fight _weapontype))
      (set `self.CurrentReceivingDamage` (* (`self.CurrentReceivingDamage`) _damagemodifier))
      (bind _damagemodifier_2 (`/Game/RTSMultiplayer/CombatSubsystem/Blueprints/I_AbleToFight.GetDamageReceiveModifierForDamageType` _asi_able_to_fight _damagetype))
      (set `self.CurrentReceivingDamage` (* (`self.CurrentReceivingDamage`) _damagemodifier_2)))
    (:`CastFailed`
      (`KismetSystemLibrary.PrintString` "CombatComponent: Actor to Attack must implement I_AbleToFight interface." true true (struct :`R` 1.0 :`G` 0.038718 :`A` 1.0) 5.0))))

(fn `ChangeCurrentReceivingDamageByArmor`
  (bind _stats (`self.GetOwnerStats`))
  (bind (_value _returnvalue) (`BlueprintMapLibrary.Map_Find` _stats "NewEnumerator6"))
  (if _returnvalue
    (set `self.CurrentReceivingDamage` (* (`self.CurrentReceivingDamage`) (- 1.0 (`/Game/RTSMultiplayer/StatsSubsystem/Blueprints/StatsFunctionLibrary.ArmorToReducePercentage` (break `/Game/RTSMultiplayer/StatsSubsystem/Blueprints/S_Stat` _value)))))))

(fn `ChangeCurrentReceivingDamageByMagicResistance`
  (bind _stats (`self.GetOwnerStats`))
  (bind (_value _returnvalue) (`BlueprintMapLibrary.Map_Find` _stats "NewEnumerator7"))
  (if _returnvalue
    (set `self.CurrentReceivingDamage` (* (`self.CurrentReceivingDamage`) (- 1.0 (`/Game/RTSMultiplayer/StatsSubsystem/Blueprints/StatsFunctionLibrary.MagicResistanceToReducePercentage` (break `/Game/RTSMultiplayer/StatsSubsystem/Blueprints/S_Stat` _value)))))))

(fn `GetOwnerStats`
  (returns (Stats :type "Map of /Game/RTSMultiplayer/StatsSubsystem/Blueprints/E_Stat Enum to /Game/RTSMultiplayer/StatsSubsystem/Blueprints/S_Stat Structure"))
  (bind _asi_have_stats (cast `/Game/RTSMultiplayer/StatsSubsystem/Blueprints/I_HaveStats` (`self.GetOwner`))
    (:`then`
      (bind _statscomponent (`/Game/RTSMultiplayer/StatsSubsystem/Blueprints/I_HaveStats.GetStatsComponent` _asi_have_stats))
      (return (`/Game/RTSMultiplayer/StatsSubsystem/Blueprints/StatsComponent.Stats` _statscomponent)))
    (:`CastFailed`
      (`KismetSystemLibrary.PrintString` "CombatComponent: owner must implement I_HaveStats interface." true true (struct :`R` 1.0 :`G` 0.038718 :`A` 1.0) 5.0))))

(fn `GetOwnerStatsComponent`
  (returns (StatsComponent :type "/Game/RTSMultiplayer/StatsSubsystem/Blueprints/StatsComponent Object Reference"))
  (bind _asi_have_stats (cast `/Game/RTSMultiplayer/StatsSubsystem/Blueprints/I_HaveStats` (`self.GetOwner`))
    (:`then`
      (bind _statscomponent (`/Game/RTSMultiplayer/StatsSubsystem/Blueprints/I_HaveStats.GetStatsComponent` _asi_have_stats))
      (return _statscomponent))
    (:`CastFailed`
      (`KismetSystemLibrary.PrintString` "CombatComponent: owner must implement I_HaveStats interface." true true (struct :`R` 1.0 :`G` 0.038718 :`A` 1.0) 5.0))))

(fn `TryToAbsorbDamage`
  (bind _asi_effect_receiver (cast `/Game/RTSMultiplayer/EffectsSubsystem/Blueprints/I_EffectReceiver` (`self.GetOwner`)))
  (bind _effectcomponent (`/Game/RTSMultiplayer/EffectsSubsystem/Blueprints/I_EffectReceiver.GetEffectComponent` _asi_effect_receiver))
  (for _array_element (`/Game/RTSMultiplayer/EffectsSubsystem/Blueprints/EffectComponent.CurrentEffects` _effectcomponent)
    (bind _returnvalue (`GameplayStatics.GetObjectClass` _array_element))
    (if (or (== _returnvalue "/Game/RTSMultiplayer/EffectsSubsystem/Blueprints/DamageAbsorbEffect.DamageAbsorbEffect_C") (`KismetMathLibrary.ClassIsChildOf` _returnvalue "/Game/RTSMultiplayer/EffectsSubsystem/Blueprints/DamageAbsorbEffect.DamageAbsorbEffect_C"))
      (bind _asdamage_absorb_effect (cast `/Game/RTSMultiplayer/EffectsSubsystem/Blueprints/DamageAbsorbEffect` _array_element))
      (if (> (`/Game/RTSMultiplayer/EffectsSubsystem/Blueprints/DamageAbsorbEffect.AbsorbAmount` _asdamage_absorb_effect) 0.0)
        (`/Game/RTSMultiplayer/EffectsSubsystem/Blueprints/DamageAbsorbEffect.ReceiveDamage` _asdamage_absorb_effect (`self.CurrentReceivingDamage`))
        (bind _absorbamount (`/Game/RTSMultiplayer/EffectsSubsystem/Blueprints/DamageAbsorbEffect.AbsorbAmount` _asdamage_absorb_effect))
        (if (< _absorbamount 0.0)
          (set `self.CurrentReceivingDamage` (* _absorbamount -1.0))
          (else
            (set `self.CurrentReceivingDamage` 0.0)))))))