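; I_AbleToFight is a Blueprint interface in the RTS multiplayer combat subsystem for anything that can take part in combat.
; It exposes the implementer's combat component, faction and homing target component.
; It also declares calls to start and query an attack cooldown, and to get received-damage modifiers by weapon type and by damage type.
; The functions hold no logic, only empty or default returns.
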(fn `GetCombatComponent`
  (returns (CombatComponent :type "/Game/RTSMultiplayer/CombatSubsystem/Blueprints/CombatComponent Object Reference"))
  (return null))

(fn `GetDamageReceiveModifierForDamageType`
  (params (DamageType :type "/Game/RTSMultiplayer/CombatSubsystem/Blueprints/E_DamageType Enum" :default "NewEnumerator0"))
  (returns (DamageModifier :type "Float (double-precision)"))
  (return 0.0))

(fn `GetDamageReceiveModifierForWeaponType`
  (params (WeaponType :type "/Game/RTSMultiplayer/CombatSubsystem/Blueprints/E_WeaponType Enum" :default "NewEnumerator0"))
  (returns (DamageModifier :type "Float (double-precision)"))
  (return 0.0))

(fn `GetFactionAsAbleToFight`
  (returns (Faction :type "/Game/RTSMultiplayer/RTSCoreBP/E_Faction Enum"))
  (return "NewEnumerator0"))

(fn `GetHomingTargetComponent`
  (returns (HomingTargetComponent :type "PrimitiveComponent Object Reference"))
  (return null))

(fn `IsAttackOnCooldown?`
  (returns (`IsOnCooldown?` :type Boolean))
  (return false))

(fn `StartAttackCooldown`
  (params (CooldownTime :type "Float (double-precision)")))