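; Input receiver for the RTS player controller, handling ability hotkeys, camera rotation and right-click orders.
; Ability keys forward to the HUD ability bar, and gates let mouse axes drive spring arm yaw and clamped pitch while rotate is held.
; Right click seeks a quick-use ability of the hovered non-friendly object shared by all selected actors, firing it at the saved hit, otherwise ordering a move.
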(event `ServingAbilitySlotKeyPressed`
  (params (Key :type "Key Structure"))
  ;[1 1 1] Ability binding.
  (`/Game/RTSMultiplayer/AbilitySubsystem/Widgets/W_AbilityBar.ServingAbilityKeyPressed` (`/Game/RTSMultiplayer/RTSCoreUI/Widgets/W_PlayerHUD.W_AbilityBar` (`/Game/RTSMultiplayer/RTSCharacters/Blueprints/RTSPlayerController.PlayerHUD` (`self.PlayerController`))) Key))

(event `AbilitySlotKeyPressed`
  (params (Key :type "Key Structure"))
  ;[1 1 1] Ability binding.
  (`/Game/RTSMultiplayer/AbilitySubsystem/Widgets/W_AbilityBar.AbilityKeyPressed` (`/Game/RTSMultiplayer/RTSCoreUI/Widgets/W_PlayerHUD.W_AbilityBar` (`/Game/RTSMultiplayer/RTSCharacters/Blueprints/RTSPlayerController.PlayerHUD` (`self.PlayerController`))) Key))

(event `RotateRight`
  (params (Axis :type "Float (double-precision)")))

(event `MouseX`
  (params (AxisValue :type "Float (double-precision)"))
  (bind _playercontroller (`self.PlayerController`))
  (bind _springarm (`/Game/RTSMultiplayer/RTSCharacters/Blueprints/BasePlayerCharacter.SpringArm` (cast `/Game/RTSMultiplayer/RTSCharacters/Blueprints/BasePlayerCharacter` (`Controller.K2_GetPawn` _playercontroller) :!pure true)))
  (bind (_returnvalue_roll _returnvalue_pitch _returnvalue_yaw) (`KismetMathLibrary.BreakRotator` (`SceneComponent.K2_GetComponentRotation` _springarm)))
  ;[1 1 1] Camera rotation.
  (`/Engine/EditorBlueprintResources/StandardMacros.Gate` true :!label _label
    (:`Exit`
      (`SceneComponent.K2_SetWorldRotation` _springarm (`KismetMathLibrary.MakeRotator` _returnvalue_roll _returnvalue_pitch (+ _returnvalue_yaw (* (`/Game/RTSMultiplayer/RTSCharacters/Blueprints/RTSPlayerController.CameraRotationSensitivity` _playercontroller) AxisValue))) false false))))

(event `RotateReleased`
  (bind _playercontroller (`self.PlayerController`))
  (bind _playercontroller_2 (`self.PlayerController`))
  (bind _springarm (`/Game/RTSMultiplayer/RTSCharacters/Blueprints/BasePlayerCharacter.SpringArm` (cast `/Game/RTSMultiplayer/RTSCharacters/Blueprints/BasePlayerCharacter` (`Controller.K2_GetPawn` _playercontroller_2) :!pure true)))
  (bind (_returnvalue_roll _returnvalue_pitch _returnvalue_yaw) (`KismetMathLibrary.BreakRotator` (`SceneComponent.K2_GetComponentRotation` _springarm)))
  ;[1 1 1] Camera rotation.
  (`|ExecutionSequence`
    (:`then_0`
      (goto _label :!via `Close`))
    (:`then_1`
      (goto _label_2 :!via `Close`))))

(event `RotatePressed`
  (bind _playercontroller (`self.PlayerController`))
  (bind _playercontroller_2 (`self.PlayerController`))
  (bind _springarm (`/Game/RTSMultiplayer/RTSCharacters/Blueprints/BasePlayerCharacter.SpringArm` (cast `/Game/RTSMultiplayer/RTSCharacters/Blueprints/BasePlayerCharacter` (`Controller.K2_GetPawn` _playercontroller_2) :!pure true)))
  (bind (_returnvalue_roll _returnvalue_pitch _returnvalue_yaw) (`KismetMathLibrary.BreakRotator` (`SceneComponent.K2_GetComponentRotation` _springarm)))
  ;[1 1 1] Camera rotation.
  (`|ExecutionSequence`
    (:`then_0`
      (goto _label :!via `Open`))
    (:`then_1`
      (goto _label_2 :!via `Open`))))

(event `MouseY`
  (params (AxisValue :type "Float (double-precision)"))
  (bind _playercontroller (`self.PlayerController`))
  (bind _playercontroller_2 (`self.PlayerController`))
  (bind _springarm (`/Game/RTSMultiplayer/RTSCharacters/Blueprints/BasePlayerCharacter.SpringArm` (cast `/Game/RTSMultiplayer/RTSCharacters/Blueprints/BasePlayerCharacter` (`Controller.K2_GetPawn` _playercontroller_2) :!pure true)))
  (bind (_returnvalue_roll _returnvalue_pitch _returnvalue_yaw) (`KismetMathLibrary.BreakRotator` (`SceneComponent.K2_GetComponentRotation` _springarm)))
  ;[1 1 1] Camera rotation.
  (`/Engine/EditorBlueprintResources/StandardMacros.Gate` true :!label _label_2
    (:`Exit`
      (`SceneComponent.K2_SetWorldRotation` _springarm (`KismetMathLibrary.MakeRotator` _returnvalue_roll (`KismetMathLibrary.FClamp` (+ _returnvalue_pitch (* (`/Game/RTSMultiplayer/RTSCharacters/Blueprints/RTSPlayerController.CameraRotationSensitivity` _playercontroller_2) AxisValue)) (`/Game/RTSMultiplayer/RTSCharacters/Blueprints/RTSPlayerController.CameraPitchMin` _playercontroller) (`/Game/RTSMultiplayer/RTSCharacters/Blueprints/RTSPlayerController.CameraPitchMax` _playercontroller)) _returnvalue_yaw) false false))))

(event `Attached`)

(event `Detached`)

(event `LeftMouseButtonPressed`
  (params (Key :type "Key Structure")))

(event `LeftMouseButtonReleased`
  (params (Key :type "Key Structure")))

(event `CtrlLeftMouseButtonPressed`
  (params (Key :type "Key Structure")))

(event `ShiftLeftMouseButtonPressed`
  (params (Key :type "Key Structure")))

(event `CtrlShiftLeftMouseButtonPressed`
  (params (Key :type "Key Structure")))

(event `RightMouseButtonPressed`
  (params (Key :type "Key Structure"))
  ;[1 1 1] On right click. Trying to quick use ability, move otherwise.
  (bind _success (`self.TryUseAppropriateAbility`))
  (if (not _success)
    (`/Game/RTSMultiplayer/RTSCharacters/Blueprints/RTSPlayerController.MoveUnderMousePosition` (`self.PlayerController`))))

(event `OnQuickAbilityUsed`
  (params (Ability :type "/Game/RTSMultiplayer/AbilitySubsystem/Blueprints/Ability Object Reference"))
  ;[1 1 1] On right click. Trying to quick use ability, move otherwise.
  (bind _astarget_ability (cast `/Game/RTSMultiplayer/AbilitySubsystem/Blueprints/TargetAbility` Ability))
  (`/Game/RTSMultiplayer/AbilitySubsystem/Blueprints/TargetAbility.OnTargetChosen` _astarget_ability (`self.QuickAbilitySavedHitResult`))
  (bind _asbase_player_character (cast `/Game/RTSMultiplayer/RTSCharacters/Blueprints/BasePlayerCharacter` (`Controller.K2_GetPawn` (`self.PlayerController`))))
  (remove `/Game/RTSMultiplayer/RTSCharacters/Blueprints/BasePlayerCharacter.AbilityUsed` _asbase_player_character (`|CreateDelegate` :!event `OnQuickAbilityUsed`)))

(event `RightMouseButtonReleased`
  (params (Key :type "Key Structure")))

(event `TryUseAppropriateSkill`)

(fn `TryUseAppropriateAbility`
  (returns (Success :type Boolean))
  (locals (`DoesActorHaveAbility?` :type Boolean) (AbilityClass :type "/Game/RTSMultiplayer/AbilitySubsystem/Blueprints/Ability Class Reference"))
  (bind _hitresult (`PlayerController.GetHitResultUnderCursorByChannel` (`self.PlayerController`) "TraceTypeQuery1" true))
  (bind (_bblockinghit _binitialoverlap _time _distance _location _impactpoint _normal _impactnormal _physmat _hitactor) (`GameplayStatics.BreakHitResult` _hitresult))
  (if (== (`KismetArrayLibrary.Array_Length` (`/Game/RTSMultiplayer/SelectionSubsystem/Widgets/W_SelectionEnvironment.SelectedActors` (`/Game/RTSMultiplayer/RTSCharacters/Blueprints/RTSPlayerController.SelectionEnvironment` (`self.PlayerController`)))) 0)
    (return false)
    (else
      (set `self.QuickAbilitySavedHitResult` _hitresult)
      (bind _asbase_rtsunit (cast `/Game/RTSMultiplayer/RTSCharacters/Blueprints/BaseRTSUnit` _hitactor)
        (:`then`
          (if (`|EnumEquality` (`/Game/RTSMultiplayer/RTSCharacters/Blueprints/BasePlayerCharacter.PlayerFaction` (cast `/Game/RTSMultiplayer/RTSCharacters/Blueprints/BasePlayerCharacter` (`Controller.K2_GetPawn` (`self.PlayerController`)) :!pure true)) (`/Game/RTSMultiplayer/RTSCharacters/Blueprints/BaseRTSUnit.Faction` _asbase_rtsunit))
            (return false)
            (else
              _)))
        (:`CastFailed`
          _))
      (bind _asi_quick_use_object (cast `/Game/RTSMultiplayer/InputSubsystem/Blueprints/I_QuickUseObject` _hitactor)
        (:`then`
          (bind _abilityclasses (`/Game/RTSMultiplayer/InputSubsystem/Blueprints/I_QuickUseObject.GetQuickUseAbilityClass` _asi_quick_use_object))
          (for _array_element (`/Game/RTSMultiplayer/SelectionSubsystem/Widgets/W_SelectionEnvironment.SelectedActors` (`/Game/RTSMultiplayer/RTSCharacters/Blueprints/RTSPlayerController.SelectionEnvironment` (`self.PlayerController`)))
            (bind _asi_selectable (cast `/Game/RTSMultiplayer/SelectionSubsystem/Blueprints/I_Selectable` _array_element)
              (:`then`
                (bind _abilities (`/Game/RTSMultiplayer/SelectionSubsystem/Blueprints/I_Selectable.GetAbilities` _asi_selectable))
                (for _array_element_2 _abilities
                  (if (== (`local.AbilityClass`) null)
                    (if (`KismetArrayLibrary.Array_Contains` _abilityclasses (break `/Game/RTSMultiplayer/AbilitySubsystem/Data/S_AbilityInfo` _array_element_2))
                      (set `local.AbilityClass` (break `/Game/RTSMultiplayer/AbilitySubsystem/Data/S_AbilityInfo` _array_element_2))
                      (set `local.DoesActorHaveAbility?` true :!label _label)
                      (break))
                    (elif (== (`local.AbilityClass`) (break `/Game/RTSMultiplayer/AbilitySubsystem/Data/S_AbilityInfo` _array_element_2))
                      (goto _label))))
                (if (`local.DoesActorHaveAbility?`)
                  (set `local.DoesActorHaveAbility?` false)
                  (else
                    (return false))))
              (:`CastFailed`
                (return false))))
          (bind _asbase_player_character (cast `/Game/RTSMultiplayer/RTSCharacters/Blueprints/BasePlayerCharacter` (`Controller.K2_GetPawn` (`self.PlayerController`)))
            (:`then`
              (add `/Game/RTSMultiplayer/RTSCharacters/Blueprints/BasePlayerCharacter.AbilityUsed` _asbase_player_character (`|CreateDelegate` :!event `OnQuickAbilityUsed`))
              (`/Game/RTSMultiplayer/RTSCharacters/Blueprints/BasePlayerCharacter.SpawnAndUseAbility` _asbase_player_character (`local.AbilityClass`) (`/Game/RTSMultiplayer/SelectionSubsystem/Widgets/W_SelectionEnvironment.SelectedActors` (`/Game/RTSMultiplayer/RTSCharacters/Blueprints/RTSPlayerController.SelectionEnvironment` (`self.PlayerController`))))
              (return true))
            (:`CastFailed`
              (return false))))
        (:`CastFailed`
          (return false))))))