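; Input receiver for RTS unit selection that turns left-click, Ctrl and Shift variants into drag-selection calls on SelectionEnvironment.
; Clicking own-faction or non-selectable targets starts a drag, with modifiers setting add-to-selection and select-all-by-type.
; Clicking another faction's actor clears the selection and, unless fog hides it, shows it in HUD info and effect widgets and highlights it via its alien selector.
; Each new press deselects that alien unit first.
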(event `DeselectPossibleAlienUnit`
  ;[1 1 1] Deselect possible alien unit.
  (bind _alienselectedunit (`self.AlienSelectedUnit`)
    (:`then`
      (bind _asi_selectable (cast `/Game/RTSMultiplayer/SelectionSubsystem/Blueprints/I_Selectable` _alienselectedunit))
      (bind _selector (`/Game/RTSMultiplayer/SelectionSubsystem/Blueprints/I_Selectable.GetAlienSelector` _asi_selectable))
      (`/Game/RTSMultiplayer/SelectionSubsystem/Blueprints/Selector.Deselect` _selector))
    (:`else`)))

(event `self.LeftMouseButtonPressed`
  (params (Key :type "Key Structure"))
  (bind _selectionenvironment (`self.SelectionEnvironment`))
  (bind _playercontroller (`self.PlayerController`))
  (bind (_bblockinghit _binitialoverlap _time _distance _location _impactpoint _normal _impactnormal _physmat _hitactor) (`GameplayStatics.BreakHitResult` (`PlayerController.GetHitResultUnderCursorByChannel` _playercontroller "TraceTypeQuery1" true)))
  (bind _array (`|MakeArray` _hitactor))
  ;[1 1 1] Left mouse pressed. Show unit info if it was pressed on enemy's unit.
  ; Start select if it was pressed on player's unit.
  (`self.DeselectPossibleAlienUnit`)
  (bind _asi_selectable (cast `/Game/RTSMultiplayer/SelectionSubsystem/Blueprints/I_Selectable` _hitactor)
    (:`then`
      (bind _faction (`/Game/RTSMultiplayer/SelectionSubsystem/Blueprints/I_Selectable.GetFactionAsSelectable` _asi_selectable))
      (if (`|EnumEquality` _faction (`/Game/RTSMultiplayer/RTSCharacters/Blueprints/BasePlayerCharacter.PlayerFaction` (cast `/Game/RTSMultiplayer/RTSCharacters/Blueprints/BasePlayerCharacter` (`Controller.K2_GetPawn` _playercontroller) :!pure true)))
        (if (not (`KismetInputLibrary.Key_IsModifierKey` Key)) :!label _label
          (`/Game/RTSMultiplayer/SelectionSubsystem/Widgets/W_SelectionEnvironment.OnDragStart` (`self.SelectionEnvironment`) false false))
        (else
          (`/Game/RTSMultiplayer/SelectionSubsystem/Widgets/W_SelectionEnvironment.DeselectAll` _selectionenvironment)
          (`/Game/RTSMultiplayer/SelectionSubsystem/Widgets/W_SelectionEnvironment.CallActorsSelected` _selectionenvironment)
          (bind _asi_can_affect_fog (cast `/Game/RTSMultiplayer/FogSubsystem/Blueprints/I_CanAffectFog` _hitactor)
            (:`then`
              (bind _visible (`/Game/RTSMultiplayer/FogSubsystem/Blueprints/I_CanAffectFog.IsVisible?` _asi_can_affect_fog))
              (if _visible
                (`/Game/RTSMultiplayer/SelectionSubsystem/Widgets/W_SelectedUnitInfo.OnActorsSelected` (`/Game/RTSMultiplayer/RTSCoreUI/Widgets/W_PlayerHUD.W_SelectedUnitInfo` (`/Game/RTSMultiplayer/RTSCharacters/Blueprints/RTSPlayerController.PlayerHUD` (`self.PlayerController`))) _array :!label _label_2)
                (`/Game/RTSMultiplayer/EffectsSubsystem/Widgets/W_EffectBar.OnActorsSelected` (`/Game/RTSMultiplayer/RTSCoreUI/Widgets/W_PlayerHUD.W_EffectBar` (`/Game/RTSMultiplayer/RTSCharacters/Blueprints/RTSPlayerController.PlayerHUD` (`self.PlayerController`))) _array)
                (bind _asi_selectable_2 (cast `/Game/RTSMultiplayer/SelectionSubsystem/Blueprints/I_Selectable` _hitactor))
                (bind _selector (`/Game/RTSMultiplayer/SelectionSubsystem/Blueprints/I_Selectable.GetAlienSelector` _asi_selectable_2))
                (`/Engine/EditorBlueprintResources/StandardMacros.IsValid` _selector
                  (:`Is Valid`
                    (set `self.AlienSelectedUnit` _hitactor)
                    (`/Game/RTSMultiplayer/SelectionSubsystem/Blueprints/Selector.Select` _selector)))))
            (:`CastFailed`
              (goto _label_2))))))
    (:`CastFailed`
      (goto _label))))

(event `self.LeftMouseButtonReleased`
  (params (Key :type "Key Structure"))
  (bind _selectionenvironment (`self.SelectionEnvironment`))
  (if (`/Game/RTSMultiplayer/SelectionSubsystem/Widgets/W_SelectionEnvironment.SelectionInProcess?` _selectionenvironment)
    (`/Game/RTSMultiplayer/SelectionSubsystem/Widgets/W_SelectionEnvironment.OnDragStop` _selectionenvironment)))

(event `self.CtrlLeftMouseButtonPressed`
  (params (Key :type "Key Structure"))
  (`self.DeselectPossibleAlienUnit`)
  (`/Game/RTSMultiplayer/SelectionSubsystem/Widgets/W_SelectionEnvironment.OnDragStart` (`self.SelectionEnvironment`) true false))

(event `self.ShiftLeftMouseButtonPressed`
  (params (Key :type "Key Structure"))
  (`self.DeselectPossibleAlienUnit`)
  (`/Game/RTSMultiplayer/SelectionSubsystem/Widgets/W_SelectionEnvironment.OnDragStart` (`self.SelectionEnvironment`) false true))

(event `self.CtrlShiftLeftMouseButtonPressed`
  (params (Key :type "Key Structure"))
  (`self.DeselectPossibleAlienUnit`)
  (`/Game/RTSMultiplayer/SelectionSubsystem/Widgets/W_SelectionEnvironment.OnDragStart` (`self.SelectionEnvironment`) true true))