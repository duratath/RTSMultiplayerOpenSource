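; Input receiver for the ability targeting state in the RTS multiplayer input subsystem.
; While attached it switches to game-only input with a crosshair cursor, restoring game-and-UI input and the default cursor on detach.
; Left-click release broadcasts the cursor's visibility trace hit as the chosen target, and the rotate axis is forwarded.
; Right-click release aborts the controlled character's active ability; ability slot keys are ignored.
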(event `self.Attached`
  (bind _playercontroller (`self.PlayerController`))
  (`WidgetBlueprintLibrary.SetInputMode_GameOnly` _playercontroller)
  (set `PlayerController.CurrentMouseCursor` "Crosshairs" _playercontroller))

(event `self.Detached`
  (bind _playercontroller (`self.PlayerController`))
  (`WidgetBlueprintLibrary.SetInputMode_GameAndUIEx` _playercontroller null "DoNotLock" false)
  (set `PlayerController.CurrentMouseCursor` "Default" _playercontroller))

(event `self.LeftMouseButtonReleased`
  (params (Key :type "Key Structure"))
  (`self.TargetChosen` (`PlayerController.GetHitResultUnderCursorByChannel` (`self.PlayerController`) "TraceTypeQuery1" true)))

(event `self.RightMouseButtonReleased`
  (params (Key :type "Key Structure"))
  (bind _asbase_player_character (cast `/Game/RTSMultiplayer/RTSCharacters/Blueprints/BasePlayerCharacter` (`Controller.K2_GetPawn` (`self.PlayerController`))))
  (bind _ability (`/Game/RTSMultiplayer/RTSCharacters/Blueprints/BasePlayerCharacter.Ability` _asbase_player_character))
  (`/Engine/EditorBlueprintResources/StandardMacros.IsValid` _ability
    (:`Is Valid`
      (`/Game/RTSMultiplayer/AbilitySubsystem/Blueprints/Ability.Abort` _ability))))

(event `self.RightMouseButtonPressed`
  (params (Key :type "Key Structure")))

(event `self.RotateRight`
  (params (Axis :type "Float (single-precision)"))
  (`self.OnRotateRight` Axis))

(event `self.AbilitySlotKeyPressed`
  (params (Key :type "Key Structure")))